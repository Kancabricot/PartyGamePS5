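; Player character Blueprint that interacts with, carries, hands over and throws items.
; Box traces in front of the capsule drive interface messages for interacting, taking items and giving them to desks; held items attach to a hand socket.
; Holding Action with an item halts acceleration, aims by stick with a debug-drawn predicted arc, then throws on release.
; Moving plays a tilt timeline and smoke, while menu mode forwards input to MenuRef.
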(event `InputMovementMenu`
  ;[1 1 1] Movement in menu
  (if false
    (`/Engine/EditorBlueprintResources/StandardMacros.DoOnce` false
      (:`Completed`
        (message `/Game/Blueprints/Interface/BPI_InteractionInMenu.ButtonUp` (`self.MenuRef`))))
    (elif (< (`self.Action Value Y`) -40.0)
      (`/Engine/EditorBlueprintResources/StandardMacros.DoOnce` false :!label _label
        (:`Completed`
          (message `/Game/Blueprints/Interface/BPI_InteractionInMenu.ButtonDown` (`self.MenuRef`))
          (`KismetSystemLibrary.Delay` 0.2)
          (`self.ResetInputMovementMenu`))))))

(event `self.ReceiveBeginPlay`
  (bind (_returnvalue_roll _returnvalue_pitch) (`KismetMathLibrary.BreakRotator` (`self.K2_GetActorRotation`)))
  (`EnhancedInputSubsystemInterface.AddMappingContext` (pcsubsystem `EnhancedInputLocalPlayerSubsystem` (`GameplayStatics.GetPlayerController` (`self.Player Index`))) (`self.Mapping Context`) 0 (struct))
  (set `self.RotationYaw` _returnvalue_pitch))

(event `ResetInputMovementMenu`
  ;[1 1 1] Movement in menu
  (goto _label :!via `Reset`))

(event `EnhancedInput|/Game/Input/Actions/IA_Move`
  (params (ActionValue :type "Vector2D Structure") (ElapsedSeconds :type "Float (double-precision)") (TriggeredSeconds :type "Float (double-precision)") (InputAction :type "InputAction Object Reference" :default "/Game/Input/Actions/IA_Move.IA_Move"))
  (bind (_returnvalue_roll _returnvalue_pitch _returnvalue_yaw) (`KismetMathLibrary.BreakRotator` (`self.K2_GetActorRotation`)))
  (:`Triggered`
    (set `self.Action Value X` ActionValue_X)
    (set `self.Action Value Y` ActionValue_Y)
    (if (`self.b_InMenu`)
      (`self.InputMovementMenu`)))
  (:`Started`
    (`TimelineComponent.SetPlayRate` (`self.Mouvement`) 1.0)
    (`ActorComponent.Activate` (`self.NS_WalkSmoke`) false)
    (bind (_direction _newtrack_0) (`Timeline|Mouvement` :!via `PlayFromStart` :!label _label_2)
      (:`Update`
        (`self.K2_SetActorRotation` (`KismetMathLibrary.MakeRotator` _returnvalue_roll (`KismetMathLibrary.Lerp` 0.0 20.0 _newtrack_0) _returnvalue_yaw)))))
  (:`Completed`
    (`ActorComponent.Deactivate` (`self.NS_WalkSmoke`))
    (`TimelineComponent.SetPlayRate` (`self.Mouvement`) 5.0)
    (goto _label_2 :!via `Reverse`)))

(event `EnhancedInput|/Game/Input/Actions/IA_Action`
  (params (ActionValue :type Boolean) (ElapsedSeconds :type "Float (double-precision)") (TriggeredSeconds :type "Float (double-precision)") (InputAction :type "InputAction Object Reference" :default "/Game/Input/Actions/IA_Action.IA_Action"))
  (bind _capsulecomponent (`self.CapsuleComponent`))
  (bind _radiusspheretrace (`self.RadiusSphereTrace`))
  (bind _returnvalue (+ (`SceneComponent.K2_GetComponentLocation` _capsulecomponent) (* (`SceneComponent.GetForwardVector` _capsulecomponent) (`self.DistanceSphereTrace`))))
  (:`Triggered`
    (if (`self.b_canThrow`)
      (`self.RotationForThrowing`)))
  (:`Started`
    (bind _outhits (`KismetSystemLibrary.BoxTraceMulti` _returnvalue _returnvalue (`KismetMathLibrary.MakeVector` _radiusspheretrace _radiusspheretrace 200.0) (struct) "TraceTypeQuery1"))
    (for _array_element _outhits
      (if (`self.b_HaveItem`)
        (set `self.b_canThrow` true)
        (set `CharacterMovementComponent.MaxAcceleration` 0.0 (`self.CharacterMovement`))
        (set `self.ThrowingStrengh` 1000.0)
        (else
          (bind (_bblockinghit _binitialoverlap _time _distance _location _impactpoint _normal _impactnormal _physmat _hitactor) (`GameplayStatics.BreakHitResult` _array_element))
          (cast `/Game/Blueprints/Interface/BPI_Interact` _hitactor)
          (message `/Game/Blueprints/Interface/BPI_Interact.Interact` _hitactor)))))
  (:`Completed`
    (if (`self.b_canThrow`)
      (`self.ThrowItem`)
      (set `CharacterMovementComponent.MaxAcceleration` 1e+17 (`self.CharacterMovement`)))))

(event `EnhancedInput|/Game/Input/Actions/IA_TakeItem`
  (params (ActionValue :type Boolean) (ElapsedSeconds :type "Float (double-precision)") (TriggeredSeconds :type "Float (double-precision)") (InputAction :type "InputAction Object Reference" :default "/Game/Input/Actions/IA_TakeItem.IA_TakeItem"))
  (bind _capsulecomponent (`self.CapsuleComponent`))
  (bind _radiusspheretrace (`self.RadiusSphereTrace`))
  (bind _returnvalue (+ (`SceneComponent.K2_GetComponentLocation` _capsulecomponent) (* (`SceneComponent.GetForwardVector` _capsulecomponent) (`self.DistanceSphereTrace`))))
  (:`Started`
    (if (not (`self.b_InMenu`))
      (bind _outhits (`KismetSystemLibrary.BoxTraceMulti` _returnvalue _returnvalue (`KismetMathLibrary.MakeVector` _radiusspheretrace _radiusspheretrace 200.0) (struct) "TraceTypeQuery1"))
      (if (`self.b_HaveItem`)
        (for _array_element _outhits
          (if (`self.b_HaveItem`)
            (bind _return (message `/Game/Blueprints/Interface/BPI_TakeItem.GiveItemToDesk` (`.HitActor` (`GameplayStatics.BreakHitResult` _array_element)) (`self.ActorAttach`)))
            (if _return
              (set `self.b_HaveItem` false))
            (else
              (break))))
        (if (`self.b_HaveItem`)
          (set `self.ThrowingStrengh` 0.0)
          (`self.ThrowItem`))
        (else
          (for _array_element_2 _outhits
            (bind _return_2 (message `/Game/Blueprints/Interface/BPI_TakeItem.TakeItem` (`.HitActor` (`GameplayStatics.BreakHitResult` _array_element_2)) self))
            (if _return_2
              (set `self.b_HaveItem` true)
              (break)))))
      (else
        (message `/Game/Blueprints/Interface/BPI_InteractionInMenu.ButtonA` (`self.MenuRef`))))))

(event `TakeItem`
  (params (Color :type "Float (single-precision)") (Actor :type "Actor Object Reference"))
  (bind _mesh (`self.Mesh`))
  (bind _rootcomponent (`Actor.RootComponent` Actor))
  (`KismetSystemLibrary.PrintString` (`KismetSystemLibrary.GetDisplayName` Actor))
  (set `self.b_canThrow` false)
  (bind _output_get (set `self.ActorAttach` Actor))
  (`self.SetActorEnableCollision` _output_get false)
  (`KismetSystemLibrary.DelayUntilNextTick`)
  (`SceneComponent.K2_AttachToComponent` _rootcomponent _mesh (`SkinnedMeshComponent.GetSocketBoneName` _mesh "HandS") "SnapToTarget" "SnapToTarget" "KeepWorld" true)
  (`SceneComponent.K2_SetWorldLocation` _rootcomponent (`SceneComponent.K2_GetComponentLocation` (`self.Scene`)) false false)
  (if (not (== (`self.ActorAttach`) null))
    (set `self.b_HaveItem` true)))

(fn `GetMenu`
  (params (MenuRef :type "Widget Object Reference"))
  (set `self.MenuRef` MenuRef)
  (set `self.b_InMenu` true))

(fn `PreviewForThrowing`
  (locals (MaxThrow :type Integer :default 30))
  (bind _output_get (set `self.ThrowVelocity` (* (`SceneComponent.GetForwardVector` (`self.ThrowingLocation`)) (* (`local.MaxThrow`) (`KismetMathLibrary.VSizeXY` (`KismetMathLibrary.MakeVector` (`self.Action Value X`) (`self.Action Value Y`)))))))
  (`GameplayStatics.Blueprint_PredictProjectilePath_Advanced` (make `PredictProjectilePathParams` (`SceneComponent.K2_GetComponentLocation` (`self.ThrowingLocation`)) _output_get false 0.0 1.0 true "ECC_WorldStatic" _ _ 20.0 0.0 "ForOneFrame")))

(fn `RotationForThrowing`
  (bind _returnvalue_roll (`KismetMathLibrary.BreakRotator` (`KismetMathLibrary.MakeRotFromY` (`KismetMathLibrary.MakeVector` (`self.Action Value X`) (`self.Action Value Y`)))))
  (bind _returnvalue (`KismetMathLibrary.FWrap` _returnvalue_roll 0.0 359.0))
  (set `self.RotRef` _returnvalue)
  (`SceneComponent.K2_SetWorldRotation` (`self.CapsuleComponent`) (`KismetMathLibrary.MakeRotator` 0.0 0.0 _returnvalue) false false)
  (`self.PreviewForThrowing`))

(fn `ThrowItem`
  (locals (MaxThrow :type Integer :default 50))
  (bind _actorattach (`self.ActorAttach`))
  (bind _rootcomponent (`Actor.RootComponent` _actorattach))
  (`/Engine/EditorBlueprintResources/StandardMacros.IsValid` _actorattach
    (:`Is Valid`
      (`self.K2_DetachFromActor` _actorattach "KeepWorld" "KeepWorld" "KeepWorld")
      (`self.SetActorEnableCollision` _actorattach true)
      (`SceneComponent.K2_SetWorldLocation` _rootcomponent (`SceneComponent.K2_GetComponentLocation` (`self.ThrowingLocation`)) false false)
      (`SceneComponent.K2_SetWorldRotation` :`self` _rootcomponent)
      (message `/Game/Blueprints/Interface/BPI_TakeItem.DettachItem` _actorattach (`self.ThrowVelocity`))
      (set `self.ActorAttach` null)
      (set `self.b_canThrow` false)
      (set `self.b_HaveItem` false))))

(fn `UserConstructionScript`)