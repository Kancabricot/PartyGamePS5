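; BP_CreateLocalPlayer sets up two-player local play and holds helper functions for Joy-Con controllers.
; On BeginPlay it creates both local players, spawns and possesses a BP_Player at separate PlayerStarts with per-player input mapping contexts, then points player 0's view at BP_camera.
; Joy-Con functions connect controllers with IMU, attach two in landscape grip, or detach and disconnect all; this graph never calls connect or disconnect.
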(event `self.ReceiveBeginPlay`
  (`|ExecutionSequence`
    (:`then_0`
      (bind _outactors (`GameplayStatics.GetAllActorsOfClass` "/Script/Engine.PlayerStart"))
      (set `self.PlayerStartRefs` _outactors))
    (:`then_1`
      (`GameplayStatics.CreatePlayer` 0)
      (bind _returnvalue (`|SpawnActorFromClass` "/Game/Blueprints/Player/BP_Player.BP_Player_C" (`self.GetTransform` (`|GetArrayItem` (`self.PlayerStartRefs`))) "Undefined" "MultiplyWithRoot" null "/Game/Input/IMC_Player1.IMC_Player1" 0 self null))
      (`Controller.Possess` (`GameplayStatics.GetPlayerController` 0) _returnvalue)
      (`GameplayStatics.CreatePlayer` 1)
      (bind _returnvalue_2 (`|SpawnActorFromClass` "/Game/Blueprints/Player/BP_Player.BP_Player_C" (`self.GetTransform` (`|GetArrayItem` (`self.PlayerStartRefs`) 1)) "Undefined" "MultiplyWithRoot" null "/Game/Input/IMC_Player2.IMC_Player2" 1 self null))
      (`Controller.Possess` (`GameplayStatics.GetPlayerController` 1) _returnvalue_2))
    (:`then_2`
      (`self.SetUpCam`))))

(event `SetUpCam`
  (bind _returnvalue (`GameplayStatics.GetActorOfClass` "/Game/Blueprints/BP_camera.BP_camera_C"))
  (`PlayerController.SetViewTargetWithBlend` (`GameplayStatics.GetPlayerController` 0) _returnvalue 0.0 "VTBlend_Linear" 0.0 false))

(fn `AttachJoycon`
  (params (GripIndex :type Integer) (ControlleurIndex :type Integer))
  (bind _joycons (`JoyConDriverFunctionLibrary.GetConnectedJoyCons`))
  (`JoyConDriverFunctionLibrary.AttachJoyCon` (`.ControllerId` (break `JoyConInformation` (`|GetArrayItem` _joycons ControlleurIndex))) GripIndex)
  (`JoyConDriverFunctionLibrary.SetJoyConGripMode` GripIndex "Landscape"))

(fn `ConnectJoycon`
  (`JoyConDriverFunctionLibrary.ResumeJoyConConnection`)
  (bind _joycons (`JoyConDriverFunctionLibrary.SearchForJoyCons`))
  (for _array_element _joycons
    (bind _success (`JoyConDriverFunctionLibrary.ConnectJoyCon` _array_element true true))
    (`KismetSystemLibrary.PrintString` "GG" _success))
  (`self.AttachJoycon` 0)
  (`self.AttachJoycon` 1 1))

(fn `DisconnectJoycon`
  (bind _joycons (`JoyConDriverFunctionLibrary.GetAttachedJoyCons`))
  (for _array_element _joycons
    (`JoyConDriverFunctionLibrary.DetachJoyCon` (`.ControllerId` (break `JoyConInformation` _array_element))))
  (bind _joycons_2 (`JoyConDriverFunctionLibrary.GetConnectedJoyCons`))
  (for _array_element_2 _joycons_2
    (`JoyConDriverFunctionLibrary.DisconnectJoyCon` (`.ControllerId` (break `JoyConInformation` _array_element_2)))))

(fn `UserConstructionScript`)