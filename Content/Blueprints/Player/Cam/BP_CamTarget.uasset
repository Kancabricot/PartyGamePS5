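; BP_CamTarget is a camera target actor that follows the average position of a set of player actors within a limited band.
; CamTargetLocation stores the player array and starts a fast looping timer that averages their locations.
; The actor snaps to that average only while BMove is true, meaning its Y lies within a fixed distance of the start.
; BMove updates after each move, so the limit applies one timer step late.
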(event `self.ReceiveBeginPlay`
  (set `self.StartLocation` (`self.K2_GetActorLocation`)))

(event `CamTargetLocation`
  (params (PlayerTab :type "Array of /Game/Blueprints/Player/Player/BP_Player Object Reference"))
  (set `self.Player Tab` PlayerTab)
  (`KismetSystemLibrary.K2_SetTimerDelegate` (delegate `SetLoc`) 0.01 true))

(event `SetLoc`
  (bind (_startlocation_x _startlocation_y) (`KismetMathLibrary.BreakVector` (`self.StartLocation`)))
  (bind (_averagelocation_x _averagelocation_y) (`KismetMathLibrary.BreakVector` (`self.AverageLocation`)))
  (bind (_startlocation_x_2 _startlocation_y_2) (`KismetMathLibrary.BreakVector` (`self.StartLocation`)))
  (bind (_averagelocation_x_2 _averagelocation_y_2) (`KismetMathLibrary.BreakVector` (`self.AverageLocation`)))
  (bind _returnvalue (`GameplayStatics.GetActorArrayAverageLocation` (`self.Player Tab`)))
  (bind _output_get (set `self.AverageLocation` _returnvalue))
  (if (`self.b_Move`)
    (`self.K2_SetActorLocation` _output_get))
  (if (and (> (+ _startlocation_y_2 350.0) _averagelocation_y_2) (< (- _startlocation_y 350.0) _averagelocation_y))
    (set `self.b_Move` true)
    (else
      (set `self.b_Move` false))))

(fn `UserConstructionScript`)