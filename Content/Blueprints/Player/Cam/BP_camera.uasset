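; Shared camera actor that drifts toward a target actor's Y position and widens its view when the first two players move apart.
; SetLocationCam stores the target and players, then starts a fast looping timer that interpolates location and FOV.
; Past a distance threshold it eases to a raised FOV and X-offset position, otherwise back to its start.
; The construction script applies editable spring arm, angle and FOV presets.
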(event `self.ReceiveBeginPlay`
  (bind (_returnvalue_x _returnvalue_y _returnvalue_z) (`KismetMathLibrary.BreakVector` (`self.K2_GetActorLocation`)))
  (set `self.Interpe` (`KismetMathLibrary.MakeVector` (+ _returnvalue_x 50.0) _returnvalue_y _returnvalue_z))
  (set `self.StartPos` (`self.K2_GetActorLocation`)))

(event `SetLocationCam`
  (params (TargerCam :type "/Game/Blueprints/Player/Cam/BP_CamTarget Object Reference") (TabPlayer :type "Array of /Game/Blueprints/Player/Player/BP_Player Object Reference"))
  (set `self.Tab Player` TabPlayer)
  (set `self.Targer Cam` TargerCam)
  (`KismetSystemLibrary.K2_SetTimerDelegate` (delegate `Set loc`) 0.001 true))

(event `Set loc`
  (bind (_returnvalue_x _returnvalue_y _returnvalue_z) (`KismetMathLibrary.BreakVector` (`self.K2_GetActorLocation`)))
  (bind _camera (`self.Camera`))
  (bind _tab_player (`self.Tab Player`))
  (bind _camera_2 (`self.Camera`))
  (bind (_returnvalue_x_2 _returnvalue_y_2) (`KismetMathLibrary.BreakVector` (`self.K2_GetActorLocation` (`self.Targer Cam`))))
  (`self.K2_SetActorLocation` (`KismetMathLibrary.VInterpTo` (`self.K2_GetActorLocation`) (`KismetMathLibrary.MakeVector` _returnvalue_x _returnvalue_y_2 _returnvalue_z) (`GameplayStatics.GetWorldDeltaSeconds`) 0.05))
  (if (> (`self.GetDistanceTo` (`|GetArrayItem` _tab_player) (`|GetArrayItem` _tab_player 1)) 1250.0)
    (set `CameraComponent.FieldOfView` (`KismetMathLibrary.FInterpTo` (`CameraComponent.FieldOfView` _camera_2) (+ (`self.FOV`) 4.0) (`GameplayStatics.GetWorldDeltaSeconds`) 0.05) _camera_2)
    (`self.K2_SetActorLocation` (`KismetMathLibrary.VInterpTo` (`self.K2_GetActorLocation`) (`self.Interpe`) (`GameplayStatics.GetWorldDeltaSeconds`) 0.1))
    (else
      (set `CameraComponent.FieldOfView` (`KismetMathLibrary.FInterpTo` (`CameraComponent.FieldOfView` _camera) (`self.FOV`) (`GameplayStatics.GetWorldDeltaSeconds`) 0.05) _camera)
      (`self.K2_SetActorLocation` (`KismetMathLibrary.VInterpTo` (`self.K2_GetActorLocation`) (`self.StartPos`) (`GameplayStatics.GetWorldDeltaSeconds`) 0.1)))))

(fn `ModifyPresets`
  (bind _camera (`self.Camera`))
  (set `SpringArmComponent.TargetArmLength` (`self.DistanceFromCenter`) (`self.SpringArm`))
  (`SceneComponent.K2_SetRelativeRotation` _camera (`KismetMathLibrary.MakeRotator` 0.0 (`self.CamPitch`)) false false)
  (`CameraComponent.SetFieldOfView` _camera (`self.FOV`))
  (`SceneComponent.K2_SetRelativeRotation` (`self.CenterRef`) (`KismetMathLibrary.MakeRotator` 0.0 (* (`self.AngleOfPitchView`) -1.0) (`self.AngleOfYawView`)) false false))

(fn `UserConstructionScript`
  (`self.ModifyPresets`))