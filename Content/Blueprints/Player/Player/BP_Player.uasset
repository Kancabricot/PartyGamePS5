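; Player character for a multiplayer game with Joy-Con support, handling per-player input mapping, menu input, movement lean and smoke, and debug player switching.
; Box traces drive interacting, taking items and handing them to desks through interface messages.
; Holding action with an item stops movement, aims by stick with rumble and previews the predicted path with spline meshes.
; Release or Joy-Con shake throws, using a suggested-arc velocity when snapping to a drop position.
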(event `self.ReceiveBeginPlay`
  ;[1 1 1] BeginPlay
  (bind _joycons (`JoyConDriverFunctionLibrary.GetAttachedJoyCons`))
  (if (not (`KismetArrayLibrary.Array_IsEmpty` _joycons))
    (set `self.AdditionalOffSetForSwitch` 44.0)
    (if (`.IsLeft` (break `JoyConInformation` (`|GetArrayItem` _joycons (`self.Player Index`))))
      (set `self.Mapping Context` "/Game/Input/IMC_Player1.IMC_Player1")
      (else
        (set `self.Mapping Context` "/Game/Input/IMC_Player2.IMC_Player2")))
    (`self.SetInput`)
    (else
      (set `self.AdditionalOffSetForSwitch` 1.0)
      (`self.SetInput`)))
  ;;[1 1 1] DebugConnectJoycon
  (bind _returnvalue (`|CreateWidget` "/Game/Blueprints/Widgets/WG_DebugJoycon.WG_DebugJoycon_C"))
  (`UserWidget.AddToViewport` _returnvalue 0))

(event `InputMovementMenu`
  ;[1 1 1] Movement in menu
  (if false
    (`/Engine/EditorBlueprintResources/StandardMacros.DoOnce` false
      (:`Completed`
        (message `/Game/Blueprints/Interface/BPI_InteractionInMenu.ButtonUp` (`self.MenuRef`))))
    (elif (< (`self.Action Value Y`) -40.0)
      (`/Engine/EditorBlueprintResources/StandardMacros.DoOnce` false :!label _label
        (:`Completed`
          (message `/Game/Blueprints/Interface/BPI_InteractionInMenu.ButtonDown` (`self.MenuRef`))
          (`KismetSystemLibrary.Delay` 0.2)
          (`self.ResetInputMovementMenu`))))))

(event `EnhancedInput|/Game/Input/Actions/IA_Move`
  (params (ActionValue :type "Vector2D Structure") (ElapsedSeconds :type "Float (double-precision)") (TriggeredSeconds :type "Float (double-precision)") (InputAction :type "InputAction Object Reference" :default "/Game/Input/Actions/IA_Move.IA_Move"))
  (bind (_returnvalue_roll _returnvalue_pitch _returnvalue_yaw) (`KismetMathLibrary.BreakRotator` (`self.K2_GetActorRotation`)))
  ;[1 1 1] Player Movement
  (:`Triggered`
    (set `self.Action Value X` ActionValue_X)
    (set `self.Action Value Y` ActionValue_Y))
  (:`Started`
    (set `self.MaxThrowPower` 18.0)
    (if (not (<= (`CharacterMovementComponent.GetMaxAcceleration` (`self.CharacterMovement`)) 0.0))
      (`TimelineComponent.SetPlayRate` (`self.Mouvement`) 1.0)
      (`ActorComponent.Activate` (`self.NS_WalkSmoke`) false)
      (bind (_direction _newtrack_0) (`Timeline|Mouvement` :!via `PlayFromStart` :!label _label_2)
        (:`Update`
          (`self.K2_SetActorRotation` (`KismetMathLibrary.MakeRotator` _returnvalue_roll (`KismetMathLibrary.Lerp` 0.0 20.0 _newtrack_0) _returnvalue_yaw))))))
  (:`Completed`
    (set `self.MaxThrowPower` 0.0)
    (`ActorComponent.Deactivate` (`self.NS_WalkSmoke`))
    (`TimelineComponent.SetPlayRate` (`self.Mouvement`) 5.0)
    (goto _label_2 :!via `Reverse`)))

(event `ResetInputMovementMenu`
  ;[1 1 1] Movement in menu
  (goto _label :!via `Reset`))

(event `EnhancedInput|/Game/Input/Actions/IA_SwitchPlayer`
  (params (ActionValue :type Boolean) (ElapsedSeconds :type "Float (double-precision)") (TriggeredSeconds :type "Float (double-precision)") (InputAction :type "InputAction Object Reference" :default "/Game/Input/Actions/IA_SwitchPlayer.IA_SwitchPlayer"))
  ;[1 1 1] Switch Player Pour debug
  (:`Started`
    (if (== (`self.Player Index`) 0)
      (bind _outactors (`GameplayStatics.GetAllActorsOfClass` "BP_Player_C"))
      (for _array_element _outactors
        (if (== (`/Game/Blueprints/Player/Player/BP_Player.Player Index` _array_element) 1)
          (`Controller.Possess` (`GameplayStatics.GetPlayerController` 0) _array_element)
          (`/Game/Blueprints/Player/Player/BP_CreateLocalPlayer.SetUpCam` (`self.LocalPlayerRef`) :!label _label_3)))
      (else
        (bind _outactors_2 (`GameplayStatics.GetAllActorsOfClass` "BP_Player_C"))
        (for _array_element_2 _outactors_2
          (if (== (`/Game/Blueprints/Player/Player/BP_Player.Player Index` _array_element_2) 0)
            (`Controller.Possess` (`GameplayStatics.GetPlayerController` 0) _array_element_2)
            (goto _label_3)))))))

(event `EnhancedInput|/Game/Input/Actions/IA_Action`
  (params (ActionValue :type Boolean) (ElapsedSeconds :type "Float (double-precision)") (TriggeredSeconds :type "Float (double-precision)") (InputAction :type "InputAction Object Reference" :default "/Game/Input/Actions/IA_Action.IA_Action"))
  (bind (_predictresult _spline) (`self.PreviewForThrowing`))
  (bind _capsulecomponent (`self.CapsuleComponent`))
  (bind _radiusspheretrace (`self.RadiusSphereTrace`))
  (bind _returnvalue (+ (`SceneComponent.K2_GetComponentLocation` _capsulecomponent) (* (`SceneComponent.GetForwardVector` _capsulecomponent) (`self.DistanceSphereTrace`))))
  (:`Triggered`
    (if (`self.b_canThrow`)
      (`self.RotationForThrowing`)
      (`self.ArcSpline` _predictresult _spline)))
  (:`Started`
    (bind _outhits (`KismetSystemLibrary.BoxTraceMulti` _returnvalue _returnvalue (`KismetMathLibrary.MakeVector` _radiusspheretrace _radiusspheretrace 200.0) (struct) "TraceTypeQuery1"))
    (for _array_element _outhits
      (if (`self.b_HaveItem`)
        (set `self.b_canThrow` true)
        (set `self.ThrowingStrengh` 1000.0)
        (set `CharacterMovementComponent.MaxAcceleration` 0.0 (`self.CharacterMovement`))
        (else
          (bind (_bblockinghit _binitialoverlap _time _distance _location _impactpoint _normal _impactnormal _physmat _hitactor) (`GameplayStatics.BreakHitResult` _array_element))
          (cast `/Game/Blueprints/Interface/BPI_Interact` _hitactor)
          (bind _output_get (set `self.InteractRef` _hitactor))
          (message `/Game/Blueprints/Interface/BPI_Interact.Interact` _output_get)
          (set `CharacterMovementComponent.MaxAcceleration` 0.0 (`self.CharacterMovement`))))))
  (:`Completed`
    (set `CharacterMovementComponent.MaxAcceleration` 1e+17 (`self.CharacterMovement`))
    (if (`self.b_canThrow`)
      (`self.ThrowItem`))))

(event `EnhancedInput|/Game/Input/Actions/IA_TakeItem`
  (params (ActionValue :type Boolean) (ElapsedSeconds :type "Float (double-precision)") (TriggeredSeconds :type "Float (double-precision)") (InputAction :type "InputAction Object Reference" :default "/Game/Input/Actions/IA_TakeItem.IA_TakeItem"))
  (bind _capsulecomponent (`self.CapsuleComponent`))
  (bind _radiusspheretrace (`self.RadiusSphereTrace`))
  (bind _returnvalue (+ (`SceneComponent.K2_GetComponentLocation` _capsulecomponent) (* (`SceneComponent.GetForwardVector` _capsulecomponent) (`self.DistanceSphereTrace`))))
  (:`Started`
    (if (not (`self.b_InMenu`))
      (bind _outhits (`KismetSystemLibrary.BoxTraceMulti` _returnvalue _returnvalue (`KismetMathLibrary.MakeVector` _radiusspheretrace _radiusspheretrace 200.0) (struct) "TraceTypeQuery1"))
      (if (`self.b_HaveItem`)
        (for _array_element _outhits
          (if (`self.b_HaveItem`)
            (bind _return (message `/Game/Blueprints/Interface/BPI_TakeItem.GiveItemToDesk` (`.HitActor` (`GameplayStatics.BreakHitResult` _array_element)) (`self.ActorAttach`)))
            (if _return
              (set `self.b_HaveItem` false))
            (else
              (break))))
        (if (`self.b_HaveItem`)
          (set `self.ThrowVelocity` (0.0 0.0 0.0))
          (`self.ThrowItem`))
        (else
          (for _array_element_2 _outhits
            (bind _return_2 (message `/Game/Blueprints/Interface/BPI_TakeItem.TakeItem` (`.HitActor` (`GameplayStatics.BreakHitResult` _array_element_2)) self))
            (if _return_2
              (set `self.b_HaveItem` true)
              (break)))))
      (else
        (message `/Game/Blueprints/Interface/BPI_InteractionInMenu.ButtonA` (`self.MenuRef`))))))

(event `TakeItem`
  (params (Actor :type "Actor Object Reference"))
  (bind _mesh (`self.Mesh`))
  (bind _rootcomponent (`Actor.RootComponent` Actor))
  (set `self.b_canThrow` false)
  (bind _output_get (set `self.ActorAttach` Actor))
  (`self.SetActorEnableCollision` _output_get false)
  (`KismetSystemLibrary.DelayUntilNextTick`)
  (`SceneComponent.K2_AttachToComponent` _rootcomponent _mesh (`SkinnedMeshComponent.GetSocketBoneName` _mesh "HandS") "SnapToTarget" "SnapToTarget" "KeepWorld" true)
  (`SceneComponent.K2_SetWorldLocation` _rootcomponent (`SceneComponent.K2_GetComponentLocation` (`self.ItemLocation`)) false false)
  (if (not (== (`self.ActorAttach`) null))
    (set `self.b_HaveItem` true)))

(event `self.Sphere.OnComponentBeginOverlap`
  (params (OverlappedComponent :type "PrimitiveComponent Object Reference") (OtherActor :type "Actor Object Reference") (OtherComp :type "PrimitiveComponent Object Reference") (OtherBodyIndex :type Integer) (bFromSweep :type Boolean) (SweepResult :type "HitResult Structure (by ref)"))
  ;[1 0 0] A REMPLACER ( snap )
  (bind (_dropposition _b_cansnap) (message `/Game/Blueprints/Interface/BPI_Snap.GetSnapValue` OtherActor (`self.ActorAttach`)))
  (if _b_cansnap
    (set `self.Drop Position` _dropposition)
    (set `self.CanSnap` true)))

(event `self.Sphere.OnComponentEndOverlap`
  (params (OverlappedComponent :type "PrimitiveComponent Object Reference") (OtherActor :type "Actor Object Reference") (OtherComp :type "PrimitiveComponent Object Reference") (OtherBodyIndex :type Integer))
  ;[1 0 0] A REMPLACER ( snap )
  (set `self.CanSnap` false))

(event `self.ReceiveTick`
  (params (DeltaSeconds :type "Float (single-precision)"))
  (if (and (>= (`KismetMathLibrary.VSize` (`.Accelerometer` (`JoyConDriverFunctionLibrary.GetJoyConAccelerometer` 0))) 2.0) (`self.b_canThrow`))
    (`self.ThrowItem`)))

(fn `ArcSpline`
  (params (PathResult :type "PredictProjectilePathResult Structure") (SplineRef :type "SplineComponent Object Reference"))
  (locals (PointLocation :type "Array of Vector Structure") (HaveSpline :type Boolean :default true) (Spline :type "SplineComponent Object Reference"))
  (bind _pathdata (break `PredictProjectilePathResult` PathResult))
  (bind _splinemesh1 (`self.SplineMesh1`))
  (bind _returnvalue (`KismetArrayLibrary.Array_LastIndex` _pathdata))
  (bind _output_location (break `PredictProjectilePathPointData` (`|GetArrayItem` _pathdata _returnvalue)))
  (`|ExecutionSequence`
    (:`then_0`
      (`self.ClearMeshThrow` (`local.SplineRef`) (`self.SplineMesh1`)))
    (:`then_1`
      (for _array_element _pathdata
        (`SplineComponent.AddSplinePoint` (`local.SplineRef`) (break `PredictProjectilePathPointData` _array_element) "Local" true))
      (`SplineComponent.SetSplinePointType` (`local.SplineRef`) _returnvalue "CurveClamped" true)
      (`SceneComponent.K2_SetWorldLocation` (`self.EndSpline`) _output_location false false)
      (for _index (range (`SplineComponent.GetNumberOfSplinePoints` (`local.SplineRef`)))
        (bind _returnvalue_2 (`AddComponent|NODE_AddSplineMeshComponent-3` :`bManualAttachment` true))
        (`KismetArrayLibrary.Array_Add` (`self.SplineMesh1`) _returnvalue_2)
        (bind (_location _tangent) (`SplineComponent.GetLocationAndTangentAtSplinePoint` (`local.SplineRef`) _index "Local"))
        (bind (_location_2 _tangent_2) (`SplineComponent.GetLocationAndTangentAtSplinePoint` (`local.SplineRef`) (+ _index 1) "Local"))
        (`SplineMeshComponent.SetStartAndEnd` _returnvalue_2 _location _tangent _location_2 _tangent_2 true))
      (if (`self.IsSnap`)
        (`PrimitiveComponent.SetMaterial` _splinemesh1 0 "/Game/Assets/Materials/Throw/M_Throw_Inst.M_Throw_Inst")
        (else
          (`PrimitiveComponent.SetMaterial` _splinemesh1 0 "/Game/Assets/Materials/Throw/M_Throw.M_Throw"))))))

(fn `ClearMeshThrow`
  (params (Spline :type "SplineComponent Object Reference") (SplineMesh :type "Array of SplineMeshComponent Object Reference (by ref)"))
  (`SplineComponent.ClearSplinePoints` Spline true)
  (`ActorComponent.K2_DestroyComponent` SplineMesh)
  (`KismetArrayLibrary.Array_Clear` SplineMesh))

(fn `GetMenu`
  (params (MenuRef :type "Widget Object Reference"))
  (set `self.MenuRef` MenuRef)
  (set `self.b_InMenu` true))

(fn `PreviewForThrowing`
  (returns (PredictResult :type "PredictProjectilePathResult Structure") (Spline :type "SplineComponent Object Reference"))
  (locals (IntensityFFC :type "Float (double-precision)" :default 2.0) (MeshSpline :type "SplineMeshComponent Object Reference") (Bool :type "Object Object Reference" :default "true") (PointLocation :type "Array of Vector Structure") (Spli :type "SplineComponent Object Reference"))
  (bind _forcefeedback (`self.ForceFeedback`))
  (bind _returnvalue (`KismetMathLibrary.VSizeXY` (`KismetMathLibrary.MakeVector` (* (`self.Action Value X`) (`self.AdditionalOffSetForSwitch`)) (* (`self.Action Value Y`) (`self.AdditionalOffSetForSwitch`)))))
  (`ForceFeedbackComponent.Play` _forcefeedback 0.0)
  (`ForceFeedbackComponent.SetIntensityMultiplier` _forcefeedback (/ (`KismetMathLibrary.NormalizeToRange` (* _returnvalue (`self.MaxThrowPower`)) 0.0 200.0) (`local.IntensityFFC`)))
  (bind _output_get (set `self.ThrowVelocity` (* (`SceneComponent.GetForwardVector` (`self.ThrowingLocation`)) (* (`self.MaxThrowPower`) _returnvalue))))
  (bind _predictresult (`GameplayStatics.Blueprint_PredictProjectilePath_Advanced` (make `PredictProjectilePathParams` (`SceneComponent.K2_GetComponentLocation` (`self.ItemLocation`)) _output_get true 0.0 20.0 true "ECC_WorldStatic" _ (`|MakeArray` (`self.ActorAttach`) self :!type "Actor Object Reference") 10.0)))
  (if (`self.CanSnap`)
    (set `self.IsSnap` true)
    (`self.Snap` (`self.ActuTurret`) (`self.Spline1`))
    (else
      (set `self.IsSnap` false)
      (`self.ClearMeshThrow` (`self.Spline1`) (`self.SplineMesh2`))
      (`PrimitiveComponent.SetMaterial` (`self.SplineMesh1`) 0 "/Game/Assets/Materials/Throw/M_Throw.M_Throw")
      (`PrimitiveComponent.SetMaterial` (`self.EndSpline`) 0 "/Game/Assets/Materials/Throw/M_Throw.M_Throw")))
  (return _predictresult (`self.Spline`)))

(fn `RotationForThrowing`
  (bind _returnvalue_roll (`KismetMathLibrary.BreakRotator` (`KismetMathLibrary.MakeRotFromY` (`KismetMathLibrary.MakeVector` (* (`self.Action Value X`) (`self.AdditionalOffSetForSwitch`)) (* (`self.Action Value Y`) (`self.AdditionalOffSetForSwitch`))))))
  (bind _returnvalue (`KismetMathLibrary.FWrap` _returnvalue_roll _returnvalue_roll 360.0))
  (`SceneComponent.SetVisibility` (`self.EndSpline`) true false)
  (set `self.RotRef` _returnvalue)
  (`SceneComponent.K2_SetWorldRotation` (`self.CapsuleComponent`) (`KismetMathLibrary.MakeRotator` 0.0 0.0 _returnvalue) false false))

(fn `SetInput`
  (bind (_returnvalue_roll _returnvalue_pitch) (`KismetMathLibrary.BreakRotator` (`self.K2_GetActorRotation`)))
  (`EnhancedInputSubsystemInterface.AddMappingContext` (pcsubsystem `EnhancedInputLocalPlayerSubsystem` (`GameplayStatics.GetPlayerController` (`self.Player Index`))) (`self.Mapping Context`) 0 (struct))
  (set `self.RotationYaw` _returnvalue_pitch))

(fn `Snap`
  (params (Turret :type "/Game/Blueprints/Turret/Blueprint/BP_Turret Object Reference") (Spline :type "SplineComponent Object Reference"))
  (locals (LocalSpine :type "SplineComponent Object Reference"))
  (bind _localspine (`local.LocalSpine`))
  (bind _returnvalue (`SceneComponent.K2_GetComponentLocation` (`self.ItemLocation`)))
  (set `local.LocalSpine` Spline)
  (bind _outlaunchvelocity (`GameplayStatics.SuggestProjectileVelocity_CustomArc` _returnvalue (`self.Drop Position`)))
  (bind _output_get (set `self.SnapVelocity` _outlaunchvelocity))
  (bind _predictresult (`GameplayStatics.Blueprint_PredictProjectilePath_Advanced` (make `PredictProjectilePathParams` _returnvalue _output_get true 10.0 20.0 true "ECC_WorldDynamic" _ (`|MakeArray` (`self.ActorAttach`) self :!type "Actor Object Reference") 10.0 0.0 "ForOneFrame")))
  (`|ExecutionSequence`
    (:`then_0`
      (`self.ClearMeshThrow` (`local.LocalSpine`) (`self.SplineMesh2`)))
    (:`then_1`
      (bind _pathdata (break `PredictProjectilePathResult` _predictresult))
      (for _array_element _pathdata
        (`SplineComponent.AddSplinePoint` (`local.LocalSpine`) (break `PredictProjectilePathPointData` _array_element) "Local" true))
      (bind _returnvalue_2 (`KismetArrayLibrary.Array_LastIndex` _pathdata))
      (`SplineComponent.SetSplinePointType` (`local.LocalSpine`) _returnvalue_2 "CurveClamped" true)
      (bind _output_location (break `PredictProjectilePathPointData` (`|GetArrayItem` _pathdata _returnvalue_2)))
      (`SceneComponent.K2_SetWorldLocation` (`self.EndSpline1`) _output_location false false)
      (for _index (range (`SplineComponent.GetNumberOfSplinePoints` (`local.LocalSpine`)))
        (bind _returnvalue_3 (`AddComponent|NODE_AddSplineMeshComponent-6` :`bManualAttachment` true))
        (`KismetArrayLibrary.Array_Add` (`self.SplineMesh2`) _returnvalue_3)
        (bind (_location _tangent) (`SplineComponent.GetLocationAndTangentAtSplinePoint` _localspine _index "Local"))
        (bind (_location_2 _tangent_2) (`SplineComponent.GetLocationAndTangentAtSplinePoint` _localspine (+ _index 1) "Local"))
        (`SplineMeshComponent.SetStartAndEnd` _returnvalue_3 _location _tangent _location_2 _tangent_2 true))
      (`PrimitiveComponent.SetMaterial` (`self.SplineMesh1`) 0 "/Game/Assets/Materials/Throw/M_Throw_Inst.M_Throw_Inst")
      (`PrimitiveComponent.SetMaterial` (`self.EndSpline`) 0 "/Game/Assets/Materials/Throw/M_Throw_Inst.M_Throw_Inst"))))

(fn `ThrowItem`
  (locals (MaxThrow :type Integer :default 50))
  (bind _actorattach (`self.ActorAttach`))
  (bind _rootcomponent (`Actor.RootComponent` _actorattach))
  (`/Engine/EditorBlueprintResources/StandardMacros.IsValid` _actorattach
    (:`Is Valid`
      (`self.K2_DetachFromActor` _actorattach "KeepWorld" "KeepWorld" "KeepWorld")
      (`self.SetActorEnableCollision` _actorattach true)
      (`SceneComponent.K2_SetWorldLocation` _rootcomponent (`SceneComponent.K2_GetComponentLocation` (`self.ThrowingLocation`)) false false)
      (`SceneComponent.K2_SetWorldRotation` :`self` _rootcomponent)
      (message `/Game/Blueprints/Interface/BPI_TakeItem.DettachItem` _actorattach (`KismetMathLibrary.SelectVector` (`self.SnapVelocity`) (`self.ThrowVelocity`) (`self.IsSnap`)))
      (set `self.ActorAttach` null)
      (set `self.b_canThrow` false)
      (set `self.b_HaveItem` false)
      ;[1 1 1] Clear Spline preview Mesh
      (`self.ClearMeshThrow` (`self.Spline`) (`self.SplineMesh1`))
      (`self.ClearMeshThrow` (`self.Spline1`) (`self.SplineMesh2`))
      (`SceneComponent.SetVisibility` (`self.EndSpline`) false false)
      (`ForceFeedbackComponent.Stop` (`self.ForceFeedback`)))))

(fn `UserConstructionScript`)