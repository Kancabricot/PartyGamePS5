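; BP_Throw is a helper actor that carries a thrown target actor along an arc of predefined points, then destroys itself.
; On BeginPlay it fits its spline to PointLocation, lowered for turrets, and notifies the target, while a timeline eases travel speed from fast to slower.
; Tick moves the target by spline distance, pitch-spinning scrap.
; At the spline's end it sends an end message unless TouchGround is set.
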(event `self.ReceiveBeginPlay`
  (bind _pointlocation (`self.PointLocation`))
  (bind _pointlocation_2 (`self.PointLocation`))
  (message `/Game/Blueprints/Interface/BPI_Throw.GetInfo` (`self.ActorTarget`) self)
  (for _index (range 21)
    (bind _returnvalue (`KismetArrayLibrary.Array_IsValidIndex` _pointlocation_2 _index))
    (`SplineComponent.SetLocationAtSplinePoint` (`self.Spline`) _index (- (select `bool` _returnvalue :`false` (`|GetArrayItem` _pointlocation (- (`KismetArrayLibrary.Array_Length` _pointlocation) 1)) :`true` (`|GetArrayItem` _pointlocation_2 _index)) (select `bool` (`.bSuccess` (cast `/Game/Blueprints/Turret/Blueprint/BP_Turrets` (`self.ActorTarget`) :!pure true)) :`true` (0.0 0.0 100.0) :!type "Vector Structure")) "World" true)
    (if _returnvalue
      (`SplineComponent.SetTangentAtSplinePoint` (`self.Spline`) _index (0.0 0.0 0.0) "World" true)))
  (`KismetSystemLibrary.Delay` 0.01)
  (set `self.b_CanThrow` true)
  (message `/Game/Blueprints/Interface/BPI_Throw.OnThrow` (`self.ActorTarget`))
  (`TimelineComponent.SetPlayRate` (`self.TL speed`) (/ 1.0 1.3))
  (bind (_direction _ease_speed) (`Timeline|TL speed` :!via `PlayFromStart`)
    (:`Update`
      (set `self.SplineSpeed` (`KismetMathLibrary.Lerp` 4000.0 900.0 _ease_speed)))))

(event `self.ReceiveTick`
  (params (DeltaSeconds :type "Float (single-precision)"))
  (bind _actortarget (`self.ActorTarget`))
  ;[1 1 1] todo
  (if (`self.b_CanThrow`)
    (set `self.DistanceAlongSpline` (+ (* DeltaSeconds (`self.SplineSpeed`)) (`self.DistanceAlongSpline`)))
    (bind _actortarget_2 (`self.ActorTarget`)
      (:`then`
        (`SceneComponent.K2_SetRelativeLocation` (`Actor.RootComponent` _actortarget_2) (.location (`SplineComponent.GetTransformAtDistanceAlongSpline` (`self.Spline`) (`self.DistanceAlongSpline`) "World" false)) false false)
        (`|ExecutionSequence`
          (:`then_0`
            (bind _spline (`self.Spline`)
              (:`then`
                (if (>= (`self.DistanceAlongSpline`) (`SplineComponent.GetSplineLength` _spline))
                  (if (not (`self.Touch Ground`))
                    (message `/Game/Blueprints/Interface/BPI_Throw.EndSpline` (`self.ActorTarget`)))
                  (`self.K2_DestroyActor`)))
              (:`else`)))
          (:`then_1`
            (if (`.bSuccess` (cast `/Game/Blueprints/Enemie/Blueprint/BP_Scrap` _actortarget :!pure true))
              (bind (_direction _newtrack_0) (`Timeline|rota`)
                (:`Update`
                  (`/Engine/EditorBlueprintResources/StandardMacros.IsValid` _actortarget
                    (:`Is Valid`
                      (`self.K2_SetActorRotation` (`self.ActorTarget`) (`KismetMathLibrary.MakeRotator` 0.0 (`KismetMathLibrary.Lerp` 0.0 360.0 _newtrack_0)) false)))))))))
      (:`else`
        (`self.K2_DestroyActor`)))))

(fn `UserConstructionScript`)