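; Local two-player setup actor that possesses the level's BP_Player pawns and pairs Joy-Cons at game start.
; BeginPlay resets Joy-Cons, creates the second local player, assigns indices and mapping contexts, then attaches both controllers in landscape grip.
; It spawns a camera target at the players' average location and points player 0's view at the shared BP_camera.
; Disconnect check and reconnect events handle pausing with a widget, but the check's timer is unwired.
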(event `self.ReceiveBeginPlay`
  (bind _output (`|GetArrayItem` (`self.PLayerArrayRef`)))
  (bind _output_2 (`|GetArrayItem` (`self.PLayerArrayRef`) 1))
  ;[1 1 1] Comment
  (`self.DisconnectJoycon`)
  (`|ExecutionSequence`
    (:`then_0`
      (bind _outactors (`GameplayStatics.GetAllActorsOfClass` "/Game/Blueprints/Player/Player/BP_Player.BP_Player_C"))
      (set `self.PLayerArrayRef` _outactors)
      (set `/Game/Blueprints/Player/Player/BP_Player.Player Index` 0 _output)
      (set `/Game/Blueprints/Player/Player/BP_Player.Mapping Context` "/Game/Input/IMC_Player1.IMC_Player1" _output)
      (set `/Game/Blueprints/Player/Player/BP_Player.LocalPlayerRef` self _output)
      (`Controller.Possess` (`GameplayStatics.GetPlayerController` 0) _output)
      (`GameplayStatics.CreatePlayer` 1)
      (set `/Game/Blueprints/Player/Player/BP_Player.Player Index` 1 _output_2)
      (set `/Game/Blueprints/Player/Player/BP_Player.Mapping Context` "/Game/Input/IMC_Player2.IMC_Player2" _output_2)
      (set `/Game/Blueprints/Player/Player/BP_Player.LocalPlayerRef` self _output_2)
      (`Controller.Possess` (`GameplayStatics.GetPlayerController` 1) _output_2)
      (`self.ConnectJoycon`)
      (`/Game/Blueprints/Player/Player/BP_Player.SetOrder` (`|GetArrayItem` (`self.PLayerArrayRef`)))
      (`/Game/Blueprints/Player/Player/BP_Player.SetOrder` _output_2)
      (bind _returnvalue (`GameplayStatics.GetActorArrayAverageLocation` (`self.PLayerArrayRef`)))
      (bind _returnvalue_2 (`|SpawnActorFromClass` "/Game/Blueprints/Player/Cam/BP_CamTarget.BP_CamTarget_C" (`KismetMathLibrary.MakeTransform` _returnvalue) "Undefined" "MultiplyWithRoot" null null))
      (set `self.CamTarget` _returnvalue_2)
      (`self.SetUpCam`)
      (`self.ConnectJoycon`))))

(event `VeriifConnetion`
  (bind _joycons (`JoyConDriverFunctionLibrary.SearchForJoyCons`))
  (bind _output_get (set `self.Joycons` _joycons))
  (if (`KismetArrayLibrary.Array_IsEmpty` _output_get)
    (`GameplayStatics.SetGamePaused` true :!label _label)
    (bind _returnvalue (`|CreateWidget` "/Game/Blueprints/Widgets/WG_Disconecte.WG_Disconecte_C"))
    (bind _output_get_2 (set `self.NewVar` _returnvalue))
    ;[1 1 1] Comment
    (`UserWidget.AddToViewport` _output_get_2 0)
    (elif (< (`KismetArrayLibrary.Array_Length` _output_get) 2)
      (switch `int` (`.ControllerId` (break `JoyConInformation` (`|GetArrayItem` (`self.Joycons`))))
        (:`0`
          (goto _label))
        (:`1`
          (goto _label))))))

(event `TryReconectJoycon`
  (bind _success (`self.ConnectJoycon`))
  (if _success
    (`Widget.RemoveFromParent` (`self.NewVar`))
    (`GameplayStatics.SetGamePaused` false)))

(event `SetUpCam`
  ;[1 1 1] Comment
  (bind _returnvalue (`GameplayStatics.GetActorOfClass` "/Game/Blueprints/Player/Cam/BP_camera.BP_camera_C"))
  (bind _output_get (set `self.CamRef` _returnvalue))
  (`/Game/Blueprints/Player/Cam/BP_CamTarget.CamTargetLocation` (`self.CamTarget`) (`self.PLayerArrayRef`) (`SceneComponent.K2_GetComponentLocation` (`/Game/Blueprints/Player/Cam/BP_camera.CenterRef` _output_get)))
  (`self.Possses`))

(fn `AttachJoycon`
  (params (GripIndex :type Integer) (ControlleurIndex :type Integer))
  (bind _joycons (`JoyConDriverFunctionLibrary.GetConnectedJoyCons`))
  (bind _success (`JoyConDriverFunctionLibrary.AttachJoyCon` (`.ControllerId` (break `JoyConInformation` (`|GetArrayItem` _joycons ControlleurIndex))) GripIndex))
  (`JoyConDriverFunctionLibrary.SetJoyConGripMode` GripIndex "Landscape")
  (if _success
    (set `self.NBJoyconConnected` (+ (`self.NBJoyconConnected`) 1))))

(fn `ConnectJoycon`
  (returns (Success :type Boolean))
  (`JoyConDriverFunctionLibrary.ResumeJoyConConnection`)
  (bind _joycons (`JoyConDriverFunctionLibrary.SearchForJoyCons`))
  (for _array_element _joycons
    (bind _success (`JoyConDriverFunctionLibrary.ConnectJoyCon` _array_element true true)))
  (`self.AttachJoycon` 0)
  (`self.AttachJoycon` 1 1)
  (return _success))

(fn `DisconnectJoycon`
  (bind _joycons (`JoyConDriverFunctionLibrary.GetAttachedJoyCons`))
  (for _array_element _joycons
    (`JoyConDriverFunctionLibrary.DetachJoyCon` (`.ControllerId` (break `JoyConInformation` _array_element))))
  (bind _joycons_2 (`JoyConDriverFunctionLibrary.GetConnectedJoyCons`))
  (for _array_element_2 _joycons_2
    (`JoyConDriverFunctionLibrary.DisconnectJoyCon` (`.ControllerId` (break `JoyConInformation` _array_element_2))))
  (set `self.NBJoyconConnected` 0))

(fn `Possses`
  (`PlayerController.SetViewTargetWithBlend` (`GameplayStatics.GetPlayerController` 0) (`self.CamRef`) 0.0 "VTBlend_Linear" 0.0 false)
  (`/Game/Blueprints/Player/Cam/BP_camera.SetLocationCam` (`self.CamRef`) (`self.CamTarget`) (`self.PLayerArrayRef`)))

(fn `UserConstructionScript`)