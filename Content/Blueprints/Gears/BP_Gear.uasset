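; BP_Gear is a gear actor that spins continuously at a fixed speed in either direction.
; The construction script assigns the Gear mesh variable to its static mesh component, so the mesh is set per instance or default.
; On BeginPlay, the SensHoraire (clockwise) boolean picks the sign of the RotatingMovement component's single-axis rotation rate, which then drives the spin without Tick logic.
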(event `self.ReceiveBeginPlay`
  (if (not (`self.Sens Horaire`))
    (set `RotatingMovementComponent.RotationRate` (struct :`Yaw` -180.0) (`self.RotatingMovement`))
    (else
      (set `RotatingMovementComponent.RotationRate` (struct :`Yaw` 180.0) (`self.RotatingMovement`)))))

(fn `UserConstructionScript`
  (`StaticMeshComponent.SetStaticMesh` (`self.StaticMesh`) (`self.Gear`)))