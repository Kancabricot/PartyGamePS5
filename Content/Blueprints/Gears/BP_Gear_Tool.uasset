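; Gear actor that places three tool actors in the level and sets its gear to a fixed rotation.
; On BeginPlay it spawns each tool class at the world transform of its matching placement component.
; It also starts a timer, with a negative start delay offsetting the interval, whose event snaps the gear to an absolute half-turn world rotation without interpolation.
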(event `self.ReceiveBeginPlay`
  (`self.Spawn tools`)
  (`KismetSystemLibrary.K2_SetTimerDelegate` (delegate `Turn Gear`) 5.0 false -5.0))

(event `Turn Gear`
  (`SceneComponent.K2_SetWorldRotation` (`self.Gear`) (struct :`Yaw` 180.0) false false))

(event `Spawn tools`
  (`|SpawnActorFromClass` (`self.Tool 1`) (`SceneComponent.K2_GetComponentToWorld` (`self.Tool Placement 1`)) "Undefined" "MultiplyWithRoot" null null)
  (`|SpawnActorFromClass` (`self.Tool 2`) (`SceneComponent.K2_GetComponentToWorld` (`self.Tool Placement 2`)) "Undefined" "MultiplyWithRoot" null null)
  (`|SpawnActorFromClass` (`self.Tool 3`) (`SceneComponent.K2_GetComponentToWorld` (`self.Tool Placement 3`)) "Undefined" "MultiplyWithRoot" null null))

(fn `UserConstructionScript`)