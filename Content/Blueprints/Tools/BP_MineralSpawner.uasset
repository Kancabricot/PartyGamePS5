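; BP_MineralSpawner is a station actor that keeps one mineral available at its item location.
; A looping two-second timer spawns an actor of the configured MineralType at the ItemLocation transform whenever the stored Item is no longer valid.
; It exposes a set of per-station Interact functions, returning itself from InteractMineralSpawner and nothing from the others, which lets callers identify the station type.
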(event `self.ReceiveBeginPlay`
  (`KismetSystemLibrary.K2_SetTimerDelegate` (delegate `Spawn Material`) 2.0 true -1.0))

(event `Spawn Material`
  (`/Engine/EditorBlueprintResources/StandardMacros.IsValid` (`self.Item`)
    (:`Is Not Valid`
      (bind _returnvalue (`|SpawnActorFromClass` (`self.Mineral Type`) (`SceneComponent.K2_GetComponentToWorld` (`self.ItemLocation`)) "Undefined" "MultiplyWithRoot" null null))
      (set `self.Item` _returnvalue))))

(fn `InteractDesk`
  (returns (Desk :type "/Game/Blueprints/Tools/BP_Desk Object Reference"))
  (return null))

(fn `InteractFurnance`
  (returns (Furnance :type "/Game/Blueprints/Tools/BP_Furnance Object Reference"))
  (return null))

(fn `InteractMineralSpawner`
  (returns (`Mineral Spawner` :type "/Game/Blueprints/Tools/BP_MineralSpawner Object Reference"))
  (return self))

(fn `InteractMixer`
  (returns (Mixer :type "/Game/Blueprints/Tools/BP_Mixer Object Reference"))
  (return null))

(fn `InteractPress`
  (returns (Press :type "/Game/Blueprints/Tools/BP_Press Object Reference"))
  (return null))

(fn `InteractSpout`
  (returns (Spout :type "/Game/Blueprints/Tools/BP_Spout Object Reference"))
  (return null))

(fn `InteractWorkBench`
  (returns (Workbench :type "/Game/Blueprints/Tools/BP_Etabli Object Reference"))
  (return null))

(fn `UserConstructionScript`)