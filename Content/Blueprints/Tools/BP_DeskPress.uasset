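; Desk press tool that stamps molten zinc, copper or brass into the matching gear when interacted with.
; Interact plays a timeline that moves the press between top and down positions, ignoring further interactions until it finishes.
; Near the peak of the stroke, each update calls MakeGear, which switches the ingredient enum to its gear type and refreshes it through SetIngredients.
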(event `self.ReceiveBeginPlay`
  (`parent.ReceiveBeginPlay`))

(event `/Game/Blueprints/Interface/BPI_Interact.Interact`
  (bind (_press_down_position_x _press_down_position_y _press_down_position_z) (`KismetMathLibrary.BreakVector` (`self.Press Down Position`)))
  (bind (_press_top_position_x _press_top_position_y _press_top_position_z) (`KismetMathLibrary.BreakVector` (`self.Press Top Position`)))
  (if (not (`self.b_IsPress`))
    (set `self.b_IsPress` true)
    (bind (_direction _newtrack_0) (`Timeline|Timeline` :!via `PlayFromStart`)
      (:`Update`
        (if (> _newtrack_0 0.9)
          (`self.MakeGear`))
        (`SceneComponent.K2_SetRelativeLocation` (`self.Press`) (`KismetMathLibrary.MakeVector` 0.0 0.0 (`KismetMathLibrary.Lerp` _press_top_position_z _press_down_position_z _newtrack_0)) false false))
      (:`Finished`
        (set `self.b_IsPress` false)))))

(fn `MakeGear`
  (switch `/Game/Blueprints/Enums/Enum_Ingredients` (`self.Enum_Ingredients`)
    (:`NewEnumerator4`
      (set `self.Enum_Ingredients` "NewEnumerator7")
      (`self.SetIngredients` null))
    (:`NewEnumerator5`
      (set `self.Enum_Ingredients` "NewEnumerator8")
      (`self.SetIngredients` null))
    (:`NewEnumerator6`
      (set `self.Enum_Ingredients` "NewEnumerator9")
      (`self.SetIngredients` null))))

(fn `UserConstructionScript`
  (`parent.UserConstructionScript`))