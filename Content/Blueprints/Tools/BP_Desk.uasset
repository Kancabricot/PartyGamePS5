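; BP_Desk is a desk that holds one crafting ingredient, from zinc mineral through processed parts to turrets, for a player to take.
; An ingredient enum drives the displayed mesh and material through a switch, refreshed on BeginPlay and whenever SetIngredient stores a new item.
; TakeIngredient copies the enum to the player, updates their mesh, then resets the desk to Default, which clears the display.
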(event `self.ReceiveBeginPlay`
  (`self.SetIngredients` (`self.Ingredients`) (`self.Enum_Ingredients`)))

(event `/Game/Blueprints/Interface/BPI_SetIngredients.TakeIngredient`
  (params (Player :type "/Game/Blueprints/BP_Player Object Reference"))
  (set `/Game/Blueprints/BP_Player.Enum_Ingrediants` (`self.Enum_Ingredients`) Player)
  (`/Game/Blueprints/BP_Player.SetIngredientsMesh` Player)
  (set `self.Enum_Ingredients` "NewEnumerator3")
  (`self.SetIngredients` (`self.Ingredients`) (`self.Enum_Ingredients`)))

(fn `SetIngredient`
  (params (E_Ingredients :type "/Game/Blueprints/Enums/Enum_Ingredients Enum" :default "NewEnumerator3"))
  (set `self.Enum_Ingredients` E_Ingredients)
  (`self.SetIngredients` (`self.Ingredients`) (`self.Enum_Ingredients`))
  (return))

(fn `SetIngredients`
  (params (Target :type "StaticMeshComponent Object Reference") (Selection :type "/Game/Blueprints/Enums/Enum_Ingredients Enum" :default "NewEnumerator3"))
  (bind _target (`local.Target`))
  (switch `/Game/Blueprints/Enums/Enum_Ingredients` Selection
    (:`NewEnumerator3`
      ;[1 1 1] Mineral
      (`self.SetMeshAndMaterial` _target))
    (:`NewEnumerator0`
      (`self.SetMeshAndMaterial` _target "/Game/Assets/Mineral.Mineral" "/Game/Assets/Materials/Zinc/M_Zinc_Mineral.M_Zinc_Mineral"))
    (:`NewEnumerator4`
      ;[1 1 1] molted
      (`self.SetMeshAndMaterial` (`local.Target`) "/Game/Assets/Ingot.Ingot" "/Game/Assets/Materials/Zinc/M_Fusion_Zinc.M_Fusion_Zinc"))
    (:`NewEnumerator7`
      ;[1 1 1] Gear
      (`self.SetMeshAndMaterial` (`local.Target`) "/Game/Assets/Gears/Thibault/Gear5.Gear5" "/Game/Assets/Materials/Zinc/M_Zinc.M_Zinc"))
    (:`NewEnumerator11`
      ;[1 1 1] Tige
      (`self.SetMeshAndMaterial` (`local.Target`) "/Game/Assets/Materials/Zinc/Import/ZincTige.ZincTige" "/Game/Assets/Materials/Zinc/M_Zinc.M_Zinc"))
    (:`NewEnumerator10`
      ;[1 1 1] Turret
      (`self.SetMeshAndMaterial` (`local.Target`) "/Game/Assets/Turret/Turret.Turret" "/Game/Assets/Materials/Zinc/M_Zinc.M_Zinc"))
    (:`NewEnumerator12`
      (`self.SetMeshAndMaterial` (`local.Target`) "/Game/Assets/Turret/Big_Turret.Big_Turret" "/Game/Assets/Materials/Zinc/M_Zinc.M_Zinc"))
    (:`NewEnumerator13`
      (`self.SetMeshAndMaterial` (`local.Target`) "/Game/Assets/Turret/Sniper_T.Sniper_T" "/Game/Assets/Materials/Zinc/M_Zinc.M_Zinc"))))

(fn `SetMeshAndMaterial`
  (params (Target :type "StaticMeshComponent Object Reference") (NewMesh :type "StaticMesh Object Reference") (NewMaterial :type "MaterialInterface Object Reference"))
  (`StaticMeshComponent.SetStaticMesh` Target NewMesh)
  (`PrimitiveComponent.SetMaterial` Target 0 NewMaterial))

(fn `UserConstructionScript`)