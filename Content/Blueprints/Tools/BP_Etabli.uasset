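; BP_Etabli is the workbench actor among the game's tool Blueprints.
; It has a set of per-station Interact functions for desk, furnace, mineral spawner, mixer, press, spout and workbench.
; Only InteractWorkBench returns self and the rest return empty, so the functions act as a type query in place of a cast.
; The event graph and construction script hold no logic.
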(fn `InteractDesk`
  (returns (Desk :type "/Game/Blueprints/Tools/BP_Desk Object Reference"))
  (return null))

(fn `InteractFurnance`
  (returns (Furnance :type "/Game/Blueprints/Tools/BP_Furnance Object Reference"))
  (return null))

(fn `InteractMineralSpawner`
  (returns (`Mineral Spawner` :type "/Game/Blueprints/Tools/BP_MineralSpawner Object Reference"))
  (return null))

(fn `InteractMixer`
  (returns (Mixer :type "/Game/Blueprints/Tools/BP_Mixer Object Reference"))
  (return null))

(fn `InteractPress`
  (returns (Press :type "/Game/Blueprints/Tools/BP_Press Object Reference"))
  (return null))

(fn `InteractSpout`
  (returns (Spout :type "/Game/Blueprints/Tools/BP_Spout Object Reference"))
  (return null))

(fn `InteractWorkBench`
  (returns (Workbench :type "/Game/Blueprints/Tools/BP_Etabli Object Reference"))
  (return self))

(fn `UserConstructionScript`)