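; Desk furnace that melts a placed ingredient over time and shows progress on a WG_Temperature widget.
; Tick raises PercentMelt by a fixed per-frame step for one ingredient type with Niagara active; at full, MeltMineral switches the ingredient enum and the effect stops.
; Other ingredient types only activate the effect, while a missing or non-ingredient actor resets progress.
; Interact is empty, and the DecrementeHeat cooldown function is not called here.
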(event `self.ReceiveBeginPlay`
  (`parent.ReceiveBeginPlay`)
  (bind _aswg_temperature (cast `/Game/Blueprints/Widgets/WG_Temperature` (`WidgetComponent.GetWidget` (`self.Widget`))))
  (set `self.WGRef` _aswg_temperature))

(event `self.ReceiveTick`
  (params (DeltaSeconds :type "Float (single-precision)"))
  (bind _percentmelt (`self.PercentMelt`))
  (`/Game/Blueprints/Widgets/WG_Temperature.SetTimer` (`self.WGRef`) (`self.PercentMelt`))
  (bind _actor (`self.Actor`)
    (:`then`
      (bind _asbp_ingredients (cast `/Game/Blueprints/BP_Ingredients` _actor)
        (:`then`
          (if (`|EnumEquality` (`/Game/Blueprints/BP_Ingredients.Enum_Ingredients` _asbp_ingredients) "NewEnumerator0")
            (if (< _percentmelt 100.0)
              (set `self.PercentMelt` (+ _percentmelt 0.5))
              (if (not (`ActorComponent.IsActive` (`self.Niagara`))) :!label _label
                (`ActorComponent.Activate` (`self.Niagara`) false))
              (else
                (`self.MeltMineral`)
                (`ActorComponent.Deactivate` (`self.Niagara`))))
            (else
              (goto _label))))
        (:`CastFailed`
          (set `self.PercentMelt` 0.0 :!label _label_2))))
    (:`else`
      (goto _label_2))))

(event `/Game/Blueprints/Interface/BPI_Interact.Interact`)

(fn `DecrementeHeat`
  (bind _furnaceheat (`self.FurnaceHeat`))
  (if (> _furnaceheat 0.0)
    (bind _output_get (set `self.FurnaceHeat` (- _furnaceheat 0.01)))
    (`KismetSystemLibrary.PrintString` (`KismetStringLibrary.Conv_DoubleToString` _output_get) true true (struct :`G` 0.66 :`B` 1.0 :`A` 1.0) 0.001)
    (else
      (`ActorComponent.SetActive` (`self.Niagara`) false false))))

(fn `MeltMineral`
  (bind _asbp_ingredients (cast `/Game/Blueprints/BP_Ingredients` (`self.Actor`)))
  (set `/Game/Blueprints/BP_Ingredients.Enum_Ingredients` "NewEnumerator4" _asbp_ingredients)
  (set `self.Enum_Ingredients` "NewEnumerator4"))

(fn `UserConstructionScript`
  (`parent.UserConstructionScript`))