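; Desk saw tool Blueprint that cuts the ingredient placed on it, currently only turning a Zinc Ingot into a ZincTige.
; SetIngredient resets the Ingredients component to its start position and applies the given ingredient enum.
; Interact plays a timeline that sweeps the component toward EndItem, then CutItem swaps the enum and updates Ingredients, with a leftover debug print.
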(event `self.ReceiveBeginPlay`
  (`parent.ReceiveBeginPlay`))

(event `/Game/Blueprints/Interface/BPI_Interact.Interact`
  (bind (_direction _track) (`Timeline|SawTimeline` :!via `PlayFromStart`)
    (:`Update`
      (`SceneComponent.K2_SetRelativeLocation` (`self.Ingredients`) (`KismetMathLibrary.VLerp` (0.0 0.0 90.0) (`SceneComponent.RelativeLocation` (`self.EndItem`)) _track) true false))
    (:`Finished`
      (`self.CutItem`))))

(event `/Game/Blueprints/Interface/BPI_SetIngredients.SetIngredient`
  (params (E_Ingredients :type "/Game/Blueprints/Enums/Enum_Ingredients Enum" :default "NewEnumerator3"))
  (`SceneComponent.K2_SetRelativeLocation` (`self.Ingredients`) (0.0 0.0 90.0) false false)
  (bind _output_get (set `self.Enum_Ingredients` E_Ingredients))
  (`self.SetIngredients` (`self.Ingredients`) _output_get))

(fn `CutItem`
  (switch `/Game/Blueprints/Enums/Enum_Ingredients` (`self.Enum_Ingredients`)
    (:`NewEnumerator4`
      (bind _output_get (set `self.Enum_Ingredients` "NewEnumerator11"))
      (`self.SetIngredients` (`self.Ingredients`) _output_get)
      (`KismetSystemLibrary.PrintString` "Hello"))))

(fn `UserConstructionScript`
  (`parent.UserConstructionScript`))