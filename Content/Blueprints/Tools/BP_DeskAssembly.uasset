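; BP_DeskAssembly is an assembly desk that holds up to two ingredients and combines a specific pair into a new one.
; SetIngredient fills the first slot if empty, otherwise overwrites the second, updating that slot's display.
; TakeIngredient hands the player the first slot's item, falling back to the second, then clears that slot.
; Interact checks for the hard-coded pair in either order, leaving the result in the first slot and emptying the second.
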(event `self.ReceiveBeginPlay`
  (`parent.ReceiveBeginPlay`))

(event `/Game/Blueprints/Interface/BPI_SetIngredients.SetIngredient`
  (params (E_Ingredients :type "/Game/Blueprints/Enums/Enum_Ingredients Enum" :default "NewEnumerator3"))
  (if (`|EnumEquality` (`self.Enum_Ingredients`) "NewEnumerator3")
    (set `self.Enum_Ingredients` E_Ingredients)
    (`self.SetIngredients` (`self.Ingredients`) (`self.Enum_Ingredients`))
    (else
      (bind _output_get (set `self.Enum_IngredientsNumber2` E_Ingredients))
      (`self.SetIngredients` (`self.Ingredients1`) _output_get))))

(event `/Game/Blueprints/Interface/BPI_SetIngredients.TakeIngredient`
  (params (Player :type "/Game/Blueprints/BP_Player Object Reference"))
  (if (not (`|EnumEquality` (`self.Enum_Ingredients`) "NewEnumerator3"))
    (set `/Game/Blueprints/BP_Player.Enum_Ingrediants` (`self.Enum_Ingredients`) Player)
    (`/Game/Blueprints/BP_Player.SetIngredientsMesh` Player)
    (set `self.Enum_Ingredients` "NewEnumerator3")
    (`self.SetIngredients` (`self.Ingredients`) (`self.Enum_Ingredients`))
    (else
      (set `/Game/Blueprints/BP_Player.Enum_Ingrediants` (`self.Enum_IngredientsNumber2`) Player)
      (`/Game/Blueprints/BP_Player.SetIngredientsMesh` Player)
      (set `self.Enum_IngredientsNumber2` "NewEnumerator3")
      (`self.SetIngredients` (`self.Ingredients1`) (`self.Enum_IngredientsNumber2`)))))

(event `/Game/Blueprints/Interface/BPI_Interact.Interact`
  (if (or (and (`|EnumEquality` (`self.Enum_Ingredients`) "NewEnumerator4") (`|EnumEquality` "NewEnumerator7" (`self.Enum_IngredientsNumber2`))) (and (`|EnumEquality` (`self.Enum_Ingredients`) "NewEnumerator7") (`|EnumEquality` "NewEnumerator4" (`self.Enum_IngredientsNumber2`))))
    (set `self.Enum_IngredientsNumber2` "NewEnumerator3")
    (`self.SetIngredients` (`self.Ingredients1`) (`self.Enum_IngredientsNumber2`))
    (set `self.Enum_Ingredients` "NewEnumerator10")
    (`self.SetIngredients` (`self.Ingredients`) (`self.Enum_Ingredients`))))

(fn `UserConstructionScript`
  (`parent.UserConstructionScript`))