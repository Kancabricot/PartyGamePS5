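; BP_Ingredients is an ingredient actor that players can pick up and throw, applying its configured mesh and material on BeginPlay.
; TakeItem passes it to the player and disables collision and physics, while GiveItemToDesk always returns false.
; DettachItem restores both, applies the given velocity and starts a timeline.
; The timeline destroys the actor only if BIsGrab is false, yet both TakeItem and DettachItem set it true.
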(event `/Game/Blueprints/Interface/BPI_TakeItem.DettachItem`
  (params (Impulse :type "Vector Structure"))
  (`PrimitiveComponent.SetCollisionEnabled` (`self.Item`) "QueryAndPhysics")
  (`PrimitiveComponent.SetSimulatePhysics` (`self.Item`) true)
  (`PrimitiveComponent.SetPhysicsLinearVelocity` (`self.Item`) Impulse false "None")
  (set `self.b_IsGrab` true)
  (`self.StartDelay`))

(event `self.ReceiveBeginPlay`
  (`self.SetMesh`))

(event `StartDelay`
  (`Timeline|Timeline` :!via `PlayFromStart`
    (:`Finished`
      (if (not (`self.b_IsGrab`))
        (`self.K2_DestroyActor`)))))

(event `SpawnCatch`
  (`PrimitiveComponent.SetCollisionEnabled` (`self.Item`) "NoCollision"))

(fn `GiveItemToDesk`
  (params (ActorTarget :type "Actor Object Reference"))
  (returns (Return :type Boolean))
  (return false))

(fn `SetMesh`
  (`self.SetMeshAndMaterial` (`self.Item`) (`self.Mesh`) (`self.Material`)))

(fn `SetMeshAndMaterial`
  (params (Target :type "StaticMeshComponent Object Reference") (NewMesh :type "StaticMesh Object Reference") (NewMaterial :type "MaterialInterface Object Reference"))
  (`StaticMeshComponent.SetStaticMesh` Target NewMesh)
  (`PrimitiveComponent.SetMaterial` Target 0 NewMaterial))

(fn `TakeItem`
  (params (Player :type "/Game/Blueprints/Player/BP_Player Object Reference"))
  (returns (Return :type Boolean))
  (`/Game/Blueprints/Player/BP_Player.TakeItem` Player 0.0 self)
  (`PrimitiveComponent.SetCollisionEnabled` (`self.Item`) "NoCollision")
  (`PrimitiveComponent.SetSimulatePhysics` (`self.Item`) false)
  (set `self.b_IsGrab` true)
  (return true))

(fn `UserConstructionScript`)