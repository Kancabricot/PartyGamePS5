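; BP_RoboticArm is a robotic arm actor that moves between preset world positions using timelines.
; Move lerps the actor between two indexed Location array points, then advances both indices with wraparound.
; Step2 plays a bug animation, slides the arm to Phase2Location after a delay, then reverses back once, guarded by a flag.
; BeginPlay is empty, and the looping move timer and delayed Step2 trigger are disconnected.
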(event `self.ReceiveBeginPlay`)

(event `Call Move`
  (`self.Move `))

(event `Move`
  (bind (_direction _move_alpha) (`Timeline|TL_Move` :!via `PlayFromStart`)
    (:`Update`
      (`self.K2_SetActorLocation` (`KismetMathLibrary.VLerp` (`|GetArrayItem` (`self.Location `) (`self.Location Index `)) (`|GetArrayItem` (`self.Location `) (`self.Location Index + 1`)) _move_alpha)))
    (:`Finished`
      (if (> (+ (`self.Location Index + 1`) 1) (- (`KismetArrayLibrary.Array_Length` (`self.Location `)) 2))
        (set `self.Location Index + 1` 0)
        (else
          (set `self.Location Index + 1` (+ (`self.Location Index + 1`) 1))))
      (if (> (+ (`self.Location Index `) 1) (- (`KismetArrayLibrary.Array_Length` (`self.Location `)) 2))
        (set `self.Location Index ` 0)
        (else
          (set `self.Location Index ` (+ (`self.Location Index `) 1)))))))

(event `Step 2`
  (`SkeletalMeshComponent.PlayAnimation` (`self.SkeletalMesh`) "/Game/Assets/roboticArm/Animations/A_Arm_Bug_bug.A_Arm_Bug_bug" false)
  (`KismetSystemLibrary.Delay` 2.0)
  (set `self.Temp Actor Location` (`self.K2_GetActorLocation`))
  (bind (_direction _alpha) (`Timeline|TL_Step2` :!via `PlayFromStart` :!label _label)
    (:`Update`
      (`self.K2_SetActorLocation` (`KismetMathLibrary.VLerp` (`self.Temp Actor Location`) (`self.Phase 2 location`) _alpha)))
    (:`Finished`
      (if (not (`self.b_Step2_is_finished`))
        (`KismetSystemLibrary.Delay` 2.0)
        (`self.End Step 2`)
        (set `self.b_Step2_is_finished` true)))))

(event `End Step 2`
  (goto _label :!via `ReverseFromEnd`))

(fn `UserConstructionScript`)