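; BP_Storage is a storage machine that dispenses ingredients to players and refuses items given to it.
; A timeline moves the displayed item vertically, and the construction script sets its mesh for the Gear Zinc ingredient.
; TakeItem spawns a BP_Ingredients copy of the display far off in Z and hands it to the player.
; It also shows a fixed gear icon on the player's widget and starts a looping RotateWidget timer.
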(event `self.ReceiveBeginPlay`
  (bind (_direction _movement) (`Timeline|Movement`)
    (:`Update`
      (`SceneComponent.K2_SetRelativeLocation` (`self.Item`) (`KismetMathLibrary.MakeVector` 0.0 0.0 (`KismetMathLibrary.Lerp` 100.0 200.0 _movement)) false false))))

(fn `GiveItemToDesk`
  (params (ActorTarget :type "Actor Object Reference"))
  (returns (Return :type Boolean))
  (return false))

(fn `TakeItem`
  (params (Player :type "/Game/Blueprints/Player/Player/BP_Player Object Reference"))
  (returns (Return :type Boolean))
  (bind _item (`self.Item`))
  (bind _widget (`/Game/Blueprints/Player/Player/BP_Player.Widget` Player))
  (bind _output_get (set `self.ActuPlayer` Player))
  (bind _returnvalue (`KismetSystemLibrary.K2_SetTimer` _output_get "RotateWidget" 0.1 true))
  (set `self.ActuTimer` _returnvalue)
  (bind _returnvalue_2 (`|SpawnActorFromClass` "/Game/Blueprints/Machine/BP_Ingredients.BP_Ingredients_C" (`KismetMathLibrary.MakeTransform` (0.0 0.0 1000000.0)) "Undefined" "MultiplyWithRoot" null (`StaticMeshComponent.StaticMesh` _item) (`PrimitiveComponent.GetMaterial` _item 0) (`self.Ingredient`) null null))
  (set `/Game/Blueprints/Machine/BP_Ingredients.ActuPlayer` Player _returnvalue_2)
  (bind _aswg_icon (cast `/Game/Blueprints/Arrow/WG_Icon` (`WidgetComponent.GetWidget` _widget))
    (:`then`
      (`/Game/Blueprints/Arrow/WG_Icon.SetImage` _aswg_icon "/Game/Blueprints/Arrow/PictoEngrenage_cercle.PictoEngrenage_cercle")
      (`SceneComponent.SetVisibility` _widget true false))
    (:`CastFailed`
      _))
  (`/Game/Blueprints/Player/Player/BP_Player.TakeItem` Player _returnvalue_2)
  (`/Game/Blueprints/Machine/BP_Ingredients.SpawnCatch` _returnvalue_2)
  (return true))

(fn `UserConstructionScript`
  (switch `/Game/Blueprints/Enums/Enum_Ingredients` (`self.Ingredient`)
    (:`NewEnumerator7`
      (`StaticMeshComponent.SetStaticMesh` (`self.Item`) "/Engine/BasicShapes/Sphere.Sphere"))))