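; Smelter machine that turns dropped BP_Scrap into BP_Turret items for the player.
; Overlapping scrap is destroyed while a timeline spins the crushers and fills the melt tank.
; Holding Interact runs a looping timer that tilts the vat and drains the tank into the turret mold; release tilts it back.
; A full mold triggers a timeline, then swaps material, letting TakeItem spawn a turret into the player's hands and reset the mold.
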(event `self.TriggerCrusher.OnComponentBeginOverlap`
  (params (OverlappedComponent :type "PrimitiveComponent Object Reference") (OtherActor :type "Actor Object Reference") (OtherComp :type "PrimitiveComponent Object Reference") (OtherBodyIndex :type Integer) (bFromSweep :type Boolean) (SweepResult :type "HitResult Structure (by ref)"))
  (bind _asbp_scrap (cast `/Game/Blueprints/Enemie/Blueprint/BP_Scrap` OtherActor))
  (`self.K2_DestroyActor` _asbp_scrap)
  (bind (_direction _newtrack_0) (`Timeline|T_Crusher` :!via `PlayFromStart`)
    (:`Update`
      (bind (_returnvalue_roll _returnvalue_pitch) (`KismetMathLibrary.BreakRotator` (`KismetMathLibrary.RLerp` (struct) (struct :`Pitch` 720.0) _newtrack_0)))
      (`SceneComponent.K2_SetRelativeRotation` (`self.Crusher2`) (`KismetMathLibrary.NegateRotator` (`KismetMathLibrary.MakeRotator` 0.0 _returnvalue_pitch)) false false)
      (`SceneComponent.K2_SetRelativeRotation` (`self.Crusher1`) (`KismetMathLibrary.MakeRotator` 0.0 _returnvalue_pitch) false false)
      (`SceneComponent.K2_SetRelativeLocation` (`self.MeltedScrapbac`) (`KismetMathLibrary.VLerp` (64.505291 -1.651919 -76.402662) (64.505291 -1.651919 -16.402662) _newtrack_0) false false)
      (set `self.SmeltTank` _newtrack_0))))

(event `/Game/Blueprints/Interface/BPI_Interact.Interact`
  (if (`self.b_NeedMelt`)
    (set `self.b_IsPressed` true)
    (bind _returnvalue (`KismetSystemLibrary.K2_SetTimerDelegate` (delegate `Smelt`) 0.01 true))
    (if (not (`KismetSystemLibrary.K2_IsValidTimerHandle` (`self.TimeSmelt`)))
      (set `self.TimeSmelt` _returnvalue))))

(event `/Game/Blueprints/Interface/BPI_Interact.Release`
  (set `self.b_IsPressed` false))

(event `Smelt`
  (if (`self.b_IsPressed`)
    (if (`self.b_CuveIsDown`)
      (if (not (<= (`self.SmeltTank`) 0.0))
        (bind _output_get (set `self.SmeltTank` (- (`self.SmeltTank`) 0.01)))
        (`SceneComponent.K2_SetRelativeLocation` (`self.MeltedTurret`) (`KismetMathLibrary.VLerp` (5.627284 -119.742409 47.895939) (5.627284 -119.742409 -21.223185) _output_get) false false)
        (`SceneComponent.K2_SetRelativeLocation` (`self.MeltedScrapbac`) (`KismetMathLibrary.VLerp` (64.505291 -1.651919 -76.402662) (64.505291 -1.651919 -16.402662) _output_get) false false)
        (bind _output_get_2 (set `self.PaternTank` (+ (`self.PaternTank`) 0.01)))
        (if (>= _output_get_2 1.0)
          (`self.StartCuveUp`)
          (`self.MeltPatern`)))
      (else
        (`self.StartCuveDown`)))
    (else
      (`KismetSystemLibrary.K2_PauseTimerHandle` (`self.TimeSmelt`))
      (`/Engine/EditorBlueprintResources/StandardMacros.DoOnce` false :!label _label
        (:`Completed`
          (`self.StartCuveUp`))))))

(event `MeltPatern`
  (`Timeline|T_Patern` :!via `PlayFromStart`
    (:`Finished`
      (`PrimitiveComponent.SetMaterial` (`self.MeltedTurret`) 0 "/Engine/EditorMaterials/Camera/CineMat.CineMat")
      (set `self.b_NeedMelt` false))))

(event `StartCuveDown`
  (`|ExecutionSequence`
    (:`then_0`
      (goto _label :!via `Reset`))
    (:`then_1`
      (bind (_direction _newtrack_0) (`Timeline|T_Cuve` :!label _label_2)
        (:`Update`
          (`SceneComponent.K2_SetRelativeRotation` (`self.Cuve`) (`KismetMathLibrary.RLerp` (struct) (struct :`Pitch` 100.0) _newtrack_0) false false))
        (:`Finished`
          (if (> _newtrack_0 0.5)
            (set `self.b_CuveIsDown` true)))))))

(event `StartCuveUp`
  (set `self.b_CuveIsDown` false)
  (goto _label_2 :!via `Reverse`))

(fn `GetSnapValue`
  (params (ActorToThrow :type "Actor Object Reference"))
  (returns (DropPosition :type "Vector Structure") (b_CanSnap :type Boolean))
  (cast `/Game/Blueprints/Enemie/Blueprint/BP_Scrap` ActorToThrow
    (:`then`
      (return (`SceneComponent.K2_GetComponentLocation` (`self.Crusher2`)) true))
    (:`CastFailed`
      (return (0.0 0.0 0.0) false))))

(fn `GiveItemToDesk`
  (params (ActorTarget :type "Actor Object Reference"))
  (returns (Return :type Boolean))
  (return false))

(fn `TakeItem`
  (params (Player :type "/Game/Blueprints/Player/Player/BP_Player Object Reference"))
  (returns (Return :type Boolean))
  (bind _meltedturret (`self.MeltedTurret`))
  (if (not (`self.b_NeedMelt`))
    (bind _returnvalue (`|SpawnActorFromClass` "/Game/Blueprints/Turret/Blueprint/BP_Turret.BP_Turret_C" (`KismetMathLibrary.MakeTransform` (0.0 0.0 0.0)) "Undefined" "MultiplyWithRoot" null false (`self.DechargeSpeed`) null))
    (set `/Game/Blueprints/Turret/Blueprint/BP_Turret.b_IsGrab` true _returnvalue)
    (`/Game/Blueprints/Player/Player/BP_Player.TakeItem` Player _returnvalue)
    (`/Game/Blueprints/Turret/Blueprint/BP_Turret.SpawnCatch` _returnvalue)
    (set `self.PaternTank` 0.0)
    (`SceneComponent.K2_SetRelativeLocation` _meltedturret (5.627284 -119.742409 -21.223185) false false)
    (`PrimitiveComponent.SetMaterial` _meltedturret 0 "/Engine/MapTemplates/Materials/BasicAsset01.BasicAsset01")
    (set `self.b_NeedMelt` true)
    (return true)
    (else
      (return false))))

(fn `UserConstructionScript`)