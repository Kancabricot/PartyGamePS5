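; Manager that shuffles the positions of the three printer machines and updates the BP_BaseSlime actors to match.
; Shuffle flags the request if any printer is crafting, otherwise it animates printers and slime bases.
; ShuffleMachine waits on no printer switching, randomizes stored transforms, recursively retrying when multiple slots stay unchanged, then moves the printers.
; Ray follows after a delay, closing each slime base's door and re-detecting its slime type.
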(event `self.ReceiveBeginPlay`
  ;[1 1 1] BeginPlay
  (bind _outactors (`GameplayStatics.GetAllActorsOfClass` "/Game/Blueprints/Machine/BP_BaseSlime.BP_BaseSlime_C"))
  (set `self.BaseSlimeRefs` _outactors))

(event `Shuffle`
  (bind _printer_ref (`self.Printer ref`))
  ;[1 1 1] SuffleEvent
  ;;[1 1 1] DelayBeforeShuffle
  (if (or (`/Game/Blueprints/Machine/BP_Slime.IsCrafting` (`|GetArrayItem` _printer_ref)) (`/Game/Blueprints/Machine/BP_Slime.IsCrafting` (`|GetArrayItem` _printer_ref 1)) (`/Game/Blueprints/Machine/BP_Slime.IsCrafting` (`|GetArrayItem` _printer_ref 2)))
    ;;[1 1 1] Keep Shuffle in memory if machine is crafting
    (set `self.b_NeedToShuffle` true)
    (else
      (for _array_element (`self.Printer ref`)
        ;;[1 1 1] Next shuffle
        (`/Game/Blueprints/Machine/BP_Slime.Anim` _array_element true))
      (for _array_element_2 (`self.BaseSlimeRefs`)
        (`/Game/Blueprints/Machine/BP_BaseSlime.Anim` _array_element_2)))))

(event `Ray`
  (`KismetSystemLibrary.Delay` 1.0)
  (bind _outactors (`GameplayStatics.GetAllActorsOfClass` "/Game/Blueprints/Machine/BP_BaseSlime.BP_BaseSlime_C"))
  (for _array_element _outactors
    (`/Game/Blueprints/Machine/BP_BaseSlime.CloseDoort` _array_element)
    (`/Game/Blueprints/Machine/BP_BaseSlime.DetectTypeOfSlime` _array_element)))

(fn `ShuffleMachine`
  (locals (TempRef :type "/Game/Blueprints/Enums/Enum_Kit Enum") (ActuPrinter :type "/Game/Blueprints/Machine/BP_Slime Object Reference") (TypeToChange :type "Array of /Game/Blueprints/Enums/Enum_Kit Enum") (LatestTransformTab :type "Array of Transform Structure") (Verif :type "Array of Boolean") (NeedToShuffle :type Boolean) (NeedToShuffle2 :type Boolean))
  (bind _trasnfortemp (`self.TrasnforTemp`))
  (bind _printer_ref (`self.Printer ref`))
  ;[1 1 1] SuffleFunction
  (if (not (or (`/Game/Blueprints/Machine/BP_Slime.IsSwitching` (`|GetArrayItem` _printer_ref)) (`/Game/Blueprints/Machine/BP_Slime.IsSwitching` (`|GetArrayItem` _printer_ref 1)) (`/Game/Blueprints/Machine/BP_Slime.IsSwitching` (`|GetArrayItem` _printer_ref 2))))
    (set `local.LatestTransformTab` _trasnfortemp)
    (if (>= (`KismetArrayLibrary.Array_Length` _trasnfortemp) 3)
      (`KismetArrayLibrary.Array_Shuffle` (`self.TrasnforTemp`))
      (for (_array_element _array_index) (`local.LatestTransformTab`)
        (if (== _array_element (`|GetArrayItem` (`self.TrasnforTemp`) _array_index))
          (if (`local.NeedToShuffle`)
            (set `local.NeedToShuffle2` true)
            (else
              (set `local.NeedToShuffle` true)))))
      (if (and (`local.NeedToShuffle`) (`local.NeedToShuffle2`))
        (`KismetArrayLibrary.Array_Clear` (`local.LatestTransformTab`))
        (`self.ShuffleMachine`)
        (else
          (for (_array_element_2 _array_index_2) (`self.Printer ref`)
            (bind _output (`|GetArrayItem` (`self.TrasnforTemp`) _array_index_2))
            (`/Game/Blueprints/Machine/BP_Slime.ReversiAim` _array_element_2 (.z (.location _output)) true 0)
            (`self.K2_SetActorTransform` _array_element_2 (`KismetMathLibrary.MakeTransform` (`KismetMathLibrary.MakeVector` (.x (.location _output)) (.y (.location _output)) (.z (.location _output))) (.rotation _output) (.scale _output)) false false)
            (set `/Game/Blueprints/Machine/BP_Slime.IsInTab` false _array_element_2))
          (`self.Ray`)
          (`KismetArrayLibrary.Array_Clear` (`local.LatestTransformTab`))
          (for _array_element_3 (`self.Printer ref`)
            (`/Game/Blueprints/Machine/BP_Slime.cleartab` _array_element_3)))))))

(fn `UserConstructionScript`
  (if (> (`self.MinDuration`) (`self.MaxDuration`))
    (set `self.MaxDuration` (`self.MinDuration`))))