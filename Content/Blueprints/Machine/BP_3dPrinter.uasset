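; 3D printer machine that turns scrap into turret kits of the type set on the printer.
; Scrap entering its box while awake is destroyed and its value banked; reaching the threshold starts crafting, deducts the cost and begins sleep.
; After a short delay it spawns a BP_TurretKit and launches it along the arrow.
; Type sets the cube's color, which turns gray during the timed cooldown and is restored on wakeup.
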(event `CreateAddons`
  (set `self.IsCrafting` true)
  (`KismetSystemLibrary.Delay` 1.5)
  (bind _returnvalue (`|SpawnActorFromClass` "/Game/Blueprints/Turret/Blueprint/BP_TurretKit.BP_TurretKit_C" (`KismetMathLibrary.MakeTransform` (`SceneComponent.K2_GetComponentLocation` (`self.Scene`)) (struct) (2.0 2.0 2.0)) "Undefined" "MultiplyWithRoot" null (`self.TypeOfPrinter`) null null))
  (`PrimitiveComponent.SetAllPhysicsLinearVelocity` (`/Game/Blueprints/Turret/Blueprint/BP_TurretKit.Kit` _returnvalue) (* (`SceneComponent.GetForwardVector` (`self.Arrow`)) 1000.0) false)
  (set `self.IsCrafting` false))

(event `self.Box.OnComponentBeginOverlap`
  (params (OverlappedComponent :type "PrimitiveComponent Object Reference") (OtherActor :type "Actor Object Reference") (OtherComp :type "PrimitiveComponent Object Reference") (OtherBodyIndex :type Integer) (bFromSweep :type Boolean) (SweepResult :type "HitResult Structure (by ref)"))
  (if (not (`self.isSleeping`))
    (bind _asbp_scrap (cast `/Game/Blueprints/Enemie/Blueprint/BP_Scrap` OtherActor))
    (set `self.As BP Scrap` _asbp_scrap)
    (set `self.NbScrap` (+ (`/Game/Blueprints/Enemie/Blueprint/BP_Scrap.Value` (`self.As BP Scrap`)) (`self.NbScrap`)))
    (`self.K2_DestroyActor` (`self.As BP Scrap`))
    (if (>= (`self.NbScrap`) (`self.ScrapNeeded`))
      (`self.CreateAddons`)
      (set `self.NbScrap` (- (`self.NbScrap`) (`self.ScrapNeeded`)))
      (`self.SleepPhase`))))

(event `SleepPhase`
  (`PrimitiveComponent.SetMaterial` (`self.Cube`) 0 "/Engine/TemplateResources/MI_Template_BaseGray_03_Metal.MI_Template_BaseGray_03_Metal")
  (set `self.isSleeping` true)
  (`KismetSystemLibrary.Delay` 10.0)
  (`self.Wakeup`))

(event `self.ReceiveBeginPlay`
  (`|ExecutionSequence`
    (:`then_0`
      (bind _returnvalue (`GameplayStatics.GetActorOfClass` "/Game/Blueprints/Machine/BP_GestionMachine.BP_GestionMachine_C"))
      (set `self.GestionMachine` _returnvalue))))

(event `Wakeup`
  (set `self.isSleeping` false)
  (`self.ChangeMat`))

(fn `ChangeMat`
  (bind _cube (`self.Cube`))
  (switch `/Game/Blueprints/Enums/Enum_Kit` (`self.TypeOfPrinter`)
    (:`NewEnumerator0`
      (`PrimitiveComponent.SetMaterial` _cube 0 "/Game/Blueprints/Machine/MatPlaceholder/M_RedP.M_RedP"))
    (:`NewEnumerator1`
      (`PrimitiveComponent.SetMaterial` _cube 0 "/Game/Blueprints/Machine/MatPlaceholder/M_GreenP.M_GreenP"))
    (:`NewEnumerator2`
      (`PrimitiveComponent.SetMaterial` _cube 0 "/Game/Blueprints/Machine/MatPlaceholder/M_BlueP.M_BlueP"))))

(fn `UserConstructionScript`
  (bind _cube (`self.Cube`))
  (switch `/Game/Blueprints/Enums/Enum_Kit` (`self.TypeOfPrinter`)
    (:`NewEnumerator0`
      (`PrimitiveComponent.SetMaterial` _cube 0 "/Game/Blueprints/Machine/MatPlaceholder/M_RedP.M_RedP"))
    (:`NewEnumerator1`
      (`PrimitiveComponent.SetMaterial` _cube 0 "/Game/Blueprints/Machine/MatPlaceholder/M_GreenP.M_GreenP"))
    (:`NewEnumerator2`
      (`PrimitiveComponent.SetMaterial` _cube 0 "/Game/Blueprints/Machine/MatPlaceholder/M_BlueP.M_BlueP"))))