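; Grabbable ingredient item that a player carries and can throw, with a configurable mesh and material.
; Taking it disables physics, shows its icon on the player's widget and starts a looping widget-rotation timer.
; Detaching launches it with physics, and a Timeline then destroys it unless it is grabbed again.
; Custom depth stencil drives highlighting, and an animated arrow widget on BP_Assembler marks the target.
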(event `SpawnCatch`
  (`PrimitiveComponent.SetCollisionEnabled` (`self.Item`) "NoCollision"))

(event `/Game/Blueprints/Interface/BPI_TakeItem.DettachItem`
  (params (Impulse :type "Vector Structure"))
  (`SceneComponent.SetVisibility` (`/Game/Blueprints/Player/Player/BP_Player.Widget` (`self.ActuPlayer`)) false false)
  (`KismetSystemLibrary.K2_PauseTimerHandle` (`self.ActuTimer`))
  (`/Game/Blueprints/Arrow/wg_arrow.Stop` (`self.As Wg Arrow`))
  (set `self.launchVelocity` Impulse)
  (`PrimitiveComponent.SetCollisionEnabled` (`self.Item`) "QueryAndPhysics")
  (`PrimitiveComponent.SetSimulatePhysics` (`self.Item`) true)
  (`PrimitiveComponent.SetPhysicsLinearVelocity` (`self.Item`) (`self.launchVelocity`) false "None")
  (set `self.b_IsGrab` false)
  (`self.StartDelay`))

(event `self.ReceiveBeginPlay`
  (bind _returnvalue (`GameplayStatics.GetActorOfClass` "/Game/Blueprints/Machine/BP_Assembler.BP_Assembler_C"))
  (bind _output_get (set `self.AssembleurRef` _returnvalue))
  (bind _aswg_arrow (cast `/Game/Blueprints/Arrow/wg_arrow` (`WidgetComponent.GetWidget` (`/Game/Blueprints/Machine/BP_Assembler.Widget` _output_get))))
  (set `self.As Wg Arrow` _aswg_arrow))

(event `StartDelay`
  (`Timeline|Timeline` :!via `PlayFromStart`
    (:`Finished`
      (if (not (`self.b_IsGrab`))
        (`self.K2_DestroyActor`)))))

(event `/Game/Blueprints/Interface/BPI_TakeItem.ActiveHighlight`
  (`PrimitiveComponent.SetCustomDepthStencilValue` (`self.Item`) 1))

(event `/Game/Blueprints/Interface/BPI_TakeItem.DeactiveHighlight`
  (`PrimitiveComponent.SetCustomDepthStencilValue` (`self.Item`) 0)
  (`PrimitiveComponent.SetCustomDepthStencilValue` (`/Game/Blueprints/Machine/BP_Assembler.Assembleur_Assembleur` (`self.AssembleurRef`)) 0))

(event `/Game/Blueprints/Interface/BPI_HightLiteTarget.HightLiteTarget`
  (bind _as_wg_arrow (`self.As Wg Arrow`))
  (`SceneComponent.SetVisibility` (`/Game/Blueprints/Machine/BP_Assembler.Widget` (`self.AssembleurRef`)) true false)
  (`/Game/Blueprints/Arrow/wg_arrow.Play` _as_wg_arrow)
  (`/Game/Blueprints/Arrow/wg_arrow.ChangeImage` _as_wg_arrow "/Game/Blueprints/Arrow/Picto_Sphere3D.Picto_Sphere3D"))

(fn `GiveItemToDesk`
  (params (ActorTarget :type "Actor Object Reference"))
  (returns (Return :type Boolean))
  (return false))

(fn `SetMesh`
  (`self.SetMeshAndMaterial` (`self.Item`) (`self.Mesh`) (`self.Material`)))

(fn `SetMeshAndMaterial`
  (params (Target :type "StaticMeshComponent Object Reference") (NewMesh :type "StaticMesh Object Reference") (NewMaterial :type "MaterialInterface Object Reference"))
  (`StaticMeshComponent.SetStaticMesh` Target NewMesh)
  (`PrimitiveComponent.SetMaterial` Target 0 NewMaterial))

(fn `TakeItem`
  (params (Player :type "/Game/Blueprints/Player/Player/BP_Player Object Reference"))
  (returns (Return :type Boolean))
  (bind _widget (`/Game/Blueprints/Player/Player/BP_Player.Widget` (`self.ActuPlayer`)))
  (bind _output_get (set `self.ActuPlayer` Player))
  (bind _returnvalue (`KismetSystemLibrary.K2_SetTimer` _output_get "RotateWidget" 0.1 true))
  (set `self.ActuTimer` _returnvalue)
  (bind _aswg_icon (cast `/Game/Blueprints/Arrow/WG_Icon` (`WidgetComponent.GetWidget` _widget)))
  (`/Game/Blueprints/Arrow/WG_Icon.SetImage` _aswg_icon "/Game/Blueprints/Arrow/Picto_Sphere3D.Picto_Sphere3D")
  (`SceneComponent.SetVisibility` _widget true false)
  (`/Game/Blueprints/Player/Player/BP_Player.TakeItem` Player self)
  (`PrimitiveComponent.SetCollisionEnabled` (`self.Item`) "NoCollision")
  (`PrimitiveComponent.SetSimulatePhysics` (`self.Item`) false)
  (set `self.b_IsGrab` true)
  (return true))

(fn `UserConstructionScript`)