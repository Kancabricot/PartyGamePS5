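; Charging station machine that recharges the battery of a BP_Turret placed in its trigger, one turret at a time.
; An overlap with the turret's base snaps it to the station, disables its physics and pauses its discharge timer.
; A looping timer, paused while idle, adds charge until the next step would reach full, then swaps the charging effect for a finished one.
; The turret receives a charger reference, and ResetChargingPoint frees the station.
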(event `self.ReceiveBeginPlay`
  (bind _returnvalue (`KismetSystemLibrary.K2_SetTimer` null "ChargeTurret" 0.5 true -0.5))
  (bind _output_get (set `self.TimerCharge` _returnvalue))
  (`KismetSystemLibrary.K2_PauseTimerHandle` _output_get))

(event `self.TriggerCharge.OnComponentBeginOverlap`
  (params (OverlappedComponent :type "PrimitiveComponent Object Reference") (OtherActor :type "Actor Object Reference") (OtherComp :type "PrimitiveComponent Object Reference") (OtherBodyIndex :type Integer) (bFromSweep :type Boolean) (SweepResult :type "HitResult Structure (by ref)"))
  (bind _asbp_turret (cast `/Game/Blueprints/Turret/Blueprint/BP_Turret` OtherActor))
  (if (and (not (`self.b_HaveTurretInCharge`)) (== OtherComp (`/Game/Blueprints/Turret/Blueprint/BP_Turret.Base` _asbp_turret)))
    (bind _output_get (set `self.TurretRef` _asbp_turret))
    (`self.PlaceTurretInChargingPoint` _output_get)
    (`SceneComponent.SetVisibility` (`/Game/Blueprints/Turret/Blueprint/BP_Turret.Eclair` _asbp_turret) false false)
    (`ActorComponent.Deactivate` (`/Game/Blueprints/Turret/Blueprint/BP_Turret.Niagara` _asbp_turret))
    (`KismetSystemLibrary.K2_PauseTimerHandle` (`/Game/Blueprints/Turret/Blueprint/BP_Turret.DechargeTurretTimer` _asbp_turret))))

(fn `ChargeTurret`
  (bind _returnvalue (+ (`/Game/Blueprints/Turret/Blueprint/BP_Turret.BaterieCharge` (`self.TurretRef`)) (`self.ChargeValue`)))
  (if (< _returnvalue 100.0)
    (set `/Game/Blueprints/Turret/Blueprint/BP_Turret.BaterieCharge` _returnvalue (`self.TurretRef`))
    (else
      (`NiagaraFunctionLibrary.SpawnSystemAtLocation` "/Game/VFX/Turrets/Energy/EnergyCharging/NS_ChargingFinished.NS_ChargingFinished" (+ (`SceneComponent.K2_GetComponentLocation` (`self.DefaultSceneRoot`)) (0.0 0.0 50.0)))
      (`KismetSystemLibrary.K2_PauseTimerHandle` (`self.TimerCharge`))
      (`/Engine/EditorBlueprintResources/StandardMacros.IsValid` (`self.NSCharging`)
        (:`Is Valid`
          (`ActorComponent.K2_DestroyComponent` (`self.NSCharging`)))))))

(fn `PlaceTurretInChargingPoint`
  (params (TurretTarget :type "/Game/Blueprints/Turret/Blueprint/BP_Turret Object Reference"))
  (bind _returnvalue (`SceneComponent.K2_GetComponentLocation` (`self.DefaultSceneRoot`)))
  (`SceneComponent.K2_SetWorldLocation` (`/Game/Blueprints/Turret/Blueprint/BP_Turret.Base` TurretTarget) _returnvalue false false)
  (bind _returnvalue_2 (`NiagaraFunctionLibrary.SpawnSystemAtLocation` "/Game/VFX/Turrets/Energy/EnergyCharging/NS_EnergyCharging.NS_EnergyCharging" (+ _returnvalue (0.0 0.0 50.0))))
  (set `self.NSCharging` _returnvalue_2)
  (`PrimitiveComponent.SetSimulatePhysics` (`/Game/Blueprints/Turret/Blueprint/BP_Turret.Base` (`local.TurretTarget`)) false)
  (set `/Game/Blueprints/Turret/Blueprint/BP_Turret.ChargerRef` self (`local.TurretTarget`))
  (`KismetSystemLibrary.K2_UnPauseTimerHandle` (`self.TimerCharge`))
  (set `self.b_HaveTurretInCharge` true))

(fn `ResetChargingPoint`
  (set `self.b_HaveTurretInCharge` false)
  (`ActorComponent.K2_DestroyComponent` (`self.NSCharging`))
  (`KismetSystemLibrary.K2_PauseTimerHandle` (`self.TimerCharge`)))

(fn `UserConstructionScript`)