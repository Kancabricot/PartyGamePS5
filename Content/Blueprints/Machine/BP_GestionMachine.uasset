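; BP_GestionMachine manages a set of printer machines, periodically randomizing which type each one is.
; After a random delay between MinDuration and MaxDuration, it shuffles TypeTab, assigns types to PrinterRef, wakes each printer and calls AnimTemp, then reschedules itself.
; If any of the first three printers is crafting, it only sets BNeedToShuffle and the loop stops.
; The construction script keeps MaxDuration at least MinDuration.
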(event `self.ReceiveBeginPlay`
  ;[1 1 1] BeginPlay
  (`self.Shuffle`))

(event `Shuffle`
  (bind _printer_ref (`self.Printer ref`))
  ;[1 1 1] SuffleEvent
  ;;[1 1 1] DelayBeforeShuffle
  (`KismetSystemLibrary.Delay` (`KismetMathLibrary.RandomFloatInRange` (`self.MinDuration`) (`self.MaxDuration`)))
  (if (or (`/Game/Blueprints/Machine/BP_3dPrinter.IsCrafting` (`|GetArrayItem` _printer_ref)) (`/Game/Blueprints/Machine/BP_3dPrinter.IsCrafting` (`|GetArrayItem` _printer_ref 1)) (`/Game/Blueprints/Machine/BP_3dPrinter.IsCrafting` (`|GetArrayItem` _printer_ref 2)))
    ;;[1 1 1] Keep Shuffle in memory if machine is crafting
    (set `self.b_NeedToShuffle` true)
    (else
      (`self.ShuffleMachine`)
      ;;[1 1 1] Next shuffle
      (`self.Shuffle`))))

(fn `ShuffleMachine`
  (locals (TempRef :type "/Game/Blueprints/Enums/Enum_Kit Enum") (ActuPrinter :type "/Game/Blueprints/Machine/BP_3dPrinter Object Reference"))
  (bind _actuprinter (`local.ActuPrinter`))
  ;[1 1 1] SuffleFunction
  (`KismetArrayLibrary.Array_Shuffle` (`self.TypeTab`))
  (for (_array_element _array_index) (`self.Printer ref`)
    (bind _output_get (set `local.ActuPrinter` _array_element))
    (set `/Game/Blueprints/Machine/BP_3dPrinter.TypeOfPrinter` (`|GetArrayItem` (`self.TypeTab`) _array_index) _output_get)
    (set `/Game/Blueprints/Machine/BP_3dPrinter.isSleeping` false _actuprinter)
    (`/Game/Blueprints/Machine/BP_3dPrinter.AnimTemp` _actuprinter)))

(fn `UserConstructionScript`
  (if (> (`self.MinDuration`) (`self.MaxDuration`))
    (set `self.MaxDuration` (`self.MinDuration`))))