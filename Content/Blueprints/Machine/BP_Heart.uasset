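; BP_Heart is the defended core machine that loses life when enemies reach it, ending the game at zero.
; An overlapping BP_Enemie plays its jump, with damage timed to that duration, then dies and notifies any tutorial manager once.
; Damage animates the WG_Heart widget's life bar through a timeline.
; At zero life, it stops all enemies, explodes, shakes the camera, pauses and shows the losing end screen.
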(event `self.TriggerDamage.OnComponentBeginOverlap`
  (params (OverlappedComponent :type "PrimitiveComponent Object Reference") (OtherActor :type "Actor Object Reference") (OtherComp :type "PrimitiveComponent Object Reference") (OtherBodyIndex :type Integer) (bFromSweep :type Boolean) (SweepResult :type "HitResult Structure (by ref)"))
  (bind _tutomanagerref (`self.TutoManagerRef`))
  (bind _asbp_enemie (cast `/Game/Blueprints/Enemie/Blueprint/BP_Enemie` OtherActor))
  (bind _montage_length (`/Game/Blueprints/Enemie/Blueprint/BP_Enemie.PlayJump` _asbp_enemie))
  (`KismetSystemLibrary.K2_SetTimer` null "Check Damage" _montage_length)
  (`KismetSystemLibrary.Delay` _montage_length)
  (`/Engine/EditorBlueprintResources/StandardMacros.IsValid` _asbp_enemie
    (:`Is Valid`
      (`/Game/Blueprints/Enemie/Blueprint/BP_Enemie.Death` _asbp_enemie))
    (:`Is Not Valid`
      _))
  (`KismetSystemLibrary.Delay` 0.1)
  (`/Engine/EditorBlueprintResources/StandardMacros.IsValid` _tutomanagerref
    (:`Is Valid`
      (`/Game/Blueprints/Tutorial/BP_TutorialManager.Heart` _tutomanagerref)
      (set `self.TutoManagerRef` null))))

(event `self.ReceiveBeginPlay`
  (bind _maxlife (`self.MaxLife`))
  (bind _returnvalue (/ (`self.Old Life`) (`self.MaxLife`)))
  (`|ExecutionSequence`
    (:`then_0`
      (bind _aswg_heart (cast `/Game/Blueprints/Widgets/WG_Heart` (`WidgetComponent.GetWidget` (`self.Widget`))))
      (set `self.As WG Heart` _aswg_heart)
      (set `self.Old Life` _maxlife)
      (set `self.Current life` _maxlife))
    (:`then_1`
      (`/Game/Blueprints/Widgets/WG_Heart.Set Life Bar` (`self.As WG Heart`) _returnvalue)
      (`/Game/Blueprints/Widgets/WG_Heart.Set Text` (`self.As WG Heart`) _returnvalue))))

(event `TimedShake`
  (`KismetSystemLibrary.Delay` 1.86)
  (`PlayerController.ClientStartCameraShake` :`self` (`GameplayStatics.GetPlayerController` 0) :`Shake` "/Game/Blueprints/Enemie/Blueprint/BP_CamShakeExplosion.BP_CamShakeExplosion_C" :`Scale` 50.0)
  (`KismetSystemLibrary.Delay` 1.5)
  (`GameplayStatics.SetGamePaused` true)
  (bind _returnvalue (`|CreateWidget` "/Game/Blueprints/Widgets/WG_EndGame.WG_EndGame_C" (`GameplayStatics.GetPlayerController` 0)))
  (`UserWidget.AddToViewport` _returnvalue 0)
  (`WidgetBlueprintLibrary.SetInputMode_UIOnlyEx` (`GameplayStatics.GetPlayerController` 0) _returnvalue))

(event `Smooth lIfe Bar`
  (bind _returnvalue (/ (`self.Current life`) (`self.MaxLife`)))
  (set `self.TL_LifeIsPlaying` true)
  (bind (_direction _alpha) (`Timeline|TL_Life` :!via `PlayFromStart`)
    (:`Update`
      (`/Game/Blueprints/Widgets/WG_Heart.Set Life Bar` (`self.As WG Heart`) (`KismetMathLibrary.Lerp` (/ (`self.Old Life`) (`self.MaxLife`)) _returnvalue _alpha)))
    (:`Finished`
      (set `self.Old Life` (`self.Current life`))
      (`/Game/Blueprints/Widgets/WG_Heart.Set Text` (`self.As WG Heart`) _returnvalue)
      (set `self.TL_LifeIsPlaying` false))))

(fn `Check Damage`
  (set `self.Current life` (- (`self.Old Life`) 1.0))
  (if (not (`self.TL_LifeIsPlaying`))
    (`self.Smooth lIfe Bar`))
  (if (<= (`self.Current life`) 0.0)
    (`self.End Game`)
    (return)
    (else
      (return))))

(fn `End Game`
  (bind _outactors (`GameplayStatics.GetAllActorsOfClass` "/Game/Blueprints/Enemie/Blueprint/BP_Enemie.BP_Enemie_C"))
  (for _array_element _outactors
    (`/Game/Blueprints/Enemie/Blueprint/BP_Enemie.StopMoving` _array_element))
  (`GameplayStatics.PlaySound2D` "/Game/Sound/SFX_SC/Enemis_Sc/Krash_Survolte_SC/SC_SFX_Krash_Survolte_Explosion_02.SC_SFX_Krash_Survolte_Explosion_02" 1.0 1.0 0.0 null null)
  (`NiagaraFunctionLibrary.SpawnSystemAtLocation` "/Game/VFX/VFX/Coeur/V1/NS_CoreExplosion.NS_CoreExplosion" (`SceneComponent.K2_GetComponentLocation` (`self.Sphere_Energy`)))
  (`self.TimedShake`)
  (return))

(fn `UserConstructionScript`)