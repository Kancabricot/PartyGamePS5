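; BP_conveyorbelt is a conveyor belt actor that moves two static meshes along a spline.
; Each Tick advances a distance per mesh by SplineSpeed and places that mesh at the matching local spline location and rotation.
; The second mesh starts 3.5 seconds after BeginPlay, staggering the pair.
; When either mesh begins overlapping the Box, its distance resets to zero, looping it back to the spline start.
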(event `self.ReceiveBeginPlay`
  (`KismetSystemLibrary.Delay` 3.5)
  (set `self.GO` true))

(event `self.ReceiveTick`
  (params (DeltaSeconds :type "Float (single-precision)"))
  (bind (_returnvalue_location _returnvalue_rotation) (`KismetMathLibrary.BreakTransform` (`SplineComponent.GetTransformAtDistanceAlongSpline` (`self.Spline`) (`self.DistanceAlongSpline_2`) "Local" false)))
  (bind (_returnvalue_location_2 _returnvalue_rotation_2) (`KismetMathLibrary.BreakTransform` (`SplineComponent.GetTransformAtDistanceAlongSpline` (`self.Spline`) (`self.DistanceAlongSpline`) "Local" false)))
  (`|ExecutionSequence`
    (:`then_0`
      (set `self.DistanceAlongSpline` (+ (* DeltaSeconds (`self.SplineSpeed`)) (`self.DistanceAlongSpline`)))
      (`SceneComponent.K2_SetRelativeTransform` (`self.StaticMesh`) (`KismetMathLibrary.MakeTransform` _returnvalue_location_2 _returnvalue_rotation_2) false false))
    (:`then_1`
      (if (`self.GO`)
        (set `self.DistanceAlongSpline_2` (+ (* DeltaSeconds (`self.SplineSpeed`)) (`self.DistanceAlongSpline_2`)))
        (`SceneComponent.K2_SetRelativeTransform` (`self.StaticMesh1`) (`KismetMathLibrary.MakeTransform` _returnvalue_location _returnvalue_rotation) false false)))))

(event `self.Box.OnComponentBeginOverlap`
  (params (OverlappedComponent :type "PrimitiveComponent Object Reference") (OtherActor :type "Actor Object Reference") (OtherComp :type "PrimitiveComponent Object Reference") (OtherBodyIndex :type Integer) (bFromSweep :type Boolean) (SweepResult :type "HitResult Structure (by ref)"))
  (if (== OtherComp (`self.StaticMesh`))
    (set `self.DistanceAlongSpline` 0.0)
    (elif (== OtherComp (`self.StaticMesh1`))
      (set `self.DistanceAlongSpline_2` 0.0))))

(fn `UserConstructionScript`)