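; BP_Charger is a turret charging station with three snap points.
; An overlapping turret base is snapped to a free point with physics off, and the turret's effects and discharge timer are stopped.
; A looping timer raises battery charge toward 100, but only for the turret in the first slot.
; ResetChargePoint frees a turret's slot, and GetSnapValue offers the first point as a drop position for turrets.
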(event `self.TriggerSnapCharge.OnComponentBeginOverlap`
  (params (OverlappedComponent :type "PrimitiveComponent Object Reference") (OtherActor :type "Actor Object Reference") (OtherComp :type "PrimitiveComponent Object Reference") (OtherBodyIndex :type Integer) (bFromSweep :type Boolean) (SweepResult :type "HitResult Structure (by ref)"))
  (bind _asbp_turret (cast `/Game/Blueprints/Turret/Blueprint/BP_Turret` OtherActor))
  (bind _base (`/Game/Blueprints/Turret/Blueprint/BP_Turret.Base` _asbp_turret))
  (if (== OtherComp _base)
    (`self.SetTurretInCharge` _base _asbp_turret)
    (bind _eclair (`/Game/Blueprints/Turret/Blueprint/BP_Turret.Eclair` _asbp_turret))
    (`SkeletalMeshComponent.Stop` _eclair)
    (`SceneComponent.SetVisibility` _eclair false false)
    (`ActorComponent.Deactivate` (`/Game/Blueprints/Turret/Blueprint/BP_Turret.Niagara` _asbp_turret))
    (`KismetSystemLibrary.K2_PauseTimerHandle` (`/Game/Blueprints/Turret/Blueprint/BP_Turret.DechargeTurretTimer` _asbp_turret))))

(event `ChargeTurret`
  (bind _returnvalue (`KismetSystemLibrary.K2_SetTimerDelegate` (delegate `ChargeEvent`) 0.1 true))
  (if (not (`KismetSystemLibrary.K2_IsValidTimerHandle` (`self.ChargeTimer`)))
    (set `self.ChargeTimer` _returnvalue)))

(event `ChargeEvent`
  (bind _turretchargepoint1 (`self.TurretChargePoint1`))
  (`/Engine/EditorBlueprintResources/StandardMacros.IsValid` (`self.TurretChargePoint1`)
    (:`Is Valid`
      (bind _output_get (set `/Game/Blueprints/Turret/Blueprint/BP_Turret.BaterieCharge` (+ (`/Game/Blueprints/Turret/Blueprint/BP_Turret.BaterieCharge` _turretchargepoint1) 0.2) _turretchargepoint1))
      (if (>= _output_get 100.0)
        (`KismetSystemLibrary.K2_PauseTimerHandle` (`self.ChargeTimer`))))
    (:`Is Not Valid`
      (`KismetSystemLibrary.K2_PauseTimerHandle` (`self.ChargeTimer`)))))

(fn `GetSnapValue`
  (params (ActorToThrow :type "Actor Object Reference"))
  (returns (DropPosition :type "Vector Structure") (b_CanSnap :type Boolean))
  (cast `/Game/Blueprints/Turret/Blueprint/BP_Turret` ActorToThrow
    (:`then`
      (return (`SceneComponent.K2_GetComponentLocation` (`self.ChargePoint01`)) true))
    (:`CastFailed`
      (return (0.0 0.0 0.0) false))))

(fn `ResetChargePoint`
  (params (TurretTarget :type "/Game/Blueprints/Turret/Blueprint/BP_Turret Object Reference"))
  (if (== TurretTarget (`self.TurretChargePoint1`))
    (set `self.TurretChargePoint1` null)
    (elif (== (`local.TurretTarget`) (`self.TurretChargePoint2`))
      (set `self.TurretChargePoint2` null)
      (elif (== (`local.TurretTarget`) (`self.TurretChargePoint3`))
        (set `self.TurretChargePoint3` null)))))

(fn `SetTurretInCharge`
  (params (Target :type "StaticMeshComponent Object Reference") (TurretTarget :type "/Game/Blueprints/Turret/Blueprint/BP_Turret Object Reference"))
  (bind _turrettarget (`local.TurretTarget`))
  (bind _turrettarget_2 (`local.TurretTarget`))
  (bind _turrettarget_3 (`local.TurretTarget`))
  (if (== (`self.TurretChargePoint1`) null)
    (`SceneComponent.K2_SetWorldLocation` (`local.Target`) (`SceneComponent.K2_GetComponentLocation` (`self.ChargePoint01`)) false false)
    (set `self.TurretChargePoint1` _turrettarget_2)
    (set `/Game/Blueprints/Turret/Blueprint/BP_Turret.ChargerRef` self _turrettarget_2)
    (`PrimitiveComponent.SetSimulatePhysics` (`local.Target`) false)
    (`self.ChargeTurret`)
    (elif (== (`self.TurretChargePoint2`) null)
      (`SceneComponent.K2_SetWorldLocation` (`local.Target`) (`SceneComponent.K2_GetComponentLocation` (`self.ChargePoint02`)) false false)
      (set `self.TurretChargePoint2` _turrettarget_3)
      (set `/Game/Blueprints/Turret/Blueprint/BP_Turret.ChargerRef` self _turrettarget_3)
      (`PrimitiveComponent.SetSimulatePhysics` (`local.Target`) false)
      (`self.ChargeTurret`)
      (elif (== (`self.TurretChargePoint3`) null)
        (`SceneComponent.K2_SetWorldLocation` (`local.Target`) (`SceneComponent.K2_GetComponentLocation` (`self.ChargePoint03`)) false false)
        (set `self.TurretChargePoint3` _turrettarget)
        (set `/Game/Blueprints/Turret/Blueprint/BP_Turret.ChargerRef` self _turrettarget)
        (`PrimitiveComponent.SetSimulatePhysics` (`local.Target`) false)
        (`self.ChargeTurret`)))))

(fn `UserConstructionScript`)