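; Assembler machine that turns an ingredient dropped into its box into a turret addon.
; An empty slot consumes the ingredient and spins the rollers; one specific type starts a timed craft with Niagara effect and progress widget, while ingredients arriving mid-craft are thrown back.
; Timelines drive rollers, timer and addon ejection, which ends in physics simulation.
; It also provides a snap point for ingredients and advances the tutorial once on reset.
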(event `self.ReceiveBeginPlay`
  (bind _aswg_temperature (cast `/Game/Blueprints/Widgets/WG_Temperature` (`WidgetComponent.GetWidget` (`self.Widget`))))
  (set `self.WGBar` _aswg_temperature))

(event `self.Box.OnComponentBeginOverlap`
  (params (OverlappedComponent :type "PrimitiveComponent Object Reference") (OtherActor :type "Actor Object Reference") (OtherComp :type "PrimitiveComponent Object Reference") (OtherBodyIndex :type Integer) (bFromSweep :type Boolean) (SweepResult :type "HitResult Structure (by ref)"))
  (bind _asbp_ingredients (cast `/Game/Blueprints/Machine/BP_Ingredients` OtherActor))
  (if (not (`self.b_IsCooking`))
    (if (`|EnumEquality` (`self.Enum_Ingredients`) "NewEnumerator14")
      (set `self.Enum_Ingredients` (`/Game/Blueprints/Machine/BP_Ingredients.Enum_Ingredients` _asbp_ingredients))
      (`StaticMeshComponent.SetStaticMesh` (`self.StaticMesh`) null)
      (`self.K2_DestroyActor` _asbp_ingredients)
      (`self.CheckAssembly`)
      (bind (_direction _newtrack_0) (`Timeline|RotationCrusher` :!via `PlayFromStart`)
        (:`Update`
          (bind (_returnvalue_roll _returnvalue_pitch) (`KismetMathLibrary.BreakRotator` (`KismetMathLibrary.RLerp` (struct :`Yaw` 90.0) (struct :`Pitch` -720.0 :`Yaw` 90.0) _newtrack_0)))
          (`SceneComponent.K2_SetRelativeRotation` (`self.Assembleur_AssembleurRond2`) (`KismetMathLibrary.MakeRotator` 0.0 _returnvalue_pitch 90.0) false false)
          (bind (_returnvalue_roll_2 _returnvalue_pitch_2) (`KismetMathLibrary.BreakRotator` (`KismetMathLibrary.RLerp` (struct :`Yaw` 90.0) (struct :`Pitch` 720.0 :`Yaw` 90.0) _newtrack_0)))
          (`SceneComponent.K2_SetRelativeRotation` (`self.Assembleur_AssembleurRond3`) (`KismetMathLibrary.MakeRotator` 0.0 _returnvalue_pitch_2 90.0) false false))))
    (else
      (message `/Game/Blueprints/Interface/BPI_TakeItem.DettachItem` _asbp_ingredients (* (`SceneComponent.GetForwardVector` (`self.ThrowingLocation`)) 500)))))

(event `DropAddon`
  (bind _returnvalue (`|SpawnActorFromClass` "/Game/Blueprints/Turret/Blueprint/BP_TurretAddon.BP_TurretAddon_C" (`KismetMathLibrary.MakeTransform` (`SceneComponent.K2_GetComponentLocation` (`self.PosAddonStart`))) "Undefined" "MultiplyWithRoot" null null (`self.AddonType`) self null))
  (`self.ResetAssembly`)
  (bind (_direction _movement) (`Timeline|MovementAddon` :!via `PlayFromStart` :!label _label)
    (:`Update`
      (bind _addon (`/Game/Blueprints/Turret/Blueprint/BP_TurretAddon.Addon` _returnvalue))
      (`SceneComponent.K2_SetWorldLocation` _addon (`KismetMathLibrary.VLerp` (`SceneComponent.K2_GetComponentLocation` (`self.PosAddonStart`)) (`SceneComponent.K2_GetComponentLocation` (`self.PosAddonFinal`)) _movement) false false))
    (:`Finished`
      (`PrimitiveComponent.SetSimulatePhysics` _addon true))))

(event `StopMovementAddon`
  (goto _label :!via `Stop`))

(event `CreateStage`
  (`ActorComponent.Activate` (`self.NS_Craft`) false)
  (set `self.b_IsCooking` true)
  (bind (_direction _timervalue) (`Timeline|Delay` :!via `PlayFromStart`)
    (:`Update`
      (`/Game/Blueprints/Widgets/WG_Temperature.SetTimer` (`self.WGBar`) _timervalue))
    (:`Finished`
      (`self.DropAddon`))))

(fn `CheckAssembly`
  (if (`|EnumEquality` (`self.Enum_Ingredients`) "NewEnumerator7")
    (`self.CreateStage`)))

(fn `GetSnapValue`
  (params (ActorToThrow :type "Actor Object Reference"))
  (returns (DropPosition :type "Vector Structure") (b_CanSnap :type Boolean))
  (cast `/Game/Blueprints/Machine/BP_Ingredients` ActorToThrow
    (:`then`
      (return (`SceneComponent.K2_GetComponentLocation` (`self.Assembleur_AssembleurRond2`)) true))
    (:`CastFailed`
      (return (0.0 0.0 0.0) false))))

(fn `ResetAssembly`
  (`/Game/Blueprints/Widgets/WG_Temperature.SetTimer` (`self.WGBar`) 0.0)
  (set `self.Enum_Ingredients` "NewEnumerator14")
  (`StaticMeshComponent.SetStaticMesh` (`self.StaticMesh1`) null)
  (`StaticMeshComponent.SetStaticMesh` (`self.StaticMesh`) null)
  (`ActorComponent.Deactivate` (`self.NS_Craft`))
  (set `self.b_IsCooking` false)
  (`self.Tuto`))

(fn `Tuto`
  (if (`self.b_IsTuto`)
    (bind _foundwidgets (`WidgetBlueprintLibrary.GetAllWidgetsOfClass` "/Game/Blueprints/Widgets/WG_Tutorial.WG_Tutorial_C"))
    (`/Game/Blueprints/Widgets/WG_Tutorial.IncrementTuto` (`|GetArrayItem` _foundwidgets))
    (set `self.b_IsTuto` false)))

(fn `UserConstructionScript`)