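; Slime base machine with a hatch, an LCD that shows the slime's printer type, and an optional cage assignment.
; Anim plays a sound and opens the hatch through a timeline-driven "open" morph target.
; CloseDoort plays the closing sound, line-traces along an arrow for a BP_Slime, colors the LCD red, green or blue, and sets or clears its Cage.
; The timeline reverse is unwired, so CloseDoort does not animate the hatch.
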(event `Anim`
  (`GameplayStatics.PlaySound2D` "/Game/Sound/SFX_SC/Slime_Sc/SC_SFX_Trappe_Ouvre_01.SC_SFX_Trappe_Ouvre_01" 1.0 1.0 0.0 null null)
  (`self.OpenDoor `))

(event `self.ReceiveBeginPlay`
  (`SkeletalMeshComponent.SetMorphTarget` (`self.PR_fermoir_00`) "open" 1.0 true))

(event `OpenDoor`
  (bind _direction (`Timeline|Timeline`)
    (:`Update`
      (`SkeletalMeshComponent.SetMorphTarget` (`self.PR_fermoir_00`) "open" (`self.Lerp`) false))
    (:`Finished`
      (switch `ETimelineDirection` _direction))))

(event `CloseDoort`
  (bind _returnvalue (`SceneComponent.K2_GetComponentLocation` (`self.Arrow`)))
  (`GameplayStatics.PlaySound2D` "/Game/Sound/SFX_SC/Slime_Sc/SC_SFX_Trappe_Ferme_01.SC_SFX_Trappe_Ferme_01" 1.0 1.0 0.0 null null)
  (`KismetSystemLibrary.PrintString` "back")
  (bind _outhit (`KismetSystemLibrary.LineTraceSingle` _returnvalue (+ _returnvalue (* (`SceneComponent.GetForwardVector` (`self.Arrow`)) 500.0)) "TraceTypeQuery1"))
  (bind _asbp_slime (cast `/Game/Blueprints/Machine/BP_Slime` (`.HitActor` (`GameplayStatics.BreakHitResult` _outhit))))
  (switch `/Game/Blueprints/Enums/Enum_Kit` (`/Game/Blueprints/Machine/BP_Slime.TypeOfPrinter` _asbp_slime)
    (:`NewEnumerator0`
      (`PrimitiveComponent.SetMaterial` (`self.PR_socleSlime_00`) 2 "/Game/Assets/Assembleur/Mat/lcd_Red.lcd_Red"))
    (:`NewEnumerator1`
      (`PrimitiveComponent.SetMaterial` (`self.PR_socleSlime_00`) 2 "/Game/Assets/Assembleur/Mat/lcd_Green.lcd_Green"))
    (:`NewEnumerator2`
      (`PrimitiveComponent.SetMaterial` (`self.PR_socleSlime_00`) 2 "/Game/Assets/Assembleur/Mat/lcd_Blue.lcd_Blue")))
  (if (`self.HasCage`)
    (set `/Game/Blueprints/Machine/BP_Slime.cage` (`self.WhatCage`) _asbp_slime)
    (else
      (set `/Game/Blueprints/Machine/BP_Slime.cage` null _asbp_slime))))

(fn `UserConstructionScript`)