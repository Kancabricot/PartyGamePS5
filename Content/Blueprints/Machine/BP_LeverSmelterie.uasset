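; BP_LeverSmelterie is an interactive lever that switches a linked smeltery.
; Interact and Reset share one toggle that plays or reverses a single timeline based on the BIsON state, swinging the lever pivot between two angles.
; When the timeline finishes, it flips BIsON and, if the smeltery reference is valid, calls its StartInteract with the inverse of the new state and itself as the lever reference.
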(event `Reset`
  (if (`self.b_IsON`) :!label _label
    (bind (_direction _newtrack_0) (`Timeline|LeverTimelineOFF` :!label _label_2)
      (:`Update`
        (`SceneComponent.K2_SetRelativeRotation` (`self.PivotLever`) (`KismetMathLibrary.RLerp` (struct :`Pitch` 50.0) (struct :`Pitch` -50.0) _newtrack_0) false false))
      (:`Finished`
        (set `self.b_IsON` (not (`self.b_IsON`)))
        (bind _smelteryref (`self.SmelteryRef`)
          (:`then`
            (`/Game/Blueprints/Machine/BP_Smelterie.StartInteract` _smelteryref (not (`self.b_IsON`)) self))
          (:`else`))))
    (else
      (goto _label_2 :!via `Reverse`))))

(event `/Game/Blueprints/Interface/BPI_Interact.Interact`
  (goto _label))

(fn `UserConstructionScript`)