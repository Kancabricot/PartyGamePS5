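; BP_Slime is a colour-typed slime machine that takes scrap and produces turret kits, then sleeps.
; Overlapping scrap is absorbed and starts crafting; CreateAddons launches one kit, or three for golden scrap.
; Timers drive the sleep bar, which player hits speed up, and rotation toward nearby players.
; It also swaps faces through a dynamic material, plays tunnel animations for BP_GestionSlime shuffles, and supports tutorial hooks.
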(event `self.ReceiveBeginPlay`
  ;[1 1 1] BeginPlay
  (bind _returnvalue (`GameplayStatics.GetActorOfClass` "/Game/Blueprints/Machine/BP_GestionSlime.BP_GestionSlime_C"))
  (set `self.GestionMachine` _returnvalue)
  (bind _returnvalue_2 (`PrimitiveComponent.CreateDynamicMaterialInstance` (`self.Rebl_Chewing_01`) 1 (`self.EyesMat`) "None"))
  (set `self.DynamicM` _returnvalue_2)
  (set `self.FirstRotation` (`SceneComponent.K2_GetComponentRotation` (`self.Rebl_Chewing_01`)))
  ;;[1 1 1] Widgets Ref
  (bind _aswg_slime_sleeping (cast `/Game/Blueprints/Widgets/WG_SlimeSleeping` (`WidgetComponent.GetWidget` (`self.WidgetSleep`))))
  (bind _output_get (set `self.As WG Slime Sleeping` _aswg_slime_sleeping))
  (`Widget.SetVisibility` _output_get "Hidden")
  (`SceneComponent.SetVisibility` (`self.widgetScrap`) false false)
  (bind _aswg_circle (cast `/Game/Blueprints/Widgets/WG_Circle` (`WidgetComponent.GetWidget` (`self.Widget_Circle`))))
  (set `self.As WG Circle` _aswg_circle))

(event `Show Widgets`
  ;[1 1 1] Scrap Widgets Tuto
  (if (not (or (`self.IsCrafting`) (`self.b_Tuto_is_Inactactive`) (`self.isSleeping`)))
    (`/Game/Blueprints/Widgets/WG_Circle.Play Circle Animation` (`self.As WG Circle`))
    (`SceneComponent.SetVisibility` (`self.widgetScrap`) true false)))

(event `Hide Widgets`
  ;[1 1 1] Scrap Widgets Tuto
  (if (not (or (`self.IsCrafting`) (`self.b_Tuto_is_Inactactive`) (`self.isSleeping`)))
    (`SceneComponent.SetVisibility` (`self.widgetScrap`) false false)))

(event `Anim`
  (bind _returnvalue (`self.GetTransform`))
  (bind (_returnvalue_x _returnvalue_y _returnvalue_z) (`KismetMathLibrary.BreakVector` (`self.K2_GetActorLocation`)))
  (`KismetArrayLibrary.Array_Add` (`/Game/Blueprints/Machine/BP_GestionSlime.TrasnforTemp` (`self.GestionMachine`)) (`KismetMathLibrary.MakeTransform` (.location _returnvalue) (`KismetMathLibrary.MakeRotator` (.roll (.rotation _returnvalue)) (.pitch (.rotation _returnvalue)) (.yaw (.rotation _returnvalue))) (.scale _returnvalue)))
  ;[1 1 1] Animation
  (`KismetSystemLibrary.Delay` 1.0)
  (`|PlayMontage` (`self.Rebl_Chewing_01`) "/Game/Animation/AnimBp/Slime/Montage/EnterTunel.EnterTunel"
    (:`then`
      (bind (_direction _newtrack_0) (`Timeline|Timeline`)
        (:`Update`
          (`self.K2_SetActorLocation` (`KismetMathLibrary.MakeVector` _returnvalue_x _returnvalue_y (`KismetMathLibrary.Lerp` _returnvalue_z (+ _returnvalue_z -5.0) _newtrack_0))))
        (:`Finished`
          (if (`self.b_IsTuto`)
            (set `self.b_Tuto_is_Inactactive` true)
            (else
              (`self.Suflle`))))))))

(event `PlayAnime`
  (params (WhatFace :type Integer))
  (bind (_nbframe _face) (`self.GetGoodFace` WhatFace))
  ;[1 1 1] PlayFaceAnime
  (`self.ChangeFacialAnim` _nbframe _face))

(event `SleepPhase`
  (bind _niagara (`self.Niagara`))
  ;[1 1 1] Sleep and wake up
  (`Widget.SetVisibility` (`self.As WG Slime Sleeping`) "Visible")
  (`ActorComponent.Activate` _niagara false)
  (`SceneComponent.SetVisibility` _niagara true false)
  (set `self.isSleeping` true)
  (bind _returnvalue (`KismetSystemLibrary.K2_SetTimerDelegate` (delegate `TimerSleep`) (`self.TimerDuration`) true -1.0))
  (set `self.DelayTimer` _returnvalue))

(event `TimerSleep`
  ;[1 1 1] Sleep and wake up
  (bind _output_get (set `self.ActuSleepDuration` (+ (`self.ActuSleepDuration`) 1.0)))
  (`/Game/Blueprints/Widgets/WG_SlimeSleeping.Set Slime Sleep Bar` (`self.As WG Slime Sleeping`) _output_get (`self.MaxSleepDuration`))
  (if (>= (`self.ActuSleepDuration`) (`self.MaxSleepDuration`))
    (`self.Wakeup`)))

(event `Suflle`
  ;[1 1 1] Animation
  (`/Game/Blueprints/Machine/BP_GestionSlime.ShuffleMachine` (`self.GestionMachine`)))

(event `Wakeup`
  (bind _niagara (`self.Niagara`))
  ;[1 1 1] Sleep and wake up
  (`ActorComponent.Deactivate` _niagara)
  (`SceneComponent.SetVisibility` _niagara false false)
  (set `self.isSleeping` false)
  (`Widget.SetVisibility` (`self.As WG Slime Sleeping`) "Hidden")
  (bind _output_get (set `self.ActuSleepDuration` 0.0))
  (`/Game/Blueprints/Widgets/WG_SlimeSleeping.Set Slime Sleep Bar` (`self.As WG Slime Sleeping`) _output_get (`self.MaxSleepDuration`))
  (`KismetSystemLibrary.K2_PauseTimerHandle` (`self.DelayTimer`))
  (set `self.TimerDuration` 1.0)
  (`/Game/Blueprints/Widgets/WG_SlimeSleeping.ChangeBack` (`self.As WG Slime Sleeping`)))

(event `/Game/Blueprints/Interface/BPI_Interact.Interact`
  (params (Player :type "/Game/Blueprints/Player/Player/BP_Player Object Reference"))
  (bind _interactplayer (`self.InteractPlayer`))
  (bind _skeletalmesh (`/Game/Blueprints/Player/Player/BP_Player.SkeletalMesh` (`self.InteractPlayer`)))
  (bind _floatingpawnmovement (`/Game/Blueprints/Player/Player/BP_Player.FloatingPawnMovement` _interactplayer))
  (bind (_returnvalue_roll _returnvalue_pitch _returnvalue_yaw) (`KismetMathLibrary.BreakRotator` (`KismetMathLibrary.FindLookAtRotation` (`SceneComponent.K2_GetComponentLocation` _skeletalmesh) (`SceneComponent.K2_GetComponentLocation` (`self.Rebl_Chewing_01`)))))
  ;[1 1 1] Interact
  (set `self.InteractPlayer` Player)
  (if (`self.isSleeping`)
    (set `self.b_IsTuto` false)
    (`KismetSystemLibrary.K2_PauseTimerHandle` (`self.DelayTimer`))
    (set `self.TimerDuration` 0.5)
    (`self.SleepPhase`)
    (set `self.Hit` true)
    (`/Game/Blueprints/Widgets/WG_SlimeSleeping.ChangeColor` (`self.As WG Slime Sleeping`))
    (`|PlayMontage` (`/Game/Blueprints/Player/Player/BP_Player.SkeletalMesh` (`self.InteractPlayer`)) "/Game/Animation/Montage/AM_Hitting.AM_Hitting"
      (:`then`
        (set `/Game/Blueprints/Player/Player/BP_Player.StopMovementRotation` true _interactplayer)
        (set `FloatingPawnMovement.MaxSpeed` 0.0 _floatingpawnmovement)
        (set `FloatingPawnMovement.Acceleration` 0.0 _floatingpawnmovement)
        (`SceneComponent.K2_SetWorldRotation` _skeletalmesh (`KismetMathLibrary.MakeRotator` 0.0 0.0 (+ _returnvalue_yaw 240.0)) false false)))))

(event `ReversiAim`
  (params (`Z Transform` :type "Float (double-precision)"))
  (bind (_returnvalue_x _returnvalue_y _returnvalue_z) (`KismetMathLibrary.BreakVector` (`self.K2_GetActorLocation`)))
  ;[1 1 1] Animation
  (`|PlayMontage` (`self.Rebl_Chewing_01`) "/Game/Animation/AnimBp/Slime/Montage/EnterTunel.EnterTunel"
    (:`then`
      (bind (_direction _newtrack_0) (`Timeline|Timeline_0`)
        (:`Update`
          (`self.K2_SetActorLocation` (`KismetMathLibrary.MakeVector` _returnvalue_x _returnvalue_y (`KismetMathLibrary.Lerp` (- _returnvalue_z `Z Transform`) `Z Transform` _newtrack_0))))
        (:`Finished`
          (if (`self.b_IsTuto`)
            (set `self.b_Tuto_is_Inactactive` false)))))))

(event `self.lookArea.OnComponentBeginOverlap`
  (params (OverlappedComponent :type "PrimitiveComponent Object Reference") (OtherActor :type "Actor Object Reference") (OtherComp :type "PrimitiveComponent Object Reference") (OtherBodyIndex :type Integer) (bFromSweep :type Boolean) (SweepResult :type "HitResult Structure (by ref)"))
  ;[1 1 1] Look at player
  (if (not (`self.isSleeping`))
    (cast `/Game/Blueprints/Player/Player/BP_Player` OtherActor)
    (set `self.LookActor` OtherActor)
    (bind _returnvalue (`KismetSystemLibrary.K2_SetTimerDelegate` (delegate `LookPlayer`) 0.01 true))
    (set `self.looktimer` _returnvalue)))

(event `Revien`
  (`KismetSystemLibrary.K2_PauseTimerHandle` (`self.DelayTimer`))
  (set `self.TimerDuration` 1.0)
  (`/Game/Blueprints/Widgets/WG_SlimeSleeping.ChangeBack` (`self.As WG Slime Sleeping`))
  (`self.SleepPhase`))

(event `LookPlayer`
  (bind (_returnvalue_roll _returnvalue_pitch _returnvalue_yaw) (`KismetMathLibrary.BreakRotator` (`KismetMathLibrary.RInterpTo` (`SceneComponent.K2_GetComponentRotation` (`self.Rebl_Chewing_01`)) (`KismetMathLibrary.FindLookAtRotation` (`SceneComponent.K2_GetComponentLocation` (`self.Rebl_Chewing_01`)) (`self.K2_GetActorLocation` (`self.LookActor`))) (`GameplayStatics.GetWorldDeltaSeconds`) 0.8)))
  ;[1 1 1] Look at player
  (if (not (`self.isSleeping`))
    (bind _rebl_chewing_01 (`self.Rebl_Chewing_01`)
      (:`then`
        (`SceneComponent.K2_SetWorldRotation` _rebl_chewing_01 (`KismetMathLibrary.MakeRotator` 0.0 0.0 _returnvalue_yaw) false false))
      (:`else`))))

(event `self.gIVEbOX.OnComponentBeginOverlap`
  (params (OverlappedComponent :type "PrimitiveComponent Object Reference") (OtherActor :type "Actor Object Reference") (OtherComp :type "PrimitiveComponent Object Reference") (OtherBodyIndex :type Integer) (bFromSweep :type Boolean) (SweepResult :type "HitResult Structure (by ref)"))
  (bind (_returnvalue_x _returnvalue_y _returnvalue_z) (`KismetMathLibrary.BreakVector` (`SceneComponent.K2_GetComponentLocation` (`self.Rebl_Chewing_01`))))
  (bind (_returnvalue_x_2 _returnvalue_y_2) (`KismetMathLibrary.BreakVector` (`KismetMathLibrary.VInterpTo` (`self.K2_GetActorLocation` (`self.As BP Scrap`)) (`SceneComponent.K2_GetComponentLocation` (`self.Rebl_Chewing_01`)) (`GameplayStatics.GetWorldDeltaSeconds`) 10.0)))
  ;[1 1 1] When box is given
  (if (and (not (`self.isSleeping`)) (not (`self.IsSwitching`)) (not (`self.IsCrafting`)) (not (`self.b_Tuto_is_Inactactive`)))
    (bind _cage (`self.cage`)
      (:`then`
        (if (not (`/Game/Blueprints/LevelPrototyping/BP_LaserCage.GateActivated` _cage))
          (bind _asbp_scrap (cast `/Game/Blueprints/Enemie/Blueprint/BP_Scrap` OtherActor :!label _label))
          (set `self.As BP Scrap` _asbp_scrap)
          (set `self.NbScrap` (+ (`/Game/Blueprints/Enemie/Blueprint/BP_Scrap.Value` (`self.As BP Scrap`)) (`self.NbScrap`)))
          (`PrimitiveComponent.SetPhysicsLinearVelocity` (`/Game/Blueprints/Enemie/Blueprint/BP_Scrap.StaticMesh` (`self.As BP Scrap`)) (0.0 0.0 0.0) false "None")
          (`|ExecutionSequence`
            (:`then_0`
              (`self.SetActorEnableCollision` (`self.As BP Scrap`) false)
              (`Timeline|GoTo` :!via `PlayFromStart`
                (:`Update`
                  (`self.K2_SetActorLocation` (`self.As BP Scrap`) (`KismetMathLibrary.MakeVector` _returnvalue_x_2 _returnvalue_y_2 _returnvalue_z) false false))
                (:`Finished`
                  (`/Game/Blueprints/Enemie/Blueprint/BP_Scrap.FunctionDestroyActor` (`self.As BP Scrap`)))))
            (:`then_1`
              (set `self.GrabScrap` true)
              (set `self.IsCrafting` true)
              (`KismetSystemLibrary.Delay` (`self.CraftingDuration`))
              (set `self.IsCrafting` false)))))
      (:`else`
        (goto _label)))))

(event `self.lookArea.OnComponentEndOverlap`
  (params (OverlappedComponent :type "PrimitiveComponent Object Reference") (OtherActor :type "Actor Object Reference") (OtherComp :type "PrimitiveComponent Object Reference") (OtherBodyIndex :type Integer))
  ;[1 1 1] Look at player
  (cast `/Game/Blueprints/Player/Player/BP_Player` OtherActor)
  (set `self.LookActor` null)
  (`KismetSystemLibrary.K2_PauseTimerHandle` (`self.looktimer`))
  (bind _returnvalue (`KismetSystemLibrary.K2_SetTimerDelegate` (delegate `ReturnToPlace`) 0.01 true))
  (set `self.Timer` _returnvalue))

(event `CreateAddons`
  (bind _gestionmachine (`self.GestionMachine`))
  (bind _returnvalue (`SceneComponent.K2_GetComponentLocation` (`self.Scene`)))
  ;[1 1 1] CreateAddons event
  (set `self.NbScrap` (- (`self.NbScrap`) (`self.ScrapNeeded`) 0))
  (set `self.IsCrafting` false)
  (`NiagaraFunctionLibrary.SpawnSystemAtLocation` "/Game/VFX/VFX/Distributeur/StarSuccess/NS_StarSuccess.NS_StarSuccess" _returnvalue)
  (cast `/Game/Blueprints/Enemie/Blueprint/BP_GoldenScrap` (`self.As BP Scrap`)
    (:`then`
      (bind _index (`/Game/Blueprints/Macro/ML_Macro.ForLoopWithDelay` 0 2 2.0 -2.0)
        (:`LoopBody`
          (bind _returnvalue_2 (`|SpawnActorFromClass` "/Game/Blueprints/Turret/Blueprint/BP_TurretKit.BP_TurretKit_C" (`KismetMathLibrary.MakeTransform` _returnvalue (struct) (0.8 0.8 0.8)) "Undefined" "MultiplyWithRoot" null (`KismetMathLibrary.RandomIntegerInRange` -99999 999999) (`self.TypeOfPrinter`) null :!label _label_2))
          (if (`self.b_Give_TutoManager_Ref_`)
            (set `/Game/Blueprints/Turret/Blueprint/BP_TurretKit.BP_TutorialManager` (`self.TutorialmanagerRef`) _returnvalue_2))
          (`PrimitiveComponent.SetAllPhysicsLinearVelocity` (`/Game/Blueprints/Turret/Blueprint/BP_TurretKit.Kit` _returnvalue_2) (* (`SceneComponent.GetForwardVector` (select `int` _index :`0` (`self.Arrow`) :`1` (`self.Arrow1`) :`2` (`self.Arrow2`))) 1000.0) false))
        (:`Complete`
          (set `self.IsCrafting` false :!label _label_3)
          (`self.SleepPhase`)
          (`/Engine/EditorBlueprintResources/StandardMacros.IsValid` _gestionmachine
            (:`Is Valid`
              (if (`/Game/Blueprints/Machine/BP_GestionSlime.b_NeedToShuffle` _gestionmachine)
                (`/Game/Blueprints/Machine/BP_GestionSlime.ShuffleMachine` _gestionmachine)))
            (:`Is Not Valid`
              _))
          (bind _tutorialmanagerref (`self.TutorialmanagerRef`)
            (:`then`
              (`/Game/Blueprints/Tutorial/BP_TutorialManager.Slime` _tutorialmanagerref))
            (:`else`)))))
    (:`CastFailed`
      (`|ExecutionSequence`
        (:`then_0`
          (goto _label_2))
        (:`then_1`
          (goto _label_3))))))

(event `ReturnToPlace`
  (bind _rebl_chewing_01 (`self.Rebl_Chewing_01`))
  ;[1 1 1] Look at player
  (`SceneComponent.K2_SetWorldRotation` _rebl_chewing_01 (`KismetMathLibrary.RInterpTo` (`SceneComponent.K2_GetComponentRotation` _rebl_chewing_01) (`self.FirstRotation`) (`GameplayStatics.GetWorldDeltaSeconds`) 1.0) false false)
  (if (== (`SceneComponent.K2_GetComponentRotation` (`self.Rebl_Chewing_01`)) (`self.FirstRotation`) :`ErrorTolerance` 1.0)
    (`KismetSystemLibrary.K2_PauseTimerHandle` (`self.Timer`))))

(fn `ChangeFacialAnim`
  (params (nbFrame :type "Float (single-precision)") (Face :type "Texture Object Reference"))
  (`MaterialInstanceDynamic.SetScalarParameterValue` (`self.DynamicM`) "Nombre D'image" nbFrame)
  (`MaterialInstanceDynamic.SetTextureParameterValue` (`self.DynamicM`) "Texture" Face))

(fn `GetGoodFace`
  (params (WhatFace :type Integer))
  (returns (nbFrame :type "Float (double-precision)") (Face :type "Texture Object Reference"))
  (bind _face (break `/Game/Blueprints/Machine/FaceStructure` (`BlueprintMapLibrary.Map_Find` (`self.MapsTypeFace`) (`self.TypeOfPrinter`))))
  (bind _keys (`BlueprintMapLibrary.Map_Keys` _face))
  (bind _output (`|GetArrayItem` _keys WhatFace))
  (return (`BlueprintMapLibrary.Map_Find` _face _output) _output))

(fn `Spit Out Scraps`
  (bind _returnvalue (- (`self.NbScrap`) (`self.ScrapNeeded`)))
  (if (<= _returnvalue 3)
    (bind _returnvalue_2 (`|SpawnActorFromClass` "/Game/Blueprints/Enemie/Blueprint/BP_Scrap.BP_Scrap_C" (`KismetMathLibrary.MakeTransform` (`SceneComponent.K2_GetComponentLocation` (`self.Scrap Spawn`))) "Undefined" "MultiplyWithRoot" null _returnvalue null))
    (set `/Game/Blueprints/Enemie/Blueprint/BP_Scrap.Value` _returnvalue _returnvalue_2)
    (`PrimitiveComponent.SetPhysicsLinearVelocity` (`/Game/Blueprints/Enemie/Blueprint/BP_Scrap.StaticMesh` _returnvalue_2) (`self.Impulse Scrap`) false "None")))

(fn `UserConstructionScript`
  (bind _rebl_chewing_01 (`self.Rebl_Chewing_01`))
  (bind _rebl_chewing_01_2 (`self.Rebl_Chewing_01`))
  (bind _rebl_chewing_01_3 (`self.Rebl_Chewing_01`))
  (switch `/Game/Blueprints/Enums/Enum_Kit` (`self.TypeOfPrinter`)
    (:`NewEnumerator0`
      (`PrimitiveComponent.SetMaterial` _rebl_chewing_01_2 0 "/Game/Assets/Assembleur/Mat/Slime_Inst_Red.Slime_Inst_Red")
      (`SkeletalMeshComponent.SetSkeletalMeshAsset` _rebl_chewing_01_2 "/Game/Assets/Assembleur/Slime/Slime_v4.Slime_v4")
      (set `self.EyesMat` "/Game/Assets/Assembleur/Mat/M_FaceSlime_red.M_FaceSlime_red"))
    (:`NewEnumerator1`
      (`SkeletalMeshComponent.SetSkeletalMeshAsset` _rebl_chewing_01 "/Game/Assets/Assembleur/Slime/Slime_v4.Slime_v4")
      (`PrimitiveComponent.SetMaterial` _rebl_chewing_01 0 "/Game/Assets/Assembleur/Mat/Slime_Inst_green.Slime_Inst_green")
      (set `self.EyesMat` "/Game/Assets/Assembleur/Mat/M_FaceSlime_green.M_FaceSlime_green"))
    (:`NewEnumerator2`
      (`PrimitiveComponent.SetMaterial` _rebl_chewing_01_3 0 "/Game/Assets/Assembleur/Mat/Slime_Inst_Blue.Slime_Inst_Blue")
      (`SkeletalMeshComponent.SetSkeletalMeshAsset` _rebl_chewing_01_3 "/Game/Assets/Assembleur/Slime/Slime_v4.Slime_v4")
      (set `self.EyesMat` "/Game/Assets/Assembleur/Mat/M_FaceSlime_blue.M_FaceSlime_blue")))
  (`PrimitiveComponent.SetMaterial` (`self.Rebl_Chewing_01`) 1 (`self.EyesMat`)))