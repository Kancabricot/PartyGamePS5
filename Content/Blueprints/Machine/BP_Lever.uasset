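; BP_Lever is an interactable machine lever that tilts its mesh one way or the other depending on which side the player stands.
; Left and right trigger boxes set overlap flags when BP_Player enters and clear them when any overlap ends.
; Interact checks left first, then right, and plays a timeline that lerps the mesh from its current rotation toward an opposite pitch offset from its BeginPlay rotation.
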(event `self.ReceiveBeginPlay`
  (set `self.StartRota` (`SceneComponent.K2_GetComponentRotation` (`self.StaticMesh`))))

(event `/Game/Blueprints/Interface/BPI_Interact.Interact`
  (params (Player :type "/Game/Blueprints/Player/Player/BP_Player Object Reference"))
  (bind (_startrota_roll _startrota_pitch _startrota_yaw) (`KismetMathLibrary.BreakRotator` (`self.StartRota`)))
  (bind (_startrota_roll_2 _startrota_pitch_2 _startrota_yaw_2) (`KismetMathLibrary.BreakRotator` (`self.StartRota`)))
  (bind _returnvalue (`SceneComponent.K2_GetComponentRotation` (`self.StaticMesh`)))
  (if (`self.LeftOverlap`)
    (bind (_direction _newtrack_0) (`Timeline|Timeline` :!via `PlayFromStart`)
      (:`Update`
        (`KismetSystemLibrary.PrintString` "hhjjjjjjjjj")
        (`SceneComponent.K2_SetWorldRotation` (`self.StaticMesh`) (`KismetMathLibrary.RLerp` _returnvalue (`KismetMathLibrary.MakeRotator` _startrota_roll (+ _startrota_pitch -50.0) _startrota_yaw) _newtrack_0 true) false false)))
    (elif (`self.RightOverlap`)
      (`KismetSystemLibrary.PrintString` "sdqdq")
      (bind (_direction_2 _newtrack_0_2) (`Timeline|Timeline_0` :!via `PlayFromStart`)
        (:`Update`
          (`KismetSystemLibrary.PrintString` "hhjjjjjjjjj")
          (`SceneComponent.K2_SetWorldRotation` (`self.StaticMesh`) (`KismetMathLibrary.RLerp` _returnvalue (`KismetMathLibrary.MakeRotator` _startrota_roll_2 (+ _startrota_pitch_2 50.0) _startrota_yaw_2) _newtrack_0_2 true) false false))))))

(event `self.RightBox.OnComponentBeginOverlap`
  (params (OverlappedComponent :type "PrimitiveComponent Object Reference") (OtherActor :type "Actor Object Reference") (OtherComp :type "PrimitiveComponent Object Reference") (OtherBodyIndex :type Integer) (bFromSweep :type Boolean) (SweepResult :type "HitResult Structure (by ref)"))
  (cast `/Game/Blueprints/Player/Player/BP_Player` OtherActor)
  (set `self.RightOverlap` true))

(event `self.LeftBox.OnComponentBeginOverlap`
  (params (OverlappedComponent :type "PrimitiveComponent Object Reference") (OtherActor :type "Actor Object Reference") (OtherComp :type "PrimitiveComponent Object Reference") (OtherBodyIndex :type Integer) (bFromSweep :type Boolean) (SweepResult :type "HitResult Structure (by ref)"))
  (cast `/Game/Blueprints/Player/Player/BP_Player` OtherActor)
  (set `self.LeftOverlap` true))

(event `self.RightBox.OnComponentEndOverlap`
  (params (OverlappedComponent :type "PrimitiveComponent Object Reference") (OtherActor :type "Actor Object Reference") (OtherComp :type "PrimitiveComponent Object Reference") (OtherBodyIndex :type Integer))
  (set `self.RightOverlap` false))

(event `self.LeftBox.OnComponentEndOverlap`
  (params (OverlappedComponent :type "PrimitiveComponent Object Reference") (OtherActor :type "Actor Object Reference") (OtherComp :type "PrimitiveComponent Object Reference") (OtherBodyIndex :type Integer))
  (set `self.LeftOverlap` false))

(fn `UserConstructionScript`)