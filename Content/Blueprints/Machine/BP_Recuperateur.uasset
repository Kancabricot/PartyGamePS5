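; BP_Recuperateur is a scrap collector machine that turns deposited scrap into 3D printer jobs.
; While unlocked, its box overlap adds each BP_Scrap's value to a running total and destroys it.
; At the required total, it shuffles its printer array, calls CreateAddons on the first, and deducts the cost.
; If HasAkit is already set, it locks instead and prints a debug string.
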(event `self.Box.OnComponentBeginOverlap`
  (params (OverlappedComponent :type "PrimitiveComponent Object Reference") (OtherActor :type "Actor Object Reference") (OtherComp :type "PrimitiveComponent Object Reference") (OtherBodyIndex :type Integer) (bFromSweep :type Boolean) (SweepResult :type "HitResult Structure (by ref)"))
  (bind _3dprinter (`self.3dPrinter`))
  (if (not (`self.isLock`))
    (bind _asbp_scrap (cast `/Game/Blueprints/Enemie/Blueprint/BP_Scrap` OtherActor))
    (set `self.NbScrap` (+ (`/Game/Blueprints/Enemie/Blueprint/BP_Scrap.Value` _asbp_scrap) (`self.NbScrap`)))
    (`self.K2_DestroyActor` _asbp_scrap)
    (if (>= (`self.NbScrap`) (`self.ScrapNeeded`))
      (if (not (`self.HasAkit`))
        (`KismetArrayLibrary.Array_Shuffle` _3dprinter)
        (`/Game/Blueprints/Machine/BP_3dPrinter.CreateAddons` (`|GetArrayItem` _3dprinter) self)
        (set `self.NbScrap` (- (`self.NbScrap`) (`self.ScrapNeeded`)))
        (else
          (set `self.isLock` true)
          (`KismetSystemLibrary.PrintString` "Hello"))))))

(fn `UserConstructionScript`)