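; BP_Scrap is a physics-driven scrap item that a player can pick up and that can be launched when detached.
; TakeItem hands the actor to the player, flags it as grabbed and turns off its mesh collision and physics.
; DettachItem restores collision and physics and sets the mesh velocity to the given impulse, leaving the grabbed flag untouched.
; GiveItemToDesk always returns false, and the overlap handlers are empty.
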(event `self.Box.OnComponentBeginOverlap`
  (params (OverlappedComponent :type "PrimitiveComponent Object Reference") (OtherActor :type "Actor Object Reference") (OtherComp :type "PrimitiveComponent Object Reference") (OtherBodyIndex :type Integer) (bFromSweep :type Boolean) (SweepResult :type "HitResult Structure (by ref)")))

(event `/Game/Blueprints/Interface/BPI_TakeItem.DettachItem`
  (params (Impulse :type "Vector Structure"))
  (bind _staticmesh (`self.StaticMesh`))
  (bind _output_get (set `self.Impulse` Impulse))
  (`PrimitiveComponent.SetCollisionEnabled` _staticmesh "QueryAndPhysics")
  (`PrimitiveComponent.SetSimulatePhysics` _staticmesh true)
  (`PrimitiveComponent.SetPhysicsLinearVelocity` (`self.StaticMesh`) _output_get false "None"))

(fn `GiveItemToDesk`
  (params (ActorTarget :type "Actor Object Reference"))
  (returns (Return :type Boolean))
  (return false))

(fn `TakeItem`
  (params (Player :type "/Game/Blueprints/Player/BP_Player Object Reference"))
  (returns (Return :type Boolean))
  (`/Game/Blueprints/Player/BP_Player.TakeItem` Player 0.0 self)
  (`PrimitiveComponent.SetCollisionEnabled` (`self.StaticMesh`) "NoCollision")
  (set `self.b_IsGrab` true)
  (`PrimitiveComponent.SetSimulatePhysics` (`self.StaticMesh`) false)
  (return false))

(fn `UserConstructionScript`)