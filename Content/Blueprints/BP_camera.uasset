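; BP_camera is a camera rig Blueprint that frames a center reference point using preset framing variables.
; Its construction script calls ModifyPresets, which applies distance to the spring arm length, pitch and field of view to the camera, and negated view angle to CenterRef's pitch.
; The presets apply at construction time, and BeginPlay does nothing.
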(event `self.ReceiveBeginPlay`)

(fn `ModifyPresets`
  (bind _camera (`self.Camera`))
  (set `SpringArmComponent.TargetArmLength` (`self.DistanceFromCenter`) (`self.SpringArm`))
  (`SceneComponent.K2_SetRelativeRotation` _camera (`KismetMathLibrary.MakeRotator` 0.0 (`self.CamPitch`)) false false)
  (`CameraComponent.SetFieldOfView` _camera (`self.FOV`))
  (`SceneComponent.K2_SetRelativeRotation` (`self.CenterRef`) (`KismetMathLibrary.MakeRotator` 0.0 (* (`self.AngleOfView`) -1.0)) false false))

(fn `UserConstructionScript`
  (`self.ModifyPresets`))