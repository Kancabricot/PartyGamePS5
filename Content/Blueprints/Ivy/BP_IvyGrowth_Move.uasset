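; Ivy actor that grows along a spline, then turns into a physics-driven cable with foliage.
; A looping timer extends spline mesh stem segments, while random leaf meshes scale up segment by segment after a delay.
; Once growth ends, it destroys the spline meshes, shows the Cable and makes added static meshes follow its particle locations.
; Cable ticking and the timer stop a few seconds later, freezing the result.
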(event `self.ReceiveBeginPlay`
  (`ActorComponent.SetComponentTickEnabled` (`self.Cable`) false)
  (`self.ClearTable`)
  (bind _returnvalue (`KismetSystemLibrary.K2_SetTimerDelegate` (delegate `StartStem`) 0.01 true))
  (set `self.TimerStem` _returnvalue)
  (`KismetSystemLibrary.Delay` (`self.DelayBeforeLeave`))
  (set `self.spawnLeave` true))

(event `StartStem`
  (`self.StemGrowth`)
  (`self.LeavesGrowth`)
  (if (> (`SplineComponent.GetSplineLength` (`self.Spline`)) (+ (`self.StemDistance`) (`self.SegmentLength`)))
    _
    (elif (`KismetArrayLibrary.Array_IsEmpty` (`self.MeshFoliage`))
      (`KismetSystemLibrary.Delay` (`self.DelayBeforeLeave`))
      (`/Engine/EditorBlueprintResources/StandardMacros.DoOnce` false
        (:`Completed`
          ;[1 1 1] Destroy Static Ivy
          (for _array_element (`self.AllStem`)
            (`/Engine/EditorBlueprintResources/StandardMacros.IsValid` _array_element
              (:`Is Valid`
                (`ActorComponent.K2_DestroyComponent` _array_element))))
          (`SceneComponent.SetVisibility` (`self.Cable`) true false)
          (`ActorComponent.Activate` (`self.Pouf`) false)
          ;[1 1 1] initalize static mesh on cable
          (`ActorComponent.SetComponentTickEnabled` (`self.Cable`) true)
          (for _array_element_2 (`CableComponent.GetCableParticleLocations` (`self.Cable`))
            (bind _returnvalue (`AddComponent|NODE_AddStaticMeshComponent-0` :`RelativeTransform` (`KismetMathLibrary.MakeTransform` _array_element_2)))
            (`KismetArrayLibrary.Array_Add` (`self.MeshFoliage`) _returnvalue))
          ;[1 1 1] stop Physics on cable
          (`KismetSystemLibrary.Delay` 6.0)
          (`ActorComponent.SetComponentTickEnabled` (`self.Cable`) false)
          (`KismetSystemLibrary.K2_ClearAndInvalidateTimerHandle` (`self.TimerStem`))))
      (else
        ;[1 1 1] update static mesh position on cable
        (for (_array_element_3 _array_index) (`self.MeshFoliage`)
          (`SceneComponent.K2_SetWorldLocation` _array_element_3 (`|GetArrayItem` (`CableComponent.GetCableParticleLocations` (`self.Cable`)) _array_index) false false))))))

(fn `ClearTable`
  (`KismetArrayLibrary.Array_Clear` (`self.MeshFoliage`))
  (`KismetArrayLibrary.Array_Clear` (`self.AllStem`)))

(fn `LeavesGrowth`
  (bind _leavesdistance (`self.LeavesDistance`))
  (bind _currentleaves (`self.CurrentLeaves`))
  (bind _leavesgrowthalpha (`self.LeavesGrowthAlpha`))
  (bind _spline (`self.Spline`))
  (bind _returnvalue (+ _leavesdistance (`self.SegmentLength`)))
  (if (`self.spawnLeave`)
    (if (> (`SplineComponent.GetSplineLength` (`self.Spline`)) (+ (`self.StemDistance`) (`self.SegmentLength`)))
      (`self.CurrentLeaves`
        (:`then`
          _)
        (:`else`
          (bind _returnvalue_2 (`AddComponent|NODE_AddSplineMeshComponent-1`))
          (bind _output_get (set `self.CurrentLeaves` _returnvalue_2))
          (`KismetArrayLibrary.Array_Add` (`self.AllStem`) _output_get)
          (`StaticMeshComponent.SetStaticMesh` _output_get (`KismetArrayLibrary.Array_Random` (`self.LeavesMeshes`)))))
      (`SplineMeshComponent.SetStartAndEnd` (`self.CurrentLeaves`) (`SplineComponent.GetLocationAtDistanceAlongSpline` _spline _leavesdistance "Local") (`SplineComponent.GetDirectionAtDistanceAlongSpline` _spline _leavesdistance "Local") (`SplineComponent.GetLocationAtDistanceAlongSpline` _spline _returnvalue "Local") (`SplineComponent.GetDirectionAtDistanceAlongSpline` _spline _returnvalue "Local") true)
      (`SplineMeshComponent.SetStartScale` _currentleaves (`KismetMathLibrary.MakeVector2D` _leavesgrowthalpha _leavesgrowthalpha) true)
      (`SplineMeshComponent.SetEndScale` _currentleaves (`KismetMathLibrary.MakeVector2D` _leavesgrowthalpha _leavesgrowthalpha) true)
      (bind _output_get_2 (set `self.LeavesGrowthAlpha` (+ (`self.LeavesGrowthAlpha`) (* (`GameplayStatics.GetWorldDeltaSeconds`) (`self.GrowthRate`)))))
      (if (> _output_get_2 1.0)
        (set `self.LeavesGrowthAlpha` 0.0)
        (set `self.LeavesDistance` (+ (`self.LeavesDistance`) (`self.SegmentLength`)))
        (set `self.CurrentLeaves` null)))))

(fn `StemGrowth`
  (bind _spline (`self.Spline`))
  (bind _stemdistance (`self.StemDistance`))
  (bind _returnvalue (`SplineComponent.GetLocationAtDistanceAlongSpline` _spline _stemdistance "Local"))
  (bind _returnvalue_2 (+ _stemdistance (`self.SegmentLength`)))
  (if (> (`SplineComponent.GetSplineLength` (`self.Spline`)) (+ (`self.StemDistance`) (`self.SegmentLength`)))
    (`self.CurrentStem`
      (:`then`
        _)
      (:`else`
        (bind _returnvalue_3 (`AddComponent|NODE_AddSplineMeshComponent-0`))
        (bind _output_get (set `self.CurrentStem` _returnvalue_3))))
    (`KismetArrayLibrary.Array_Add` (`self.AllStem`) _output_get)
    (`SplineMeshComponent.SetStartAndEnd` (`self.CurrentStem`) _returnvalue (`SplineComponent.GetDirectionAtDistanceAlongSpline` _spline _stemdistance "Local") (`KismetMathLibrary.VLerp` _returnvalue (`SplineComponent.GetLocationAtDistanceAlongSpline` _spline _returnvalue_2 "Local") (`self.StemGrowthAlpha`)) (`SplineComponent.GetDirectionAtDistanceAlongSpline` _spline _returnvalue_2 "Local") true)
    (bind _output_get_2 (set `self.StemGrowthAlpha` (+ (`self.StemGrowthAlpha`) (* (`GameplayStatics.GetWorldDeltaSeconds`) (`self.GrowthRate`)))))
    (if (> _output_get_2 1.0)
      (set `self.StemGrowthAlpha` 0.0)
      (set `self.StemDistance` (+ (`self.StemDistance`) (`self.SegmentLength`)))
      (set `self.CurrentStem` null))))

(fn `UserConstructionScript`)