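; Static ivy actor that lays stems and leaves along an editable spline.
; The construction script chains spline meshes in fixed-length sections, optionally scaled by actor X scale or limited to full-length pieces, with tangents clamped to section length.
; SpawnLeaves, separate from construction, replaces leaves with evenly spaced random meshes, randomizing scale and multiplying spline rotation by a random factor.
; ClearSplinePoints resets the spline to two points and destroys the stem meshes.
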(fn `ClearSplinePoints`
  (bind _spline (`self.Spline`))
  (`SplineComponent.ClearSplinePoints` _spline true)
  (`SplineComponent.AddSplinePoint` _spline (0.0 0.0 0.0) "Local" true)
  (`SplineComponent.AddSplinePoint` _spline (0.0 50.0 0.0) "Local" true)
  (for _array_element (`self.SplineMeshes`)
    (if (`KismetSystemLibrary.IsValid` _array_element)
      (`ActorComponent.K2_DestroyComponent` _array_element))))

(fn `get end pos/ angent`
  (params (Index :type Integer))
  (returns (Position :type "Vector Structure") (Tangent :type "Vector Structure"))
  (bind _spline (`self.Spline`))
  (bind _returnvalue (* (+ Index 1) (`self.Section Length`)))
  (return (`SplineComponent.GetLocationAtDistanceAlongSpline` _spline _returnvalue "Local") (`KismetMathLibrary.ClampVectorSize` (`SplineComponent.GetTangentAtDistanceAlongSpline` _spline _returnvalue "Local") 0.0 (`self.Section Length`))))

(fn `get start pos/tangent`
  (params (Index :type Integer))
  (returns (Position :type "Vector Structure") (Tangent :type "Vector Structure"))
  (bind _spline (`self.Spline`))
  (bind _returnvalue (* Index (`self.Section Length`)))
  (return (`SplineComponent.GetLocationAtDistanceAlongSpline` _spline _returnvalue "Local") (`KismetMathLibrary.ClampVectorSize` (`SplineComponent.GetTangentAtDistanceAlongSpline` _spline _returnvalue "Local") 0.0 (`self.Section Length`))))

(fn `SpawnLeaves`
  (bind _spline (`self.Spline`))
  (bind _nbfeuilles (`self.NbFeuilles`))
  (bind _returnvalue (`SplineComponent.GetSplineLength` _spline))
  (for _array_element (`self.Leaves`)
    (if (`KismetSystemLibrary.IsValid` _array_element)
      (`ActorComponent.K2_DestroyComponent` _array_element)))
  (if (`self.AutoLeaves`)
    (set `self.NbFeuilles` (`KismetMathLibrary.FTrunc` (/ _returnvalue (`self.LeavesDistances`)))))
  (bind _output_get (set `self.Section Length` (/ _returnvalue _nbfeuilles)))
  (bind _output_get_2 (set `self.LeavesDistance` _output_get))
  (for _ (range (+ (- _nbfeuilles 2) 1))
    ;[1 1 1] Leaves
    (bind _returnvalue_2 (`AddComponent|NODE_AddStaticMeshComponent-1` :`RelativeTransform` (`KismetMathLibrary.MakeTransform` (`SplineComponent.GetLocationAtDistanceAlongSpline` _spline _output_get_2 "Local") (* (`SplineComponent.GetRotationAtDistanceAlongSpline` _spline _output_get_2 "Local") (`KismetMathLibrary.RandomFloatInRange` 0.0 180.0)) (`KismetMathLibrary.Conv_DoubleToVector` (`KismetMathLibrary.RandomFloatInRange` 1.2 2.0)))))
    (`KismetArrayLibrary.Array_Add` (`self.Leaves`) _returnvalue_2)
    (`StaticMeshComponent.SetStaticMesh` _returnvalue_2 (`KismetArrayLibrary.Array_Random` (`self.LeavesMeshes`)))
    (set `self.LeavesDistance` (+ (`self.LeavesDistance`) (`self.Section Length`)))))

(fn `UserConstructionScript`
  (bind _returnvalue_x (`KismetMathLibrary.BreakVector` (`self.GetActorScale3D`)))
  ;[1 1 1] done
  (if (`self.AllowScaling ?`)
    (set `self.Section Length` (* _returnvalue_x 100.0)))
  (if (`self.Must be full length meshes`)
    ;;[1 1 1] must be full length
    (for _index (range (`KismetMathLibrary.FTrunc` (/ (`SplineComponent.GetSplineLength` (`self.Spline`)) (`self.Section Length`))))
      (set `self.Loop Index` _index)
      (bind _returnvalue (`AddComponent|NODE_AddSplineMeshComponent-2` :!label _label))
      (`KismetArrayLibrary.Array_Add` (`self.SplineMeshes`) _returnvalue)
      (`StaticMeshComponent.SetStaticMesh` _returnvalue (`self.Spline Mesh`))
      (`SplineMeshComponent.SetForwardAxis` _returnvalue "X" true)
      (bind (_position _tangent) (`self.get start pos/tangent` (`self.Loop Index`)))
      (bind (_position_2 _tangent_2) (`self.get end pos/ angent` (`self.Loop Index`)))
      (`SplineMeshComponent.SetStartAndEnd` _returnvalue _position _tangent _position_2 _tangent_2 true))
    (else
      (for _index_2 (range (+ (`KismetMathLibrary.FTrunc` (/ (`SplineComponent.GetSplineLength` (`self.Spline`)) (`self.Section Length`))) 1))
        (set `self.Loop Index` _index_2)
        (goto _label)))))