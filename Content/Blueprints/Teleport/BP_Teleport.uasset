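; Teleporter Blueprint that moves actors standing in its trigger volume to a linked teleporter, OtherTP.
; TriggerTP overlap events maintain an array of actors inside, using an IsValid flag to skip duplicates.
; The TeleportActor event, not called within this Blueprint, moves each tracked actor without sweep, preserving its world-space offset from this teleporter at the destination.
; It removes each actor from the array while still iterating over it.
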(event `self.TriggerTP.OnComponentBeginOverlap`
  (params (OverlappedComponent :type "PrimitiveComponent Object Reference") (OtherActor :type "Actor Object Reference") (OtherComp :type "PrimitiveComponent Object Reference") (OtherBodyIndex :type Integer) (bFromSweep :type Boolean) (SweepResult :type "HitResult Structure (by ref)"))
  (for _array_element (`self.ActorToTPArray`)
    (if (== _array_element OtherActor)
      (set `self.IsValid` false)))
  (if (`self.IsValid`)
    (`KismetArrayLibrary.Array_Add` (`self.ActorToTPArray`) OtherActor)
    (set `self.IsValid` true)
    (else
      (set `self.IsValid` true))))

(event `self.TriggerTP.OnComponentEndOverlap`
  (params (OverlappedComponent :type "PrimitiveComponent Object Reference") (OtherActor :type "Actor Object Reference") (OtherComp :type "PrimitiveComponent Object Reference") (OtherBodyIndex :type Integer))
  (`KismetArrayLibrary.Array_RemoveItem` (`self.ActorToTPArray`) OtherActor))

(event `TeleportActor`
  (bind _actortotparray (`self.ActorToTPArray`))
  (for _array_element _actortotparray
    (`self.K2_SetActorLocation` _array_element (`self.CalculateRelativeLocation` _array_element) false false)
    (`KismetArrayLibrary.Array_RemoveItem` _actortotparray _array_element)))

(fn `CalculateRelativeLocation`
  (params (ActorTarget :type "Actor Object Reference"))
  (returns (ReturnValue :type "Vector Structure"))
  (return (+ (- (`self.K2_GetActorLocation` ActorTarget) (`self.K2_GetActorLocation`)) (`self.K2_GetActorLocation` (`self.OtherTP`)))))

(fn `UserConstructionScript`)