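; Child Blueprint of an enemy, the Survolté Scrap variant, that drops a golden scrap when it dies.
; Its Death override spawns BP_GoldenScrap at the enemy's location, enables physics on its mesh and launches it with a random velocity along positive X, Y and Z.
; It then calls the parent Death; the event graph holds only disabled default nodes.
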(fn `Death`
  (bind _returnvalue (`KismetMathLibrary.RandomFloatInRange` 0.0 500.0))
  (bind _returnvalue_2 (`|SpawnActorFromClass` "/Game/Blueprints/Enemie/Blueprint/BP_GoldenScrap.BP_GoldenScrap_C" (`KismetMathLibrary.MakeTransform` (`self.K2_GetActorLocation`)) "Undefined" "MultiplyWithRoot" null 0 null))
  (bind _staticmesh (`/Game/Blueprints/Enemie/Blueprint/BP_Scrap.StaticMesh` _returnvalue_2))
  (`PrimitiveComponent.SetSimulatePhysics` _staticmesh true)
  (`PrimitiveComponent.SetPhysicsLinearVelocity` _staticmesh (`KismetMathLibrary.MakeVector` _returnvalue (`KismetMathLibrary.RandomFloatInRange` 0.0 500.0) _returnvalue) false "None")
  (`parent.Death`))

(fn `UserConstructionScript`
  (`parent.UserConstructionScript`))