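; BP_LooseZone is the core that enemies attack, acting as the lose condition and owning the life HUD.
; Each BP_Enemie overlapping its box explodes, is destroyed, shakes the camera and costs one life, updating the WG_HUD counter it creates on BeginPlay.
; At zero life, EndGame stops all enemies and plays the core explosion with camera shakes, then after timed delays shows the losing WG_EndGame screen and pauses.
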(event `self.Box.OnComponentBeginOverlap`
  (params (OverlappedComponent :type "PrimitiveComponent Object Reference") (OtherActor :type "Actor Object Reference") (OtherComp :type "PrimitiveComponent Object Reference") (OtherBodyIndex :type Integer) (bFromSweep :type Boolean) (SweepResult :type "HitResult Structure (by ref)"))
  (bind _asbp_enemie (cast `/Game/Blueprints/Enemie/Blueprint/BP_Enemie` OtherActor))
  (`NiagaraFunctionLibrary.SpawnSystemAtLocation` "/Game/VFX/Turrets/TurretExplosion/NS_Turret_Explosion.NS_Turret_Explosion" (`SceneComponent.K2_GetComponentLocation` (`self.SpawnNiagaraLocation`)) (struct) (2.0 2.0 2.0))
  (`self.K2_DestroyActor` _asbp_enemie)
  (`self.CheckDamage`)
  (`PlayerController.ClientStartCameraShake` :`self` (`GameplayStatics.GetPlayerController` 0) :`Shake` "/Game/Blueprints/Enemie/Blueprint/BP_CamShake.BP_CamShake_C" :`Scale` 10.0))

(event `self.ReceiveBeginPlay`
  (`|ExecutionSequence`
    (:`then_0`
      (bind _returnvalue (`|CreateWidget` "/Game/Blueprints/Widgets/WG_HUD.WG_HUD_C"))
      (bind _output_get (set `self.HealthRef` _returnvalue))
      (`UserWidget.AddToViewport` _output_get 0)
      (set `self.Life` (`self.MaxLife`)))
    (:`then_1`
      (`/Game/Blueprints/Widgets/WG_HUD.SetText` (`self.HealthRef`) (`self.Life`)))))

(event `TimedShake`
  (`KismetSystemLibrary.Delay` 1.86)
  (`PlayerController.ClientStartCameraShake` :`self` (`GameplayStatics.GetPlayerController` 0) :`Shake` "/Game/Blueprints/Enemie/Blueprint/BP_CamShakeExplosion.BP_CamShakeExplosion_C" :`Scale` 50.0)
  (`KismetSystemLibrary.Delay` 1.5)
  (bind _returnvalue (`|CreateWidget` "/Game/Blueprints/Widgets/WG_EndGame.WG_EndGame_C"))
  (`UserWidget.AddToViewport` _returnvalue 0)
  (`GameplayStatics.SetGamePaused` true))

(fn `CheckDamage`
  (set `self.Life` (- (`self.Life`) 1))
  (`/Game/Blueprints/Widgets/WG_HUD.SetText` (`self.HealthRef`) (`self.Life`))
  (if (<= (`self.Life`) 0)
    (`self.End Game`)
    (return)
    (else
      (return))))

(fn `End Game`
  (bind _outactors (`GameplayStatics.GetAllActorsOfClass` "/Game/Blueprints/Enemie/Blueprint/BP_Enemie.BP_Enemie_C"))
  (for _array_element _outactors
    (`/Game/Blueprints/Enemie/Blueprint/BP_Enemie.StopMoving` _array_element))
  (`LegacyCameraShake.StartLegacyCameraShake` null)
  (`NiagaraFunctionLibrary.SpawnSystemAtLocation` "/Game/VFX/Coeur/NS_CoreExplosion.NS_CoreExplosion" (`SceneComponent.K2_GetComponentLocation` (`self.SpawnNiagaraLocation`)))
  (`self.TimedShake`)
  (return))

(fn `UserConstructionScript`)