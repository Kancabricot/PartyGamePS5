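; Tutorial enemy child Blueprint whose death triggers the third wave of the tutorial.
; It overrides Death to call ThirdWave on the tutorial manager reference, if valid, before running the parent death logic.
; All other behavior is inherited, as the event graph holds only disabled placeholder nodes and the construction script just calls its parent.
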(fn `Death`
  (bind _tutomanager_ref (`self.TutoManager ref`)
    (:`then`
      (`/Game/Blueprints/Tutorial/BP_TutorialManager.Third Wave` _tutomanager_ref))
    (:`else`
      _))
  (`parent.Death`))

(fn `UserConstructionScript`
  (`parent.UserConstructionScript`))