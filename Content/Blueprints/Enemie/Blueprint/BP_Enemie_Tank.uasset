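; BP_Enemie_Tank is the tank enemy variant, a child Blueprint that customizes the stats and death of its parent enemy.
; SetStats passes PDAEnemystat tank values to the parent, with the inputs apparently swapped: life feeds MaxWalkSpeed and speed feeds MaxLife.
; Death fires DeathShake, a large-radius world camera shake at the actor's location, before running the parent death logic.
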(event `self.ReceiveBeginPlay`
  (`parent.ReceiveBeginPlay`))

(event `DeathShake`
  (`GameplayStatics.PlayWorldCameraShake` "/Game/Blueprints/LevelPrototyping/CameraShakes/BP_CS_TankDie.BP_CS_TankDie_C" (`self.K2_GetActorLocation`) 0.0 50000.0 0.5))

(fn `Death`
  (`self.DeathShake`)
  (`parent.Death`))

(fn `SetStats`
  (params (`Max Walk Speed` :type "Float (single-precision)") (MaxLife :type "Float (double-precision)"))
  (`parent.SetStats` (`/Game/Blueprints/Enemie/Blueprint/DataAsset/PDA_Enemie.EnemieTankLife` (`self.PDA_Enemystat `)) (`/Game/Blueprints/Enemie/Blueprint/DataAsset/PDA_Enemie.TankEnemieSpeed` (`self.PDA_Enemystat `))))

(fn `UserConstructionScript`
  (`parent.UserConstructionScript`))