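; BP_PorteEnnemi is an enemy door Blueprint with a neon material that can flicker between red and black.
; On BeginPlay it creates a dynamic material instance from slot 1 of its static mesh.
; FlickeringNeon turns the neon off, plays a timeline that lerps the Base Color between red and black, then turns it back on.
; LightOnNeon and LightOffNeon set the color directly to red or black.
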(event `self.ReceiveBeginPlay`
  (bind _staticmeshcomponent (`self.StaticMeshComponent`))
  (bind _returnvalue (`PrimitiveComponent.CreateDynamicMaterialInstance` _staticmeshcomponent 1 (`PrimitiveComponent.GetMaterial` _staticmeshcomponent 1) "None"))
  (set `self.DMI_neon` _returnvalue))

(event `Flickering Neon`
  (`self.Light Off Neon`)
  (bind (_direction _lerp_color_alpha) (`Timeline|Timeline` :!via `PlayFromStart`)
    (:`Update`
      (`MaterialInstanceDynamic.SetVectorParameterValue` (`self.DMI_neon`) "Base Color" (`KismetMathLibrary.LinearColorLerp` (struct :`R` 1.0 :`B` 0.045186 :`A` 1.0) (struct) _lerp_color_alpha)))
    (:`Finished`
      (`self.Light On Neon`))))

(event `Light On Neon`
  (`MaterialInstanceDynamic.SetVectorParameterValue` (`self.DMI_neon`) "Base Color" (struct :`R` 1.0 :`B` 0.045186 :`A` 1.0)))

(event `Light Off Neon`
  (`MaterialInstanceDynamic.SetVectorParameterValue` (`self.DMI_neon`) "Base Color" (struct :`A` 1.0)))

(fn `UserConstructionScript`)