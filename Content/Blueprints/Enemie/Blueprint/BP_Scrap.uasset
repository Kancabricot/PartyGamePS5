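; BP_Scrap is a carryable scrap pickup that self-destroys after a set duration and points to the smeltery.
; TakeItem hands it to the player, disables physics and collision, and shows a gear icon with a looping rotation timer.
; DettachItem hides the icon, pauses the timer, stops the arrow and launches the mesh with an impulse, ignoring pawns.
; Highlighting uses custom depth stencil, HightLiteTarget plays the smeltery's arrow widget, and desks always refuse it.
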(event `self.ReceiveBeginPlay`
  (`|ExecutionSequence`
    (:`then_0`
      (bind _returnvalue (`GameplayStatics.GetActorOfClass` "/Game/Blueprints/Machine/BP_Smelterie.BP_Smelterie_C"))
      (set `self.SmelteriRef` _returnvalue))
    (:`then_1`
      (`KismetSystemLibrary.Delay` (`self.DurationBeforeDestroy`))
      (`self.K2_DestroyActor`))))

(event `self.Box.OnComponentBeginOverlap`
  (params (OverlappedComponent :type "PrimitiveComponent Object Reference") (OtherActor :type "Actor Object Reference") (OtherComp :type "PrimitiveComponent Object Reference") (OtherBodyIndex :type Integer) (bFromSweep :type Boolean) (SweepResult :type "HitResult Structure (by ref)"))
  (cast `/Game/Blueprints/Enemie/Blueprint/BP_Scrap` OtherActor))

(event `/Game/Blueprints/Interface/BPI_TakeItem.DettachItem`
  (params (Impulse :type "Vector Structure"))
  (bind _staticmesh (`self.StaticMesh`))
  (`KismetSystemLibrary.K2_PauseTimerHandle` (`self.ActuTimer`))
  (`/Game/Blueprints/Arrow/wg_arrow.Stop` (`self.As Wg Arrow`))
  (`SceneComponent.SetVisibility` (`/Game/Blueprints/Player/Player/BP_Player.Widget` (`self.ActuPlayer`)) false false)
  (bind _output_get (set `self.Impulse` Impulse))
  (`PrimitiveComponent.SetCollisionEnabled` _staticmesh "QueryAndPhysics")
  (`PrimitiveComponent.SetCollisionResponseToChannel` (`self.StaticMesh`) "ECC_Pawn" "ECR_Ignore")
  (`PrimitiveComponent.SetSimulatePhysics` _staticmesh true)
  (`PrimitiveComponent.SetPhysicsLinearVelocity` (`self.StaticMesh`) _output_get false "None")
  (set `self.b_IsGrab` false))

(event `SetLoc`)

(event `/Game/Blueprints/Interface/BPI_TakeItem.ActiveHighlight`
  (`PrimitiveComponent.SetCustomDepthStencilValue` (`self.StaticMesh`) 1))

(event `/Game/Blueprints/Interface/BPI_TakeItem.DeactiveHighlight`
  (`PrimitiveComponent.SetCustomDepthStencilValue` (`self.StaticMesh`) 0))

(event `/Game/Blueprints/Interface/BPI_HightLiteTarget.HightLiteTarget`
  (bind _widget (`/Game/Blueprints/Machine/BP_Smelterie.Widget` (`self.SmelteriRef`)))
  (`SceneComponent.SetVisibility` _widget true false)
  (bind _aswg_arrow (cast `/Game/Blueprints/Arrow/wg_arrow` (`WidgetComponent.GetWidget` _widget)))
  (bind _output_get (set `self.As Wg Arrow` _aswg_arrow))
  (`/Game/Blueprints/Arrow/wg_arrow.Play` _aswg_arrow)
  (`/Game/Blueprints/Arrow/wg_arrow.Play` _output_get))

(fn `GiveItemToDesk`
  (params (ActorTarget :type "Actor Object Reference"))
  (returns (Return :type Boolean))
  (return false))

(fn `TakeItem`
  (params (Player :type "/Game/Blueprints/Player/Player/BP_Player Object Reference"))
  (returns (Return :type Boolean))
  (bind _widget (`/Game/Blueprints/Player/Player/BP_Player.Widget` (`self.ActuPlayer`)))
  (bind _output_get (set `self.ActuPlayer` Player))
  (bind _returnvalue (`KismetSystemLibrary.K2_SetTimer` _output_get "RotateWidget" 0.1 true))
  (set `self.ActuTimer` _returnvalue)
  (bind _aswg_icon (cast `/Game/Blueprints/Arrow/WG_Icon` (`WidgetComponent.GetWidget` _widget)))
  (`/Game/Blueprints/Arrow/WG_Icon.SetImage` _aswg_icon "/Game/Blueprints/Arrow/PictoEngrenage_carre__1_.PictoEngrenage_carre__1_")
  (`SceneComponent.SetVisibility` _widget true false)
  (`/Game/Blueprints/Player/Player/BP_Player.TakeItem` Player self)
  (`PrimitiveComponent.SetCollisionEnabled` (`self.StaticMesh`) "NoCollision")
  (set `self.b_IsGrab` true)
  (`PrimitiveComponent.SetSimulatePhysics` (`self.StaticMesh`) false)
  (return true))

(fn `UserConstructionScript`)