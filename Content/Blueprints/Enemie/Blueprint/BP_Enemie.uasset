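; Enemy character that follows a spline path, takes hit and burn damage, and bursts into physics scrap on death.
; AI movement repeatedly targets the next spline key, while a timeline-driven tool mode slides it along the spline, then respawns it through SpawnerTool.
; TakeDamage flashes a dynamic material and skips the death check when invincible.
; Burn uses a looping timer with an overlay and Niagara effect, and can kill regardless of invincibility.
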(event `self.ReceiveBeginPlay`
  ;[1 1 1] BeginPlay
  (`|ExecutionSequence`
    (:`then_0`
      ;;[1 1 1] SetMax Life
      (set `self.Life` (`self.MaxLife`))
      ;;[1 1 1] Mat when is invincible
      (if (`self.b_IsInvicible`)
        (`PrimitiveComponent.SetMaterial` (`self.EnemyMesh`) 0 "/Engine/MapTemplates/Materials/BasicAsset01.BasicAsset01")))
    (:`then_1`
      ;;[1 1 1] Create Mat When hit
      (bind _returnvalue (`PrimitiveComponent.CreateDynamicMaterialInstance` (`self.EnemyMesh`) 0 null "None"))
      (set `self.KlangMaterialRef` _returnvalue)
      (set `CharacterMovementComponent.MaxWalkSpeed` (`self.MaxSpeed`) (`self.CharacterMovement`)))
    (:`then_2`
      ;;[1 1 1] Move To Targert
      (bind _spline (`self.Spline`)
        (:`then`
          (set `self.SplineRef` (`/Game/Blueprints/Enemie/SplineEnnemis/BP_Spline_Enemy_Path.Spline` _spline)))
        (:`else`
          _))
      (`self.MoveAlongSpline`)
      (`self.Anim`))))

(event `Get Hit`
  ;[1 1 1] Event when get hit for Changing mat
  (if true
    (bind (_direction _newtrack_0) (`Timeline|Timeline` :!via `PlayFromStart` :!label _label)
      (:`Update`
        (`MaterialInstanceDynamic.SetScalarParameterValue` (`self.KlangMaterialRef`) "HitTime" _newtrack_0)))))

(event `StopTimeline`
  ;[1 1 1] Event when get hit for Changing mat
  (goto _label :!via `Stop`))

(event `Anim`
  (bind (_returnvalue_roll _returnvalue_pitch _returnvalue_yaw) (`KismetMathLibrary.BreakRotator` (`SceneComponent.K2_GetComponentRotation` (`self.Mesh`))))
  ;[1 0.1615 0.1615] Anim Temp
  (`/Engine/EditorBlueprintResources/StandardMacros.FlipFlop`
    (:`A`
      (bind (_direction _newtrack_0) (`Timeline|Timeline_0` :!label _label_2)
        (:`Update`
          (`SceneComponent.K2_SetWorldRotation` (`self.EnemyMesh`) (`KismetMathLibrary.MakeRotator` 0.0 0.0 (`KismetMathLibrary.Lerp` _returnvalue_yaw (- _returnvalue_yaw 10.0) _newtrack_0)) false false))
        (:`Finished`
          (`self.Anim`))))
    (:`B`
      (goto _label_2 :!via `Reverse`))))

(event `MoveAlongSpline`
  (bind _splineref (`self.SplineRef`))
  ;[1 1 1] Move along the spline
  (if (not (`self.Stop`))
    (`KismetSystemLibrary.Delay` 0.05)
    (`/Engine/EditorBlueprintResources/StandardMacros.IsValid` (`self.SplineRef`)
      (:`Is Valid`
        (bind _output_get (set `self.Destination` (`SplineComponent.GetLocationAtSplineInputKey` _splineref (+ (`SplineComponent.FindInputKeyClosestToWorldLocation` _splineref (`self.K2_GetActorLocation` self)) 1.0) "World")))
        (`AITask_MoveTo.AIMoveTo` (`AIBlueprintHelperLibrary.GetAIController` self) _output_get null -1.0 "Disable" "Enable" true false true
          (:`OnRequestFailed`
            (`KismetSystemLibrary.PrintString` "failed"))
          (:`OnMoveFinished`
            (`self.MoveAlongSpline`)
            (`KismetSystemLibrary.PrintString` "ggg")))))))

(event `StopMoving`
  (set `self.Stop` true)
  (`NavMovementComponent.StopActiveMovement` (`self.CharacterMovement`)))

(event `MoveAlongSplineInTool`
  (bind (_direction _movementintool) (`Timeline|MoveInTool` :!via `PlayFromStart`)
    (:`Update`
      (bind _returnvalue (`KismetMathLibrary.Lerp` 0.0 (`SplineComponent.GetSplineLength` (`self.SplineRef`)) _movementintool))
      (`self.K2_SetActorTransform` (`KismetMathLibrary.MakeTransform` (+ (`SplineComponent.GetLocationAtDistanceAlongSpline` (`self.SplineRef`) _returnvalue "World") (0.0 0.0 50.0)) (`SplineComponent.GetRotationAtDistanceAlongSpline` (`self.SplineRef`) _returnvalue "World"))))
    (:`Finished`
      (`/Game/Blueprints/Debug/BP_SpawnEnemy.Spawn` (`self.SpawnerTool`))
      (`self.K2_DestroyActor`))))

(fn `BurnStart`
  (bind _burntick (`self.BurnTick`))
  (bind _returnvalue (`NiagaraFunctionLibrary.SpawnSystemAttached` "/Game/VFX/VFX/Turrets/FlameThrower/V2/NS_IgniteEffect.NS_IgniteEffect" (`self.EnemyMesh`) "None" (0.0 0.0 0.0) (struct) "KeepRelativeOffset" true))
  (set `self.NS_Ignite` _returnvalue)
  (`MeshComponent.SetOverlayMaterial` (`self.EnemyMesh`) "/Game/VFX/VFX/Turrets/FlameThrower/V2/MI_IgniteOverlay.MI_IgniteOverlay")
  (bind _returnvalue_2 (`KismetSystemLibrary.K2_SetTimer` null "DamageBurn" _burntick true (- 0.0 _burntick)))
  (set `self.BurnTimer` _returnvalue_2)
  (set `self.BurnTimeLeft` 25.0))

(fn `CheckLife`
  (params (Life :type "Float (double-precision)"))
  (bind _enemymesh (`self.EnemyMesh`))
  (if (<= Life 0.0)
    (if (not (`self.Dead`))
      (`NiagaraFunctionLibrary.SpawnSystemAtLocation` null (`self.K2_GetActorLocation`))
      (`self.StopTimeline`)
      (`NavMovementComponent.StopActiveMovement` (`self.CharacterMovement`))
      (`PrimitiveComponent.SetCollisionEnabled` _enemymesh "NoCollision")
      (`PrimitiveComponent.SetCollisionEnabled` (`self.CapsuleComponent`) "NoCollision")
      (`PrimitiveComponent.SetCollisionResponseToChannel` _enemymesh "ECC_GameTraceChannel1" "ECR_Ignore")
      (`PrimitiveComponent.SetCollisionResponseToChannel` (`self.CapsuleComponent`) "ECC_GameTraceChannel1" "ECR_Ignore")
      (`self.Death`))))

(fn `DamageBurn`
  (bind _returnvalue (- (`self.BurnTimeLeft`) (`self.BurnTick`)))
  (bind _output_get (set `self.Life` (- (`self.Life`) (`self.BurnHitDamage`))))
  (`self.CheckLife` _output_get)
  (if (<= _returnvalue 0.0)
    (`KismetSystemLibrary.K2_PauseTimerHandle` (`self.BurnTimer`))
    (`MeshComponent.SetOverlayMaterial` (`self.EnemyMesh`) null)
    (else
      (set `self.BurnTimeLeft` _returnvalue))))

(fn `Death`
  (bind _returnvalue (`KismetMathLibrary.RandomFloatInRange` 0.0 500.0))
  (for _ (range 3)
    (bind _returnvalue_2 (`|SpawnActorFromClass` "/Game/Blueprints/Enemie/Blueprint/BP_Scrap.BP_Scrap_C" (`KismetMathLibrary.MakeTransform` (`self.K2_GetActorLocation`)) "Undefined" "MultiplyWithRoot" null null))
    (bind _staticmesh (`/Game/Blueprints/Enemie/Blueprint/BP_Scrap.StaticMesh` _returnvalue_2))
    (`PrimitiveComponent.SetSimulatePhysics` _staticmesh true)
    (`PrimitiveComponent.SetPhysicsLinearVelocity` _staticmesh (`KismetMathLibrary.MakeVector` _returnvalue (`KismetMathLibrary.RandomFloatInRange` 0.0 500.0) _returnvalue) false "None"))
  (bind _spawnertool (`self.SpawnerTool`)
    (:`then`
      (`/Game/Blueprints/Debug/BP_SpawnEnemy.Spawn` _spawnertool))
    (:`else`
      _))
  (`NiagaraFunctionLibrary.SpawnSystemAtLocation` "/Game/VFX/VFX/Ennemies/NS_KlangExplosion.NS_KlangExplosion" (`self.K2_GetActorLocation`))
  (`self.K2_DestroyActor`)
  (set `self.Dead` true))

(fn `GetDistanceToObjectif`
  (returns (Distance :type "Float (double-precision)"))
  (return (`SplineComponent.FindInputKeyClosestToWorldLocation` (`/Game/Blueprints/Enemie/SplineEnnemis/BP_Spline_Enemy_Path.Spline` (`self.Spline`)) (`self.K2_GetActorLocation` self))))

(fn `GiveItemToDesk`
  (params (ActorTarget :type "Actor Object Reference"))
  (returns (Return :type Boolean))
  (return false))

(fn `TakeDamage`
  (params (Damage :type "Float (double-precision)"))
  (bind _output_get (set `self.Life` (- (`self.Life`) Damage)))
  (`self.Get Hit`)
  (if (not (`self.b_IsInvicible`))
    (`self.CheckLife` _output_get)))

(fn `UserConstructionScript`)