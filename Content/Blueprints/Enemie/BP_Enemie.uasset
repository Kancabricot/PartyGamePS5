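; Enemy character that follows the level's BP_Spline_Enemy_Path, takes damage and drops scrap on death.
; It repeatedly AI-moves one spline key beyond its closest point, while a FlipFlop timeline sways the mesh's yaw.
; Damage lowers Life and drives a HitTime material flash; at zero it spawns a crystal explosion and physics-simulated BP_Scrap, then destroys itself.
; Member-attachment and item-grab logic is disconnected.
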(event `self.ReceiveBeginPlay`
  ;[1 1 1] BeginPlay
  (`|ExecutionSequence`
    (:`then_0`
      ;;[1 1 1] SetMax Life
      (set `self.Life` (`self.MaxLife`))
      (bind _returnvalue (`GameplayStatics.GetActorOfClass` "/Game/Blueprints/Enemie/SplineEnnemis/BP_Spline_Enemy_Path.BP_Spline_Enemy_Path_C"))
      (set `self.Spline` _returnvalue))
    (:`then_1`
      ;;[1 1 1] Create Mat When hit
      (bind _returnvalue_2 (`PrimitiveComponent.CreateDynamicMaterialInstance` (`self.StaticMesh`) 0 null "None"))
      (set `self.KlangMaterialRef` _returnvalue_2))
    (:`then_2`
      ;;[1 1 1] Move To Targert
      (`self.Anim` :!label _label))
    (:`then_3`
      (`self.MoveAlongSpline`))))

(event `MoveAlongSpline`
  (bind _spline (`/Game/Blueprints/Enemie/SplineEnnemis/BP_Spline_Enemy_Path.Spline` (`self.Spline`)))
  ;[1 1 1] Move along the spline
  (bind _output_get (set `self.Destination` (`SplineComponent.GetLocationAtSplineInputKey` _spline (+ (`SplineComponent.FindInputKeyClosestToWorldLocation` _spline (`self.K2_GetActorLocation` self)) 1.0) "World")))
  (`AITask_MoveTo.AIMoveTo` (`AIBlueprintHelperLibrary.GetAIController` self) _output_get null -1.0 "Disable"
    (:`OnMoveFinished`
      (`self.MoveAlongSpline`))))

(event `Get Hit`
  ;[1 1 1] Event when get hit for Changing mat
  (bind (_direction _newtrack_0) (`Timeline|Timeline` :!via `PlayFromStart` :!label _label_2)
    (:`Update`
      (`MaterialInstanceDynamic.SetScalarParameterValue` (`self.KlangMaterialRef`) "HitTime" _newtrack_0))))

(event `StopTimeline`
  ;[1 1 1] Event when get hit for Changing mat
  (goto _label_2 :!via `Stop`))

(event `Anim`
  (bind (_returnvalue_roll _returnvalue_pitch _returnvalue_yaw) (`KismetMathLibrary.BreakRotator` (`SceneComponent.K2_GetComponentRotation` (`self.Mesh`))))
  (`/Engine/EditorBlueprintResources/StandardMacros.FlipFlop`
    (:`A`
      (bind (_direction _newtrack_0) (`Timeline|Timeline_0` :!label _label_3)
        (:`Update`
          (`SceneComponent.K2_SetWorldRotation` (`self.StaticMesh`) (`KismetMathLibrary.MakeRotator` 0.0 0.0 (`KismetMathLibrary.Lerp` _returnvalue_yaw (- _returnvalue_yaw 10.0) _newtrack_0)) false false))
        (:`Finished`
          (goto _label))))
    (:`B`
      (goto _label_3 :!via `Reverse`))))

(event `/Game/Blueprints/Interface/BPI_TakeItem.DettachItem`
  (params (Impulse :type "Vector Structure")))

(fn `CheckLife`
  (params (Life :type "Float (double-precision)"))
  (bind _staticmesh (`self.StaticMesh`))
  (bind _box (`self.Box`))
  (if (<= Life 0.0)
    (if (not (`self.Dead`))
      (`NiagaraFunctionLibrary.SpawnSystemAtLocation` "/Game/VFX/Ennemies/NS_Ennemy_Explosion_Crystal.NS_Ennemy_Explosion_Crystal" (`self.K2_GetActorLocation`))
      (`self.StopTimeline`)
      (`NavMovementComponent.StopActiveMovement` (`self.CharacterMovement`))
      (`PrimitiveComponent.SetCollisionEnabled` _staticmesh "NoCollision")
      (`PrimitiveComponent.SetCollisionEnabled` (`self.CapsuleComponent`) "NoCollision")
      (`PrimitiveComponent.SetCollisionResponseToChannel` _staticmesh "ECC_GameTraceChannel1" "ECR_Ignore")
      (`PrimitiveComponent.SetCollisionResponseToChannel` (`self.CapsuleComponent`) "ECC_GameTraceChannel1" "ECR_Ignore")
      (bind _returnvalue (`|SpawnActorFromClass` "/Game/Blueprints/BP_Scrap.BP_Scrap_C" (`KismetMathLibrary.MakeTransform` (`KismetMathLibrary.RandomPointInBoundingBox` (`SceneComponent.K2_GetComponentLocation` _box) (`BoxComponent.BoxExtent` _box))) "Undefined" "MultiplyWithRoot" null null))
      (`PrimitiveComponent.SetSimulatePhysics` (`/Game/Blueprints/BP_Scrap.StaticMesh` _returnvalue) true)
      (`self.K2_DestroyActor`)
      (set `self.Dead` true))))

(fn `ChooseNewMembers`
  (returns (Mesh :type "StaticMesh Object Reference")))

(fn `ChosseLocation`
  (returns (Namesocket :type "Name (by ref)")))

(fn `CreateNewMembers`)

(fn `GiveItemToDesk`
  (params (ActorTarget :type "Actor Object Reference"))
  (returns (Return :type Boolean))
  (return false))

(fn `TakeDamage`
  (params (Damage :type "Float (double-precision)"))
  (bind _output_get (set `self.Life` (- (`self.Life`) Damage)))
  (`self.Get Hit`)
  (`self.CheckLife` _output_get))

(fn `TakeItem`
  (params (Player :type "/Game/Blueprints/Player/BP_Player Object Reference"))
  (returns (Return :type Boolean)))

(fn `UserConstructionScript`)