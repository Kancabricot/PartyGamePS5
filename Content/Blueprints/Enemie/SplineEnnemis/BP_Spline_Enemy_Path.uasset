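; Enemy path actor that lays a visible spline route with checkpoints and controls an alarm post-process effect.
; Construction rebuilds spline meshes from either the main or step-two spline, with offset and scale adjustments.
; It also places a checkpoint component at each spline point and stores straight-line distances between consecutive checkpoints.
; BeginPlay puts a dynamic alarm material on the level's PostProcessVolume, which Warning and RemovePostPro switch on and off.
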(event `self.ReceiveBeginPlay`
  (bind _returnvalue (`GameplayStatics.GetActorOfClass` "/Script/Engine.PostProcessVolume"))
  (set `self.PostPro` _returnvalue)
  (bind _returnvalue_2 (`KismetMaterialLibrary.CreateDynamicMaterialInstance` "/Game/Assets/Mats/M_PPAlarm_Inst.M_PPAlarm_Inst"))
  (set `self.MatPostPro` _returnvalue_2)
  (bind _output_get (set `self.Post Process Settings` (make `PostProcessSettings` :`WeightedBlendables` (make `WeightedBlendables` (`|MakeArray` (make `WeightedBlendable` 1.0 _returnvalue_2))))))
  (set `PostProcessVolume.Settings` _output_get (`self.PostPro`))
  (`MaterialInstanceDynamic.SetScalarParameterValue` (`self.MatPostPro`) "Activation" 0.0))

(event `Warning`
  (`MaterialInstanceDynamic.SetScalarParameterValue` (`self.MatPostPro`) "Activation" 1.0))

(event `RemovePostPro`
  (`MaterialInstanceDynamic.SetScalarParameterValue` (`self.MatPostPro`) "Activation" 0.0))

(fn `AddBoxCollision`
  (params (RelativeTransform :type "Transform Structure"))
  (bind _returnvalue (`AddComponent|NODE_AddSceneComponent-0`))
  (`KismetArrayLibrary.Array_AddUnique` (`self.CheckPointArray`) _returnvalue)
  (`SceneComponent.K2_SetWorldLocationAndRotation` _returnvalue RelativeTransform_Location RelativeTransform_Rotation false false))

(fn `ChangeSpline`
  (bind _offsetzpath (`self.OffSetZPath`))
  (bind _returnvalue (select `bool` (`self.b_IsStep2`) :`false` (`self.Spline`) :`true` (`self.SplineStep2`)))
  (bind _returnvalue_2 (select `bool` (`self.b_IsStep2`) :`false` (`self.Spline`) :`true` (`self.SplineStep2`)))
  (bind _returnvalue_3 (`SceneComponent.K2_GetComponentLocation` (select `bool` (`self.b_IsStep2`) :`false` (`self.Spline`) :`true` (`self.SplineStep2`) :!type "SceneComponent Object Reference")))
  (`ActorComponent.K2_DestroyComponent` (`self.PathMesh`))
  (`KismetArrayLibrary.Array_Clear` (`self.PathMesh`))
  (bind _outhit (`KismetSystemLibrary.LineTraceSingle` _returnvalue_3 (+ _returnvalue_3 (* (`KismetMathLibrary.NegateVector` (`KismetMathLibrary.Vector_Up`)) 100.0)) "TraceTypeQuery1"))
  (set `self.Location` (`.Location` (`GameplayStatics.BreakHitResult` _outhit)))
  (`KismetArrayLibrary.Array_Clear` (`self.CheckPointArray`))
  (`KismetArrayLibrary.Array_Clear` (`self.DistanceArray`))
  (for _index (range (`SplineComponent.GetNumberOfSplinePoints` (select `bool` (`self.b_IsStep2`) :`false` (`self.Spline`) :`true` (`self.SplineStep2`))))
    (bind _returnvalue_4 (`AddComponent|NODE_AddSplineMeshComponent-4` :`bManualAttachment` true))
    (`KismetArrayLibrary.Array_Add` (`self.PathMesh`) _returnvalue_4)
    (bind (_location _tangent) (`SplineComponent.GetLocationAndTangentAtSplinePoint` _returnvalue_2 _index "World"))
    (`self.AddBoxCollision` (`KismetMathLibrary.MakeTransform` (`KismetMathLibrary.MakeVector` (.x _location) (.y _location) (.z _location))))
    (bind _returnvalue_5 (+ _index 1))
    (bind (_location_2 _tangent_2) (`SplineComponent.GetLocationAndTangentAtSplinePoint` _returnvalue_2 _returnvalue_5 "World"))
    (`SplineMeshComponent.SetStartAndEnd` _returnvalue_4 (`KismetMathLibrary.MakeVector` (+ (.x _location) (`self.OffSetXPath`)) (+ (.y _location) (`self.OffSetYPath`)) (+ (.z _location) _offsetzpath)) _tangent (`KismetMathLibrary.MakeVector` (+ (.x _location_2) (`self.OffSetXPath`)) (+ (.y _location_2) (`self.OffSetYPath`)) (+ (.z _location_2) _offsetzpath)) _tangent_2 true)
    (bind (_returnvalue_x _returnvalue_y) (`KismetMathLibrary.BreakVector` (`SplineComponent.GetScaleAtSplinePoint` _returnvalue _index)))
    (`SplineMeshComponent.SetStartScale` _returnvalue_4 (`KismetMathLibrary.MakeVector2D` (+ _returnvalue_x (`self.Scale X`)) (+ _returnvalue_y (`self.Scale Y`))) true)
    (bind (_returnvalue_x_2 _returnvalue_y_2) (`KismetMathLibrary.BreakVector` (`SplineComponent.GetScaleAtSplinePoint` _returnvalue _returnvalue_5)))
    (`SplineMeshComponent.SetEndScale` _returnvalue_4 (`KismetMathLibrary.MakeVector2D` (+ _returnvalue_x_2 (`self.Scale X`)) (+ _returnvalue_y_2 (`self.Scale Y`))) true))
  (`self.GetDistanceBox`))

(fn `GetDistanceBox`
  (for (_array_element _array_index) (`self.CheckPointArray`)
    (bind _returnvalue (- _array_index 1))
    (if (not (< _returnvalue 0))
      (`KismetArrayLibrary.Array_Add` (`self.DistanceArray`) (`KismetMathLibrary.VSize` (- (`SceneComponent.K2_GetComponentLocation` (`|GetArrayItem` (`self.CheckPointArray`) _returnvalue)) (`SceneComponent.K2_GetComponentLocation` _array_element)))))))

(fn `GiveSpline`
  (returns (ReturnValue :type "SplineComponent Object Reference"))
  (return (select `bool` (`self.b_IsStep2`) :`false` (`self.Spline`) :`true` (`self.SplineStep2`))))

(fn `UserConstructionScript`
  (`self.ChangeSpline`))