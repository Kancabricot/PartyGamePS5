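; Shield-bearing enemy Blueprint whose shield absorbs bullet damage, extending its parent's BeginPlay and construction.
; BeginPlay fills ShieldLife from MaxShieldLife.
; Box overlaps with BP_Bullet subtract its damage, doubled when the bullet equals BP_Bullet_Expolif, and destroy the shield mesh and box at zero.
; An untargeted DestroyActor, acting on the enemy itself, follows every bullet hit regardless of remaining shield.
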(event `self.ReceiveBeginPlay`
  (`parent.ReceiveBeginPlay`)
  (set `self.ShieldLife` (`self.MaxShieldLife`)))

(event `self.Box.OnComponentBeginOverlap`
  (params (OverlappedComponent :type "PrimitiveComponent Object Reference") (OtherActor :type "Actor Object Reference") (OtherComp :type "PrimitiveComponent Object Reference") (OtherBodyIndex :type Integer) (bFromSweep :type Boolean) (SweepResult :type "HitResult Structure (by ref)"))
  (bind _asbp_bullet (cast `/Game/Blueprints/Turret/Bullet/BP_Bullet` OtherActor))
  (bind _damage (`/Game/Blueprints/Turret/Bullet/BP_Bullet.Damage` _asbp_bullet))
  (set `self.ShieldLife` (- (`self.ShieldLife`) (`KismetMathLibrary.SelectFloat` (* _damage 2.0) _damage (== _asbp_bullet "/Game/Blueprints/Turret/Bullet/BP_Bullet_Expolif.BP_Bullet_Expolif"))))
  (if (<= (`self.ShieldLife`) 0.0)
    (`ActorComponent.K2_DestroyComponent` (`self.StaticMesh1`))
    (`ActorComponent.K2_DestroyComponent` (`self.Box`)))
  (`self.K2_DestroyActor`))

(fn `UserConstructionScript`
  (`parent.UserConstructionScript`))