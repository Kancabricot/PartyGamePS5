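; BP_RibambelledeKram is an enemy that splits into several BP_Kram actors when it dies.
; CheckLife tests the life value and, at zero or below, spawns the BP_Kram actors in a loop at its own location.
; Each spawn receives its TargetMovement, then the enemy stops its timeline and destroys itself.
; BeginPlay and the construction script only call the parent class.
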(event `self.ReceiveBeginPlay`
  (`parent.ReceiveBeginPlay`))

(fn `CheckLife`
  (params (Life :type "Float (double-precision)"))
  (if (<= Life 0.0)
    (for _ (range 3)
      (`|SpawnActorFromClass` "/Game/Blueprints/Enemie/BP_Kram.BP_Kram_C" (`KismetMathLibrary.MakeTransform` (`self.K2_GetActorLocation`)) "Undefined" "MultiplyWithRoot" null (`self.TargetMovement`) null))
    (`self.StopTimeline`)
    (`self.K2_DestroyActor`)))

(fn `UserConstructionScript`
  (`parent.UserConstructionScript`))