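; BP_GrandKrash is an enemy Blueprint that slowly regenerates its own health.
; On BeginPlay it runs the parent logic, then starts a looping one-second timer that calls Heal by function name.
; Heal adds a fixed amount to Life only while it is below MaxLife, without clamping, so the last tick can overshoot the maximum.
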(event `self.ReceiveBeginPlay`
  (`parent.ReceiveBeginPlay`)
  (`KismetSystemLibrary.K2_SetTimer` null "Heal" 1.0 true -1.0))

(fn `Heal`
  (bind _life (`self.Life`))
  (if (not (>= _life (`self.MaxLife`)))
    (set `self.Life` (+ _life 2.0))))

(fn `UserConstructionScript`
  (`parent.UserConstructionScript`))