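; BP_Clock is a damageable clock actor with hit points that enemies wear down on contact, triggering the lose screen.
; Life starts at MaxHp on BeginPlay, and each BP_Ennemy overlapping the Trigger component is destroyed and costs one point through SetLife.
; SetLife passes the new value to CheckLife, which at zero or below creates the WG_Loose widget, adds it to the viewport and calls its EndGame.
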(event `self.ReceiveBeginPlay`
  (set `self.ActuLife` (`self.MaxHp`)))

(event `self.Trigger.OnComponentBeginOverlap`
  (params (OverlappedComponent :type "PrimitiveComponent Object Reference") (OtherActor :type "Actor Object Reference") (OtherComp :type "PrimitiveComponent Object Reference") (OtherBodyIndex :type Integer) (bFromSweep :type Boolean) (SweepResult :type "HitResult Structure (by ref)"))
  (bind _asbp_ennemy (cast `/Game/Blueprints/Ennemie/BP_Ennemy` OtherActor))
  (`self.K2_DestroyActor` _asbp_ennemy)
  (`self.SetLife` 1.0))

(fn `CheckLife`
  (params (Life :type "Float (double-precision)"))
  (returns (TotalLife :type "Float (double-precision)"))
  (locals (WidgetRef :type "/Game/Blueprints/Widgets/WG_Loose Object Reference"))
  (if (<= Life 0.0)
    (bind _returnvalue (`|CreateWidget` "/Game/Blueprints/Widgets/WG_Loose.WG_Loose_C"))
    (bind _output_get (set `local.WidgetRef` _returnvalue))
    (`UserWidget.AddToViewport` _returnvalue 0)
    (`UserWidget.AddToViewport` _output_get 0)
    (`/Game/Blueprints/Widgets/WG_Loose.EndGame` (`local.WidgetRef`))
    (else
      (return Life))))

(fn `SetLife`
  (params (Damage :type "Float (double-precision)"))
  (bind _output_get (set `self.ActuLife` (- (`self.ActuLife`) Damage)))
  (`self.CheckLife` _output_get))

(fn `UserConstructionScript`)