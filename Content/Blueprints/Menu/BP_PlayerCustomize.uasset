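; Menu preview actor for player customization that lets a player cycle through accessory meshes.
; SwitchAccessory steps through the PDAPlayerAccessory list with wraparound and applies the selected mesh to the Accessory component.
; Each switch plays a grab animation and star Niagara effect, replacing the looping idle started on BeginPlay.
; The selection is also written to the game instance's HatMeshArray at the given player index.
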(event `self.ReceiveBeginPlay`
  (`SkeletalMeshComponent.PlayAnimation` (`self.Player`) "/Game/Characters/Clic/AS_Idle_00.AS_Idle_00" true)
  (bind _asbp_game_instance (cast `/Game/Blueprints/GameInstance/Bp_GameInstance` (`GameplayStatics.GetGameInstance`)))
  (set `self.GameInstanceRef` _asbp_game_instance))

(event `SwitchAccessory`
  (params (Input :type Integer) (PlayerIndex :type Integer))
  (bind _returnvalue (+ (`self.IndexAccessoryArray`) Input))
  (bind _returnvalue_2 (`KismetArrayLibrary.Array_Length` (`/Game/Blueprints/Player/DataAsset/PDA_PlayerAccessory.PlayerAccessory` (`self.PDA_PlayerAccessory`))))
  (bind _output (`|GetArrayItem` (`/Game/Blueprints/Player/DataAsset/PDA_PlayerAccessory.PlayerAccessory` (`self.PDA_PlayerAccessory`)) (`self.IndexAccessoryArray`)))
  (if (>= _returnvalue _returnvalue_2)
    (set `self.IndexAccessoryArray` 0)
    (elif (< _returnvalue 0)
      (set `self.IndexAccessoryArray` (- _returnvalue_2 1))
      (else
        (set `self.IndexAccessoryArray` _returnvalue))))
  (`|ExecutionSequence`
    (:`then_0`
      (set `self.ActualAccessory` _output)
      (`StaticMeshComponent.SetStaticMesh` (`self.Accessory`) _output)
      (`SkeletalMeshComponent.PlayAnimation` (`self.Player`) "/Game/Characters/Clic/AS_Grab_00.AS_Grab_00" false)
      (`NiagaraFunctionLibrary.SpawnSystemAtLocation` "/Game/VFX/VFX/Distributeur/StarSuccess/NS_StarSuccess.NS_StarSuccess" (`SceneComponent.K2_GetComponentLocation` (`self.Accessory`))))
    (:`then_1`
      (`KismetArrayLibrary.Array_Set` (`/Game/Blueprints/GameInstance/Bp_GameInstance.HatMeshArray` (`self.GameInstanceRef`)) PlayerIndex _output))))

(fn `UserConstructionScript`)