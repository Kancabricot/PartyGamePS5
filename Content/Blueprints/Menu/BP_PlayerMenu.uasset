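; BP_PlayerMenu is the player-side input handler for menus, set up for Joy-Con controllers.
; On BeginPlay it resets existing Joy-Con links, searches, reconnects and attaches them, adding the menu Enhanced Input mapping context for player 0.
; Up, down, accept and decline actions are forwarded as messages to the menu reference supplied through GetMenu.
; Up and down use thresholded DoOnce latches, so each push fires only once.
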(event `self.ReceiveBeginPlay`
  (bind _returnvalue (pcsubsystem `EnhancedInputLocalPlayerSubsystem` (`GameplayStatics.GetPlayerController` 0)))
  (bind _joycons (`JoyConDriverFunctionLibrary.GetAttachedJoyCons`))
  (for _array_element _joycons
    (`JoyConDriverFunctionLibrary.DetachJoyCon` (`.ControllerId` (break `JoyConInformation` _array_element))))
  (bind _joycons_2 (`JoyConDriverFunctionLibrary.GetConnectedJoyCons`))
  (for _array_element_2 _joycons_2
    (`JoyConDriverFunctionLibrary.DisconnectJoyCon` (`.ControllerId` (break `JoyConInformation` _array_element_2))))
  (`JoyConDriverFunctionLibrary.ResumeJoyConConnection`)
  (bind _joycons_3 (`JoyConDriverFunctionLibrary.SearchForJoyCons`))
  (for _array_element_3 _joycons_3
    (`JoyConDriverFunctionLibrary.ConnectJoyCon` _array_element_3 true true))
  (bind _joycons_4 (`JoyConDriverFunctionLibrary.GetConnectedJoyCons`))
  (for _array_element_4 _joycons_4
    (`JoyConDriverFunctionLibrary.AttachJoyCon` (`.ControllerId` (break `JoyConInformation` _array_element_4)))
    (`/Engine/EditorBlueprintResources/StandardMacros.IsValid` _returnvalue
      (:`Is Valid`
        (`EnhancedInputSubsystemInterface.AddMappingContext` _returnvalue "/Game/Input/IMC_InputMenu.IMC_InputMenu" 0 (struct))))))

(event `EnhancedInput|/Game/Input/Actions/InputMenu/IA_MenuUp`
  (params (ActionValue :type "Float (double-precision)") (ElapsedSeconds :type "Float (double-precision)") (TriggeredSeconds :type "Float (double-precision)") (InputAction :type "InputAction Object Reference" :default "/Game/Input/Actions/InputMenu/IA_MenuUp.IA_MenuUp"))
  (:`Triggered`
    (if (> ActionValue 0.5)
      (`/Engine/EditorBlueprintResources/StandardMacros.DoOnce` false :!label _label
        (:`Completed`
          (message `/Game/Blueprints/Interface/BPI_InteractionInMenu.ButtonUp` (`self.Menu Ref`))))
      (else
        (goto _label :!via `Reset`)))))

(event `EnhancedInput|/Game/Input/Actions/InputMenu/IA_MenuDown`
  (params (ActionValue :type "Float (double-precision)") (ElapsedSeconds :type "Float (double-precision)") (TriggeredSeconds :type "Float (double-precision)") (InputAction :type "InputAction Object Reference" :default "/Game/Input/Actions/InputMenu/IA_MenuDown.IA_MenuDown"))
  (:`Triggered`
    (if (< ActionValue -0.5)
      (`/Engine/EditorBlueprintResources/StandardMacros.DoOnce` false :!label _label_2
        (:`Completed`
          (message `/Game/Blueprints/Interface/BPI_InteractionInMenu.ButtonDown` (`self.Menu Ref`))))
      (else
        (goto _label_2 :!via `Reset`)))))

(event `EnhancedInput|/Game/Input/Actions/InputMenu/IA_MenuRight`
  (params (ActionValue :type "Float (double-precision)") (ElapsedSeconds :type "Float (double-precision)") (TriggeredSeconds :type "Float (double-precision)") (InputAction :type "InputAction Object Reference" :default "/Game/Input/Actions/InputMenu/IA_MenuRight.IA_MenuRight")))

(event `EnhancedInput|/Game/Input/Actions/InputMenu/IA_MenuLeft`
  (params (ActionValue :type "Float (double-precision)") (ElapsedSeconds :type "Float (double-precision)") (TriggeredSeconds :type "Float (double-precision)") (InputAction :type "InputAction Object Reference" :default "/Game/Input/Actions/InputMenu/IA_MenuLeft.IA_MenuLeft")))

(event `EnhancedInput|/Game/Input/Actions/InputMenu/IA_MenuAccept`
  (params (ActionValue :type Boolean) (ElapsedSeconds :type "Float (double-precision)") (TriggeredSeconds :type "Float (double-precision)") (InputAction :type "InputAction Object Reference" :default "/Game/Input/Actions/InputMenu/IA_MenuAccept.IA_MenuAccept"))
  (:`Started`
    (message `/Game/Blueprints/Interface/BPI_InteractionInMenu.ButtonA` (`self.Menu Ref`))))

(event `EnhancedInput|/Game/Input/Actions/InputMenu/IA_MenuDecline`
  (params (ActionValue :type Boolean) (ElapsedSeconds :type "Float (double-precision)") (TriggeredSeconds :type "Float (double-precision)") (InputAction :type "InputAction Object Reference" :default "/Game/Input/Actions/InputMenu/IA_MenuDecline.IA_MenuDecline"))
  (:`Started`
    (message `/Game/Blueprints/Interface/BPI_InteractionInMenu.ButtonB` (`self.Menu Ref`))))

(fn `GetMenu`
  (params (MenuRef :type "Widget Object Reference"))
  (set `self.Menu Ref` MenuRef))

(fn `UserConstructionScript`)