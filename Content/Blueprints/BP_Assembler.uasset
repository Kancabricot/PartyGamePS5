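; Assembler station that combines two ingredients into a turret addon.
; Overlapping ingredients fill two enum slots and are destroyed, while any arriving during cooking are thrown back out.
; CheckAssembly matches three order-independent pairs to a color value; an unmatched pair stays, with later ingredients overwriting the second slot.
; A match runs a timeline driving the widget bar, then spawns and launches the colored BP_TurretAddon and empties both slots.
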(event `self.ReceiveBeginPlay`
  (bind _aswg_temperature (cast `/Game/Blueprints/Widgets/WG_Temperature` (`WidgetComponent.GetWidget` (`self.Widget`))))
  (set `self.WGBar` _aswg_temperature))

(event `self.Box.OnComponentBeginOverlap`
  (params (OverlappedComponent :type "PrimitiveComponent Object Reference") (OtherActor :type "Actor Object Reference") (OtherComp :type "PrimitiveComponent Object Reference") (OtherBodyIndex :type Integer) (bFromSweep :type Boolean) (SweepResult :type "HitResult Structure (by ref)"))
  (bind _asbp_ingredients (cast `/Game/Blueprints/BP_Ingredients` OtherActor))
  (if (not (`self.b_IsCooking`))
    (if (`|EnumEquality` (`self.Enum_Ingredients`) "NewEnumerator14")
      (bind _enum_ingredients (`/Game/Blueprints/BP_Ingredients.Enum_Ingredients` _asbp_ingredients))
      (set `self.Enum_Ingredients` _enum_ingredients)
      (else
        (set `self.Enum_IngredientsNumber2` _enum_ingredients)))
    (`self.K2_DestroyActor` _asbp_ingredients)
    (`self.CheckAssembly`)
    (else
      (message `/Game/Blueprints/Interface/BPI_TakeItem.DettachItem` _asbp_ingredients (* (`SceneComponent.GetForwardVector` (`self.ThrowingLocation`)) 500)))))

(event `CreateStage`
  (set `self.b_IsCooking` true)
  (bind (_direction _timervalue) (`Timeline|Delay` :!via `PlayFromStart`)
    (:`Update`
      (`/Game/Blueprints/Widgets/WG_Temperature.SetTimer` (`self.WGBar`) _timervalue))
    (:`Finished`
      (bind _returnvalue (`|SpawnActorFromClass` "/Game/Blueprints/Turret/BP_TurretAddon.BP_TurretAddon_C" (`KismetMathLibrary.MakeTransform` (`SceneComponent.K2_GetComponentLocation` (`self.ThrowingLocation`))) "Undefined" "MultiplyWithRoot" null (make `/Game/Blueprints/Turret/Struc_Turret` 0.33 4.0 250.0 false (`KismetMathLibrary.FTrunc` (`self.Color`))) null))
      (message `/Game/Blueprints/Interface/BPI_TakeItem.DettachItem` _returnvalue (* (`SceneComponent.GetForwardVector` (`self.ThrowingLocation`)) 500))
      (`/Game/Blueprints/Widgets/WG_Temperature.SetTimer` (`self.WGBar`) 0.0)
      (set `self.Enum_Ingredients` "NewEnumerator14")
      (set `self.Enum_IngredientsNumber2` "NewEnumerator14")
      (set `self.b_IsCooking` false))))

(fn `CheckAssembly`
  (if (or (and (`|EnumEquality` (`self.Enum_Ingredients`) "NewEnumerator4") (`|EnumEquality` "NewEnumerator7" (`self.Enum_IngredientsNumber2`))) (and (`|EnumEquality` (`self.Enum_Ingredients`) "NewEnumerator7") (`|EnumEquality` "NewEnumerator4" (`self.Enum_IngredientsNumber2`))))
    (set `self.Color` 2.0)
    (`self.CreateStage`)
    (elif (or (and (`|EnumEquality` (`self.Enum_Ingredients`) "NewEnumerator4") (`|EnumEquality` "NewEnumerator11" (`self.Enum_IngredientsNumber2`))) (and (`|EnumEquality` (`self.Enum_Ingredients`) "NewEnumerator11") (`|EnumEquality` "NewEnumerator4" (`self.Enum_IngredientsNumber2`))))
      (set `self.Color` 1.0)
      (`self.CreateStage`)
      (elif (or (and (`|EnumEquality` (`self.Enum_Ingredients`) "NewEnumerator11") (`|EnumEquality` "NewEnumerator7" (`self.Enum_IngredientsNumber2`))) (and (`|EnumEquality` (`self.Enum_Ingredients`) "NewEnumerator7") (`|EnumEquality` "NewEnumerator11" (`self.Enum_IngredientsNumber2`))))
        (set `self.Color` 0.0)
        (`self.CreateStage`)))))

(fn `CreateAddon`)

(fn `UserConstructionScript`)