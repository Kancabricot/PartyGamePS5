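; BP_Baterie is a battery pickup actor that the player can grab and release as a physics object.
; TakeItem hands the actor to the player, disables physics and collision on its Cylinder mesh and flags it as grabbed.
; DettachItem restores collision and physics, sets the mesh velocity from the supplied impulse and clears the flag.
; GiveItemToDesk always returns false, so the battery never reports a successful hand-off to a desk.
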(event `/Game/Blueprints/Interface/BPI_TakeItem.DettachItem`
  (params (Impulse :type "Vector Structure"))
  (bind _cylinder (`self.Cylinder`))
  (`PrimitiveComponent.SetCollisionEnabled` _cylinder "QueryAndPhysics")
  (`PrimitiveComponent.SetSimulatePhysics` _cylinder true)
  (`PrimitiveComponent.SetPhysicsLinearVelocity` (`self.Cylinder`) Impulse false "None")
  (set `self.b_IsGrab` false))

(fn `GiveItemToDesk`
  (params (ActorTarget :type "Actor Object Reference"))
  (returns (Return :type Boolean))
  (return false))

(fn `TakeItem`
  (params (Player :type "/Game/Blueprints/Player/BP_Player Object Reference"))
  (returns (Return :type Boolean))
  (`/Game/Blueprints/Player/BP_Player.TakeItem` Player 0.0 self)
  (`PrimitiveComponent.SetCollisionEnabled` (`self.Cylinder`) "NoCollision")
  (set `self.b_IsGrab` true)
  (`PrimitiveComponent.SetSimulatePhysics` (`self.Cylinder`) false)
  (return true))

(fn `UserConstructionScript`)