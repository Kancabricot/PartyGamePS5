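; BP_Storgare is an ingredient dispenser that hands the player a fresh item of its configured Ingredient type.
; The construction script picks the displayed Item mesh from the Ingredient enum, and a timeline animates its height on BeginPlay.
; TakeItem spawns a BP_Ingredients copying that mesh, material and type, passes it to the player and calls SpawnCatch.
; GiveItemToDesk always returns false, so it accepts no items back.
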(event `self.ReceiveBeginPlay`
  (bind (_direction _movement) (`Timeline|Movement`)
    (:`Update`
      (`SceneComponent.K2_SetRelativeLocation` (`self.Item`) (`KismetMathLibrary.MakeVector` 0.0 0.0 (`KismetMathLibrary.Lerp` 100.0 200.0 _movement)) false false))))

(fn `GiveItemToDesk`
  (params (ActorTarget :type "Actor Object Reference"))
  (returns (Return :type Boolean))
  (return false))

(fn `TakeItem`
  (params (Player :type "/Game/Blueprints/Player/BP_Player Object Reference"))
  (returns (Return :type Boolean))
  (bind _item (`self.Item`))
  (bind _returnvalue (`|SpawnActorFromClass` "/Game/Blueprints/BP_Ingredients.BP_Ingredients_C" (`KismetMathLibrary.MakeTransform` (0.0 0.0 0.0)) "Undefined" "MultiplyWithRoot" null (`StaticMeshComponent.StaticMesh` _item) (`PrimitiveComponent.GetMaterial` _item 0) (`self.Ingredient`) null))
  (`/Game/Blueprints/Player/BP_Player.TakeItem` Player 0.0 _returnvalue)
  (`/Game/Blueprints/BP_Ingredients.SpawnCatch` _returnvalue)
  (return true))

(fn `UserConstructionScript`
  (bind _item (`self.Item`))
  (switch `/Game/Blueprints/Enums/Enum_Ingredients` (`self.Ingredient`)
    (:`NewEnumerator0`
      (`StaticMeshComponent.SetStaticMesh` (`self.Item`) "/Engine/EditorMeshes/ArcadeEditorSphere.ArcadeEditorSphere"))
    (:`NewEnumerator4`
      (`StaticMeshComponent.SetStaticMesh` _item "/Game/Assets/Ingot.Ingot"))
    (:`NewEnumerator7`
      (`StaticMeshComponent.SetStaticMesh` _item "/Game/Assets/Gears/Thibault/Gear5.Gear5"))
    (:`NewEnumerator11`
      (`StaticMeshComponent.SetStaticMesh` _item "/Game/Assets/Materials/Zinc/Import/ZincTige.ZincTige"))
    (:`NewEnumerator14`
      (`StaticMeshComponent.SetStaticMesh` (`self.Item`) "/Engine/EditorMeshes/ArcadeEditorSphere.ArcadeEditorSphere"))))