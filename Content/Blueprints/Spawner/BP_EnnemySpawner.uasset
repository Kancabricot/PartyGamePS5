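; BP_EnnemySpawner is an enemy spawner that creates BP_Enemie actors inside a box volume when its Spawn function is called.
; Spawn picks a random point within the Spawner box, adjusting for collisions but always spawning.
; Each enemy receives a random spline from SplineRef, the scrap-drop flag and the SpawnerMaster reference stored through GetMasterRef.
; BeginPlay and the construction script are empty.
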(event `self.ReceiveBeginPlay`)

(fn `GetMasterRef`
  (params (`Spawner Master` :type "/Game/Blueprints/Spawner/BP_SpawnerMaster Object Reference"))
  (set `self.Spawner Master` `Spawner Master`))

(fn `Spawn`
  (params (Enemy :type "Object Class Reference") (b_CanDropScrap :type Boolean))
  (bind _spawner (`self.Spawner`))
  (bind _asbp_enemie (castclass `/Game/Blueprints/Enemie/Blueprint/BP_Enemie` Enemy))
  (`|SpawnActorFromClass` _asbp_enemie (`KismetMathLibrary.MakeTransform` (`KismetMathLibrary.RandomPointInBoundingBox` (`SceneComponent.K2_GetComponentLocation` _spawner) (`BoxComponent.GetScaledBoxExtent` _spawner))) "AdjustIfPossibleButAlwaysSpawn" "MultiplyWithRoot" null 200.0 null (`KismetArrayLibrary.Array_Random` (`self.SplineRef`)) (`self.Spawner Master`) false null b_CanDropScrap null))

(fn `UserConstructionScript`)