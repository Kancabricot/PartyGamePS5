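; Wave spawner master that runs the level's enemy waves, triggers phase two at a set wave and shows the win screen after the last.
; Looping one-second timers count down data-asset delays, driving the danger bar and flickering lights before each wave.
; Spawn calls itself with a delay, triggering each spawner in the wave's list, then SetUpWave loads the next.
; Sliding-door events are empty and the enemies-remaining check is disconnected.
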(event `self.ReceiveBeginPlay`
  (`self.SetDataValue`)
  (bind _aswg_wave_number (cast `/Game/Blueprints/Widgets/WG_WaveNumber` (`WidgetComponent.GetWidget` (`self.Widget_NbWaves`))))
  (set `self.As WG Wave Number` _aswg_wave_number)
  (bind _returnvalue (`KismetSystemLibrary.K2_SetTimer` null "DelayBeforeNextWave" 1.0 true -1.0))
  (bind _output_get (set `self.TBFDelayBeforeNextWave` _returnvalue))
  (`KismetSystemLibrary.K2_PauseTimerHandle` _output_get)
  (bind _aswg_danger (cast `/Game/Blueprints/Widgets/WG_Danger` (`WidgetComponent.GetWidget` (`self.WGDanger`)))
    (:`then`
      (set `self.WGDangerRef` _aswg_danger))
    (:`CastFailed`
      _))
  (`SceneComponent.SetVisibility` (`self.WGDanger`) false false)
  (`self.Set Up Wave`))

(event `CheckEnemiOnLevel`
  (bind _outactors (`GameplayStatics.GetAllActorsOfClass` "/Game/Blueprints/Enemie/Blueprint/BP_Enemie.BP_Enemie_C")))

(event `StartFirstWave`
  (bind _returnvalue (`KismetSystemLibrary.K2_SetTimer` null "DelayFirstWave" 1.0 true -1.0))
  (set `self.TBFDelayFirstWave` _returnvalue))

(event `Spawn`
  (`KismetSystemLibrary.K2_UnPauseTimerHandle` (`self.TimerCheckEnemi`))
  (if (> (`self.NBEnnemiActualWave`) 0)
    (`/Game/Blueprints/Spawner/BP_EnnemySpawner.Spawn` (`|GetArrayItem` (`self.Number Of EnemisArraySpawnerRef`) (- (`self.NBEnnemiActualWave`) 1)) null)
    (set `self.NBEnnemiActualWave` (- (`self.NBEnnemiActualWave`) 1))
    (`|ExecutionSequence`
      (:`then_0`
        (`KismetSystemLibrary.Delay` (`self.DelayBetweenSpawn`))
        (`self.Spawn`))
      (:`then_1`
        (`/Engine/EditorBlueprintResources/StandardMacros.DoOnce` false :!label _label
          (:`Completed`
            (`self.Open Sliding Door`)))))
    (else
      (`self.Set Up Wave`)
      (`KismetSystemLibrary.K2_UnPauseTimerHandle` (`self.TBFDelayBeforeNextWave`)))))

(event `Reset Door`
  (goto _label :!via `Reset`))

(event `Flickering Light`
  (bind _high_light_intensity (`self.High Light Intensity`))
  (bind _lightcomponent (`Light.LightComponent` (`self.EnemyLight Ref`)))
  (`TimelineComponent.SetPlayRate` (`self.TL_Flickering_Light`) 0.5)
  (bind (_direction _intensity) (`Timeline|TL_Flickering_Light` :!via `PlayFromStart`)
    (:`Update`
      (`LightComponent.SetIntensity` _lightcomponent (`KismetMathLibrary.Lerp` (`self.Low Light Intensity`) _high_light_intensity _intensity)))
    (:`Finished`
      (`LightComponent.SetIntensity` _lightcomponent _high_light_intensity))))

(event `Open Sliding Door`)

(event `Close Sliding Door`)

(event `New Wave Widget Update`
  (bind (_direction _alpha) (`Timeline|TL_WaveWidget` :!via `PlayFromStart`)
    (:`Update`
      (`SceneComponent.K2_SetRelativeLocation` (`self.Widget_NbWaves`) (`KismetMathLibrary.VLerp` (115.0 1693.0 341.0) (-68.0 2783.0 341.0) _alpha) false false))))

(fn `DelayBeforeNextWave`
  (bind _wgdanger (`self.WGDanger`))
  (if (>= (`self.DelayBeforeNextWaveTemp`) (`self.DelayBetweenWave`))
    (`KismetSystemLibrary.K2_PauseTimerHandle` (`self.TBFDelayBeforeNextWave`))
    (`self.Spawn`)
    (`SceneComponent.SetVisibility` (`self.WGDanger`) false false)
    (set `self.DelayBeforeNextWaveTemp` 0.0)
    (else
      (bind _output_get (set `self.DelayBeforeNextWaveTemp` (+ (`self.DelayBeforeNextWaveTemp`) 1.0)))
      (`/Game/Blueprints/Widgets/WG_Danger.Set warning BAr` (`self.WGDangerRef`) _output_get (`self.DelayBetweenWave`))
      (if (== (`self.DelayBeforeNextWaveTemp`) 3.0)
        (`/Game/Blueprints/Enemie/Blueprint/BP_PorteEnnemi.Flickering Neon` (`self.Porte_Ennemis_Ref`))
        (`self.Flickering Light`))
      (if (not (and (`SceneComponent.IsVisible` _wgdanger) (not (`self.b_IsEnd`))))
        (`SceneComponent.SetVisibility` _wgdanger true false)))))

(fn `DelayFirstWave`
  (bind _wgdanger (`self.WGDanger`))
  (bind _timebeforefirststartspawn (`self.TimeBeforeFirstStartSpawn`))
  (if (>= (`self.DelayBeforeNextWaveTemp`) (`self.TimeBeforeFirstStartSpawn`))
    (`KismetSystemLibrary.K2_PauseTimerHandle` (`self.TBFDelayFirstWave`))
    (`self.Spawn`)
    (`SceneComponent.SetVisibility` (`self.WGDanger`) false false)
    (set `self.DelayBeforeNextWaveTemp` 0.0)
    (else
      (bind _output_get (set `self.DelayBeforeNextWaveTemp` (+ (`self.DelayBeforeNextWaveTemp`) 1.0)))
      (`/Game/Blueprints/Widgets/WG_Danger.Set warning BAr` (`self.WGDangerRef`) _output_get _timebeforefirststartspawn)
      (if (== (- _timebeforefirststartspawn (`self.DelayBeforeNextWaveTemp`)) 3.0)
        (bind _porte_ennemis_ref (`self.Porte_Ennemis_Ref`)
          (:`then`
            (`/Game/Blueprints/Enemie/Blueprint/BP_PorteEnnemi.Flickering Neon` _porte_ennemis_ref)
            (`self.Flickering Light`))
          (:`else`
            _)))
      (if (not (`SceneComponent.IsVisible` _wgdanger))
        (`SceneComponent.SetVisibility` _wgdanger true false)))))

(fn `Set Up Wave`
  (bind _number_of_enemisarrayspawnerref (`self.Number Of EnemisArraySpawnerRef`))
  (bind _level_script_ref (`self.Level Script Ref`))
  (bind _returnvalue (`KismetArrayLibrary.Array_Length` (`self.NBEnemiPerWave`)))
  (`self.Close Sliding Door`)
  (`self.Reset Door`)
  (if (< (+ (`self.ActualWave`) 1) _returnvalue)
    (bind _output_get (set `self.ActualWave` (+ (`self.ActualWave`) 1)))
    (`self.New Wave Widget Update`)
    (`/Game/Blueprints/Widgets/WG_WaveNumber.Set Text Nb Waves` (`self.As WG Wave Number`) _output_get _returnvalue)
    (if (== _output_get (`/Game/Blueprints/LevelPrototyping/LevelScripting/BP_LevelScript_VS.Nb Wave Enter Phase 2` _level_script_ref))
      (`/Game/Blueprints/LevelPrototyping/LevelScripting/BP_LevelScript_VS.EnteringPhase2` _level_script_ref))
    (set `self.Number Of EnemisArraySpawnerRef` (`.NumberOfEnemis_11_2984DFEF461018F077810D8784BD6C6F` (break `/Game/Blueprints/Spawner/ST_SpawnRate+NBEnemi` (`|GetArrayItem` (`self.NBEnemiPerWave`) (`self.ActualWave`)))))
    (`KismetArrayLibrary.Array_Reverse` _number_of_enemisarrayspawnerref)
    (set `self.NBEnnemiActualWave` (`KismetArrayLibrary.Array_Length` _number_of_enemisarrayspawnerref))
    (return)
    (else
      (`KismetSystemLibrary.K2_PauseTimerHandle` (`self.TimerCheckEnemi`))
      (`GameplayStatics.SetGamePaused` true)
      (bind _returnvalue_2 (`|CreateWidget` "/Game/Blueprints/Widgets/WG_EndGame.WG_EndGame_C" (`GameplayStatics.GetPlayerController` 0) true))
      (`UserWidget.AddToViewport` _returnvalue_2 0)
      (`WidgetBlueprintLibrary.SetInputMode_UIOnlyEx` (`GameplayStatics.GetPlayerController` 0) _returnvalue_2)
      (`self.K2_DestroyActor`)
      (set `self.b_IsEnd` true)
      (return))))

(fn `SetDataValue`
  (locals (DataAsset :type "/Game/Blueprints/Debug/PDA_LevelConstructorValue Object Reference"))
  (bind _output_get (set `local.DataAsset` (`/Game/Blueprints/Debug/BFL_SetDataAsset.SetDataAsset`)))
  (set `self.TimeBeforeFirstStartSpawn` (`KismetMathLibrary.Conv_IntToDouble` (`/Game/Blueprints/Debug/PDA_LevelConstructorValue.TimeBeforeFirstWave` (`local.DataAsset`))))
  (set `self.DelayBetweenWave` (`/Game/Blueprints/Debug/PDA_LevelConstructorValue.DelayBetweenWave` (`local.DataAsset`))))

(fn `UserConstructionScript`)