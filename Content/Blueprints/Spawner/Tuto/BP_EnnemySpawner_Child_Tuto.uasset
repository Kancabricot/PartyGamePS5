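; Tutorial variant of the enemy spawner that adds a SpawnTuto function for spawning tutorial enemies.
; SpawnTuto accepts only BP_Enemie_Child_Tuto and spawns it at a random point inside the Spawner box, adjusting for collisions.
; Each enemy receives the tutorial manager, a random spline from SplineRef, the SpawnerMaster and its scrap-drop flag.
; The regular Spawn only calls the parent, with leftover unconnected nodes.
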(fn `Spawn`
  (params (Enemy :type "Object Class Reference") (b_CanDropScrap :type Boolean))
  (`parent.Spawn` Enemy b_CanDropScrap))

(fn `SpawnTuto`
  (params (Enemy :type "Object Class Reference") (b_CanDropScrap :type Boolean) (`TutoManager ` :type "/Game/Blueprints/Tutorial/BP_TutorialManager Object Reference"))
  (bind _spawner (`self.Spawner`))
  (bind _asbp_enemie_child_tuto (castclass `/Game/Blueprints/Enemie/Blueprint/ChildTuto/BP_Enemie_Child_Tuto` Enemy))
  (`|SpawnActorFromClass` _asbp_enemie_child_tuto (`KismetMathLibrary.MakeTransform` (`KismetMathLibrary.RandomPointInBoundingBox` (`SceneComponent.K2_GetComponentLocation` _spawner) (`BoxComponent.GetScaledBoxExtent` _spawner))) "AdjustIfPossibleButAlwaysSpawn" "MultiplyWithRoot" null `TutoManager ` 175.0 null (`KismetArrayLibrary.Array_Random` (`self.SplineRef`)) (`self.Spawner Master`) false null b_CanDropScrap null))

(fn `UserConstructionScript`
  (`parent.UserConstructionScript`))