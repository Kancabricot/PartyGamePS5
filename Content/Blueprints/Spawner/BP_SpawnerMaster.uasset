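; Wave director that runs a level's enemy spawning, danger countdown, scrap rewards and victory screen.
; A data asset supplies each wave's enemies and delays to function-name timers that drive the Spawner, with scrap carriers picked by a rising chance over a per-wave quota.
; Clearing a wave triggers its event and the next countdown; the last saves stars based on heart life.
; Overlapping enemies open sliding doors via a timeline.
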(event `PlayMusique`
  (bind _returnvalue (`GameplayStatics.SpawnSound2D` (`self.LevelMusique`) 1.0 1.0 0.0 null))
  (`AudioComponent.FadeIn` _returnvalue 1.0 1.0 0.0 "Linear"))

(event `self.ReceiveBeginPlay`
  (bind _returnvalue (`|CreateWidget` "/Game/Blueprints/Widgets/WG_OpenLevel.WG_OpenLevel_C"))
  (`UserWidget.AddToViewport` _returnvalue 0)
  (bind _returnvalue_2 (`GameplayStatics.GetActorOfClass` "/Game/Blueprints/Player/Cam/BP_camera.BP_camera_C"))
  (set `self.CaméraRef` _returnvalue_2)
  (`/Game/Blueprints/Spawner/BP_EnnemySpawner.GetMasterRef` (`self.Spawner`) self)
  (set `self.WGDangerRef` (cast `/Game/Blueprints/Widgets/WG_Danger` (`WidgetComponent.GetWidget` (`self.WG_Danger`)) :!pure true))
  (bind _returnvalue_3 (`KismetSystemLibrary.K2_SetTimer` null "GetTimerWave" 1.0 true))
  (bind _output_get (set `self.TimerGetTimerWave` _returnvalue_3))
  (`KismetSystemLibrary.K2_PauseTimerHandle` _output_get)
  (if (`self.b_InstantSpawn`)
    (`self.StartGame `)
    (bind _outactors (`GameplayStatics.GetAllActorsOfClass` "/Game/Blueprints/Player/Player/BP_Player.BP_Player_C"))
    (bind _output_get_2 (set `self.Players` _outactors))
    (`KismetSystemLibrary.DelayUntilNextTick`)
    (for _array_element _output_get_2
      (`self.DisableInput` _array_element (`GameplayStatics.GetPlayerController` (`/Game/Blueprints/Player/Player/BP_Player.Player Index` _array_element))))))

(event `StartWave`
  (set `/Game/Blueprints/Player/Cam/BP_camera.GameFov` true (`self.CaméraRef`))
  (`self.DelayWave`)
  (bind _returnvalue (`GameplayStatics.GetActorOfClass` "/Game/Blueprints/LevelPrototyping/BP_Event.BP_Event_C"))
  (set `self.EventRef` _returnvalue)
  (for _array_element (`self.Players`)
    (`self.EnableInput` _array_element (`GameplayStatics.GetPlayerController` (`/Game/Blueprints/Player/Player/BP_Player.Player Index` _array_element)))))

(event `AddScrap`
  (params (nb :type Integer) (Who :type "/Game/Blueprints/Enemie/Blueprint/BP_Enemie Object Reference"))
  (bind _returnvalue (`KismetMathLibrary.RandomFloatInRange` 0.0 500.0))
  (`/Engine/EditorBlueprintResources/StandardMacros.IncrementInt` (`self.NbEnemieKill`)
    (:`  `
      (if (>= (`self.NbEnemieKill`) (`self.NbEnemieNeedToSpawnScrap`))
        (bind _returnvalue_2 (`|SpawnActorFromClass` "/Game/Blueprints/Enemie/Blueprint/BP_Scrap.BP_Scrap_C" (`KismetMathLibrary.MakeTransform` (`self.K2_GetActorLocation` Who)) "Undefined" "MultiplyWithRoot" null 0 null))
        (bind _staticmesh (`/Game/Blueprints/Enemie/Blueprint/BP_Scrap.StaticMesh` _returnvalue_2))
        (`PrimitiveComponent.SetSimulatePhysics` _staticmesh true)
        (`PrimitiveComponent.SetPhysicsLinearVelocity` _staticmesh (`KismetMathLibrary.MakeVector` _returnvalue (`KismetMathLibrary.RandomFloatInRange` 0.0 500.0) _returnvalue) false "None")
        (set `self.NbEnemieKill` 0)))))

(event `OpenDoor`
  (bind (_direction _newtrack_0) (`Timeline|Timeline` :!label _label)
    (:`Update`
      (`SceneComponent.K2_SetRelativeLocation` (`self.DoorD`) (`KismetMathLibrary.VLerp` (50.0 0.0 0.0) (50.0 220.0 0.0) _newtrack_0) false false)
      (`SceneComponent.K2_SetRelativeLocation` (`self.DoorG`) (`KismetMathLibrary.VLerp` (50.0 0.0 0.0) (50.0 -220.0 0.0) _newtrack_0) false false))))

(event `CloseDoor`
  (goto _label :!via `Reverse`))

(event `self.Trigger door.OnComponentBeginOverlap`
  (params (OverlappedComponent :type "PrimitiveComponent Object Reference") (OtherActor :type "Actor Object Reference") (OtherComp :type "PrimitiveComponent Object Reference") (OtherBodyIndex :type Integer) (bFromSweep :type Boolean) (SweepResult :type "HitResult Structure (by ref)"))
  (bind _asbp_enemie (cast `/Game/Blueprints/Enemie/Blueprint/BP_Enemie` OtherActor))
  (if (not (`KismetArrayLibrary.Array_Contains` (`self.EnemyRefArray`) _asbp_enemie))
    (`KismetArrayLibrary.Array_Add` (`self.EnemyRefArray`) _asbp_enemie)
    (`self.OpenDoor`)))

(event `self.Trigger door.OnComponentEndOverlap`
  (params (OverlappedComponent :type "PrimitiveComponent Object Reference") (OtherActor :type "Actor Object Reference") (OtherComp :type "PrimitiveComponent Object Reference") (OtherBodyIndex :type Integer))
  (bind _enemyrefarray (`self.EnemyRefArray`))
  (bind _asbp_enemie (cast `/Game/Blueprints/Enemie/Blueprint/BP_Enemie` OtherActor))
  (`KismetArrayLibrary.Array_RemoveItem` _enemyrefarray _asbp_enemie)
  (if (`KismetArrayLibrary.Array_IsEmpty` _enemyrefarray)
    (`self.CloseDoor`)))

(fn `DecreaseNBEnemy`
  (bind (_enemy _timer _delayforstartwave _nbscrapperwave _eventtoplay _xnbtodestroy) (break `/Game/Blueprints/Spawner/DataSpawner/Struc_enemy` (`|GetArrayItem` (`/Game/Blueprints/Spawner/DataSpawner/PDA_Spawner.Wave` (`self.PDA_Spawner`)) (`self.ActualWave`))))
  (bind _result (`/Engine/EditorBlueprintResources/StandardMacros.DecrementInt` (`self.NBEnemyOnLevel`))
    (:`  `
      (if (< _result 1)
        (`KismetSystemLibrary.PrintString` "Nest wave or end" true true (struct :`R` 1.0 :`B` 0.541393 :`A` 1.0))
        (`Widget.SetVisibility` (`self.WGDangerRef`) "Visible")
        (if (`self.b_NextWave`)
          (`/Game/Blueprints/LevelPrototyping/BP_Event.RunRandomEvent` (`self.EventRef`) (`self.ActualWave`) _eventtoplay _xnbtodestroy)
          (`self.DelayWave`)
          (set `self.b_NextWave` false)
          (bind _level_script_ref (`self.Level Script Ref`)
            (:`then`
              (message `/Game/Blueprints/Interface/BPI_NextWave.NextWave` _level_script_ref))
            (:`else`))
          (elif (`self.b_End`)
            (`GameplayStatics.SetGlobalTimeDilation` 0.5)
            (`KismetSystemLibrary.K2_SetTimer` null "EndGame" 1.5)
            (`SceneComponent.SetVisibility` (`self.WG_Danger`) false false)))))))

(fn `DelayToSpawn`
  (if (`KismetSystemLibrary.K2_IsTimerActiveHandle` (`self.TimerGetTimerWave`))
    (`KismetSystemLibrary.K2_PauseTimerHandle` (`self.TimerGetTimerWave`))
    (`Widget.SetVisibility` (`self.WGDangerRef`) "Hidden"))
  (`KismetSystemLibrary.K2_SetTimer` null "Spawn" (`|GetArrayItem` (`.Timer_7_34564A1F4007B79FD7CE538296FCABEE` (break `/Game/Blueprints/Spawner/DataSpawner/Struc_enemy` (`|GetArrayItem` (`/Game/Blueprints/Spawner/DataSpawner/PDA_Spawner.Wave` (`self.PDA_Spawner`)) (`self.ActualWave`)))) (`self.ActualEnemy`))))

(fn `DelayWave`
  (bind ((`DelayForStartWave_16_6FDC85794CF63927DC97418BA9A160CB` _delayforstartwave) (`NbScrapPerWave_20_E6BB7E3E42B8D0BE8A758EA9F7FE5F61` _nbscrapperwave)) (break `/Game/Blueprints/Spawner/DataSpawner/Struc_enemy` (`|GetArrayItem` (`/Game/Blueprints/Spawner/DataSpawner/PDA_Spawner.Wave` (`self.PDA_Spawner`)) (`self.ActualWave`))))
  (set `self.NBScrapToGive` _nbscrapperwave)
  (bind _returnvalue (`KismetSystemLibrary.K2_SetTimer` null "DelayToSpawn" _delayforstartwave))
  (set `self.TimerWave` _returnvalue)
  (set `self.b_FirstSpawn` true)
  (`KismetSystemLibrary.K2_UnPauseTimerHandle` (`self.TimerGetTimerWave`)))

(fn `EndGame`
  (bind _heartref (`self.HeartRef`))
  (bind _heartref_2 (`self.HeartRef`))
  (bind _wg_end_game (`self.WG end Game`))
  (bind _returnvalue (`KismetMathLibrary.NormalizeToRange` (`/Game/Blueprints/Machine/BP_Heart.Current life` _heartref) 0.0 (`/Game/Blueprints/Machine/BP_Heart.MaxLife` _heartref)))
  (bind _returnvalue_2 (select `bool` (>= _returnvalue 1.0) :`false` (select `bool` (>= _returnvalue 0.5) :`false` (select `bool` (> _returnvalue 0.0) :`false` (enumliteral `/Game/Blueprints/Menu/Enumerator/E_StarUnlock` "NewEnumerator0") :`true` (enumliteral `/Game/Blueprints/Menu/Enumerator/E_StarUnlock` "NewEnumerator1")) :`true` (enumliteral `/Game/Blueprints/Menu/Enumerator/E_StarUnlock` "NewEnumerator2")) :`true` (enumliteral `/Game/Blueprints/Menu/Enumerator/E_StarUnlock` "NewEnumerator3")))
  (bind _asbp_game_instance (cast `/Game/Blueprints/GameInstance/Bp_GameInstance` (`GameplayStatics.GetGameInstance`)))
  (bind _returnvalue_3 (`GameplayStatics.GetCurrentLevelName` true))
  (`/Game/Blueprints/GameInstance/Bp_GameInstance.SaveLevelFinish` _asbp_game_instance _returnvalue_3 _returnvalue_2)
  (`GameplayStatics.SetGamePaused` true)
  (`self.WG end Game`
    (:`then`
      _)
    (:`else`
      (bind _returnvalue_4 (`|CreateWidget` "/Game/GameLocalization/WG_EndGame.WG_EndGame_C" (`GameplayStatics.GetPlayerController` 0) true (/ (`/Game/Blueprints/Machine/BP_Heart.Current life` _heartref_2) (`/Game/Blueprints/Machine/BP_Heart.MaxLife` _heartref_2)) _returnvalue_2))
      (set `self.WG end Game` _returnvalue_4)))
  (`UserWidget.AddToViewport` _wg_end_game 0)
  (`WidgetBlueprintLibrary.SetInputMode_UIOnlyEx` (`GameplayStatics.GetPlayerController` 0) _wg_end_game))

(fn `GetTimerWave`
  (`/Game/Blueprints/Widgets/WG_Danger.Set warning BAr` (`self.WGDangerRef`) (`KismetSystemLibrary.K2_GetTimerRemainingTimeHandle` (`self.TimerWave`)) (`.DelayForStartWave_16_6FDC85794CF63927DC97418BA9A160CB` (break `/Game/Blueprints/Spawner/DataSpawner/Struc_enemy` (`|GetArrayItem` (`/Game/Blueprints/Spawner/DataSpawner/PDA_Spawner.Wave` (`self.PDA_Spawner`)) (`self.ActualWave`))))))

(fn `GiveScrap`
  (returns (b_GiveScrap :type Boolean))
  (if (> (`self.NBScrapToGive`) 0)
    (set `self.randomForScrap` (`KismetMathLibrary.RandomFloatInRange` 0.0 1.0))
    (if (> (* (`self.PercentRandom`) (`self.IterationPercent`)) (`self.randomForScrap`))
      (set `self.IterationPercent` 1.0)
      (set `self.NBScrapToGive` (- (`self.NBScrapToGive`) 1))
      (`/Engine/EditorBlueprintResources/StandardMacros.IncrementInt` (`self.EnemyAlreadySpawn`)
        (:`  `
          (`/Engine/EditorBlueprintResources/StandardMacros.IncrementInt` (`self.ScrapToDelete`)
            (:`  `
              (`self.SetUpGiveScrap`)
              (return true)))))
      (else
        (set `self.IterationPercent` (+ (`self.IterationPercent`) 1.0))
        (`/Engine/EditorBlueprintResources/StandardMacros.IncrementInt` (`self.EnemyAlreadySpawn`)
          (:`  `
            (return false)))))
    (else
      (return false))))

(fn `SetUpGiveScrap`
  (bind ((`Enemy_8_2E80F32C4A371E88B9C91FB3BCDF35EC` _enemy) (`NbScrapPerWave_20_E6BB7E3E42B8D0BE8A758EA9F7FE5F61` _nbscrapperwave)) (break `/Game/Blueprints/Spawner/DataSpawner/Struc_enemy` (`|GetArrayItem` (`/Game/Blueprints/Spawner/DataSpawner/PDA_Spawner.Wave` (`self.PDA_Spawner`)) (`self.ActualWave`))))
  (for _array_element _enemy
    (if (or (== _array_element "/Game/Blueprints/Enemie/Blueprint/ChildScrap/BP_Enemie_Scrap.BP_Enemie_Scrap_C") (== _array_element "/Game/Blueprints/Enemie/Blueprint/ChildScrap/BP_Enemie_Survolté_Scrap.BP_Enemie_Survolté_Scrap_C") (== _array_element "/Game/Blueprints/Enemie/Blueprint/ChildScrap/BP_Enemie_Tank_Scrap.BP_Enemie_Tank_Scrap_C"))
      (`/Engine/EditorBlueprintResources/StandardMacros.IncrementInt` (`self.GoldenCraps`))))
  (bind _output_get (set `self.PercentRandom` (/ (`KismetMathLibrary.Conv_IntToDouble` (- _nbscrapperwave (`self.ScrapToDelete`))) (`KismetMathLibrary.Conv_IntToDouble` (- (`KismetArrayLibrary.Array_Length` _enemy) (`self.EnemyAlreadySpawn`) (`self.GoldenCraps`))))))
  (set `self.GoldenCraps` 0))

(fn `SetUpNextWave`
  (bind _returnvalue (+ (`self.ActualWave`) 1))
  (if (> (`KismetArrayLibrary.Array_Length` (`/Game/Blueprints/Spawner/DataSpawner/PDA_Spawner.Wave` (`self.PDA_Spawner`))) _returnvalue)
    (set `self.ActualWave` _returnvalue)
    (set `self.ActualEnemy` 0)
    (set `self.b_NextWave` true)
    (else
      (set `self.b_End` true))))

(fn `Spawn`
  (bind _returnvalue (+ (`self.ActualEnemy`) 1))
  (bind _enemy (break `/Game/Blueprints/Spawner/DataSpawner/Struc_enemy` (`|GetArrayItem` (`/Game/Blueprints/Spawner/DataSpawner/PDA_Spawner.Wave` (`self.PDA_Spawner`)) (`self.ActualWave`))))
  (if (`self.b_FirstSpawn`)
    (`self.SetUpGiveScrap`)
    (set `self.b_FirstSpawn` false)
    (bind _slimeref (`self.SlimeRef`)
      (:`then`
        (`/Game/Blueprints/Machine/BP_GestionSlime.Shuffle` _slimeref))
      (:`else`
        _)))
  (`/Game/Blueprints/Spawner/BP_EnnemySpawner.Spawn` (`self.Spawner`) (`|GetArrayItem` _enemy (`self.ActualEnemy`)) (`self.GiveScrap`))
  (`/Engine/EditorBlueprintResources/StandardMacros.IncrementInt` (`self.NBEnemyOnLevel`)
    (:`  `
      ;[1 1 1] blm
      (if (> (`KismetArrayLibrary.Array_Length` _enemy) _returnvalue)
        (set `self.ActualEnemy` _returnvalue)
        (`self.DelayToSpawn`)
        (else
          (set `self.ScrapToDelete` 0)
          (set `self.EnemyAlreadySpawn` 0)
          (`self.SetUpNextWave`))))))

(fn `StartGame `
  (bind _returnvalue (`|CreateWidget` "/Game/Blueprints/Widgets/WG_StartGame.WG_StartGame_C" null self))
  (`UserWidget.AddToViewport` _returnvalue 0))

(fn `UserConstructionScript`)