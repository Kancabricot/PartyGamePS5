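; BP_SpawnerMasterTest is a master spawner that periodically triggers enemy spawns across a set of referenced spawners.
; After an initial delay on BeginPlay, a self-recalling Spawn event picks a random spawner from SpawnerRefArray and tells it to spawn BP_Enemie.
; Each loop waits a random interval within a configurable min/max range.
; Holding debug key L speeds up global time dilation for testing.
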(event Custom|Spawn
  (bind _delayspawnminmax (Variables|Default|GetDelaySpawnMinMax))
  (Default|Spawn (.OutItem (Utilities|Array|Random (Variables|Default|GetSpawnerRefArray))) (Utilities|Array|MakeArray "/Game/Blueprints/Enemie/BP_Enemie.BP_Enemie_C"))
  (Utilities|FlowControl|Delay (Math|Random|RandomFloatinRange (Utilities|Array|Get(acopy) _delayspawnminmax) (Utilities|Array|Get(acopy) _delayspawnminmax 1)))
  (CallFunction|Spawn))

(event EventBeginPlay
  (Utilities|FlowControl|Delay (Variables|Default|GetTimeBeforeFirstStartSpawn))
  (CallFunction|Spawn))

(event Input|KeyboardEvents|DebugKeyL
  (params (Key :type Key%20Structure :default "None") (ActionValue :type Input%20Action%20Value%20Structure))
  ;[1 1 1] Accélération du temp en * 5
  (:Pressed
    (Utilities|Time|SetGlobalTimeDilation 5.0))
  (:Released
    (Utilities|Time|SetGlobalTimeDilation 1.0)))

(fn ConstructionScript)