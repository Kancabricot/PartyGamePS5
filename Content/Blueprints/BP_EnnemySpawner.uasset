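; BP_EnnemySpawner is an actor that endlessly spawns BP_Ennemy enemies inside a box volume.
; After an initial delay on BeginPlay, DelaySpawn waits briefly and calls Spawn, which calls DelaySpawn again to form a repeating loop with no stop condition.
; Each enemy appears at a random point within the Spawner component's box extent and receives TargetForEnnemy as its TargetMovement.
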(event `self.ReceiveBeginPlay`
  (`KismetSystemLibrary.Delay` 10.0)
  (`self.DelaySpawn`))

(event `DelaySpawn`
  (`KismetSystemLibrary.Delay` 2.0)
  (`self.Spawn`))

(fn `Spawn`
  (bind _spawner (`self.Spawner`))
  (`|SpawnActorFromClass` "/Game/Blueprints/Ennemie/BP_Ennemy.BP_Ennemy_C" (`KismetMathLibrary.MakeTransform` (`KismetMathLibrary.RandomPointInBoundingBox` (`SceneComponent.K2_GetComponentLocation` _spawner) (`BoxComponent.GetScaledBoxExtent` _spawner))) "Undefined" "MultiplyWithRoot" null (`self.TargetForEnnemy`) null)
  (`self.DelaySpawn`))

(fn `UserConstructionScript`)