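; BP_Baterie is a battery pickup that the player can carry and throw, with a physics-driven Cylinder.
; TakeItem passes it to the player and disables collision and physics; DettachItem restores both and launches it with the supplied impulse.
; While not held, overlapping a tagged World Static component reapplies a third of that impulse, first moving the actor to a ThrowingLocation if tagged "Zone".
; GiveItemToDesk always refuses.
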(event `/Game/Blueprints/Interface/BPI_TakeItem.DettachItem`
  (params (Impulse :type "Vector Structure"))
  (bind _cylinder (`self.Cylinder`))
  (bind _output_get (set `self.Impulse` Impulse))
  (`PrimitiveComponent.SetCollisionEnabled` _cylinder "QueryAndPhysics")
  (`PrimitiveComponent.SetSimulatePhysics` _cylinder true)
  (`PrimitiveComponent.SetPhysicsLinearVelocity` (`self.Cylinder`) _output_get false "None")
  (set `self.b_IsGrab` false))

(event `self.ReceiveBeginPlay`
  (`GameplayStatics.GetActorOfClass` "/Game/Blueprints/BP_Assembler.BP_Assembler_C"))

(event `self.Box.OnComponentBeginOverlap`
  (params (OverlappedComponent :type "PrimitiveComponent Object Reference") (OtherActor :type "Actor Object Reference") (OtherComp :type "PrimitiveComponent Object Reference") (OtherBodyIndex :type Integer) (bFromSweep :type Boolean) (SweepResult :type "HitResult Structure (by ref)"))
  (switch `ECollisionChannel` (`PrimitiveComponent.GetCollisionObjectType` OtherComp)
    (:`ECC_WorldStatic`
      (if (not (`self.b_IsGrab`))
        (for _array_element (`ActorComponent.ComponentTags` OtherComp)
          (if (== _array_element "Zone")
            (`self.K2_SetActorLocation` (`SceneComponent.K2_GetComponentLocation` (`/Game/Blueprints/BP_Assembler.ThrowingLocation` (`self.Other`)))))
          (`PrimitiveComponent.SetPhysicsLinearVelocity` (`self.Cylinder`) (/ (`self.Impulse`) 3.0) false "None"))))))

(fn `GiveItemToDesk`
  (params (ActorTarget :type "Actor Object Reference"))
  (returns (Return :type Boolean))
  (return false))

(fn `TakeItem`
  (params (Player :type "/Game/Blueprints/Player/BP_Player Object Reference"))
  (returns (Return :type Boolean))
  (`/Game/Blueprints/Player/BP_Player.TakeItem` Player 0.0 self)
  (`PrimitiveComponent.SetCollisionEnabled` (`self.Cylinder`) "NoCollision")
  (set `self.b_IsGrab` true)
  (`PrimitiveComponent.SetSimulatePhysics` (`self.Cylinder`) false)
  (return true))

(fn `UserConstructionScript`)