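; Carryable auto-firing turret that activates on landing and attacks BP_Enemie actors in range, configured per weight variant from DATurretType.
; Range overlaps maintain an enemy array that pauses or resumes looping timers for aiming and shooting.
; Targeting picks by distance to goal, highest HP or unglued first, then yaws the head and spawns the variant's bullet, with separate Tesla handling.
; Non-Tesla shots deplete a magazine, ending in explosion and scrap.
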(event `EventBreakLoop`
  (for (_array_element _array_index) (`/Game/Blueprints/Turret/Structure/PDA_TurretType.Weight` (`self.DA_TurretType`)) :!via `Break`
    (if (== _array_element (`self.KitWeight`))
      (set `self.IndexTurret` _array_index)
      (`self.EventBreakLoop`))))

(event `self.ReceiveBeginPlay`
  ;[1 1 1] Get right turret
  (switch `int` 0))

(event `self.TurretRange.OnComponentBeginOverlap`
  (params (OverlappedComponent :type "PrimitiveComponent Object Reference") (OtherActor :type "Actor Object Reference") (OtherComp :type "PrimitiveComponent Object Reference") (OtherBodyIndex :type Integer) (bFromSweep :type Boolean) (SweepResult :type "HitResult Structure (by ref)"))
  ;[1 1 1] Check collision + check if enemy is already in the array
  (bind _asbp_enemie (cast `/Game/Blueprints/Enemie/Blueprint/BP_Enemie` OtherActor))
  (if (`self.b_IsActivate`)
    (if (and (not (== (`Character.Mesh` _asbp_enemie) OtherComp)) (not (`KismetArrayLibrary.Array_Contains` (`self.EnemyArray`) _asbp_enemie)))
      (`KismetArrayLibrary.Array_Add` (`self.EnemyArray`) _asbp_enemie)
      ;[1 1 1] Shoot if i the first enemy in range
      (if (== (`KismetArrayLibrary.Array_Length` (`self.EnemyArray`)) 1)
        (`self.FocusTarget`)))))

(event `self.TurretRange.OnComponentEndOverlap`
  (params (OverlappedComponent :type "PrimitiveComponent Object Reference") (OtherActor :type "Actor Object Reference") (OtherComp :type "PrimitiveComponent Object Reference") (OtherBodyIndex :type Integer))
  ;[1 1 1] Check Collision and remove the enemy off range
  (bind _asbp_enemie (cast `/Game/Blueprints/Enemie/Blueprint/BP_Enemie` OtherActor))
  (`KismetArrayLibrary.Array_RemoveItem` (`self.EnemyArray`) _asbp_enemie)
  ;[1 1 1] Is doesn't have enemy stop shooting
  (if (`KismetArrayLibrary.Array_IsEmpty` (`self.EnemyArray`))
    (`self.StopShoot`)))

(event `self.collisionGround.OnComponentBeginOverlap`
  (params (OverlappedComponent :type "PrimitiveComponent Object Reference") (OtherActor :type "Actor Object Reference") (OtherComp :type "PrimitiveComponent Object Reference") (OtherBodyIndex :type Integer) (bFromSweep :type Boolean) (SweepResult :type "HitResult Structure (by ref)"))
  (cast `StaticMeshActor` OtherActor)
  (`PrimitiveComponent.SetSimulatePhysics` (`self.Base_Turret`) false)
  (`|PlayMontage` (`self.Base_Turret`) "/Game/Animation/Montage/Turret/AM_Landing.AM_Landing"
    (:`OnCompleted`
      (`self.CheckEnemySpawn`)
      (set `self.b_IsActivate` true))))

(event `/Game/Blueprints/Interface/BPI_TakeItem.DettachItem`
  (params (Impulse :type "Vector Structure"))
  (`PrimitiveComponent.SetSimulatePhysics` (`self.Base_Turret`) true)
  (set `ProjectileMovementComponent.ProjectileGravityScale` 1.0 (`self.ProjectileMovement`))
  (`PrimitiveComponent.SetPhysicsLinearVelocity` (`self.Base_Turret`) (* Impulse 2.0) false "None"))

(fn `AnimShoot`
  (`SkeletalMeshComponent.PlayAnimation` (`self.Head_Turret`) "/Game/Assets/Turret/Animations_V2/Tesla_Shot.Tesla_Shot" false))

(fn `Check Enemy`
  (`KismetSystemLibrary.PrintString` "Check enemy")
  (for _array_element (`PrimitiveComponent.GetOverlappingActors` (`self.TurretRange`) "/Game/Blueprints/Enemie/Blueprint/BP_Enemie.BP_Enemie_C")
    (bind _asbp_enemie (cast `/Game/Blueprints/Enemie/Blueprint/BP_Enemie` _array_element))
    (`KismetSystemLibrary.PrintString` (`KismetSystemLibrary.GetDisplayName` _asbp_enemie))
    (if (not (`KismetArrayLibrary.Array_Contains` (`self.EnemyArray`) _asbp_enemie))
      (`KismetArrayLibrary.Array_Add` (`self.EnemyArray`) _asbp_enemie)))
  (if (`KismetArrayLibrary.Array_IsNotEmpty` (`self.EnemyArray`))
    (`KismetSystemLibrary.K2_UnPauseTimerHandle` (`self.TimerShoot`))
    (`KismetSystemLibrary.K2_UnPauseTimerHandle` (`self.TimerView`))))

(fn `CheckEnemySpawn`
  (for _array_element (`PrimitiveComponent.GetOverlappingActors` (`self.TurretRange`) "/Game/Blueprints/Enemie/Blueprint/BP_Enemie.BP_Enemie_C")
    (bind _asbp_enemie (cast `/Game/Blueprints/Enemie/Blueprint/BP_Enemie` _array_element))
    (`KismetArrayLibrary.Array_Add` (`self.EnemyArray`) _asbp_enemie))
  (if (not (`KismetArrayLibrary.Array_IsEmpty` (`self.EnemyArray`)))
    (`self.FocusTarget`)))

(fn `Death`
  ;[1 1 1] Spawn scrap and destroy turret
  (`NiagaraFunctionLibrary.SpawnSystemAtLocation` "/Game/VFX/VFX/Turrets/Assembleur/DestructionMatiere/NS_BoltExplosion.NS_BoltExplosion" (`self.K2_GetActorLocation`) (struct) (0.0 0.0 0.0))
  (bind _returnvalue (`|SpawnActorFromClass` "/Game/Blueprints/Enemie/Blueprint/BP_Scrap.BP_Scrap_C" (`self.GetTransform`) "Undefined" "MultiplyWithRoot" null null))
  (`PrimitiveComponent.SetPhysicsLinearVelocity` (`/Game/Blueprints/Enemie/Blueprint/BP_Scrap.StaticMesh` _returnvalue) (0.0 0.0 500.0) false "None")
  (`self.K2_DestroyActor`))

(fn `FocusTarget`
  (`KismetSystemLibrary.K2_UnPauseTimerHandle` (`self.TimerShoot`))
  (`KismetSystemLibrary.K2_UnPauseTimerHandle` (`self.TimerView`)))

(fn `GetTarget`
  (returns (Target :type "/Game/Blueprints/Enemie/Blueprint/BP_Enemie Object Reference"))
  (locals (DistanceTemp :type "Float (double-precision)" :default 9999999999.0) (EnemyTarget :type "/Game/Blueprints/Enemie/Blueprint/BP_Enemie Object Reference") (LifeTemp :type "Float (double-precision)" :default 0.0))
  ;[1 1 1] Chose how get the target
  (switch `/Game/Blueprints/Turret/Structure/Enum_Target` (`|GetArrayItem` (`/Game/Blueprints/Turret/Structure/PDA_TurretType.Target` (`self.DA_TurretType`)) (`self.IndexTurret`))
    (:`NewEnumerator0`
      ;[1 1 1] Get the closer enemy to target
      (for _array_element (`self.EnemyArray`)
        (if (< (`/Game/Blueprints/Enemie/Blueprint/BP_Enemie.DistanceToTarget` _array_element) (`local.DistanceTemp`))
          (set `local.EnemyTarget` _array_element)
          (set `local.DistanceTemp` (`/Game/Blueprints/Enemie/Blueprint/BP_Enemie.DistanceToTarget` _array_element))))
      (return (`local.EnemyTarget`)))
    (:`NewEnumerator1`
      ;[1 1 1] Target the enemy with the hight hp
      (for _array_element_2 (`self.EnemyArray`)
        (if (> (`/Game/Blueprints/Enemie/Blueprint/BP_Enemie.Life` _array_element_2) (`local.LifeTemp`))
          (set `local.EnemyTarget` _array_element_2)
          (set `local.LifeTemp` (`/Game/Blueprints/Enemie/Blueprint/BP_Enemie.Life` _array_element_2))
          (set `local.DistanceTemp` (`/Game/Blueprints/Enemie/Blueprint/BP_Enemie.DistanceToTarget` _array_element_2))
          (elif (== (`/Game/Blueprints/Enemie/Blueprint/BP_Enemie.Life` _array_element_2) (`local.LifeTemp`))
            (if (< (`/Game/Blueprints/Enemie/Blueprint/BP_Enemie.DistanceToTarget` _array_element_2) (`local.DistanceTemp`))
              (set `local.EnemyTarget` _array_element_2)
              (set `local.DistanceTemp` (`/Game/Blueprints/Enemie/Blueprint/BP_Enemie.DistanceToTarget` _array_element_2))))))
      (return (`local.EnemyTarget`)))
    (:`NewEnumerator2`
      ;[1 1 1] Get closer unglue enemy to target
      (set `local.EnemyTarget` null)
      (for _array_element_3 (`self.EnemyArray`)
        (if (and (< (`/Game/Blueprints/Enemie/Blueprint/BP_Enemie.DistanceToTarget` _array_element_3) (`local.DistanceTemp`)) (not (`/Game/Blueprints/Enemie/Blueprint/BP_Enemie.b_IsGlue` _array_element_3)))
          (set `local.EnemyTarget` _array_element_3)
          (set `local.DistanceTemp` (`/Game/Blueprints/Enemie/Blueprint/BP_Enemie.DistanceToTarget` _array_element_3))))
      (bind _enemytarget (`local.EnemyTarget`)
        (:`then`
          (return _enemytarget))
        (:`else`
          ;[1 1 1] If all is glue, target the closer enemy
          (for _array_element_4 (`self.EnemyArray`)
            (if (< (`/Game/Blueprints/Enemie/Blueprint/BP_Enemie.DistanceToTarget` _array_element_4) (`local.DistanceTemp`))
              (set `local.EnemyTarget` _array_element_4)
              (set `local.DistanceTemp` (`/Game/Blueprints/Enemie/Blueprint/BP_Enemie.DistanceToTarget` _array_element_4))))
          (return (`local.EnemyTarget`)))))))

(fn `GiveItemToDesk`
  (params (ActorTarget :type "Actor Object Reference"))
  (returns (Return :type Boolean))
  (return false))

(fn `SetMesh`
  (bind _cannon (`self.Cannon`))
  (`StaticMeshComponent.SetStaticMesh` _cannon (`|GetArrayItem` (`/Game/Blueprints/Turret/Structure/PDA_TurretType.AssetCanon` (`self.DA_TurretType`)) (`self.IndexTurret`)))
  (`SceneComponent.K2_AttachToComponent` _cannon (`self.Head_Turret`) "JNT_CannonSocket" "KeepRelative" "KeepRelative" "KeepRelative" true)
  (`SceneComponent.K2_AttachToComponent` (`self.Head_Turret`) (`self.Base_Turret`) "JNT_BaseSocket" "SnapToTarget" "SnapToTarget" "SnapToTarget" true))

(fn `SetUpTurret`
  (bind _da_turrettype (`self.DA_TurretType`))
  (bind _indexturret (`self.IndexTurret`))
  (bind _output (`|GetArrayItem` (`/Game/Blueprints/Turret/Structure/PDA_TurretType.Range` (`self.DA_TurretType`)) (`self.IndexTurret`)))
  (bind _returnvalue (+ (`|GetArrayItem` (`/Game/Blueprints/Turret/Structure/PDA_TurretType.AttackSpeed` _da_turrettype) _indexturret) (`|GetArrayItem` (`/Game/Blueprints/Turret/Structure/PDA_TurretType.LoadingShoot` _da_turrettype) _indexturret)))
  ;[1 1 1] Set mesh of the turret
  (`self.SetMesh`)
  ;[1 1 1] Set range of the turret
  (`SphereComponent.SetSphereRadius` (`self.TurretRange`) _output true)
  (`SceneComponent.SetRelativeScale3D` (`self.ZoneViewer`) (`KismetMathLibrary.MakeVector` _output _output))
  ;[1 1 1] Set the fire rate
  (bind _returnvalue_2 (`KismetSystemLibrary.K2_SetTimer` null "Shoot" _returnvalue true (- 0.5 _returnvalue)))
  (bind _output_get (set `self.TimerShoot` _returnvalue_2))
  (`KismetSystemLibrary.K2_PauseTimerHandle` _output_get)
  ;[1 1 1] Set number of shoot before destruction
  (set `self.ActualMagazine` (`|GetArrayItem` (`/Game/Blueprints/Turret/Structure/PDA_TurretType.Magazine` (`self.DA_TurretType`)) (`self.IndexTurret`)))
  ;[1 1 1] Timer for view
  (bind _returnvalue_3 (`KismetSystemLibrary.K2_SetTimer` null "SetView" 0.016 true))
  (bind _output_get_2 (set `self.TimerView` _returnvalue_3))
  (`KismetSystemLibrary.K2_PauseTimerHandle` _output_get_2))

(fn `SetUpTurretTool`
  ;[1 1 1] Set up for the tool
  (for (_array_element _array_index) (`/Game/Blueprints/Turret/Structure/PDA_TurretType.Weight` (`self.DA_TurretType`))
    (if (== _array_element (`self.KitWeight`))
      (set `self.IndexTurret` _array_index)
      (`self.EventBreakLoop`)))
  (`self.SetUpTurret`))

(fn `SetView`
  (bind _target (`self.GetTarget`))
  (bind (_returnvalue_roll _returnvalue_pitch _returnvalue_yaw) (`KismetMathLibrary.BreakRotator` (`KismetMathLibrary.FindLookAtRotation` (`SceneComponent.K2_GetComponentLocation` (`self.Cannon`)) (`SceneComponent.K2_GetComponentLocation` (`Actor.RootComponent` _target)))))
  ;[1 1 1] Set the view to the target
  (if (`KismetArrayLibrary.Array_IsNotEmpty` (`self.EnemyArray`))
    (set `self.Target` _target)
    (`SceneComponent.K2_SetWorldRotation` (`self.Head_Turret`) (`KismetMathLibrary.MakeRotator` 0.0 0.0 _returnvalue_yaw) false false)))

(fn `Shoot`
  (bind _da_turrettype (`self.DA_TurretType`))
  (bind _indexturret (`self.IndexTurret`))
  (bind _output (`|GetArrayItem` (`/Game/Blueprints/Turret/Structure/PDA_TurretType.BulletType` _da_turrettype) _indexturret))
  ;[1 1 1] Spawn the bullet
  (castclass `/Game/Blueprints/Turret/Bullet/BP_BulletTesla` _output
    (:`then`
      (`self.TeslaShoot`))
    (:`CastFailed`
      (bind _asbp_bullet_parent (castclass `/Game/Blueprints/Turret/Bullet/BP_BulletParent` _output))
      (`|SpawnActorFromClass` _asbp_bullet_parent (`KismetMathLibrary.MakeTransform` (`SceneComponent.GetSocketLocation` (`self.Cannon`) "Canon") (`SceneComponent.GetSocketRotation` (`self.Head_Turret`) "Canon")) "AlwaysSpawn" "MultiplyWithRoot" null (`|GetArrayItem` (`/Game/Blueprints/Turret/Structure/PDA_TurretType.Damage` _da_turrettype) _indexturret) (`|GetArrayItem` (`/Game/Blueprints/Turret/Structure/PDA_TurretType.LoadingShoot` _da_turrettype) _indexturret) (`self.Target`) 0.0 null)
      (`KismetSystemLibrary.K2_SetTimer` null "AnimShoot" 0.34)
      ;[1 1 1] Check if the turret have bullet or destroy it
      (bind _result (`/Engine/EditorBlueprintResources/StandardMacros.DecrementFloat` (`self.ActualMagazine`))
        (:`  `
          (if (== _result 0.0)
            (`self.Death`)))))))

(fn `StopShoot`
  (`KismetSystemLibrary.K2_PauseTimerHandle` (`self.TimerShoot`))
  (`KismetSystemLibrary.K2_PauseTimerHandle` (`self.TimerView`)))

(fn `TakeItem`
  (params (Player :type "/Game/Blueprints/Player/Player/BP_Player Object Reference"))
  (returns (Return :type Boolean))
  (bind _output_get (set `self.ActuPlayer` Player))
  (if (`self.b_CanBeCaught`)
    (set `ProjectileMovementComponent.ProjectileGravityScale` 0.0 (`self.ProjectileMovement`))
    (`/Game/Blueprints/Player/Player/BP_Player.TakeItem` _output_get self)
    (set `self.b_IsGrab` true)
    (set `self.b_IsActivate` false)
    (return true)
    (else
      (return false))))

(fn `TeslaShoot`
  (bind _da_turrettype (`self.DA_TurretType`))
  (bind _indexturret (`self.IndexTurret`))
  (if (not (`/Game/Blueprints/Enemie/Blueprint/BP_Enemie.b_IsStun` (`self.Target`)))
    (`|SpawnActorFromClass` "/Game/Blueprints/Turret/Bullet/BP_BulletTesla.BP_BulletTesla_C" (`KismetMathLibrary.MakeTransform` (`SceneComponent.GetSocketLocation` (`self.Cannon`) "Canon") (`SceneComponent.GetSocketRotation` (`self.Head_Turret`) "Canon")) "AlwaysSpawn" "MultiplyWithRoot" null 600.0 (`|GetArrayItem` (`/Game/Blueprints/Turret/Structure/PDA_TurretType.Damage` _da_turrettype) _indexturret) (`|GetArrayItem` (`/Game/Blueprints/Turret/Structure/PDA_TurretType.LoadingShoot` _da_turrettype) _indexturret) (`self.Target`) 0.0 null)
    (`self.AnimShoot`)
    (else
      (`self.Shoot`))))

(fn `UserConstructionScript`)