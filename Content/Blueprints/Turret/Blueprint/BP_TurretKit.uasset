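; BP_TurretKit is a physics pickup in three colored, weighted types that merges with other kits to build a turret.
; On overlap, the lower-Numero kit leads a timeline that shakes and pulls both toward their midpoint.
; Two single kits become one unpickable combined kit that rechecks overlaps; combined plus single spawns BP_Turrets.
; The turret's KitWeight is randomly one of two values, ignoring summed Weight; older three-kit logic is disconnected.
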(event `self.ReceiveBeginPlay`
  (bind (_returnvalue_roll _returnvalue_pitch _returnvalue_yaw) (`KismetMathLibrary.BreakRotator` (`SceneComponent.K2_GetComponentRotation` (`self.Kit`))))
  ;[1 1 1] Setup
  (`self.SetValue` (`self.Kit`) (`self.KitType`))
  (`self.ChangeColor`)
  (`KismetArrayLibrary.Array_Add` (`self.KitArray`) self)
  (set `self.Roll` _returnvalue_roll)
  (set `self.Pitch` _returnvalue_pitch)
  (set `self.Yaw` _returnvalue_yaw))

(event `/Game/Blueprints/Interface/BPI_TakeItem.DettachItem`
  (params (Impulse :type "Vector Structure"))
  (bind _kit (`self.Kit`))
  ;[1 1 1] Detach and give velocity
  (`PrimitiveComponent.SetCollisionEnabled` _kit "QueryAndPhysics")
  (`PrimitiveComponent.SetSimulatePhysics` _kit true)
  (`PrimitiveComponent.SetPhysicsLinearVelocity` (`self.Kit`) Impulse false "None")
  (set `self.b_IsGrab` false))

(event `self.KitCollider.OnComponentBeginOverlap`
  (params (OverlappedComponent :type "PrimitiveComponent Object Reference") (OtherActor :type "Actor Object Reference") (OtherComp :type "PrimitiveComponent Object Reference") (OtherBodyIndex :type Integer) (bFromSweep :type Boolean) (SweepResult :type "HitResult Structure (by ref)"))
  ;[1 1 1] Trigger snap
  (bind _asbp_turret_kit (cast `/Game/Blueprints/Turret/Blueprint/BP_TurretKit` OtherActor))
  (if (and (== (`/Game/Blueprints/Turret/Blueprint/BP_TurretKit.KitCollider` _asbp_turret_kit) OtherComp) (< (`self.Numero`) (`/Game/Blueprints/Turret/Blueprint/BP_TurretKit.Numero` _asbp_turret_kit)) (not (`/Game/Blueprints/Turret/Blueprint/BP_TurretKit.b_IsInCombine` _asbp_turret_kit)) (not (`self.b_IsInCombine`)))
    (`KismetArrayLibrary.Array_Add` (`self.KitArray`) _asbp_turret_kit)
    (if true
      (`self.Combine2Kit`))))

(event `Combine2Kit`
  (bind _returnvalue (`self.K2_GetActorLocation`))
  (bind _kitarray (`self.KitArray`))
  (bind _output (`|GetArrayItem` (`self.KitArray`) 1))
  ;[1 1 1] Combine 2 kit
  (set `self.b_IsInCombine` true)
  (set `/Game/Blueprints/Turret/Blueprint/BP_TurretKit.b_IsInCombine` true _output)
  (for _array_element _kitarray
    (`KismetArrayLibrary.Array_Add` (`self.LocationBeforeCombine`) (`self.K2_GetActorLocation` _array_element)))
  (bind _returnvalue_2 (`GameplayStatics.GetActorArrayAverageLocation` _kitarray))
  (set `self.AverageLocation` _returnvalue_2)
  (bind (_direction _snapaverage) (`Timeline|SnapAverage` :!via `PlayFromStart` :!label _label)
    (:`Update`
      (`self.ShakeAndGetCloser` _snapaverage))
    (:`Finished`
      (if (not (`self.b_IsCombine`))
        (set `self.Weight` (+ (`/Game/Blueprints/Turret/Blueprint/BP_TurretKit.Weight` _output) (`self.Weight`)))
        ;;[1 1 1] Change color kit
        (if (not (`/Game/Blueprints/Turret/Blueprint/BP_TurretKit.b_IsCombine` _output))
          (set `self.Color` (`self.FinalColor`))
          (`self.ChangeColor`)
          (`/Engine/EditorBlueprintResources/StandardMacros.IsValid` _output
            (:`Is Valid`
              (set `self.KitToDelete` _output)
              (`KismetArrayLibrary.Array_RemoveItem` (`self.KitArray`) _output)
              (bind _returnvalue_3 (`AddComponent|NODE_AddStaticMeshComponent-0` :`bManualAttachment` true))
              (`self.SetValue` _returnvalue_3 (`/Game/Blueprints/Turret/Blueprint/BP_TurretKit.KitType` (`self.KitToDelete`)))
              (`SceneComponent.K2_AttachToComponent` _returnvalue_3 (`self.Kit`) "AttachSocket" "KeepRelative" "KeepRelative" "KeepRelative" true)
              (`self.K2_DestroyActor` (`self.KitToDelete`))
              (`KismetArrayLibrary.Array_Clear` (`self.LocationBeforeCombine`))
              (`NiagaraFunctionLibrary.SpawnSystemAtLocation` "/Game/VFX/VFX/Distributeur/StarSuccess/NS_StarSuccess.NS_StarSuccess" (`self.K2_GetActorLocation`) (struct) (10.0 10.0 10.0))
              (`PrimitiveComponent.SetPhysicsLinearVelocity` (`self.Kit`) (0.0 0.0 100.0) false "None")
              (set `self.b_IsCombine` true)
              (set `self.b_IsInCombine` false)
              (`self.CheckOverlaps`)))
          (else
            (set `self.Weight` (+ (`/Game/Blueprints/Turret/Blueprint/BP_TurretKit.Weight` _output) (`self.Weight`)) :!label _label_2)
            (`self.K2_DestroyActor` _output)
            (`NiagaraFunctionLibrary.SpawnSystemAtLocation` "/Game/VFX/VFX/Turrets/Creation/NS_TurretCreation.NS_TurretCreation" _returnvalue (struct) (10.0 10.0 10.0))
            (`|SpawnActorFromClass` "/Game/Blueprints/Turret/Blueprint/BP_Turrets.BP_Turrets_C" (`KismetMathLibrary.MakeTransform` _returnvalue) "AdjustIfPossibleButAlwaysSpawn" "MultiplyWithRoot" null (`KismetMathLibrary.SelectInt` 3 8 (`KismetMathLibrary.RandomBool`)) null)
            (`self.K2_DestroyActor` self)))
        (elif (not (`/Game/Blueprints/Turret/Blueprint/BP_TurretKit.b_IsCombine` _output))
          (goto _label_2))))))

(event `Combine2KitStop`
  ;[1 1 1] Combine 2 kit
  (goto _label :!via `Stop`))

(event `Combine3Kit`)

(fn `ChangeColor`
  (bind _returnvalue (`PrimitiveComponent.CreateDynamicMaterialInstance` (`self.KitCollider`) 0 "/Game/Blueprints/Turret/Blueprint/M_SphereTim.M_SphereTim" "None"))
  (`MaterialInstanceDynamic.SetVectorParameterValue` _returnvalue "Color" (`self.Color`))
  (`MaterialInstanceDynamic.SetVectorParameterValue` _returnvalue "Color2" (`self.Color`)))

(fn `CheckOverlaps`
  (for _array_element (`PrimitiveComponent.GetOverlappingActors` (`self.KitCollider`) "BP_TurretKit_C")
    (bind _asbp_turret_kit (cast `/Game/Blueprints/Turret/Blueprint/BP_TurretKit` _array_element))
    (if (not (== _asbp_turret_kit self))
      (`KismetArrayLibrary.Array_Add` (`self.KitArray`) _asbp_turret_kit)
      (`self.Combine2Kit`))))

(fn `GiveItemToDesk`
  (params (ActorTarget :type "Actor Object Reference"))
  (returns (Return :type Boolean))
  (return false))

(fn `SetValue`
  (params (Target :type "PrimitiveComponent Object Reference") (Selection :type "/Game/Blueprints/Enums/Enum_Kit Enum" :default "NewEnumerator0"))
  (locals (ColorValue :type "Float (single-precision)" :default 0.0))
  (switch `/Game/Blueprints/Enums/Enum_Kit` Selection
    (:`NewEnumerator0`
      (set `local.ColorValue` 0.0)
      (set `self.Color` (struct :`G` 1.0 :`A` 1.0))
      (set `self.Weight` 1))
    (:`NewEnumerator1`
      (set `local.ColorValue` 2.0)
      (set `self.Color` (struct :`R` 1.0 :`A` 1.0))
      (set `self.Weight` 2))
    (:`NewEnumerator2`
      (set `local.ColorValue` 1.0)
      (set `self.Color` (struct :`B` 1.0 :`A` 1.0))
      (set `self.Weight` 5)))
  (bind _returnvalue (`PrimitiveComponent.CreateDynamicMaterialInstance` Target 1 "/Game/Assets/Kit/Mats/M_RedKit.M_RedKit" "None"))
  (`MaterialInstanceDynamic.SetScalarParameterValue` _returnvalue "ColorChoice" (`local.ColorValue`)))

(fn `ShakeAndGetCloser`
  (params (LerpValue :type "Float (single-precision)"))
  (bind _output (`|GetArrayItem` (`self.KitArray`)))
  (bind _output_2 (`|GetArrayItem` (`self.KitArray`) 1))
  (bind _kit (`/Game/Blueprints/Turret/Blueprint/BP_TurretKit.Kit` _output))
  (bind _kit_2 (`/Game/Blueprints/Turret/Blueprint/BP_TurretKit.Kit` _output_2))
  (`/Engine/EditorBlueprintResources/StandardMacros.IsValid` _output
    (:`Is Valid`
      (`SceneComponent.K2_SetWorldRotation` _kit (`KismetMathLibrary.MakeRotator` (+ (`self.Roll`) (`KismetMathLibrary.RandomFloatInRange` -20.0 20.0)) (+ (`self.Pitch`) (`KismetMathLibrary.RandomFloatInRange` -20.0 20.0)) (+ (`self.Yaw`) (`KismetMathLibrary.RandomFloatInRange` -20.0 20.0))) false false)
      (`SceneComponent.K2_SetWorldLocation` _kit (`KismetMathLibrary.VLerp` (`|GetArrayItem` (`self.LocationBeforeCombine`)) (`self.AverageLocation`) LerpValue) false false)
      (`/Engine/EditorBlueprintResources/StandardMacros.IsValid` _output_2
        (:`Is Valid`
          (`SceneComponent.K2_SetWorldRotation` _kit_2 (`KismetMathLibrary.MakeRotator` (+ (`self.Roll`) (`KismetMathLibrary.RandomFloatInRange` -20.0 20.0)) (+ (`self.Pitch`) (`KismetMathLibrary.RandomFloatInRange` -20.0 20.0)) (+ (`self.Yaw`) (`KismetMathLibrary.RandomFloatInRange` -20.0 20.0))) false false)
          (`SceneComponent.K2_SetWorldLocation` _kit_2 (`KismetMathLibrary.VLerp` (`|GetArrayItem` (`self.LocationBeforeCombine`) 1) (`self.AverageLocation`) LerpValue) false false))))))

(fn `TakeItem`
  (params (Player :type "/Game/Blueprints/Player/Player/BP_Player Object Reference"))
  (returns (Return :type Boolean))
  (if (and (not (`self.b_IsInCombine`)) (not (`self.b_IsCombine`)))
    (`/Game/Blueprints/Player/Player/BP_Player.TakeItem` Player self)
    (`PrimitiveComponent.SetCollisionEnabled` (`self.Kit`) "NoCollision")
    (set `self.b_IsGrab` true)
    (`PrimitiveComponent.SetSimulatePhysics` (`self.Kit`) false)
    (return false)))

(fn `UserConstructionScript`
  (`self.SetValue` (`self.Kit`) (`self.KitType`))
  (`self.ChangeColor`))