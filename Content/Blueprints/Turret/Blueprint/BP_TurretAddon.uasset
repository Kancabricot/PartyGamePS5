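; BP_TurretAddon is a carryable, throwable turret upgrade (Range, Fire Rate or AOE, set as material at construction).
; TakeItem attaches it to a player with a rotating icon; DettachItem launches it with physics, and moving overlaps let empty-handed players catch it.
; CheckTurret sphere-traces for turrets, adds a stage to the first if inactive, then destroys the addon.
; Inactive turrets are highlighted via custom depth and icons; "Zone" overlaps reset it to the assembler's throwing location.
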(event `/Game/Blueprints/Interface/BPI_TakeItem.DettachItem`
  (params (Impulse :type "Vector Structure"))
  (bind _addon (`self.Addon`))
  (`SceneComponent.SetVisibility` (`/Game/Blueprints/Player/Player/BP_Player.Widget` (`self.ActuPlayer`)) false false)
  (`KismetSystemLibrary.K2_PauseTimerHandle` (`self.ActuTimer`))
  (for _array_element (`self.ActuTurret`)
    (`SceneComponent.SetVisibility` (`/Game/Blueprints/Turret/Blueprint/BP_Turret.Widget` _array_element) false false))
  (bind _output_get (set `self.Impulse` Impulse))
  (`PrimitiveComponent.SetCollisionEnabled` _addon "QueryAndPhysics")
  (`PrimitiveComponent.SetSimulatePhysics` _addon true)
  (`PrimitiveComponent.SetPhysicsLinearVelocity` (`self.Addon`) _output_get false "None")
  (set `self.b_IsGrab` false))

(event `self.Box.OnComponentBeginOverlap`
  (params (OverlappedComponent :type "PrimitiveComponent Object Reference") (OtherActor :type "Actor Object Reference") (OtherComp :type "PrimitiveComponent Object Reference") (OtherBodyIndex :type Integer) (bFromSweep :type Boolean) (SweepResult :type "HitResult Structure (by ref)"))
  (switch `ECollisionChannel` (`PrimitiveComponent.GetCollisionObjectType` OtherComp)
    (:`ECC_WorldStatic`
      (if (not (`self.b_IsGrab`))
        (for _array_element (`ActorComponent.ComponentTags` OtherComp)
          (if (== _array_element "Zone")
            (`self.K2_SetActorLocation` (`SceneComponent.K2_GetComponentLocation` (`/Game/Blueprints/Machine/BP_Assembler.ThrowingLocation` (`self.LinkAssembleur`)))))
          (`PrimitiveComponent.SetPhysicsLinearVelocity` (`self.Addon`) (/ (`self.Impulse`) 3.0) false "None"))))))

(event `/Game/Blueprints/Interface/BPI_TakeItem.ActiveHighlight`
  (`PrimitiveComponent.SetCustomDepthStencilValue` (`self.Addon`) 1))

(event `/Game/Blueprints/Interface/BPI_TakeItem.DeactiveHighlight`
  (`PrimitiveComponent.SetCustomDepthStencilValue` (`self.Addon`) 0)
  (for _array_element (`self.ActuTurret`)
    (`PrimitiveComponent.SetCustomDepthStencilValue` (`/Game/Blueprints/Turret/Blueprint/BP_Turret.Base` _array_element) 0)))

(event `/Game/Blueprints/Interface/BPI_HightLiteTarget.HightLiteTarget`
  (bind _outactors (`GameplayStatics.GetAllActorsOfClass` "/Game/Blueprints/Turret/Blueprint/BP_Turret.BP_Turret_C"))
  (bind _output_get (set `self.ActuTurret` _outactors))
  (for _array_element _output_get
    (if (not (`/Game/Blueprints/Turret/Blueprint/BP_Turret.b_IsActive` _array_element))
      (bind _widget (`/Game/Blueprints/Turret/Blueprint/BP_Turret.Widget` _array_element))
      (bind _aswg_ground_icon (cast `/Game/Blueprints/Arrow/wg_GroundIcon` (`WidgetComponent.GetWidget` _widget)))
      (`/Game/Blueprints/Arrow/wg_GroundIcon.ChangeImage` _aswg_ground_icon "/Game/Blueprints/Arrow/PictoCone.PictoCone")
      (`SceneComponent.SetVisibility` _widget true false)
      (`PrimitiveComponent.SetCustomDepthStencilValue` (`/Game/Blueprints/Turret/Blueprint/BP_Turret.Base` _array_element) 1))))

(event `self.Addon.OnComponentBeginOverlap`
  (params (OverlappedComponent :type "PrimitiveComponent Object Reference") (OtherActor :type "Actor Object Reference") (OtherComp :type "PrimitiveComponent Object Reference") (OtherBodyIndex :type Integer) (bFromSweep :type Boolean) (SweepResult :type "HitResult Structure (by ref)"))
  ;[1 0 0] Passe ( a modif )
  (if (> (`KismetMathLibrary.VSize` (`self.GetVelocity`)) 1.0)
    (if (not (== OtherActor (`self.ActuPlayer`)))
      (bind _asbp_player (cast `/Game/Blueprints/Player/Player/BP_Player` OtherActor))
      (bind _actorattach (`/Game/Blueprints/Player/Player/BP_Player.ActorAttach` _asbp_player))
      (if (not (== _actorattach self))
        (`KismetSystemLibrary.PrintString` (`KismetSystemLibrary.GetDisplayName` _actorattach))
        (if (not (`/Game/Blueprints/Player/Player/BP_Player.b_HaveItem` _asbp_player))
          (`/Game/Blueprints/Interface/BPI_TakeItem.TakeItem` _asbp_player))))))

(fn `CheckTurret`
  (locals (NewLocalVar :type "Float (single-precision)" :default 0.0))
  (bind _arrayturret (`self.ArrayTurret`))
  (bind _addon (`self.Addon`))
  (bind _returnvalue (`SceneComponent.K2_GetComponentLocation` (`self.Addon`)))
  (bind _output (`|GetArrayItem` _arrayturret))
  (if (not (`self.b_IsGrab`))
    (bind _outhits (`KismetSystemLibrary.SphereTraceMulti` _returnvalue _returnvalue 160.0 "TraceTypeQuery1"))
    (for _array_element _outhits
      (bind _asbp_turret (cast `/Game/Blueprints/Turret/Blueprint/BP_Turret` (`.HitActor` (`GameplayStatics.BreakHitResult` _array_element))))
      (`KismetArrayLibrary.Array_AddUnique` (`self.ArrayTurret`) _asbp_turret))
    (if (`KismetArrayLibrary.Array_IsEmpty` _arrayturret)
      _
      (elif (not (`/Game/Blueprints/Turret/Blueprint/BP_Turret.b_IsActive` _output))
        (`/Game/Blueprints/Turret/Blueprint/BP_Turret.AddStage ` _output (`SceneComponent.K2_GetComponentRotation` _addon) (`SceneComponent.K2_GetComponentLocation` _addon) (`self.AddonType`))
        (`self.K2_DestroyActor`)))))

(fn `GiveItemToDesk`
  (params (ActorTarget :type "Actor Object Reference"))
  (returns (Return :type Boolean))
  (return false))

(fn `SetUpAddon`
  (params (Value :type "Float (single-precision)"))
  (bind _returnvalue (`PrimitiveComponent.CreateDynamicMaterialInstance` (`self.Addon`) 0 "/Game/Assets/Materials/Mat/lambertBase.lambertBase" "None"))
  (`MaterialInstanceDynamic.SetScalarParameterValue` _returnvalue "ColorChoice" Value))

(fn `TakeItem`
  (params (Player :type "/Game/Blueprints/Player/Player/BP_Player Object Reference"))
  (returns (Return :type Boolean))
  (bind _creatorref (`self.CreatorRef`))
  (bind _widget (`/Game/Blueprints/Player/Player/BP_Player.Widget` (`self.ActuPlayer`)))
  (bind _output_get (set `self.ActuPlayer` Player))
  (bind _returnvalue (`KismetSystemLibrary.K2_SetTimer` _output_get "RotateWidget" 0.1 true))
  (set `self.ActuTimer` _returnvalue)
  (bind _aswg_icon (cast `/Game/Blueprints/Arrow/WG_Icon` (`WidgetComponent.GetWidget` _widget)))
  (`/Game/Blueprints/Arrow/WG_Icon.SetImage` _aswg_icon "/Game/Blueprints/Arrow/Picto_Cone3D.Picto_Cone3D")
  (`SceneComponent.SetVisibility` _widget true false)
  (`/Game/Blueprints/Player/Player/BP_Player.TakeItem` Player self)
  (`PrimitiveComponent.SetCollisionEnabled` (`self.Addon`) "NoCollision")
  (set `self.b_IsGrab` true)
  (`PrimitiveComponent.SetSimulatePhysics` (`self.Addon`) false)
  (`/Engine/EditorBlueprintResources/StandardMacros.IsValid` _creatorref
    (:`Is Valid`
      (`/Game/Blueprints/Machine/BP_Assembler.StopMovementAddon` _creatorref)
      (return true))
    (:`Is Not Valid`
      (return true))))

(fn `UserConstructionScript`
  (bind _addon (`self.Addon`))
  (switch `/Game/Blueprints/Enums/Enum_Addon` (`self.AddonType`)
    (:`NewEnumerator0`
      (`PrimitiveComponent.SetMaterial` _addon 0 "/Game/Assets/Kit/Texture/Range/M_Range.M_Range"))
    (:`NewEnumerator1`
      (`PrimitiveComponent.SetMaterial` _addon 0 "/Game/Assets/Kit/Texture/AttackSpeed/M_AtkSpeed.M_AtkSpeed"))
    (:`NewEnumerator2`
      (`PrimitiveComponent.SetMaterial` _addon 0 "/Game/Assets/Kit/Texture/AOE/M_AOE.M_AOE"))))