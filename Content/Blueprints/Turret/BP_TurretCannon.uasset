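; BP_TurretCannon is a carryable cannon that a player can pick up and throw to add to a turret.
; TakeItem hands it to the player and disables collision, while GiveItemToDesk always refuses.
; DettachItem restores physics, launches the cannon with the given velocity, then runs CheckTurret a second later.
; If not held, it sphere-traces for nearby BP_Turrets and destroys itself when the first accepts AddCannon.
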(event `/Game/Blueprints/Interface/BPI_TakeItem.DettachItem`
  (params (Impulse :type "Vector Structure"))
  (bind _cannon (`self.Cannon`))
  (`PrimitiveComponent.SetCollisionEnabled` _cannon "QueryAndPhysics")
  (`PrimitiveComponent.SetSimulatePhysics` _cannon true)
  (`PrimitiveComponent.SetPhysicsLinearVelocity` (`self.Cannon`) Impulse false "None")
  (set `self.b_IsGrab` false)
  (`KismetSystemLibrary.Delay` 1.0)
  (`self.CheckTurret`))

(fn `CheckTurret`
  (locals (NewLocalVar :type "Float (single-precision)" :default 0.0))
  (bind _arrayturret (`self.ArrayTurret`))
  (bind _returnvalue (`SceneComponent.K2_GetComponentLocation` (`self.Cannon`)))
  (if (not (`self.b_IsGrab`))
    (bind _outhits (`KismetSystemLibrary.SphereTraceMulti` _returnvalue _returnvalue 160.0 "TraceTypeQuery1"))
    (for _array_element _outhits
      (bind _asbp_turret (cast `/Game/Blueprints/Turret/BP_Turret` (`.HitActor` (`GameplayStatics.BreakHitResult` _array_element))))
      (`KismetArrayLibrary.Array_AddUnique` (`self.ArrayTurret`) _asbp_turret))
    (if (not (`KismetArrayLibrary.Array_IsEmpty` _arrayturret))
      (bind _return (`/Game/Blueprints/Turret/BP_Turret.Add Cannon` (`|GetArrayItem` _arrayturret)))
      (if _return
        (`self.K2_DestroyActor`)))))

(fn `GiveItemToDesk`
  (params (ActorTarget :type "Actor Object Reference"))
  (returns (Return :type Boolean))
  (return false))

(fn `TakeItem`
  (params (Player :type "/Game/Blueprints/Player/BP_Player Object Reference"))
  (returns (Return :type Boolean))
  (`/Game/Blueprints/Player/BP_Player.TakeItem` Player 0.0 self)
  (`PrimitiveComponent.SetCollisionEnabled` (`self.Cannon`) "NoCollision")
  (set `self.b_IsGrab` true)
  (return true))

(fn `UserConstructionScript`)