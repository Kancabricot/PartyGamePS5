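; BP_TurretSnap is a snap point that captures a single BP_Turret and pulls it into place.
; When the Base of a turret overlaps its Cube, and neither snap point nor turret is already taken, it flags both as occupied.
; It then zeroes the Base's physics velocity and uses a Timeline to lerp the Base from its captured location to the Cube's location.
; Nothing here clears those flags.
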(event `self.Cube.OnComponentBeginOverlap`
  (params (OverlappedComponent :type "PrimitiveComponent Object Reference") (OtherActor :type "Actor Object Reference") (OtherComp :type "PrimitiveComponent Object Reference") (OtherBodyIndex :type Integer) (bFromSweep :type Boolean) (SweepResult :type "HitResult Structure (by ref)"))
  (bind _asbp_turret (cast `/Game/Blueprints/Turret/BP_Turret` OtherActor))
  (bind _base (`/Game/Blueprints/Turret/BP_Turret.Base` _asbp_turret))
  (if (== OtherComp _base)
    (if (and (not (`self.b_HaveTurret`)) (not (`/Game/Blueprints/Turret/BP_Turret.b_IsSnaped` _asbp_turret)))
      (set `self.b_HaveTurret` true)
      (set `/Game/Blueprints/Turret/BP_Turret.b_IsSnaped` true _asbp_turret)
      (set `self.LocationBaseTemp` (`SceneComponent.K2_GetComponentLocation` _base))
      (`PrimitiveComponent.SetPhysicsLinearVelocity` _base (0.0 0.0 0.0) false "None")
      (bind (_direction _newtrack_0) (`Timeline|Timeline` :!via `PlayFromStart`)
        (:`Update`
          (`SceneComponent.K2_SetWorldLocation` _base (`KismetMathLibrary.VLerp` (`self.LocationBaseTemp`) (`SceneComponent.K2_GetComponentLocation` (`self.Cube`)) _newtrack_0) false false))))))

(fn `UserConstructionScript`)