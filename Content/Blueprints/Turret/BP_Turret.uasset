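; Modular turret that players build from addons, can pick up and throw once active, and that shoots enemies in range.
; Overlapping addons tween onto the base via timelines; the second adds a cannon whose meshes and stats come from the two types combined.
; When active, it yaws toward the first tracked enemy and fires bullets on a delay loop.
; A timeline destroys unfinished turrets, restarting whenever an addon arrives.
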(event `self.TriggerSnap.OnComponentBeginOverlap`
  (params (OverlappedComponent :type "PrimitiveComponent Object Reference") (OtherActor :type "Actor Object Reference") (OtherComp :type "PrimitiveComponent Object Reference") (OtherBodyIndex :type Integer) (bFromSweep :type Boolean) (SweepResult :type "HitResult Structure (by ref)"))
  ;[1 1 1] Event for snap
  (`self.SnapAddon` OtherActor))

(event `self.ReceiveBeginPlay`
  ;[1 1 1] Set life time
  (`Timeline|LifeTimeBase` :!label _label
    (:`Finished`
      (if (not (`self.b_IsActive`))
        (`self.K2_DestroyActor`)))))

(event `ResetLifeTimeBase`
  ;[1 1 1] Set life time
  (goto _label :!via `PlayFromStart`))

(event `AddStage`
  (params (WorldRotation :type "Rotator Structure") (WorldLocation :type "Vector Structure") (TargetAddonType :type "/Game/Blueprints/Enums/Enum_Addon Enum" :default "NewEnumerator0"))
  (bind _base (`self.Base`))
  (bind _addonarray (`self.AddonArray`))
  (bind _addonarray_2 (`self.AddonArray`))
  (bind _output (`|GetArrayItem` _addonarray_2 (`KismetArrayLibrary.Array_LastIndex` _addonarray_2)))
  ;[1 1 1] Add stage and snap it
  (`self.ResetLifeTimeBase`)
  (if (not (`self.b_HaveCannon`))
    (if (`KismetArrayLibrary.Array_IsEmpty` (`self.AddonArray`))
      (bind _returnvalue (`AddComponent|NODE_AddStaticMeshComponent-5` :`bManualAttachment` true))
      (bind _returnvalue_2 (`PrimitiveComponent.CreateDynamicMaterialInstance` _returnvalue 0 "/Game/Assets/Turret/Import/Mat/lambertBase.lambertBase" "None"))
      (`MaterialInstanceDynamic.SetScalarParameterValue` _returnvalue_2 "ColorChoice" (`self.SetMaterialColor` TargetAddonType))
      (bind (_direction _snapfirst) (`Timeline|MovementFirst` :!via `PlayFromStart`)
        (:`Update`
          (`SceneComponent.K2_SetWorldRotation` _returnvalue (`KismetMathLibrary.RLerp` WorldRotation (`SceneComponent.K2_GetComponentRotation` _base) _snapfirst) false false)
          (`SceneComponent.K2_SetWorldLocation` _returnvalue (`KismetMathLibrary.VLerp` WorldLocation (`SceneComponent.K2_GetComponentLocation` _base) _snapfirst) false false)
          (set `self.AddonType1` TargetAddonType))
        (:`Finished`
          (`SceneComponent.K2_AttachToComponent` _returnvalue (`self.Base`) "AddonSnap" "SnapToTarget" "SnapToTarget" "SnapToTarget" true)
          (`KismetArrayLibrary.Array_Add` (`self.AddonArray`) _returnvalue)))
      (else
        (bind _returnvalue_3 (`AddComponent|NODE_AddStaticMeshComponent-6` :`bManualAttachment` true))
        (bind _returnvalue_4 (`PrimitiveComponent.CreateDynamicMaterialInstance` _returnvalue_3 0 "/Game/Assets/Turret/Import/Mat/lambertBase.lambertBase" "None"))
        (`MaterialInstanceDynamic.SetScalarParameterValue` _returnvalue_4 "ColorChoice" (`self.SetMaterialColor` TargetAddonType))
        (bind (_direction_2 _snapfirst_2) (`Timeline|Timeline` :!via `PlayFromStart`)
          (:`Update`
            (`SceneComponent.K2_SetWorldRotation` _returnvalue_3 (`KismetMathLibrary.RLerp` WorldRotation (`SceneComponent.K2_GetComponentRotation` _output) _snapfirst_2) false false)
            (`SceneComponent.K2_SetWorldLocation` _returnvalue_3 (`KismetMathLibrary.VLerp` WorldLocation (+ (`SceneComponent.K2_GetComponentLocation` _output) (`KismetMathLibrary.MakeVector` 0.0 0.0 (.z (`.Max` (`StaticMeshComponent.GetLocalBounds` _output))))) _snapfirst_2) false false))
          (:`Finished`
            (`SceneComponent.K2_AttachToComponent` _returnvalue_3 (`|GetArrayItem` _addonarray (`KismetArrayLibrary.Array_LastIndex` _addonarray)) "AddonSnap" "KeepWorld" "KeepWorld" "KeepWorld" true)
            (`KismetArrayLibrary.Array_Add` (`self.AddonArray`) _returnvalue_3)
            (`self.Add Cannon`)
            (set `self.AddonType2` TargetAddonType)
            (`self.CreateCannon`)
            (`self.SetUpTurret`)))))))

(event `/Game/Blueprints/Interface/BPI_TakeItem.DettachItem`
  (params (Impulse :type "Vector Structure"))
  ;[1 1 1] Detach actor and throw it
  (`PrimitiveComponent.SetCollisionEnabled` (`self.Base`) "QueryAndPhysics")
  (`PrimitiveComponent.SetSimulatePhysics` (`self.Base`) true)
  (`PrimitiveComponent.SetPhysicsLinearVelocity` (`self.Base`) Impulse false "None")
  (`KismetSystemLibrary.Delay` 1.0)
  (set `self.b_IsGrab` true))

(event `self.ReceiveTick`
  (params (DeltaSeconds :type "Float (single-precision)"))
  (bind _output (`|GetArrayItem` (`self.ArrayOfTarget`)))
  (bind (_returnvalue_roll _returnvalue_pitch _returnvalue_yaw) (`KismetMathLibrary.BreakRotator` (`KismetMathLibrary.FindLookAtRotation` (`SceneComponent.K2_GetComponentLocation` (`self.Base`)) (`SceneComponent.K2_GetComponentLocation` (`Actor.RootComponent` _output)))))
  ;[1 1 1] Follow ennemy
  (if (`self.b_IsActive`)
    (`/Engine/EditorBlueprintResources/StandardMacros.IsValid` _output
      (:`Is Valid`
        (`SceneComponent.K2_SetWorldRotation` (`self.Base`) (`KismetMathLibrary.MakeRotator` 0.0 0.0 _returnvalue_yaw) false false)))))

(event `SpawnCatch`
  ;[1 1 1] In spawn delete collision
  (`PrimitiveComponent.SetCollisionEnabled` (`self.Base`) "NoCollision"))

(event `StartLifeTime`
  ;[1 1 1] Life time
  (`KismetSystemLibrary.Delay` 99999.0)
  (`self.K2_DestroyActor`))

(event `self.SphereView.OnComponentBeginOverlap`
  (params (OverlappedComponent :type "PrimitiveComponent Object Reference") (OtherActor :type "Actor Object Reference") (OtherComp :type "PrimitiveComponent Object Reference") (OtherBodyIndex :type Integer) (bFromSweep :type Boolean) (SweepResult :type "HitResult Structure (by ref)"))
  ;[1 1 1] Get Target
  (if (`self.b_IsActive`)
    (bind _asbp_ennemy (cast `/Game/Blueprints/Ennemie/BP_Ennemy` OtherActor))
    (if (== (`|GetArrayItem` (`self.ArrayOfTarget`)) null)
      (`self.ShootRiffle`))
    (`KismetArrayLibrary.Array_Add` (`self.ArrayOfTarget`) _asbp_ennemy)))

(event `DelayShoot`
  ;[1 1 1] Delay for shoot (put set timer by event)
  (`KismetSystemLibrary.Delay` (`self.FireRate`))
  (`self.ShootRiffle`))

(event `self.SphereView.OnComponentEndOverlap`
  (params (OverlappedComponent :type "PrimitiveComponent Object Reference") (OtherActor :type "Actor Object Reference") (OtherComp :type "PrimitiveComponent Object Reference") (OtherBodyIndex :type Integer))
  ;[1 1 1] Remove target
  (if (`self.b_IsActive`)
    (for _array_element (`self.ArrayOfTarget`) :!label _label_2
      (if (== _array_element OtherActor)
        (`KismetArrayLibrary.Array_RemoveItem` (`self.ArrayOfTarget`) _array_element)
        (`self.BreakLoop`)))))

(event `BreakLoop`
  ;[1 1 1] Remove target
  (goto _label_2 :!via `Break`))

(fn `Add Cannon`
  (returns (Return :type Boolean))
  (bind _addonarray (`self.AddonArray`))
  (bind _addonarray_2 (`self.AddonArray`))
  (bind _output (`|GetArrayItem` _addonarray (`KismetArrayLibrary.Array_LastIndex` _addonarray)))
  (if (not (`self.b_HaveCannon`))
    (if (not (`KismetArrayLibrary.Array_IsEmpty` (`self.AddonArray`)))
      (bind _returnvalue (`AddComponent|NODE_AddStaticMeshComponent-4` :`RelativeTransform` (`KismetMathLibrary.MakeTransform` (`KismetMathLibrary.MakeVector` 0.0 0.0 (+ (.z (.location (`SceneComponent.GetRelativeTransform` _output))) (.z (`.Max` (`StaticMeshComponent.GetLocalBounds` _output))))))))
      (`SceneComponent.K2_AttachToComponent` _returnvalue (`|GetArrayItem` _addonarray_2 (`KismetArrayLibrary.Array_LastIndex` _addonarray_2)) "AddonSnap" "SnapToTarget" "SnapToTarget" "SnapToTarget" true)
      (bind _output_get (set `self.CannonBase` _returnvalue))
      (bind _returnvalue_2 (`AddComponent|NODE_AddStaticMeshComponent-7` :`RelativeTransform` (`KismetMathLibrary.MakeTransform` (0.0 0.0 0.0))))
      (`SceneComponent.K2_AttachToComponent` _returnvalue_2 _output_get "None" "SnapToTarget" "SnapToTarget" "SnapToTarget" true)
      (set `self.CannonCannon` _returnvalue_2)
      (`SceneComponent.K2_AttachToComponent` (`self.Bullet`) _returnvalue_2 "CannonSocket" "SnapToTarget" "SnapToTarget" "SnapToTarget" true)
      (set `self.b_HaveCannon` true)
      (`self.SetUpTurret`)
      (return true))
    (else
      (return false))))

(fn `CreateCannon`
  (switch `/Game/Blueprints/Enums/Enum_Addon` (`self.AddonType1`)
    (:`NewEnumerator0`
      (switch `/Game/Blueprints/Enums/Enum_Addon` (`self.AddonType2`)
        (:`NewEnumerator0`
          (`KismetSystemLibrary.PrintString` "Sniper")
          (set `self.TurretType` "NewEnumerator4")
          (set `self.Damage` 25.0)
          (set `self.Radius` 700.0)
          (set `self.FireRate` 1.75)
          (`StaticMeshComponent.SetStaticMesh` (`self.CannonBase`) "/Game/Assets/Turret/Sniper/Tower_BaseSnipe.Tower_BaseSnipe")
          (`StaticMeshComponent.SetStaticMesh` (`self.CannonCannon`) "/Game/Assets/Turret/Sniper/Tower_SnipeCanon.Tower_SnipeCanon"))
        (:`NewEnumerator1`
          (`KismetSystemLibrary.PrintString` "Riffle")
          (set `self.TurretType` "NewEnumerator3")
          (set `self.Damage` 3.0)
          (set `self.Radius` 400.0)
          (set `self.FireRate` 0.25)
          (`StaticMeshComponent.SetStaticMesh` (`self.CannonBase`) "/Game/Assets/Turret/Riffle/Tower_MitrailBase.Tower_MitrailBase")
          (`StaticMeshComponent.SetStaticMesh` (`self.CannonCannon`) "/Game/Assets/Turret/Riffle/Tower_MitrailCanon.Tower_MitrailCanon"))
        (:`NewEnumerator2`
          (`KismetSystemLibrary.PrintString` "Mortar")
          (set `self.TurretType` "NewEnumerator5")
          (set `self.Damage` 35.0)
          (set `self.Radius` 800.0)
          (set `self.FireRate` 3.0)
          (`StaticMeshComponent.SetStaticMesh` (`self.CannonBase`) "/Game/Assets/Turret/Mortar/Tower_MortierBase.Tower_MortierBase")
          (`StaticMeshComponent.SetStaticMesh` (`self.CannonCannon`) "/Game/Assets/Turret/Mortar/Tower_MortierCanon.Tower_MortierCanon"))))
    (:`NewEnumerator1`
      (switch `/Game/Blueprints/Enums/Enum_Addon` (`self.AddonType2`)
        (:`NewEnumerator0`
          (`KismetSystemLibrary.PrintString` "Riffle")
          (set `self.TurretType` "NewEnumerator3")
          (set `self.Damage` 3.0)
          (set `self.Radius` 400.0)
          (set `self.FireRate` 0.25)
          (`StaticMeshComponent.SetStaticMesh` (`self.CannonBase`) "/Game/Assets/Turret/Riffle/Tower_MitrailBase.Tower_MitrailBase")
          (`StaticMeshComponent.SetStaticMesh` (`self.CannonCannon`) "/Game/Assets/Turret/Riffle/Tower_MitrailCanon.Tower_MitrailCanon"))
        (:`NewEnumerator1`
          (`KismetSystemLibrary.PrintString` "MiniGun")
          (set `self.TurretType` "NewEnumerator2")
          (set `self.Damage` 2.0)
          (set `self.Radius` 300.0)
          (set `self.FireRate` 0.05)
          (`StaticMeshComponent.SetStaticMesh` (`self.CannonBase`) "/Game/Assets/Turret/MachineGun/Tower_MiniGunBase.Tower_MiniGunBase")
          (`StaticMeshComponent.SetStaticMesh` (`self.CannonCannon`) "/Game/Assets/Turret/MachineGun/Tower_MiniGunCanon.Tower_MiniGunCanon"))
        (:`NewEnumerator2`
          (`KismetSystemLibrary.PrintString` "Rocket")
          (set `self.TurretType` "NewEnumerator1")
          (set `self.Damage` 8.0)
          (set `self.Radius` 300.0)
          (set `self.FireRate` 1.0)
          (`StaticMeshComponent.SetStaticMesh` (`self.CannonBase`) "/Game/Assets/Turret/Rocket/Tower_RocketBase.Tower_RocketBase")
          (`StaticMeshComponent.SetStaticMesh` (`self.CannonCannon`) "/Game/Assets/Turret/Rocket/Tower_RocketCanon.Tower_RocketCanon"))))
    (:`NewEnumerator2`
      (switch `/Game/Blueprints/Enums/Enum_Addon` (`self.AddonType2`)
        (:`NewEnumerator0`
          (`KismetSystemLibrary.PrintString` "Mortar")
          (set `self.TurretType` "NewEnumerator5")
          (set `self.Damage` 35.0)
          (set `self.Radius` 800.0)
          (set `self.FireRate` 3.0)
          (`StaticMeshComponent.SetStaticMesh` (`self.CannonBase`) "/Game/Assets/Turret/Mortar/Tower_MortierBase.Tower_MortierBase")
          (`StaticMeshComponent.SetStaticMesh` (`self.CannonCannon`) "/Game/Assets/Turret/Mortar/Tower_MortierCanon.Tower_MortierCanon"))
        (:`NewEnumerator1`
          (`KismetSystemLibrary.PrintString` "Rocket")
          (set `self.TurretType` "NewEnumerator1")
          (set `self.Damage` 8.0)
          (set `self.Radius` 300.0)
          (set `self.FireRate` 1.0)
          (`StaticMeshComponent.SetStaticMesh` (`self.CannonBase`) "/Game/Assets/Turret/Rocket/Tower_RocketBase.Tower_RocketBase")
          (`StaticMeshComponent.SetStaticMesh` (`self.CannonCannon`) "/Game/Assets/Turret/Rocket/Tower_RocketCanon.Tower_RocketCanon"))
        (:`NewEnumerator2`
          (`KismetSystemLibrary.PrintString` "Flame")
          (set `self.TurretType` "NewEnumerator0")
          (set `self.Damage` 2.0)
          (set `self.Radius` 250.0)
          (set `self.FireRate` 0.001)
          (`StaticMeshComponent.SetStaticMesh` (`self.CannonBase`) "/Game/Assets/Turret/Flame/Tower_LanceFlammeBase.Tower_LanceFlammeBase")
          (`StaticMeshComponent.SetStaticMesh` (`self.CannonCannon`) "/Game/Assets/Turret/Flame/Tower_LanceFlammeCanon.Tower_LanceFlammeCanon"))))))

(fn `GiveItemToDesk`
  (params (ActorTarget :type "Actor Object Reference"))
  (returns (Return :type Boolean))
  (return false))

(fn `SetMaterialColor`
  (params (AddonType :type "/Game/Blueprints/Enums/Enum_Addon Enum" :default "NewEnumerator0"))
  (returns (Color :type "Float (double-precision)"))
  (switch `/Game/Blueprints/Enums/Enum_Addon` AddonType
    (:`NewEnumerator0`
      (return 1.0))
    (:`NewEnumerator1`
      (return 0.0))
    (:`NewEnumerator2`
      (return 2.0))))

(fn `SetUpTurret`
  (`SphereComponent.SetSphereRadius` (`self.SphereView`) (`self.Radius`) true)
  (set `self.b_IsActive` true)
  (`self.StartLifeTime`))

(fn `ShootRiffle`
  (bind (_returnvalue_location _returnvalue_rotation) (`KismetMathLibrary.BreakTransform` (`SceneComponent.K2_GetComponentToWorld` (`self.Bullet`))))
  (`/Engine/EditorBlueprintResources/StandardMacros.IsValid` (`|GetArrayItem` (`self.ArrayOfTarget`))
    (:`Is Valid`
      (`|SpawnActorFromClass` "/Game/Blueprints/Turret/BP_Bullet.BP_Bullet_C" (`KismetMathLibrary.MakeTransform` _returnvalue_location _returnvalue_rotation) "Undefined" "MultiplyWithRoot" null (`self.Damage`) null)
      (`self.DelayShoot`))
    (:`Is Not Valid`
      (`self.DelayShoot`))))

(fn `SnapAddon`
  (params (Object :type "Object Object Reference"))
  (locals (Temp :type "/Game/Blueprints/Turret/Struc_Turret Structure"))
  (bind _asbp_turret_addon (cast `/Game/Blueprints/Turret/BP_TurretAddon` Object)
    (:`then`
      (set `local.Temp` (`/Game/Blueprints/Turret/BP_TurretAddon.Struc_Addon` _asbp_turret_addon))
      (bind (_returnvalue_location _returnvalue_rotation) (`KismetMathLibrary.BreakTransform` (`SceneComponent.K2_GetComponentToWorld` (`/Game/Blueprints/Turret/BP_TurretAddon.Addon` _asbp_turret_addon))))
      (`self.AddStage ` _returnvalue_rotation _returnvalue_location (`/Game/Blueprints/Turret/BP_TurretAddon.AddonType` _asbp_turret_addon))
      (`self.K2_DestroyActor` _asbp_turret_addon))
    (:`CastFailed`
      (bind _asbp_turret_cannon (cast `/Game/Blueprints/Turret/BP_TurretCannon` Object))
      (`self.Add Cannon`)
      (`self.K2_DestroyActor` _asbp_turret_cannon))))

(fn `TakeItem`
  (params (Player :type "/Game/Blueprints/Player/BP_Player Object Reference"))
  (returns (Return :type Boolean))
  (if (`self.b_IsActive`)
    (`/Game/Blueprints/Player/BP_Player.TakeItem` Player 0.0 self)
    (`PrimitiveComponent.SetCollisionEnabled` (`self.Base`) "NoCollision")
    (set `self.b_IsGrab` false)
    (return true)))

(fn `UserConstructionScript`)