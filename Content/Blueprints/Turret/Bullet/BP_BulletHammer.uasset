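; BP_BulletHammer is a turret hammer "bullet" that stays attached to the cannon's socket and strikes a target with damage and a slow.
; AnimHit stretches the handle by target distance, then a timeline swings it through a rotation.
; When the forward swing finishes, it applies damage, slows the still-valid target using PDAEffect values, and reverses the swing.
; Tick keeps the head sphere on the handle's HammerPoint socket.
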(event `self.ReceiveBeginPlay`
  (`self.K2_AttachToComponent` (`self.TurretCanon`) "Canon" "SnapToTarget" "SnapToTarget" "SnapToTarget" false))

(event `self.ReceiveTick`
  (params (DeltaSeconds :type "Float (single-precision)"))
  (`SceneComponent.K2_SetRelativeLocation` (`self.DefaultSceneRoot`) (0.0 0.0 0.0) false false)
  (`SceneComponent.K2_SetWorldLocation` (`self.Sphere`) (`SceneComponent.GetSocketLocation` (`self.HammerHandle`) "HammerPoint") false true)
  (`SceneComponent.K2_SetRelativeRotation` (`self.Sphere`) (`SceneComponent.RelativeRotation` (`self.HammerHandle`)) false false))

(event `AnimHit`
  (params (Target :type "/Game/Blueprints/Enemie/Blueprint/BP_Enemie Object Reference"))
  (`SceneComponent.SetRelativeScale3D` (`self.HammerHandle`) (`KismetMathLibrary.MakeVector` 6.0 6.0 (/ (`self.GetDistanceTo` Target) 2.0)))
  (bind (_direction _hitmovement) (`Timeline|HitMovement` :!via `PlayFromStart` :!label _label)
    (:`Update`
      (`SceneComponent.K2_SetRelativeRotation` (`self.HammerHandle`) (`KismetMathLibrary.RLerp` (struct) (struct :`Pitch` -90.0) _hitmovement) false false))
    (:`Finished`
      (if (`|EnumEquality` _direction "Forward")
        (`self.Attack` Target)
        (`self.ReverseAnimHit`)))))

(event `ReverseAnimHit`
  (goto _label :!via `ReverseFromEnd`))

(fn `Attack`
  (params (Target :type "/Game/Blueprints/Enemie/Blueprint/BP_Enemie Object Reference"))
  (bind _pda_effect (`self.PDA_Effect`))
  (`/Game/Blueprints/Enemie/Blueprint/BP_Enemie.TakeDamage` Target (`self.Damage`))
  (`/Engine/EditorBlueprintResources/StandardMacros.IsValid` Target
    (:`Is Valid`
      (`/Game/Blueprints/Enemie/Blueprint/BP_Enemie.Slow` Target (`/Game/Blueprints/Turret/Structure/PDA_Effect.%slowHammer` _pda_effect) (`/Game/Blueprints/Turret/Structure/PDA_Effect.SlowDurationHammer` _pda_effect)))))

(fn `UserConstructionScript`
  (`parent.UserConstructionScript`))