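; Turret bullet actor that acts as a continuous beam, hitting one enemy at a time with damage that ramps up.
; A trigger sphere sized to the turret's range queues enemies, and a looping Hit timer runs only while the queue is occupied.
; Each hit damages the first enemy, with a debug line trace from the cannon, raising damage toward a data-asset cap.
; Damage resets if the first target changes during the hit.
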(event `self.ReceiveBeginPlay`
  (bind _turretref (`self.TurretRef`))
  (set `self.Damage` (`/Game/Blueprints/Turret/Structure/PDA_Effect.DamageBase` (`self.PDA_Effect`)))
  (bind _returnvalue (`KismetSystemLibrary.K2_SetTimer` null "Hit" (`/Game/Blueprints/Turret/Structure/PDA_Effect.HitSecond` (`self.PDA_Effect`)) true))
  (bind _output_get (set `self.TimerHit` _returnvalue))
  (`KismetSystemLibrary.K2_PauseTimerHandle` _output_get)
  (`SphereComponent.SetSphereRadius` (`self.TriggerEnemy`) (`|GetArrayItem` (`/Game/Blueprints/Turret/Structure/PDA_TurretType.Range` (`/Game/Blueprints/Turret/Blueprint/BP_Turrets.DA_TurretType` _turretref)) (`/Game/Blueprints/Turret/Blueprint/BP_Turrets.IndexTurret` _turretref)) true))

(event `self.TriggerEnemy.OnComponentBeginOverlap`
  (params (OverlappedComponent :type "PrimitiveComponent Object Reference") (OtherActor :type "Actor Object Reference") (OtherComp :type "PrimitiveComponent Object Reference") (OtherBodyIndex :type Integer) (bFromSweep :type Boolean) (SweepResult :type "HitResult Structure (by ref)"))
  (bind _asbp_enemie (cast `/Game/Blueprints/Enemie/Blueprint/BP_Enemie` OtherActor))
  (if (and (== (`/Game/Blueprints/Enemie/Blueprint/BP_Enemie.Box1` _asbp_enemie) OtherComp) (not (`KismetArrayLibrary.Array_Contains` (`self.TargetArray`) _asbp_enemie)))
    (`KismetArrayLibrary.Array_Add` (`self.TargetArray`) _asbp_enemie)
    (if (== (`KismetArrayLibrary.Array_Length` (`self.TargetArray`)) 1)
      (`KismetSystemLibrary.K2_UnPauseTimerHandle` (`self.TimerHit`)))))

(event `self.TriggerEnemy.OnComponentEndOverlap`
  (params (OverlappedComponent :type "PrimitiveComponent Object Reference") (OtherActor :type "Actor Object Reference") (OtherComp :type "PrimitiveComponent Object Reference") (OtherBodyIndex :type Integer))
  (bind _targetarray (`self.TargetArray`))
  (bind _asbp_enemie (cast `/Game/Blueprints/Enemie/Blueprint/BP_Enemie` OtherActor))
  (if (== (`/Game/Blueprints/Enemie/Blueprint/BP_Enemie.Box1` _asbp_enemie) OtherComp)
    (`KismetArrayLibrary.Array_RemoveItem` _targetarray _asbp_enemie)
    (if (`KismetArrayLibrary.Array_IsEmpty` _targetarray)
      (`KismetSystemLibrary.K2_PauseTimerHandle` (`self.TimerHit`)))))

(fn `Get Enemy`
  (params (TargetArray :type "Array of /Game/Blueprints/Enemie/Blueprint/BP_Enemie Object Reference (by ref)"))
  (for _array_element TargetArray
    (if (not (`KismetArrayLibrary.Array_Contains` (`self.TargetArray`) _array_element))
      (`KismetArrayLibrary.Array_Add` (`self.TargetArray`) _array_element)))
  (if (== (`KismetArrayLibrary.Array_Length` (`self.TargetArray`)) 1)
    (`KismetSystemLibrary.K2_UnPauseTimerHandle` (`self.TimerHit`))))

(fn `Hit`
  (bind _pda_effect (`self.PDA_Effect`))
  (bind _output (`|GetArrayItem` (`self.TargetArray`)))
  (bind _returnvalue (+ (`self.Damage`) (`/Game/Blueprints/Turret/Structure/PDA_Effect.DamageAugmentation` _pda_effect)))
  (`/Engine/EditorBlueprintResources/StandardMacros.IsValid` _output
    (:`Is Valid`
      (set `self.Target` _output)
      (`KismetSystemLibrary.LineTraceSingle` :`Start` (`SceneComponent.GetSocketLocation` (`/Game/Blueprints/Turret/Blueprint/BP_Turrets.Cannon` (`self.TurretRef`)) "Canon") :`End` (`self.K2_GetActorLocation` _output) :`TraceChannel` "TraceTypeQuery1" :`DrawDebugType` "ForDuration" :`DrawTime` 0.1)
      (`/Game/Blueprints/Enemie/Blueprint/BP_Enemie.TakeDamage` _output (`self.Damage`))
      (if (== (`self.Target`) (`|GetArrayItem` (`self.TargetArray`)))
        (if (< _returnvalue (`/Game/Blueprints/Turret/Structure/PDA_Effect.MaxDamage` (`self.PDA_Effect`)))
          (set `self.Damage` _returnvalue))
        (else
          (set `self.Damage` (`/Game/Blueprints/Turret/Structure/PDA_Effect.DamageBase` _pda_effect)))))))

(fn `UserConstructionScript`
  (`parent.UserConstructionScript`))