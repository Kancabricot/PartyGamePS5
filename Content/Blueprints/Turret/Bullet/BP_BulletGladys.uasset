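; Bullet actor for the Gladys turret, a rail-shaped laser that records the enemies it touches.
; On BeginPlay it scales GladysRail by the effect data's radius and rail length, then sets its lifespan to the laser time.
; Rail overlaps add unique BP_Enemie actors to EnemyRef when Box1 matches OverlappedComponent, the rail's own component rather than the other one.
; End overlap only casts, and no damage is applied here.
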(event `self.ReceiveBeginPlay`
  (bind _pda_effect (`self.PDA_Effect`))
  (bind _radius (`/Game/Blueprints/Turret/Structure/PDA_Effect.Radius` _pda_effect))
  (`SceneComponent.SetRelativeScale3D` (`self.GladysRail`) (`KismetMathLibrary.MakeVector` _radius _radius (`/Game/Blueprints/Turret/Structure/PDA_Effect.LenghtRail` _pda_effect)))
  (`self.SetLifeSpan` (`/Game/Blueprints/Turret/Structure/PDA_Effect.LaserTime` (`self.PDA_Effect`))))

(event `self.GladysRail.OnComponentBeginOverlap`
  (params (OverlappedComponent :type "PrimitiveComponent Object Reference") (OtherActor :type "Actor Object Reference") (OtherComp :type "PrimitiveComponent Object Reference") (OtherBodyIndex :type Integer) (bFromSweep :type Boolean) (SweepResult :type "HitResult Structure (by ref)"))
  (`KismetSystemLibrary.PrintString` "Hello")
  (bind _asbp_enemie (cast `/Game/Blueprints/Enemie/Blueprint/BP_Enemie` OtherActor))
  (if (and (== (`/Game/Blueprints/Enemie/Blueprint/BP_Enemie.Box1` _asbp_enemie) OverlappedComponent) (not (`KismetArrayLibrary.Array_Contains` (`self.EnemyRef`) _asbp_enemie)))
    (`KismetArrayLibrary.Array_Add` (`self.EnemyRef`) _asbp_enemie)))

(event `self.GladysRail.OnComponentEndOverlap`
  (params (OverlappedComponent :type "PrimitiveComponent Object Reference") (OtherActor :type "Actor Object Reference") (OtherComp :type "PrimitiveComponent Object Reference") (OtherBodyIndex :type Integer))
  (cast `/Game/Blueprints/Enemie/Blueprint/BP_Enemie` OtherActor))

(fn `UserConstructionScript`
  (`parent.UserConstructionScript`))