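; BP_BulletTesla is a turret bullet that fires chain lightning, stunning and damaging enemies in succession.
; Tesla draws a Niagara beam and hit effect to the target, then schedules CheckAnotherEnemy after a short delay.
; That function sphere-traces for the nearest unstunned enemy not already hit, applies stun and damage to the current target, then jumps onward.
; The actor destroys itself when jumps run out or no new target is found.
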(event `self.ReceiveBeginPlay`
  (set `self.LastTargetPos` (`self.K2_GetActorLocation` (`self.Target`)))
  (`self.Tesla`))

(fn `CheckAnotherEnemy`
  (locals (Distance :type "Float (single-precision)" :default 99999997952.0) (TargetTemp :type "/Game/Blueprints/Enemie/Blueprint/BP_Enemie Object Reference"))
  (bind _target (`self.Target`))
  (bind _lasttargetpos (`self.LastTargetPos`))
  (bind _target_2 (`self.Target`))
  (bind _outhits (`KismetSystemLibrary.SphereTraceMultiForObjects` :`Start` _lasttargetpos :`End` _lasttargetpos :`Radius` (`/Game/Blueprints/Turret/Structure/PDA_Effect.RadiusTesla` (`self.PDA_Effect`)) :`ObjectTypes` (`|MakeArray` "ObjectTypeQuery7" :!type "EObjectTypeQuery Enum") :`DrawDebugType` (`/Game/Blueprints/Turret/Structure/PDA_Effect.Draw Debug Type Tesla` (`self.PDA_Effect`)) :`DrawTime` 1.0))
  (for _array_element _outhits
    (bind _asbp_enemie (cast `/Game/Blueprints/Enemie/Blueprint/BP_Enemie` (`.HitActor` (`GameplayStatics.BreakHitResult` _array_element))))
    (`/Engine/EditorBlueprintResources/StandardMacros.IsValid` _asbp_enemie
      (:`Is Valid`
        (`/Engine/EditorBlueprintResources/StandardMacros.IsValid` _target
          (:`Is Valid`
            (bind _returnvalue (`self.GetDistanceTo` _target _asbp_enemie))
            (bind _returnvalue_2 (< _returnvalue (`local.Distance`)))
            (bind _returnvalue_3 (not (`/Game/Blueprints/Enemie/Blueprint/BP_Enemie.b_IsStun` _asbp_enemie)))
            (if (and (not (== _asbp_enemie _target)) _returnvalue_2 _returnvalue_3)
              (if (not (`KismetArrayLibrary.Array_Contains` (`self.EnemyStunArray`) _asbp_enemie)) :!label _label
                (set `local.TargetTemp` _asbp_enemie)
                (set `local.Distance` _returnvalue))))
          (:`Is Not Valid`
            (if (and _returnvalue_2 _returnvalue_3)
              (goto _label)))))))
  (set `self.LastTargetPos` (`self.K2_GetActorLocation` _target_2))
  (`KismetArrayLibrary.Array_Add` (`self.EnemyStunArray`) _target_2)
  (`/Game/Blueprints/Enemie/Blueprint/BP_Enemie.Stun` _target_2 (`/Game/Blueprints/Turret/Structure/PDA_Effect.TeslaStunTimer` (`self.PDA_Effect`)))
  (`/Game/Blueprints/Enemie/Blueprint/BP_Enemie.TakeDamage` _target_2 (`self.Damage`))
  (if (or (== (`self.LastTarget`) (`local.TargetTemp`)) (== (`local.TargetTemp`) null))
    (`self.K2_DestroyActor`)
    (else
      (set `self.LastTarget` (`self.Target`))
      (set `self.Target` (`local.TargetTemp`))
      (`self.Tesla`))))

(fn `Tesla`
  (bind _returnvalue (`self.K2_GetActorLocation` (`self.Target`)))
  (bind _output_get (set `self.nbPossibleShoot` (- (`self.nbPossibleShoot`) 1)))
  (if (< _output_get 0)
    (`self.K2_DestroyActor`)
    (else
      (bind _returnvalue_2 (`NiagaraFunctionLibrary.SpawnSystemAtLocation` "/Game/VFX/VFX/Turrets/Tesla/Ns_Tesla.Ns_Tesla"))
      (`NiagaraComponent.SetNiagaraVariableFloat` _returnvalue_2 "BeamWidthMultiplier" 4.0)
      (`/Engine/EditorBlueprintResources/StandardMacros.IsValid` (`self.LastTarget`)
        (:`Is Valid`
          (`NiagaraComponent.SetNiagaraVariableVec3` _returnvalue_2 "BeamStartPoint" (`self.LastTargetPos`)))
        (:`Is Not Valid`
          (`NiagaraComponent.SetNiagaraVariableVec3` _returnvalue_2 "BeamStartPoint" (`self.K2_GetActorLocation`))))
      (`NiagaraComponent.SetNiagaraVariableVec3` _returnvalue_2 "BeamendPoint" _returnvalue)
      (`NiagaraFunctionLibrary.SpawnSystemAtLocation` "/Game/VFX/VFX/Turrets/Tesla/Hit/NS_TeslaHit.NS_TeslaHit" _returnvalue)
      (`KismetSystemLibrary.K2_SetTimer` null "CheckAnotherEnemy" 0.2))))

(fn `UserConstructionScript`
  (`parent.UserConstructionScript`))