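; Cannon turret projectile that homes in on its target enemy and deals explosive area damage on impact.
; BeginPlay sets projectile speed and homing, then spawns Niagara muzzle and bullet effects.
; Overlapping the target applies direct damage and a hit effect, then a debug-drawn sphere trace damages each other nearby enemy once, using PDAEffect radius and damage.
; Other enemies it overlaps are not hit directly, and it destroys itself after striking the target.
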(event `self.ReceiveBeginPlay`
  (bind _projectilemovement (`self.ProjectileMovement`))
  (bind _output_get (set `ProjectileMovementComponent.InitialSpeed` (`self.BulletSpeed`) _projectilemovement))
  (set `ProjectileMovementComponent.MaxSpeed` _output_get _projectilemovement)
  (set `ProjectileMovementComponent.HomingTargetComponent` (`Character.Mesh` (`self.Target`)) (`self.ProjectileMovement`))
  (`NiagaraFunctionLibrary.SpawnSystemAtLocation` "/Game/VFX/VFX/Turrets/Canon/MuzzleFlash/NS_CanonMF.NS_CanonMF" (`SceneComponent.K2_GetComponentLocation` (`/Game/Blueprints/Turret/Blueprint/BP_Turrets.Scene` (`self.TurretRef`))))
  (bind _returnvalue (`NiagaraFunctionLibrary.SpawnSystemAtLocation` "/Game/VFX/VFX/Turrets/Canon/NS_CanonBullet.NS_CanonBullet" (`SceneComponent.K2_GetComponentLocation` (`self.CanonBallTemp`)) (`KismetMathLibrary.FindLookAtRotation` (`self.K2_GetActorLocation`) (`self.K2_GetActorLocation` (`self.Target`)))))
  (set `self.BulletVfxRef` _returnvalue))

(event `self.CanonBallTemp.OnComponentBeginOverlap`
  (params (OverlappedComponent :type "PrimitiveComponent Object Reference") (OtherActor :type "Actor Object Reference") (OtherComp :type "PrimitiveComponent Object Reference") (OtherBodyIndex :type Integer) (bFromSweep :type Boolean) (SweepResult :type "HitResult Structure (by ref)"))
  (bind _explosionlocationtemp (`self.ExplosionLocationTemp`))
  (bind _asbp_enemie (cast `/Game/Blueprints/Enemie/Blueprint/BP_Enemie` OtherActor))
  (set `self.ExplosionLocationTemp` (`SceneComponent.K2_GetComponentLocation` (`Character.Mesh` _asbp_enemie)))
  (if (== _asbp_enemie (`self.Target`))
    (set `self.EnemyHit` _asbp_enemie)
    (`/Game/Blueprints/Enemie/Blueprint/BP_Enemie.TakeDamage` _asbp_enemie (`self.Damage`))
    (`NiagaraFunctionLibrary.SpawnSystemAtLocation` "/Game/VFX/VFX/Turrets/Canon/Hit/NS_CanonHit.NS_CanonHit" (`self.K2_GetActorLocation`))
    (`ActorComponent.Deactivate` (`self.BulletVfxRef`))
    (bind _outhits (`KismetSystemLibrary.SphereTraceMultiForObjects` :`Start` _explosionlocationtemp :`End` _explosionlocationtemp :`Radius` (`/Game/Blueprints/Turret/Structure/PDA_Effect.RadiousExplosion` (`self.PDA_Effect`)) :`ObjectTypes` (`|MakeArray` "ObjectTypeQuery7" :!type "EObjectTypeQuery Enum") :`DrawDebugType` "ForDuration"))
    (for _array_element _outhits
      (bind _asbp_enemie_2 (cast `/Game/Blueprints/Enemie/Blueprint/BP_Enemie` (`.HitActor` (`GameplayStatics.BreakHitResult` _array_element))))
      (if (!= _asbp_enemie_2 (`self.EnemyHit`))
        (if (not (`KismetArrayLibrary.Array_Contains` (`self.EnemyHitArray`) _asbp_enemie_2))
          (`KismetArrayLibrary.Array_Add` (`self.EnemyHitArray`) _asbp_enemie_2)
          (`/Game/Blueprints/Enemie/Blueprint/BP_Enemie.TakeDamage` _asbp_enemie_2 (`/Game/Blueprints/Turret/Structure/PDA_Effect.DamageExplosion` (`self.PDA_Effect`))))))
    (`self.K2_DestroyActor`)))

(fn `UserConstructionScript`
  (`parent.UserConstructionScript`))