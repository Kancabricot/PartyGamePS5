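; BP_MortarBullet is a mortar turret projectile that deals area damage to enemies.
; Half a second after spawning, it zeroes its velocity and turns on ProjectileMovement homing toward HomingTarget.
; Overlapping anything but a BP_Turret runs a multi-sphere trace of RadiusAOE at the bullet and applies Damage to BP_Enemie hits.
; It then spawns a Niagara explosion and destroys itself, with debug trace drawing and name printing left on.
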(event `self.ReceiveBeginPlay`
  (`KismetSystemLibrary.Delay` 0.5)
  (`ProjectileMovementComponent.SetVelocityInLocalSpace` (`self.ProjectileMovement`) (0.0 0.0 0.0))
  (set `ProjectileMovementComponent.HomingTargetComponent` (`self.Homing Target`) (`self.ProjectileMovement`))
  (set `ProjectileMovementComponent.bIsHomingProjectile` true (`self.ProjectileMovement`)))

(event `self.ReceiveActorBeginOverlap`
  (params (OtherActor :type "Actor Object Reference"))
  (bind (_returnvalue_x _returnvalue_y _returnvalue_z) (`KismetMathLibrary.BreakVector` (`self.K2_GetActorLocation`)))
  (bind _returnvalue (`SceneComponent.K2_GetComponentLocation` (`self.Bullet`)))
  (cast `/Game/Blueprints/Turret/BP_Turret` OtherActor
    (:`CastFailed`
      (bind _outhits (`KismetSystemLibrary.SphereTraceMulti` :`Start` _returnvalue :`End` _returnvalue :`Radius` (`self.RadiusAOE`) :`TraceChannel` "TraceTypeQuery1" :`DrawDebugType` "ForDuration"))
      (`NiagaraFunctionLibrary.SpawnSystemAtLocation` null)
      (for _array_element _outhits
        (bind _asbp_ennemy (cast `/Game/Blueprints/Ennemie/BP_Enemie` (`.HitActor` (`GameplayStatics.BreakHitResult` _array_element))))
        (`KismetSystemLibrary.PrintString` (`KismetSystemLibrary.GetDisplayName` _asbp_ennemy))
        (`/Game/Blueprints/Ennemie/BP_Enemie.TakeDamage` _asbp_ennemy (`self.Damage`)))
      (`NiagaraFunctionLibrary.SpawnSystemAtLocation` "/Game/VFX/Turrets/Rocket/NS_RocketExplosionV2.NS_RocketExplosionV2" (`KismetMathLibrary.MakeVector` _returnvalue_x _returnvalue_y _returnvalue_z))
      (`self.K2_DestroyActor`))))

(fn `UserConstructionScript`)