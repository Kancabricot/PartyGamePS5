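; BP_SniperBullet is a turret sniper projectile that damages enemies on overlap.
; Actor overlaps feed a HIt event, which ignores BP_Turret and damages a BP_Ennemy only when the Bullet component overlaps its capsule.
; A valid enemy hit or any other actor destroys the Bullet component and deactivates the Trail, leaving the actor itself in place, with debug prints.
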(event `self.ReceiveActorBeginOverlap`
  (params (OtherActor :type "Actor Object Reference"))
  (`self.HIt` OtherActor))

(event `HIt`
  (params (Actor :type "Actor Object Reference"))
  (cast `/Game/Blueprints/Turret/BP_Turret` Actor
    (:`CastFailed`
      (bind _asbp_ennemy (cast `/Game/Blueprints/Ennemie/BP_Ennemy` Actor)
        (:`then`
          (if (`PrimitiveComponent.IsOverlappingComponent` (`self.Bullet`) (`Character.CapsuleComponent` _asbp_ennemy))
            (`/Game/Blueprints/Ennemie/BP_Ennemy.TakeDamage` _asbp_ennemy (`self.Damage`))
            (`ActorComponent.K2_DestroyComponent` (`self.Bullet`) :!label _label)
            (`ActorComponent.Deactivate` (`self.Trail`))
            (`KismetSystemLibrary.PrintString` "Hello")))
        (:`CastFailed`
          (`KismetSystemLibrary.PrintString` "Hit Other")
          (goto _label))))))

(fn `UserConstructionScript`)