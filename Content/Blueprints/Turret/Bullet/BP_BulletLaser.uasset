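; Laser projectile for turrets that strikes its Target with a timed beam instead of travelling.
; On BeginPlay it spawns Niagara anticipation and beam effects, aiming the beam end slightly ahead of the target along its forward vector.
; After a short delay it rechecks the target, spawns a raised hit effect, then runs the Shoot logic to apply Damage and destroy itself.
; An invalid target at either check destroys the actor without damage.
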(event `Shoot`
  (`/Game/Blueprints/Enemie/Blueprint/BP_Enemie.TakeDamage` (`self.Target`) (`self.Damage`) :!label _label)
  (`self.K2_DestroyActor`))

(event `self.ReceiveBeginPlay`
  (bind _returnvalue (`self.K2_GetActorLocation`))
  (bind _returnvalue_2 (`self.K2_GetActorRotation`))
  (bind _target (`self.Target`))
  (bind _returnvalue_3 (+ (`SceneComponent.K2_GetComponentLocation` (`Character.Mesh` _target)) (* (`SceneComponent.GetForwardVector` (`Actor.RootComponent` _target)) 100.0)))
  (`self.Target`
    (:`then`
      (`NiagaraFunctionLibrary.SpawnSystemAtLocation` "/Game/VFX/VFX/Turrets/LaserTurret/Laser/NS_Laser_Anticipation.NS_Laser_Anticipation" _returnvalue)
      (bind _returnvalue_4 (`NiagaraFunctionLibrary.SpawnSystemAtLocation` "/Game/VFX/VFX/Turrets/LaserTurret/Laser/NS_Laser.NS_Laser" _returnvalue _returnvalue_2))
      (`FXSystemComponent.SetVectorParameter` _returnvalue_4 "BeamEndPosition" _returnvalue_3)
      (`KismetSystemLibrary.Delay` 0.34)
      (`self.Target`
        (:`then`
          (`NiagaraFunctionLibrary.SpawnSystemAtLocation` "/Game/VFX/VFX/Turrets/LaserTurret/Laser/Hit/NS_Laser_Hit.NS_Laser_Hit" (+ _returnvalue_3 (0.0 0.0 100.0)) _returnvalue_2 (2.2 2.2 2.2))
          (goto _label))
        (:`else`
          (`self.K2_DestroyActor`))))
    (:`else`
      (`self.K2_DestroyActor`))))

(fn `UserConstructionScript`
  (`parent.UserConstructionScript`))