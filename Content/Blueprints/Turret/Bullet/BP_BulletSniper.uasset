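; BP_BulletSniper is a sniper bullet projectile, filed with the turret assets, that hits enemies.
; On BeginPlay it copies BulletSpeed into the ProjectileMovement max and initial speeds.
; When the Bullet component overlaps the Mesh of a BP_Enemie, it calls that enemy's TakeDamage with a zero value, then destroys itself.
; Other overlaps are ignored, and construction only runs the parent script.
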(event `self.ReceiveBeginPlay`
  (bind _projectilemovement (`self.ProjectileMovement`))
  (bind _bulletspeed (`self.BulletSpeed`))
  (set `ProjectileMovementComponent.MaxSpeed` _bulletspeed _projectilemovement)
  (set `ProjectileMovementComponent.InitialSpeed` _bulletspeed _projectilemovement))

(event `self.Bullet.OnComponentBeginOverlap`
  (params (OverlappedComponent :type "PrimitiveComponent Object Reference") (OtherActor :type "Actor Object Reference") (OtherComp :type "PrimitiveComponent Object Reference") (OtherBodyIndex :type Integer) (bFromSweep :type Boolean) (SweepResult :type "HitResult Structure (by ref)"))
  (bind _asbp_enemie (cast `/Game/Blueprints/Enemie/Blueprint/BP_Enemie` OtherActor))
  (if (== (`Character.Mesh` _asbp_enemie) OtherComp)
    (`/Game/Blueprints/Enemie/Blueprint/BP_Enemie.TakeDamage` _asbp_enemie 0.0)
    (`self.K2_DestroyActor`)))

(fn `UserConstructionScript`
  (`parent.UserConstructionScript`))