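; BP_BulletSnow is a turret snowball projectile that builds up freeze on its target enemy.
; BeginPlay sets its speed and spawns a Niagara snowball aimed at the target; overlapping any enemy plays the hit effect and stops the snowball.
; Only the intended target receives GiveFreeze, which adds freeze from PDAEffect and slows it, or stuns and damages it at the 100 threshold.
; The bullet destroys itself on hitting its target or a non-enemy.
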(event `self.ReceiveBeginPlay`
  (bind _projectilemovement (`self.ProjectileMovement`))
  (bind _output_get (set `ProjectileMovementComponent.MaxSpeed` (`self.BulletSpeed`) _projectilemovement))
  (set `ProjectileMovementComponent.InitialSpeed` _output_get _projectilemovement)
  (bind _returnvalue (`NiagaraFunctionLibrary.SpawnSystemAtLocation` "/Game/VFX/VFX/Turrets/Canon_a_neige/NS_SnowBall.NS_SnowBall" (`SceneComponent.K2_GetComponentLocation` (`self.GlueTemp`)) (`KismetMathLibrary.FindLookAtRotation` (`self.K2_GetActorLocation`) (`self.K2_GetActorLocation` (`self.Target`)))))
  (set `self.BulletVfxRef` _returnvalue))

(event `self.GlueTemp.OnComponentBeginOverlap`
  (params (OverlappedComponent :type "PrimitiveComponent Object Reference") (OtherActor :type "Actor Object Reference") (OtherComp :type "PrimitiveComponent Object Reference") (OtherBodyIndex :type Integer) (bFromSweep :type Boolean) (SweepResult :type "HitResult Structure (by ref)"))
  (bind _asbp_enemie (cast `/Game/Blueprints/Enemie/Blueprint/BP_Enemie` OtherActor)
    (:`then`
      (`NiagaraFunctionLibrary.SpawnSystemAtLocation` "/Game/VFX/VFX/Turrets/Canon_a_neige/Hit/NS_SnowBallHit.NS_SnowBallHit" (`self.K2_GetActorLocation`))
      (`ActorComponent.Deactivate` (`self.BulletVfxRef`))
      (if (== _asbp_enemie (`self.Target`))
        (`self.GiveFreeze` _asbp_enemie)
        (`self.K2_DestroyActor` :!label _label)))
    (:`CastFailed`
      (goto _label))))

(fn `GiveFreeze`
  (params (Target :type "/Game/Blueprints/Enemie/Blueprint/BP_Enemie Object Reference"))
  (bind _pda_effect (`self.PDA_Effect`))
  (bind _target (`local.Target`))
  (bind _output_get (set `/Game/Blueprints/Enemie/Blueprint/BP_Enemie.Freeze` (+ (`/Game/Blueprints/Enemie/Blueprint/BP_Enemie.Freeze` Target) (`/Game/Blueprints/Turret/Structure/PDA_Effect.%Freeze` (`self.PDA_Effect`))) Target))
  (`/Game/Blueprints/Enemie/Blueprint/BP_Enemie.FreezeFunction` (`local.Target`) (`/Game/Blueprints/Turret/Structure/PDA_Effect.TimerFreeze` (`self.PDA_Effect`)))
  (if (>= _output_get 100.0)
    (`NiagaraFunctionLibrary.SpawnSystemAtLocation` "/Game/VFX/VFX/Turrets/Canon_a_neige/FrozeEffect/NS_FrozeEffect.NS_FrozeEffect" (`self.K2_GetActorLocation` Target))
    (`/Game/Blueprints/Enemie/Blueprint/BP_Enemie.Stun` _target (`/Game/Blueprints/Turret/Structure/PDA_Effect.StunSnow` (`self.PDA_Effect`)))
    (`/Game/Blueprints/Enemie/Blueprint/BP_Enemie.TakeDamage` _target (`self.Damage`))
    (`/Engine/EditorBlueprintResources/StandardMacros.IsValid` _target
      (:`Is Valid`
        (set `/Game/Blueprints/Enemie/Blueprint/BP_Enemie.b_IsFreeze` true _target)))
    (else
      (`/Game/Blueprints/Enemie/Blueprint/BP_Enemie.Slow` (`local.Target`) (`/Game/Blueprints/Turret/Structure/PDA_Effect.%SlowSnow` _pda_effect) (`/Game/Blueprints/Turret/Structure/PDA_Effect.SlowDurationSnow` _pda_effect)))))

(fn `UserConstructionScript`
  (`parent.UserConstructionScript`))