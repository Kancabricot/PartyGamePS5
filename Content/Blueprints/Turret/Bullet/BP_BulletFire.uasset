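; BP_BulletFire is a short-lived fire area attack for turrets that damages and ignites enemies.
; On BeginPlay it sizes its sphere to the owning turret's range and sets its lifespan from the effect's burst time.
; Enemies whose Box1 enters the sphere get a flamethrower Niagara effect, start burning and take damage.
; EnemyHit blocks duplicate hits until an end overlap removes the enemy, so re-entry can hit again.
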(event `self.ReceiveBeginPlay`
  (bind _turretref (`self.TurretRef`))
  (`SphereComponent.SetSphereRadius` (`self.Sphere`) (`|GetArrayItem` (`/Game/Blueprints/Turret/Structure/PDA_TurretType.Range` (`/Game/Blueprints/Turret/Blueprint/BP_Turrets.DA_TurretType` _turretref)) (`/Game/Blueprints/Turret/Blueprint/BP_Turrets.IndexTurret` _turretref)) true)
  (`self.SetLifeSpan` (`/Game/Blueprints/Turret/Structure/PDA_Effect.BurstLifeTime` (`self.DPA_Effect`))))

(event `self.Sphere.OnComponentBeginOverlap`
  (params (OverlappedComponent :type "PrimitiveComponent Object Reference") (OtherActor :type "Actor Object Reference") (OtherComp :type "PrimitiveComponent Object Reference") (OtherBodyIndex :type Integer) (bFromSweep :type Boolean) (SweepResult :type "HitResult Structure (by ref)"))
  (bind _asbp_enemie (cast `/Game/Blueprints/Enemie/Blueprint/BP_Enemie` OtherActor))
  (if (and (== (`/Game/Blueprints/Enemie/Blueprint/BP_Enemie.Box1` _asbp_enemie) OtherComp) (not (`KismetArrayLibrary.Array_Contains` (`self.EnemyHit`) _asbp_enemie)))
    (`KismetArrayLibrary.Array_Add` (`self.EnemyHit`) _asbp_enemie)
    (`/Engine/EditorBlueprintResources/StandardMacros.IsValid` _asbp_enemie
      (:`Is Valid`
        (`NiagaraFunctionLibrary.SpawnSystemAtLocation` "/Game/VFXToLoad/NS_FlameThrowerV2.NS_FlameThrowerV2" (+ (`SceneComponent.K2_GetComponentLocation` (`Actor.RootComponent` _asbp_enemie)) (0.0 0.0 100.0)) (`SceneComponent.K2_GetComponentRotation` (`self.DefaultSceneRoot`)) (3.0 3.0 3.0))
        (`/Game/Blueprints/Enemie/Blueprint/BP_Enemie.Burn Start` _asbp_enemie)
        (`/Game/Blueprints/Enemie/Blueprint/BP_Enemie.TakeDamage` _asbp_enemie (`self.Damage`))))))

(event `self.Sphere.OnComponentEndOverlap`
  (params (OverlappedComponent :type "PrimitiveComponent Object Reference") (OtherActor :type "Actor Object Reference") (OtherComp :type "PrimitiveComponent Object Reference") (OtherBodyIndex :type Integer))
  (bind _asbp_enemie (cast `/Game/Blueprints/Enemie/Blueprint/BP_Enemie` OtherActor))
  (if (`KismetArrayLibrary.Array_Contains` (`self.EnemyHit`) _asbp_enemie)
    (`KismetArrayLibrary.Array_RemoveItem` (`self.EnemyHit`) _asbp_enemie)))

(fn `UserConstructionScript`)