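; BP_BulletSongWave is a turret projectile that acts as an expanding wave, damaging enemies it reaches.
; On BeginPlay, the WaveScale timeline grows the CylinderTemp component flat in X and Y from zero to the end size in PDAEffect, then destroys the actor.
; Overlaps with a BP_Enemie's Box1 component apply Damage, and the EnemyHit list limits each enemy to one hit per wave.
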(event `self.ReceiveBeginPlay`
  (bind (_direction _scale) (`Timeline|WaveScale`)
    (:`Update`
      (bind _returnvalue (`KismetMathLibrary.Lerp` 0.0 (`/Game/Blueprints/Turret/Structure/PDA_Effect.WaveEndSize` (`self.PDA_Effect`)) _scale))
      (`SceneComponent.SetRelativeScale3D` (`self.CylinderTemp`) (`KismetMathLibrary.MakeVector` _returnvalue _returnvalue)))
    (:`Finished`
      (`self.K2_DestroyActor`))))

(event `self.CylinderTemp.OnComponentBeginOverlap`
  (params (OverlappedComponent :type "PrimitiveComponent Object Reference") (OtherActor :type "Actor Object Reference") (OtherComp :type "PrimitiveComponent Object Reference") (OtherBodyIndex :type Integer) (bFromSweep :type Boolean) (SweepResult :type "HitResult Structure (by ref)"))
  (bind _asbp_enemie (cast `/Game/Blueprints/Enemie/Blueprint/BP_Enemie` OtherActor))
  (if (and (== (`/Game/Blueprints/Enemie/Blueprint/BP_Enemie.Box1` _asbp_enemie) OtherComp) (not (`KismetArrayLibrary.Array_Contains` (`self.EnemyHit`) _asbp_enemie)))
    (`KismetArrayLibrary.Array_Add` (`self.EnemyHit`) _asbp_enemie)
    (`/Game/Blueprints/Enemie/Blueprint/BP_Enemie.TakeDamage` _asbp_enemie (`self.Damage`))))

(fn `UserConstructionScript`
  (`parent.UserConstructionScript`))