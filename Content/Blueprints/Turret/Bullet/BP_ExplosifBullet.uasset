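; Explosive turret bullet that deals area damage to enemies when it overlaps any actor other than a turret.
; On impact it runs a multi sphere trace on the Visibility channel at the bullet's position and damages each BP_Enemie hit.
; It then spawns a rocket explosion effect and destroys itself.
; Persistent debug drawing of the trace and "Hello" debug prints are still active.
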(event `self.ReceiveActorBeginOverlap`
  (params (OtherActor :type "Actor Object Reference"))
  (bind _returnvalue (`SceneComponent.K2_GetComponentLocation` (`self.Bullet`)))
  (cast `/Game/Blueprints/Turret/BP_Turret` OtherActor
    (:`CastFailed`
      (bind _outhits (`KismetSystemLibrary.SphereTraceMulti` :`Start` _returnvalue :`End` _returnvalue :`Radius` (`self.RadiusAOE`) :`TraceChannel` "TraceTypeQuery1" :`DrawDebugType` "Persistent"))
      (`KismetSystemLibrary.PrintString` "Hello")
      (for _array_element _outhits
        (bind _asbp_ennemy (cast `/Game/Blueprints/Ennemie/BP_Enemie` (`.HitActor` (`GameplayStatics.BreakHitResult` _array_element))))
        (`KismetSystemLibrary.PrintString` "Hello")
        (`/Game/Blueprints/Ennemie/BP_Enemie.TakeDamage` _asbp_ennemy (`self.Damage`)))
      (`NiagaraFunctionLibrary.SpawnSystemAtLocation` "/Game/VFX/Turrets/Rocket/NS_RocketExplosionV2.NS_RocketExplosionV2" (`self.K2_GetActorLocation`))
      (`self.K2_DestroyActor`))))

(fn `UserConstructionScript`)