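; Sticky bomb turret bullet that latches onto its target enemy and explodes after a fuse delay.
; On overlapping the target, it flags the enemy as bombed, attaches to a mesh socket, stops moving and plays an attached Niagara effect.
; After the effect data's delay, it spawns an explosion, damages and stuns the target, clears the flag and destroys itself.
; Stun duration reuses the fuse time value.
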(event `self.ReceiveBeginPlay`
  (bind _projectilemovement (`self.ProjectileMovement`))
  (bind _output_get (set `ProjectileMovementComponent.InitialSpeed` (`self.BulletSpeed`) _projectilemovement))
  (set `ProjectileMovementComponent.MaxSpeed` _output_get _projectilemovement))

(event `self.BombTemp.OnComponentBeginOverlap`
  (params (OverlappedComponent :type "PrimitiveComponent Object Reference") (OtherActor :type "Actor Object Reference") (OtherComp :type "PrimitiveComponent Object Reference") (OtherBodyIndex :type Integer) (bFromSweep :type Boolean) (SweepResult :type "HitResult Structure (by ref)"))
  (bind _asbp_enemie (cast `/Game/Blueprints/Enemie/Blueprint/BP_Enemie` OtherActor))
  (if (== _asbp_enemie (`self.Target`))
    (set `/Game/Blueprints/Enemie/Blueprint/BP_Enemie.b_HaveStickyBomb` true _asbp_enemie)
    (`self.K2_AttachToComponent` (`Character.Mesh` _asbp_enemie) "RootBoneSocket_StickyBomb" "KeepWorld" "KeepWorld" "KeepWorld")
    (set `MovementComponent.Velocity` (0.0 0.0 0.0) (`self.ProjectileMovement`))
    (`NiagaraFunctionLibrary.SpawnSystemAttached` "/Game/VFXToLoad/NS_GrenadeThrow.NS_GrenadeThrow" (`self.BombTemp`) "None" (0.0 0.0 0.0) (struct) "KeepRelativeOffset" true)
    (`KismetSystemLibrary.Delay` (`/Game/Blueprints/Turret/Structure/PDA_Effect.TimeBeforeExplosion` (`self.PDA_Effect`)))
    (`NiagaraFunctionLibrary.SpawnSystemAtLocation` "/Game/VFXToLoad/NS_GrenadeExplosion.NS_GrenadeExplosion" (`SceneComponent.K2_GetComponentLocation` (`self.BombTemp`)))
    (`/Game/Blueprints/Enemie/Blueprint/BP_Enemie.TakeDamage` (`self.Target`) (`self.Damage`))
    (`/Game/Blueprints/Enemie/Blueprint/BP_Enemie.Stun` (`self.Target`) (`/Game/Blueprints/Turret/Structure/PDA_Effect.TimeBeforeExplosion` (`self.PDA_Effect`)))
    (set `/Game/Blueprints/Enemie/Blueprint/BP_Enemie.b_HaveStickyBomb` false (`self.Target`))
    (`self.K2_DestroyActor`)))

(fn `UserConstructionScript`
  (`parent.UserConstructionScript`))