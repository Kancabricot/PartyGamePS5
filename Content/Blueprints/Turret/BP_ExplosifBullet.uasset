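; BP_ExplosifBullet is an explosive turret projectile that deals area damage to enemies.
; On overlap with any actor other than a BP_Turret, it runs a zero-length multi sphere trace on Visibility at the Bullet component, sized by RadiusAOE.
; It calls TakeDamage with Damage on each BP_Ennemy hit, then destroys itself.
; The trace leaves debug drawing enabled.
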(event `self.ReceiveActorBeginOverlap`
  (params (OtherActor :type "Actor Object Reference"))
  (bind _returnvalue (`SceneComponent.K2_GetComponentLocation` (`self.Bullet`)))
  (cast `/Game/Blueprints/Turret/BP_Turret` OtherActor
    (:`CastFailed`
      (bind _outhits (`KismetSystemLibrary.SphereTraceMulti` :`Start` _returnvalue :`End` _returnvalue :`Radius` (`self.RadiusAOE`) :`TraceChannel` "TraceTypeQuery1" :`DrawDebugType` "ForDuration"))
      (for _array_element _outhits
        (bind _asbp_ennemy (cast `/Game/Blueprints/Ennemie/BP_Ennemy` (`.HitActor` (`GameplayStatics.BreakHitResult` _array_element))))
        (`/Game/Blueprints/Ennemie/BP_Ennemy.TakeDamage` _asbp_ennemy (`self.Damage`)))
      (`self.K2_DestroyActor`))))

(fn `UserConstructionScript`)