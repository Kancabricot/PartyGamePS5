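; Turret actor that automatically tracks and shoots enemies entering its range.
; A sphere sized from Characteristic.Range adds and removes BP_Ennemy targets in an array, and Tick yaws the turret toward the first entry.
; An overlap with no current first target calls Shoot, which spawns BP_Bullet with the turret's Power if a target is valid.
; Shoot and DelayShoot re-call each other at the FireRate delay, even without a target.
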(event `self.ReceiveTick`
  (params (DeltaSeconds :type "Float (single-precision)"))
  (bind _output (`|GetArrayItem` (`self.ArrayOfTarget`)))
  (bind (_returnvalue_roll _returnvalue_pitch _returnvalue_yaw) (`KismetMathLibrary.BreakRotator` (`KismetMathLibrary.FindLookAtRotation` (`SceneComponent.K2_GetComponentLocation` (`self.Turret`)) (`SceneComponent.K2_GetComponentLocation` (`Actor.RootComponent` _output)))))
  (`/Engine/EditorBlueprintResources/StandardMacros.IsValid` _output
    (:`Is Valid`
      (`SceneComponent.K2_SetWorldRotation` (`self.Turret`) (`KismetMathLibrary.MakeRotator` 0.0 0.0 _returnvalue_yaw) false false))))

(event `self.SphereView.OnComponentBeginOverlap`
  (params (OverlappedComponent :type "PrimitiveComponent Object Reference") (OtherActor :type "Actor Object Reference") (OtherComp :type "PrimitiveComponent Object Reference") (OtherBodyIndex :type Integer) (bFromSweep :type Boolean) (SweepResult :type "HitResult Structure (by ref)"))
  (bind _asbp_ennemy (cast `/Game/Blueprints/Ennemie/BP_Ennemy` OtherActor))
  (if (== (`|GetArrayItem` (`self.ArrayOfTarget`)) null)
    (`self.Shoot`))
  (`KismetArrayLibrary.Array_Add` (`self.ArrayOfTarget`) _asbp_ennemy))

(event `self.SphereView.OnComponentEndOverlap`
  (params (OverlappedComponent :type "PrimitiveComponent Object Reference") (OtherActor :type "Actor Object Reference") (OtherComp :type "PrimitiveComponent Object Reference") (OtherBodyIndex :type Integer))
  (for _array_element (`self.ArrayOfTarget`) :!label _label
    (if (== _array_element OtherActor)
      (`KismetArrayLibrary.Array_RemoveItem` (`self.ArrayOfTarget`) _array_element)
      (`self.BreakLoop`))))

(event `BreakLoop`
  (goto _label :!via `Break`))

(event `self.ReceiveBeginPlay`
  (`SphereComponent.SetSphereRadius` (`self.SphereView`) (`.Range_6_1365810A496423C5DEC6BC876F7D7119` (break `/Game/Blueprints/Turret/Struc_Turret` (`self.characteristic`))) true))

(event `DelayShoot`
  (`KismetSystemLibrary.Delay` (`.FireRate_2_89E56A254847F72758C31A89A8081B61` (break `/Game/Blueprints/Turret/Struc_Turret` (`self.characteristic`))))
  (`self.Shoot`))

(fn `Shoot`
  (bind (_returnvalue_location _returnvalue_rotation) (`KismetMathLibrary.BreakTransform` (`SceneComponent.K2_GetComponentToWorld` (`self.BulletSpawn`))))
  (`/Engine/EditorBlueprintResources/StandardMacros.IsValid` (`|GetArrayItem` (`self.ArrayOfTarget`))
    (:`Is Valid`
      (`|SpawnActorFromClass` "/Game/Blueprints/Turret/BP_Bullet.BP_Bullet_C" (`KismetMathLibrary.MakeTransform` _returnvalue_location _returnvalue_rotation) "Undefined" "MultiplyWithRoot" null (`.Power_4_9DCFBFF74052EA155CEE9CB992BA8FB7` (break `/Game/Blueprints/Turret/Struc_Turret` (`self.characteristic`))) null)
      (`self.DelayShoot`))
    (:`Is Not Valid`
      (`self.DelayShoot`))))

(fn `UserConstructionScript`
  (`SphereComponent.SetSphereRadius` (`self.SphereView`) (`.Range_6_1365810A496423C5DEC6BC876F7D7119` (break `/Game/Blueprints/Turret/Struc_Turret` (`self.characteristic`))) true))