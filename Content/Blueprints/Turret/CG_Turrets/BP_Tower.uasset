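; Base turret Blueprint that tracks BP_SplineEnnemy actors inside a Range-scaled sphere and expires after a timed life.
; A timeline drains Life from LifeTime to zero, updates the WG_Turret_LifeTime widget and destroys the tower when finished.
; StartShooting sets a one-shot AttackSpeed timer to an empty SpawnProjectiles event.
; Despite its name, CalculateDistanceEnnemyCrystal keeps any valid target or takes the first tracked enemy; its crystal-distance logic is unconnected.
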(event `self.ReceiveBeginPlay`
  (bind _range (`self.Range`))
  (`SceneComponent.SetRelativeScale3D` (`self.Sphere`) (`KismetMathLibrary.MakeVector` _range _range _range))
  (bind _returnvalue (`GameplayStatics.GetActorOfClass` "/Game/Blueprints/Crystal/BP_Crystal.BP_Crystal_C"))
  (set `self.Ref Crystal` _returnvalue)
  (set `self.Life` (`self.LifeTime`))
  (bind _aswg_turret_life_time (cast `/Game/Blueprints/Widgets/WG_Turret_LifeTime` (`WidgetComponent.GetWidget` (`self.Widget`))))
  (set `self.Ref WG` _aswg_turret_life_time)
  (`self.LifeTime Calcul`))

(event `Start Shooting`
  (`KismetSystemLibrary.K2_SetTimerDelegate` (delegate `Spawn Projectiles`) (`self.Attack Speed`)))

(event `Spawn Projectiles`)

(event `self.Sphere.OnComponentBeginOverlap`
  (params (OverlappedComponent :type "PrimitiveComponent Object Reference") (OtherActor :type "Actor Object Reference") (OtherComp :type "PrimitiveComponent Object Reference") (OtherBodyIndex :type Integer) (bFromSweep :type Boolean) (SweepResult :type "HitResult Structure (by ref)"))
  (bind _asbp_spline_ennemy (cast `/Game/Blueprints/Enemie/SplineEnnemis/BP_SplineEnnemy` OtherActor))
  (`KismetArrayLibrary.Array_Add` (`self.EnnemiesArray`) _asbp_spline_ennemy))

(event `self.Sphere.OnComponentEndOverlap`
  (params (OverlappedComponent :type "PrimitiveComponent Object Reference") (OtherActor :type "Actor Object Reference") (OtherComp :type "PrimitiveComponent Object Reference") (OtherBodyIndex :type Integer))
  (bind _asbp_spline_ennemy (cast `/Game/Blueprints/Enemie/SplineEnnemis/BP_SplineEnnemy` OtherActor))
  (`KismetArrayLibrary.Array_RemoveItem` (`self.EnnemiesArray`) _asbp_spline_ennemy))

(event `LifeTime Calcul`
  (set `/Game/Blueprints/Widgets/WG_Turret_LifeTime.Lifetime` (`self.LifeTime`) (`self.Ref WG`))
  (bind (_direction _life) (`Timeline|TL_LifeTime`)
    (:`Update`
      (bind _output_get (set `self.Life` (`KismetMathLibrary.Lerp` (`self.LifeTime`) 0.0 _life)))
      (set `/Game/Blueprints/Widgets/WG_Turret_LifeTime.Lifetime` _output_get (`self.Ref WG`)))
    (:`Finished`
      (`self.K2_DestroyActor`))))

(fn `Calculate Distance Ennemy/Crystal`
  (returns (`Taget Enemy` :type "/Game/Blueprints/Enemie/SplineEnnemis/BP_SplineEnnemy Object Reference"))
  (for _array_element (`self.EnnemiesArray`)
    (`/Engine/EditorBlueprintResources/StandardMacros.IsValid` (`self.Taget Enemy`)
      (:`Is Not Valid`
        (set `self.Taget Enemy` _array_element))))
  (return (`self.Taget Enemy`)))

(fn `UserConstructionScript`)