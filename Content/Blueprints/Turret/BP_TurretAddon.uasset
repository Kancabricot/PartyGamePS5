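; BP_TurretAddon is a colored pickup that players carry and release to add a stage to a turret.
; TakeItem hands it to the player and disables collision, while DettachItem restores physics and launches it with the given impulse.
; One second later, a sphere trace gathers nearby turrets, offers StrucAddon to the first and destroys the addon if accepted.
; Its material color comes from StrucAddon, and it always refuses desk placement.
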(event `self.ReceiveBeginPlay`
  (bind _returnvalue (`PrimitiveComponent.CreateDynamicMaterialInstance` (`self.Addon`) 0 "/Game/Assets/Turret/Import/Mat/lambertBase.lambertBase" "None"))
  (`MaterialInstanceDynamic.SetScalarParameterValue` _returnvalue "ColorChoice" (`KismetMathLibrary.Conv_IntToDouble` (`.Color_21_392707AB4EE9FE28CF5BA39B5D438156` (break `/Game/Blueprints/Turret/Struc_Turret` (`self.Struc_Addon`))))))

(event `/Game/Blueprints/Interface/BPI_TakeItem.DettachItem`
  (params (Impulse :type "Vector Structure"))
  (bind _addon (`self.Addon`))
  (`PrimitiveComponent.SetCollisionEnabled` _addon "QueryAndPhysics")
  (`PrimitiveComponent.SetSimulatePhysics` _addon true)
  (`PrimitiveComponent.SetPhysicsLinearVelocity` (`self.Addon`) Impulse false "None")
  (set `self.b_IsGrab` false)
  (`KismetSystemLibrary.Delay` 1.0)
  (`self.CheckTurret`))

(fn `CheckTurret`
  (locals (NewLocalVar :type "Float (single-precision)" :default 0.0))
  (bind _arrayturret (`self.ArrayTurret`))
  (bind _returnvalue (`SceneComponent.K2_GetComponentLocation` (`self.Addon`)))
  (if (not (`self.b_IsGrab`))
    (bind _outhits (`KismetSystemLibrary.SphereTraceMulti` _returnvalue _returnvalue 160.0 "TraceTypeQuery1"))
    (for _array_element _outhits
      (bind _asbp_turret (cast `/Game/Blueprints/Turret/BP_Turret` (`.HitActor` (`GameplayStatics.BreakHitResult` _array_element))))
      (`KismetArrayLibrary.Array_AddUnique` (`self.ArrayTurret`) _asbp_turret))
    (if (not (`KismetArrayLibrary.Array_IsEmpty` _arrayturret))
      (bind _return (`/Game/Blueprints/Turret/BP_Turret.AddStage` (`|GetArrayItem` _arrayturret) (`self.Struc_Addon`)))
      (if _return
        (`self.K2_DestroyActor`)))))

(fn `GiveItemToDesk`
  (params (ActorTarget :type "Actor Object Reference"))
  (returns (Return :type Boolean))
  (return false))

(fn `TakeItem`
  (params (Player :type "/Game/Blueprints/Player/BP_Player Object Reference"))
  (returns (Return :type Boolean))
  (`/Game/Blueprints/Player/BP_Player.TakeItem` Player (`KismetMathLibrary.Conv_IntToDouble` (`.Color_21_392707AB4EE9FE28CF5BA39B5D438156` (break `/Game/Blueprints/Turret/Struc_Turret` (`self.Struc_Addon`)))) self)
  (`PrimitiveComponent.SetCollisionEnabled` (`self.Addon`) "NoCollision")
  (set `self.b_IsGrab` true)
  (return true))

(fn `UserConstructionScript`)