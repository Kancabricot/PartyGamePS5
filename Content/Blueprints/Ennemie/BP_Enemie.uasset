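; Enemy actor that walks via its AI controller to a target actor, takes damage and is destroyed when Life runs out.
; On BeginPlay it has a one-in-four chance to attach a random member mesh at a random socket, though its Life bonus is then overwritten by MaxLife.
; Each hit plays a timeline driving the HitTime parameter on a dynamic material as visual feedback.
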(event `self.ReceiveBeginPlay`
  (`self.CreateNewMembers`)
  (`AIBlueprintHelperLibrary.SimpleMoveToActor` (`AIBlueprintHelperLibrary.GetAIController` self) (`self.TargetMovement`))
  (bind _returnvalue (`PrimitiveComponent.CreateDynamicMaterialInstance` (`self.StaticMesh`) 0 null "None"))
  (set `self.KlangMaterialRef` _returnvalue)
  (set `self.Life` (`self.MaxLife`)))

(event `Get Hit`
  (bind (_direction _newtrack_0) (`Timeline|Timeline` :!via `PlayFromStart` :!label _label)
    (:`Update`
      (`MaterialInstanceDynamic.SetScalarParameterValue` (`self.KlangMaterialRef`) "HitTime" _newtrack_0))))

(event `StopTimeline`
  (goto _label :!via `Stop`))

(fn `CheckLife`
  (params (Life :type "Float (double-precision)"))
  (if (<= Life 0.0)
    (`self.StopTimeline`)
    (`self.K2_DestroyActor`)))

(fn `ChooseNewMembers`
  (returns (Mesh :type "StaticMesh Object Reference"))
  (bind _memberarray (`self.MemberArray`))
  (return (`|GetArrayItem` _memberarray (`KismetMathLibrary.RandomIntegerInRange` 0 (`KismetArrayLibrary.Array_Length` _memberarray)))))

(fn `ChosseLocation`
  (returns (Namesocket :type "Name (by ref)"))
  (return (`KismetArrayLibrary.Array_Random` (`SceneComponent.GetAllSocketNames` (`self.StaticMesh`)))))

(fn `CreateNewMembers`
  (if (== (`KismetMathLibrary.RandomIntegerInRange` 0 3) 0)
    (bind _namesocket (`self.ChosseLocation`))
    (bind _returnvalue (`AddComponent|NODE_AddStaticMeshComponent-0`))
    (bind _output_get (set `self.NewVar` _returnvalue))
    (`StaticMeshComponent.SetStaticMesh` _output_get (`self.ChooseNewMembers`))
    (`SceneComponent.K2_AttachToComponent` _output_get (`self.StaticMesh`) _namesocket "SnapToTarget" "SnapToTarget" "SnapToTarget" true)
    (set `self.Life` (+ (`self.Life`) 10.0))
    (return)))

(fn `TakeDamage`
  (params (Damage :type "Float (double-precision)"))
  (bind _output_get (set `self.Life` (- (`self.Life`) Damage)))
  (`self.Get Hit`)
  (`self.CheckLife` _output_get))

(fn `UserConstructionScript`)