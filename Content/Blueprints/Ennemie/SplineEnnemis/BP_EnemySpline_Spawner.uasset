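; BP_EnemySpline_Spawner periodically spawns BP_SplineEnnemy enemies at the start of the level's enemy path spline.
; On BeginPlay it finds the BP_Ennemy_Path_Spline actor and starts a looping timer at SpawnRate after a short initial delay.
; Each tick of that timer spawns an enemy at the first spline point, using world location and local rotation.
; A CrystalDestroy event pauses the timer to halt spawning.
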(event `self.ReceiveBeginPlay`
  (bind _returnvalue (`GameplayStatics.GetActorOfClass` "/Game/Blueprints/Ennemie/SplineEnnemis/BP_Ennemy_Path_Spline.BP_Ennemy_Path_Spline_C"))
  (set `self.Path_Spline` _returnvalue)
  (bind _returnvalue_2 (`KismetSystemLibrary.K2_SetTimerDelegate` (delegate `Spawn Enemy`) (`self.Spawn Rate`) true 2.0))
  (set `self.Timer Handler` _returnvalue_2))

(event `Spawn Enemy`
  (bind _spline (`/Game/Blueprints/Ennemie/SplineEnnemis/BP_Ennemy_Path_Spline.Spline` (`self.Path_Spline`)))
  (if true
    (`|SpawnActorFromClass` "/Game/Blueprints/Ennemie/SplineEnnemis/BP_SplineEnnemy.BP_SplineEnnemy_C" (`KismetMathLibrary.MakeTransform` (`SplineComponent.GetLocationAtSplinePoint` _spline 0 "World") (`SplineComponent.GetRotationAtSplinePoint` _spline 0 "Local")) "Undefined" "MultiplyWithRoot" null null)))

(event `/Game/Blueprints/Interface/BPI_Crystal_Interact.Crystal_Destroy`
  (`KismetSystemLibrary.K2_PauseTimerHandle` (`self.Timer Handler`)))

(fn `UserConstructionScript`)