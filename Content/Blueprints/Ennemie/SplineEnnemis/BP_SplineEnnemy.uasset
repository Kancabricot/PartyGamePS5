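; Enemy actor that travels along a spline path and explodes when destroyed.
; On BeginPlay it finds a BP_Ennemy_Path_Spline via GetActorOfClass, then a timeline, rate-scaled by TimeToComplete, moves it from start to end by distance along the spline.
; Two events, InteractWCrystal and CrystalDestroy, each spawn their own Niagara explosion and destroy the actor.
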(event `self.ReceiveBeginPlay`
  (bind _returnvalue (`GameplayStatics.GetActorOfClass` "/Game/Blueprints/Ennemie/SplineEnnemis/BP_Ennemy_Path_Spline.BP_Ennemy_Path_Spline_C"))
  (set `self.Path_Spline` _returnvalue)
  (`self.Move`))

(event `Move`
  (`TimelineComponent.SetPlayRate` (`self.TL_Move`) (/ 1.0 (`self.Time To Complete`)))
  (bind (_direction _move_track) (`Timeline|TL_Move`)
    (:`Update`
      (`self.K2_SetActorTransform` (`KismetMathLibrary.MakeTransform` (`SplineComponent.GetLocationAtDistanceAlongSpline` (`/Game/Blueprints/Ennemie/SplineEnnemis/BP_Ennemy_Path_Spline.Spline` (`self.Path_Spline`)) (`KismetMathLibrary.Lerp` 0.0 (`SplineComponent.GetSplineLength` (`/Game/Blueprints/Ennemie/SplineEnnemis/BP_Ennemy_Path_Spline.Spline` (`self.Path_Spline`))) _move_track) "World"))))))

(event `/Game/Blueprints/Interface/BPI_Crystal_Interact.Interact_W_Crystal`
  (`NiagaraFunctionLibrary.SpawnSystemAtLocation` "/Game/VFX/Ennemies/NS_Ennemy_Explosion_Crystal.NS_Ennemy_Explosion_Crystal" (`SceneComponent.K2_GetComponentLocation` (`self.DefaultSceneRoot`)))
  (`self.K2_DestroyActor`))

(event `/Game/Blueprints/Interface/BPI_Crystal_Interact.Crystal_Destroy`
  (`NiagaraFunctionLibrary.SpawnSystemAtLocation` "/Game/VFX/Ennemies/NS_Ennemy_Explosion.NS_Ennemy_Explosion" (`SceneComponent.K2_GetComponentLocation` (`self.DefaultSceneRoot`)))
  (`self.K2_DestroyActor`))

(fn `UserConstructionScript`)