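; Player Blueprint that carries one crafting ingredient at a time, from zinc materials to turrets, and interacts with objects in front of it.
; Both inputs run a sphere trace ahead of the capsule and message the hit actor through interfaces to interact, take or set ingredients, clearing the held item only on a BP_Desk.
; While holding an item, releasing Action throws it as a spawned BP_Ingredients.
; The held-ingredient enum drives the displayed mesh and material.
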(event `self.ReceiveBeginPlay`
  (`EnhancedInputSubsystemInterface.AddMappingContext` (pcsubsystem `EnhancedInputLocalPlayerSubsystem` (`GameplayStatics.GetPlayerController` (`self.Player Index`))) (`self.Mapping Context`) 0 (struct)))

(event `EnhancedInput|/Game/Input/Actions/IA_Action`
  (params (ActionValue :type Boolean) (ElapsedSeconds :type "Float (double-precision)") (TriggeredSeconds :type "Float (double-precision)") (InputAction :type "InputAction Object Reference" :default "/Game/Input/Actions/IA_Action.IA_Action"))
  (bind _capsulecomponent (`self.CapsuleComponent`))
  (bind _returnvalue (+ (`SceneComponent.K2_GetComponentLocation` _capsulecomponent) (* (`SceneComponent.GetForwardVector` _capsulecomponent) (`self.DistanceSphereTrace`))))
  (:`Started`
    (bind _outhit (`KismetSystemLibrary.SphereTraceSingle` :`Start` _returnvalue :`End` _returnvalue :`Radius` (`self.RadiusSphereTrace`) :`TraceChannel` "TraceTypeQuery1" :`DrawDebugType` "ForDuration"))
    (if (`|EnumEquality` (`self.Enum_Ingrediants`) "NewEnumerator3")
      (bind (_bblockinghit _binitialoverlap _time _distance _location _impactpoint _normal _impactnormal _physmat _hitactor) (`GameplayStatics.BreakHitResult` _outhit))
      (cast `/Game/Blueprints/Interface/BPI_Interact` _hitactor)
      (message `/Game/Blueprints/Interface/BPI_Interact.Interact` _hitactor)
      (else
        (set `self.b_canThrow` true))))
  (:`Completed`
    (`self.ThrowItem`)))

(event `EnhancedInput|/Game/Input/Actions/IA_TakeItem`
  (params (ActionValue :type Boolean) (ElapsedSeconds :type "Float (double-precision)") (TriggeredSeconds :type "Float (double-precision)") (InputAction :type "InputAction Object Reference" :default "/Game/Input/Actions/IA_TakeItem.IA_TakeItem"))
  (bind _capsulecomponent (`self.CapsuleComponent`))
  (bind _returnvalue (+ (`SceneComponent.K2_GetComponentLocation` _capsulecomponent) (* (`SceneComponent.GetForwardVector` _capsulecomponent) (`self.DistanceSphereTrace`))))
  (:`Started`
    (bind _outhit (`KismetSystemLibrary.SphereTraceSingle` :`Start` _returnvalue :`End` _returnvalue :`Radius` (`self.RadiusSphereTrace`) :`TraceChannel` "TraceTypeQuery1" :`DrawDebugType` "ForDuration"))
    (if (`|EnumEquality` (`self.Enum_Ingrediants`) "NewEnumerator3")
      (bind (_bblockinghit _binitialoverlap _time _distance _location _impactpoint _normal _impactnormal _physmat _hitactor) (`GameplayStatics.BreakHitResult` _outhit))
      (message `/Game/Blueprints/Interface/BPI_SetIngredients.TakeIngredient` _hitactor self)
      (else
        (bind _asbpi_set_ingredients (cast `/Game/Blueprints/Interface/BPI_SetIngredients` _hitactor))
        (message `/Game/Blueprints/Interface/BPI_SetIngredients.SetIngredient` _hitactor (`self.Enum_Ingrediants`))
        (cast `/Game/Blueprints/Tools/BP_Desk` _asbpi_set_ingredients)
        (set `self.Enum_Ingrediants` "NewEnumerator3")
        (`self.SetIngredientsMesh`)))))

(fn `SetIngredientsMesh`
  (bind _ingredientmesh (`self.IngredientMesh`))
  (switch `/Game/Blueprints/Enums/Enum_Ingredients` (`self.Enum_Ingrediants`)
    (:`NewEnumerator3`
      ;[1 1 1] Mineral
      (`self.SetMeshAndMaterial` _ingredientmesh))
    (:`NewEnumerator0`
      (`self.SetMeshAndMaterial` _ingredientmesh "/Game/Assets/Mineral.Mineral" "/Game/Assets/Materials/Zinc/M_Zinc_Mineral.M_Zinc_Mineral"))
    (:`NewEnumerator4`
      ;[1 1 1] molted
      (`self.SetMeshAndMaterial` (`self.IngredientMesh`) "/Game/Assets/Ingot.Ingot" "/Game/Assets/Materials/Zinc/M_Fusion_Zinc.M_Fusion_Zinc"))
    (:`NewEnumerator7`
      ;[1 1 1] Gear
      (`self.SetMeshAndMaterial` (`self.IngredientMesh`) "/Game/Assets/Gears/Thibault/Gear5.Gear5" "/Game/Assets/Materials/Zinc/M_Zinc.M_Zinc"))
    (:`NewEnumerator11`
      ;[1 1 1] Tige
      (`self.SetMeshAndMaterial` (`self.IngredientMesh`) "/Game/Assets/Materials/Zinc/Import/ZincTige.ZincTige" "/Game/Assets/Materials/Zinc/M_Zinc.M_Zinc"))
    (:`NewEnumerator10`
      ;[1 1 1] Turret
      (`self.SetMeshAndMaterial` (`self.IngredientMesh`) "/Game/Assets/Turret/Turret.Turret" "/Game/Assets/Materials/Zinc/M_Zinc.M_Zinc"))
    (:`NewEnumerator12`
      (`self.SetMeshAndMaterial` (`self.IngredientMesh`) "/Game/Assets/Turret/Big_Turret.Big_Turret" "/Game/Assets/Materials/Zinc/M_Zinc.M_Zinc"))
    (:`NewEnumerator13`
      (`self.SetMeshAndMaterial` (`self.IngredientMesh`) "/Game/Assets/Turret/Sniper_T.Sniper_T" "/Game/Assets/Materials/Zinc/M_Zinc.M_Zinc"))))

(fn `SetMeshAndMaterial`
  (params (Target :type "StaticMeshComponent Object Reference") (NewMesh :type "StaticMesh Object Reference") (NewMaterial :type "MaterialInterface Object Reference"))
  (`StaticMeshComponent.SetStaticMesh` Target NewMesh)
  (`PrimitiveComponent.SetMaterial` Target 0 NewMaterial))

(fn `ThrowItem`
  (bind _capsulecomponent (`self.CapsuleComponent`))
  (bind _ingredientmesh (`self.IngredientMesh`))
  (if (`self.b_canThrow`)
    (`|SpawnActorFromClass` "/Game/Blueprints/BP_Ingredients.BP_Ingredients_C" (`KismetMathLibrary.MakeTransform` (+ (`SceneComponent.K2_GetComponentLocation` _capsulecomponent) (* (`SceneComponent.GetForwardVector` _capsulecomponent) 80.0))) "Undefined" "MultiplyWithRoot" null (`StaticMeshComponent.StaticMesh` _ingredientmesh) (`PrimitiveComponent.GetMaterial` _ingredientmesh 0) (`self.Enum_Ingrediants`) null)
    (set `self.b_canThrow` false)
    (set `self.Enum_Ingrediants` "NewEnumerator3")
    (`self.SetIngredientsMesh`)))

(fn `UserConstructionScript`)