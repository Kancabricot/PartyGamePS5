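; BP_BaseTurretSpawner is a dispenser that hands the player a new turret base (BP_Turret) when taken from and refuses items given to it.
; TakeItem spawns a turret flagged as grabbed, passes it to the player, calls its SpawnCatch, then starts the respawn cooldown.
; The TimerRespawn timeline feeds a WG_Temperature widget as a progress bar and re-enables taking when it finishes.
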(event `ResetTimer`
  (set `self.b_HaveBaseToGive` false)
  (bind (_direction _timer) (`Timeline|TimerRespawn` :!via `PlayFromStart`)
    (:`Update`
      (`/Game/Blueprints/Widgets/WG_Temperature.SetTimer` (`self.WGBar`) _timer))
    (:`Finished`
      (set `self.b_HaveBaseToGive` true))))

(event `self.ReceiveBeginPlay`
  (bind _aswg_temperature (cast `/Game/Blueprints/Widgets/WG_Temperature` (`WidgetComponent.GetWidget` (`self.Widget`))))
  (set `self.WGBar` _aswg_temperature)
  (set `self.b_HaveBaseToGive` true)
  (`/Game/Blueprints/Widgets/WG_Temperature.SetTimer` (`self.WGBar`) 1.0))

(fn `GiveItemToDesk`
  (params (ActorTarget :type "Actor Object Reference"))
  (returns (Return :type Boolean))
  (return false))

(fn `TakeItem`
  (params (Player :type "/Game/Blueprints/Player/BP_Player Object Reference"))
  (returns (Return :type Boolean))
  (if (`self.b_HaveBaseToGive`)
    (bind _returnvalue (`|SpawnActorFromClass` "/Game/Blueprints/Turret/BP_Turret.BP_Turret_C" (`KismetMathLibrary.MakeTransform` (0.0 0.0 0.0)) "Undefined" "MultiplyWithRoot" null null))
    (set `/Game/Blueprints/Turret/BP_Turret.b_IsGrab` true _returnvalue)
    (`/Game/Blueprints/Player/BP_Player.TakeItem` Player 0.0 _returnvalue)
    (`/Game/Blueprints/Turret/BP_Turret.SpawnCatch` _returnvalue)
    (`self.ResetTimer`)
    (return true)))

(fn `UserConstructionScript`)