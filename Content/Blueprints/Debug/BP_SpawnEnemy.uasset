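; Debug enemy spawner that draws a path along a spline and, after a delay, spawns a single BP_Enemie to follow it.
; SetSpline picks the line, L or U spline (BeginPlay uses L), traces down for ground height and builds offset spline mesh segments just above it.
; Spawn passes itself and the chosen spline to the enemy, makes it movable and starts its spline movement.
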(event `self.ReceiveBeginPlay`
  (`self.SetSpline` "NewEnumerator1")
  (`self.Spawn`))

(event `Spawn`
  (`KismetSystemLibrary.Delay` 20.0)
  (bind _returnvalue (`|SpawnActorFromClass` "/Game/Blueprints/Enemie/Blueprint/BP_Enemie.BP_Enemie_C" (`KismetMathLibrary.MakeTransform` (`self.K2_GetActorLocation`)) "AlwaysSpawn" "MultiplyWithRoot" null null false 300.0 self (`self.SplineRef`) null))
  (`/Engine/EditorBlueprintResources/StandardMacros.IsValid` _returnvalue
    (:`Is Valid`
      (`SceneComponent.SetMobility` (`Actor.RootComponent` _returnvalue) "Movable")
      (`/Game/Blueprints/Enemie/Blueprint/BP_Enemie.MoveAlongSplineInTool` _returnvalue))))

(fn `SetSpline`
  (params (Selection :type "/Game/Blueprints/Debug/Enum_Spline Enum" :default "NewEnumerator0"))
  (bind (_location_x _location_y _location_z) (`KismetMathLibrary.BreakVector` (`self.Location`)))
  (bind _splineref (`self.SplineRef`))
  (bind _returnvalue (`SceneComponent.K2_GetComponentLocation` (`self.SplineRef`)))
  (switch `/Game/Blueprints/Debug/Enum_Spline` Selection
    (:`NewEnumerator0`
      (set `self.SplineRef` (`self.SplineLine`)))
    (:`NewEnumerator1`
      (set `self.SplineRef` (`self.SplineL`)))
    (:`NewEnumerator2`
      (set `self.SplineRef` (`self.SplineU`))))
  (bind _outhit (`KismetSystemLibrary.LineTraceSingle` _returnvalue (+ _returnvalue (* (`KismetMathLibrary.NegateVector` (`KismetMathLibrary.Vector_Up`)) 100.0)) "TraceTypeQuery1"))
  (set `self.Location` (+ (`.Location` (`GameplayStatics.BreakHitResult` _outhit)) (0.0 0.0 1.0)))
  (`ActorComponent.K2_DestroyComponent` (`self.MeshArray`))
  (for _index (range (`SplineComponent.GetNumberOfSplinePoints` (`self.SplineRef`)))
    (bind _returnvalue_2 (`AddComponent|NODE_AddSplineMeshComponent-0` :`bManualAttachment` true))
    (`KismetArrayLibrary.Array_Add` (`self.MeshArray`) _returnvalue_2)
    (bind (_location _tangent) (`SplineComponent.GetLocationAndTangentAtSplinePoint` _splineref _index "World"))
    (bind (_location_2 _tangent_2) (`SplineComponent.GetLocationAndTangentAtSplinePoint` _splineref (+ _index 1) "World"))
    (`SplineMeshComponent.SetStartAndEnd` _returnvalue_2 (`KismetMathLibrary.MakeVector` (+ (.x _location) (`self.OffSetXPath`)) (+ (.y _location) (`self.OffSetYPath`)) _location_z) _tangent (`KismetMathLibrary.MakeVector` (+ (.x _location_2) (`self.OffSetXPath`)) (+ (.y _location_2) (`self.OffSetYPath`)) _location_z) _tangent_2 true)))

(fn `UserConstructionScript`)