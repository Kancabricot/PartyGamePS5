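; Debug Blueprint function library that finds the level constructor data asset belonging to the current level.
; SetDataAsset scans the debug DataAsset folder non-recursively through the Asset Registry, matching asset names against the DA_LevelConstructor prefix plus the level name.
; On a match it flags that the asset exists and returns it cast to PDA_LevelConstructorValue; despite its name, it creates or modifies no asset.
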(fn `SetDataAsset`
  (returns (DataAsset :type "/Game/Blueprints/Debug/PDA_LevelConstructorValue Object Reference"))
  (locals (b_DataAssetAlreadyExist :type Boolean))
  (bind _outassetdata (`AssetRegistry.GetAssetsByPath` (`AssetRegistryHelpers.GetAssetRegistry`) "/Game/Blueprints/Debug/DataAsset" false false))
  (for _array_element _outassetdata
    (bind _returnvalue (`GameplayStatics.GetCurrentLevelName` null))
    (if (`KismetStringLibrary.EqualEqual_StrStr` (`KismetStringLibrary.Conv_NameToString` (`.AssetName` (break `AssetData` _array_element))) (`KismetStringLibrary.Concat_StrStr` "DA_LevelConstructor" _returnvalue))
      (set `local.b_DataAssetAlreadyExist` true)
      (bind _aspda_level_constructor_value (cast `/Game/Blueprints/Debug/PDA_LevelConstructorValue` (`AssetRegistryHelpers.GetAsset` _array_element)))
      (return _aspda_level_constructor_value))))