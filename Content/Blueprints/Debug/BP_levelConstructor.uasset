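; Editor-time level validation actor that checks whether a map contains the actors the game needs.
; Its construction script runs ReviewMissObject, which requires exactly one BP_CreateLocalPlayer, then checks in sequence for gameplay actors like spawners, machines, enemy spline path, camera and nav mesh volume.
; The first failure writes a French warning to its Debug text; later checks are skipped, and a passing level leaves the text untouched.
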(fn `ReviewMissObject`
  (bind _outactors (`GameplayStatics.GetAllActorsOfClass` "/Game/Blueprints/Player/Player/BP_CreateLocalPlayer.BP_CreateLocalPlayer_C"))
  (if (`KismetArrayLibrary.Array_IsNotEmpty` _outactors)
    (if (> (`KismetArrayLibrary.Array_Length` _outactors) 1)
      (`self.SetTextDebug` "Il y a trop de BP_CreateLocalPlayer")
      (else
        (bind _outactors_2 (`GameplayStatics.GetAllActorsOfClass` "/Game/Blueprints/Enemie/Blueprint/BP_LooseZone.BP_LooseZone_C"))
        (if (`KismetArrayLibrary.Array_IsEmpty` _outactors_2)
          (`self.SetTextDebug` "Manque BP_LooseZone")
          (else
            (bind _outactors_3 (`GameplayStatics.GetAllActorsOfClass` "/Game/Blueprints/Machine/BP_Storage.BP_Storage_C"))
            (if (`KismetArrayLibrary.Array_IsEmpty` _outactors_3)
              (`self.SetTextDebug` "Manque BP_Storage")
              (else
                (bind _outactors_4 (`GameplayStatics.GetAllActorsOfClass` "/Game/Blueprints/Spawner/BP_EnnemySpawner.BP_EnnemySpawner_C"))
                (if (`KismetArrayLibrary.Array_IsEmpty` _outactors_4)
                  (`self.SetTextDebug` "Manque BP_EnnemySpawner")
                  (else
                    (bind _outactors_5 (`GameplayStatics.GetAllActorsOfClass` "/Game/Blueprints/Spawner/BP_SpawnerMaster.BP_SpawnerMaster_C"))
                    (if (`KismetArrayLibrary.Array_IsEmpty` _outactors_5)
                      (`self.SetTextDebug` "Manque BP_SpawnerMaster")
                      (else
                        (bind _outactors_6 (`GameplayStatics.GetAllActorsOfClass` "/Game/Blueprints/Machine/BP_Smelterie.BP_Smelterie_C"))
                        (if (`KismetArrayLibrary.Array_IsEmpty` _outactors_6)
                          (`self.SetTextDebug` "Manque BP_Smelterie")
                          (else
                            (bind _outactors_7 (`GameplayStatics.GetAllActorsOfClass` "/Game/Blueprints/Machine/BP_Assembler.BP_Assembler_C"))
                            (if (`KismetArrayLibrary.Array_IsEmpty` _outactors_7)
                              (`self.SetTextDebug` "Manque BP_Assembler")
                              (else
                                (bind _outactors_8 (`GameplayStatics.GetAllActorsOfClass` "/Game/Blueprints/Machine/BP_Charger.BP_Charger_C"))
                                (if (`KismetArrayLibrary.Array_IsEmpty` _outactors_8)
                                  (`self.SetTextDebug` "Manque BP_Charger")
                                  (else
                                    (bind _outactors_9 (`GameplayStatics.GetAllActorsOfClass` "/Script/NavigationSystem.NavMeshBoundsVolume"))
                                    (if (`KismetArrayLibrary.Array_IsEmpty` _outactors_9)
                                      (`self.SetTextDebug` "Manque un NavMeshBoundVolume")
                                      (else
                                        (bind _outactors_10 (`GameplayStatics.GetAllActorsOfClass` "/Game/Blueprints/Enemie/SplineEnnemis/BP_Spline_Enemy_Path.BP_Spline_Enemy_Path_C"))
                                        (if (`KismetArrayLibrary.Array_IsEmpty` _outactors_10)
                                          (`self.SetTextDebug` "Manque BP_Spline_Enemy_Path")
                                          (else
                                            (bind _outactors_11 (`GameplayStatics.GetAllActorsOfClass` "/Game/Blueprints/Player/Cam/BP_camera.BP_camera_C"))
                                            (if (`KismetArrayLibrary.Array_IsEmpty` _outactors_11)
                                              (`self.SetTextDebug` "Manque BP_Camera"))))))))))))))))))))))
    (else
      (`self.SetTextDebug` "Manque BP_CreateLocalPlayer"))))

(fn `SetTextDebug`
  (params (Text :type Text))
  (locals (TextToWrite :type Text))
  (set `local.TextToWrite` Text)
  (`TextRenderComponent.K2_SetText` (`self.Debug`) (`local.TextToWrite`)))

(fn `UserConstructionScript`
  (`self.ReviewMissObject`))