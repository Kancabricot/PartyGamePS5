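; BP_CreateLocalPlayer sets up two-player local multiplayer when play begins.
; It gathers PlayerStart actors, creates local players 0 and 1, and spawns a BP_Player at each of the first two starts.
; Each pawn receives its own input mapping context, IMC_Player1 or IMC_Player2, and is possessed by its matching controller.
; Player 0's view target is then set to the BP_camera actor found in the level.
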(event `self.ReceiveBeginPlay`
  (`|ExecutionSequence`
    (:`then_0`
      (bind _outactors (`GameplayStatics.GetAllActorsOfClass` "/Script/Engine.PlayerStart"))
      (set `self.PlayerStartRefs` _outactors))
    (:`then_1`
      (`GameplayStatics.CreatePlayer` 0)
      (bind _returnvalue (`|SpawnActorFromClass` "/Game/Blueprints/Player/BP_Player.BP_Player_C" (`self.GetTransform` (`|GetArrayItem` (`self.PlayerStartRefs`))) "Undefined" "MultiplyWithRoot" null "/Game/Input/IMC_Player1.IMC_Player1" 0 null))
      (`Controller.Possess` (`GameplayStatics.GetPlayerController` 0) _returnvalue)
      (`GameplayStatics.CreatePlayer` 1)
      (bind _returnvalue_2 (`|SpawnActorFromClass` "/Game/Blueprints/Player/BP_Player.BP_Player_C" (`self.GetTransform` (`|GetArrayItem` (`self.PlayerStartRefs`) 1)) "Undefined" "MultiplyWithRoot" null "/Game/Input/IMC_Player2.IMC_Player2" 1 null))
      (`Controller.Possess` (`GameplayStatics.GetPlayerController` 1) _returnvalue_2))
    (:`then_2`
      (bind _returnvalue_3 (`GameplayStatics.GetActorOfClass` "/Game/Blueprints/BP_camera.BP_camera_C"))
      (`PlayerController.SetViewTargetWithBlend` (`GameplayStatics.GetPlayerController` 0) _returnvalue_3 0.0 "VTBlend_Linear" 0.0 false))))

(fn `UserConstructionScript`)