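; BP_TeslaVfx is a Tesla turret effect actor that throws electric beams at nearby surfaces in random directions.
; Tick runs UpdateTraces, which on a cooldown line-traces the Visibility channel along a random direction between a minimum and maximum radius.
; Each blocking hit spawns an auto-destroyed, attached Niagara system.
; It receives an actor-relative start, a world-space end nudged along the surface normal, and that normal.
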(event `self.ReceiveTick`
  (params (DeltaSeconds :type "Float (single-precision)"))
  (`self.UpdateTraces`))

(fn `UpdateTraces`
  (locals (RandomDirection :type "Vector Structure") (ImpactOffset :type "Float (double-precision)" :default 1.0))
  (bind _returnvalue (`self.K2_GetActorLocation`))
  (bind _returnvalue_2 (* (`local.RandomDirection`) (`self.MinRadius`)))
  ;[1 1 1] Check Cooldown
  (if (>= (- (`GameplayStatics.GetTimeSeconds`) (`self.LastTrace`)) (`self.TraceCooldown`))
    ;[1 1 1] Trace
    (set `local.RandomDirection` (`KismetMathLibrary.RandomUnitVector`))
    (bind _outhit (`KismetSystemLibrary.LineTraceSingle` :`Start` (+ _returnvalue _returnvalue_2) :`End` (+ _returnvalue (* (`local.RandomDirection`) (`self.MaxRadius`))) :`TraceChannel` "TraceTypeQuery1" :`DrawTime` (`self.TraceCooldown`)))
    ;[1 1 1] Reset Cooldown
    (set `self.LastTrace` (`GameplayStatics.GetTimeSeconds`))
    (bind (_bblockinghit _binitialoverlap _time _distance _location _impactpoint _normal _impactnormal) (`GameplayStatics.BreakHitResult` _outhit))
    (if _bblockinghit
      (bind _returnvalue_3 (`NiagaraFunctionLibrary.SpawnSystemAttached` "/Game/VFX/VFX/Turrets/Tesla/Ns_Tesla.Ns_Tesla" (`self.DefaultSceneRoot`) "None" (0.0 0.0 0.0) (struct) "KeepRelativeOffset" true))
      (`NiagaraComponent.SetVariableVec3` _returnvalue_3 "BeamStartPoint" _returnvalue_2)
      (`NiagaraComponent.SetVariableVec3` _returnvalue_3 "BeamendPoint" (+ _impactpoint (* _impactnormal (`local.ImpactOffset`))))
      (`NiagaraComponent.SetVariableVec3` _returnvalue_3 "ImpactNormal" _impactnormal))))

(fn `UserConstructionScript`)