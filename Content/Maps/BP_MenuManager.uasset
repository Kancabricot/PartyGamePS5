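; BP_MenuManager runs the front-end menu flow, from loading screen to two-player menu and intro.
; On BeginPlay it sets game-only input and shows WG_Loading, passing itself to the widget.
; CreateMenu swaps loading for WG_Menu, creates a second player and possesses a BP_PlayerMenu pawn for each controller, both sharing that menu.
; IntroCreation shows WG_Intro, starts its media sound and uses a fixed timer to open the tutorial level.
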(event `self.ReceiveBeginPlay`
  (`|ExecutionSequence`
    (:`then_0`
      (`WidgetBlueprintLibrary.SetInputMode_GameOnly` (`GameplayStatics.GetPlayerController` 0)))
    (:`then_1`
      (bind _returnvalue (`|CreateWidget` "/Game/GameLocalization/WG_Loading.WG_Loading_C"))
      (bind _output_get (set `self.loadingRef` _returnvalue))
      (`/Game/GameLocalization/WG_Loading.GetInfo` _output_get self)
      (`UserWidget.AddToViewport` _output_get 0))))

(event `Create Menu`
  (`Widget.RemoveFromParent` (`self.loadingRef`))
  (bind _returnvalue (`|CreateWidget` "/Game/GameLocalization/WG_Menu.WG_Menu_C"))
  (bind _output_get (set `self.WGMenuRef` _returnvalue))
  (`/Game/GameLocalization/WG_Menu.GetMenuManagerRef` _output_get self)
  (`UserWidget.AddToViewport` _output_get 0)
  (bind _returnvalue_2 (`|SpawnActorFromClass` "/Game/Blueprints/Menu/BP_PlayerMenu.BP_PlayerMenu_C" (`KismetMathLibrary.MakeTransform` (0.0 0.0 0.0)) "Undefined" "MultiplyWithRoot" null (`self.WGMenuRef`) 0 null))
  (`Controller.Possess` (`GameplayStatics.GetPlayerController` 0) _returnvalue_2)
  (`GameplayStatics.CreatePlayer` 1)
  (bind _returnvalue_3 (`|SpawnActorFromClass` "/Game/Blueprints/Menu/BP_PlayerMenu.BP_PlayerMenu_C" (`KismetMathLibrary.MakeTransform` (0.0 0.0 0.0)) "Undefined" "MultiplyWithRoot" null (`self.WGMenuRef`) 1 null))
  (`Controller.Possess` (`GameplayStatics.GetPlayerController` 1) _returnvalue_3))

(fn `IntroCreation`
  (bind _returnvalue (`|CreateWidget` "/Game/GameLocalization/WG_Intro.WG_Intro_C"))
  (`UserWidget.AddToViewport` _returnvalue 0)
  (`SynthComponent.Start` (`self.MediaSoundIntro`))
  (`KismetSystemLibrary.K2_SetTimer` null "LoadLevelTuto" 41.0))

(fn `LoadLevelTuto`
  (`GameplayStatics.OpenLevelBySoftObjectPtr` "/Game/Maps/Levels/Iterations/Level_00_Tutorial.Level_00_Tutorial"))

(fn `UserConstructionScript`)